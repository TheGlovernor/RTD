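; Procedurally scatters and removes biome foliage on the terrain's hex tiles, animating each instance in and out.
; Construction builds a hierarchical instanced mesh component per mesh, grouped by foliage type with grass-specific render settings, plus FastNoise generators seeded from TerrainGen.
; Adding filters random points by per-biome noise thresholds, picks weighted groups, then animates tiny instances after a draw delay.
; Removal sphere-traces the hex and plays that animation in reverse.
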(event Custom|AddFoliage
  (params (HexLocation :type Vector) (Biome :type Biome%20Enum :default "NewEnumerator0") (DrawDelay :type Float%20%28double-precision%29))
  (bind _biomeaddthreshold (Variables|Default|GetBiomeAddThreshold))
  (bind _value (Utilities|Map|Find _biomeaddthreshold Biome))
  (for _index (range 1 (.Value (Utilities|Map|Find (Variables|Default|GetBiomeDensity) Biome)))
    (bind _location (CallFunction|RandomPointinRadius HexLocation (Variables|Default|GetHexRadius)))
    (if (select (.Value (Utilities|Map|Find (Variables|Default|GetUseScattered) Biome)) (> _value (Class|FastNoiseWrapper|GetNoise2D (Variables|Default|GetScatteredNoise) (.X (Class|KismetMathLibrary|BreakVector3f _location)) (.Y (Class|KismetMathLibrary|BreakVector3f _location)))) (> _value (Class|FastNoiseWrapper|GetNoise2D (Variables|Default|GetCellularNoise) (.X (Class|KismetMathLibrary|BreakVector3f _location)) (.Y (Class|KismetMathLibrary|BreakVector3f _location)))))
      (bind _ismc (CallFunction|ChooseFoliage Biome))
      (bind _returnvalue (Components|InstancedStaticMesh|AddInstance _ismc (Math|Transform|MakeTransform (Math|Vector|MakeVector (.X (Class|KismetMathLibrary|BreakVector3f _location)) (.Y (Class|KismetMathLibrary|BreakVector3f _location)) (+ (.Z (Class|KismetMathLibrary|BreakVector3f _location)) 5e+01)) "0, 0, 0" "0.010000,0.010000,0.010000") false))
      (AddComponent|AddACInstanceAnim _ismc _returnvalue (Math|Transform|MakeTransform (Math|Vector|MakeVector (.X (Class|KismetMathLibrary|BreakVector3f _location)) (.Y (Class|KismetMathLibrary|BreakVector3f _location)) (+ (.Z (Class|KismetMathLibrary|BreakVector3f _location)) 5e+01)) (Math|Rotator|MakeRotator 0.0 0.0 (Math|Random|RandomFloatinRange -1.8e+02 1.8e+02))) DrawDelay 0.5 false))))

(event Custom|RemoveFoliage
  (params (HexLocation :type Vector))
  (bind _outhits (Collision|MultiSphereTraceByChannel HexLocation HexLocation (Variables|Default|GetHexRadius) "TraceTypeQuery1" false 0 "None" false))
  (for _array_element _outhits
    (for _array_element_2 (Variables|Default|GetISMCs)
      (if (== _array_element_2 (.hitcomponent _array_element))
        (AddComponent|AddACInstanceAnim _array_element_2 (.hititem _array_element) (Math|Transform|MakeTransform (.location _array_element)) 0.0 0.5 true)))))

(fn ConstructionScript
  (CallFunction|SetupInstances)
  (CallFunction|SetupNoise))

(fn SetupInstances
  (bind _keys (Utilities|Map|Keys (Variables|Default|GetFoliageGroupMap)))
  (for _array_element _keys
    (bind _returnvalue (AddComponent|AddHierarchicalInstancedStaticMeshComponent false))
    (Components|StaticMesh|SetStaticMesh _returnvalue _array_element)
    (Utilities|FlowControl|Sequence
      (:then_0
        (if (Utilities|Array|ContainsItem (Variables|Default|GetGrassGroups) (.Value (Utilities|Map|Find (Variables|Default|GetFoliageGroupMap) _array_element)))
          (Rendering|SetCustomDepthStencilValue _returnvalue 255)
          (Rendering|SetCastShadow _returnvalue false)
          (Components|InstancedStaticMesh|SetCullDistances _returnvalue 5000 7500)))
      (:then_1
        (Utilities|Array|Add (Variables|Default|GetISMCs) _returnvalue)
        (if (.ReturnValue (Utilities|Map|Find (Variables|Default|GetISMCMap) (.Value (Utilities|Map|Find (Variables|Default|GetFoliageGroupMap) _array_element))))
          (bind _output_get (LocalVariables|SetTempArray (.ismcs (.Value (Utilities|Map|Find (Variables|Default|GetISMCMap) (.Value (Utilities|Map|Find (Variables|Default|GetFoliageGroupMap) _array_element)))))))
          (Utilities|Array|Add _output_get _returnvalue)
          (Utilities|Map|Add (Variables|Default|GetISMCMap) (.Value (Utilities|Map|Find (Variables|Default|GetFoliageGroupMap) _array_element)) (Utilities|Struct|MakeS_ismcArray (LocalVariables|GetTempArray)))
          (else
            (Utilities|Map|Add (Variables|Default|GetISMCMap) (.Value (Utilities|Map|Find (Variables|Default|GetFoliageGroupMap) _array_element)) (Utilities|Struct|MakeS_ismcArray (Utilities|Array|MakeArray _returnvalue)))))))))

(fn SetupNoise
  (bind _terraingen (Variables|Default|GetTerrainGen))
  (bind _seed (Variables|/Game/Blueprints/Map/BP_TerrainGen.BP_TerrainGen_C|GetSeed _terraingen))
  (bind _returnvalue (Game|ConstructObjectfromClass "/Script/FastNoiseGenerator.FastNoiseWrapper"))
  (bind _output_get (Variables|Default|SetCellularNoise _returnvalue))
  (Class|FastNoiseWrapper|SetupFastNoise _output_get "Cellular" _seed 0.001 "Linear" "FBM" 3 2.0 1.0 1.0 "Manhattan" "CellValue")
  (bind _returnvalue_2 (Game|ConstructObjectfromClass "/Script/FastNoiseGenerator.FastNoiseWrapper"))
  (bind _output_get_2 (Variables|Default|SetScatteredNoise _returnvalue_2))
  (Class|FastNoiseWrapper|SetupFastNoise _output_get_2 "Simplex" _seed 0.01 "Linear" "FBM" 3 2.0 1.0 0.45 "Manhattan" "CellValue")
  (bind _returnvalue_3 (Game|ConstructObjectfromClass "/Script/FastNoiseGenerator.FastNoiseWrapper"))
  (bind _output_get_3 (Variables|Default|SetGrassNoise _returnvalue_3))
  (Class|FastNoiseWrapper|SetupFastNoise _output_get_3 "Cellular" _seed 0.001 "Linear" "FBM" 3 2.0 1.0 1.0 "Manhattan" "CellValue"))

(fn ChooseFoliage
  (params (Biome :type Biome%20Enum :default "NewEnumerator0"))
  (bind _biomegroupweights (Variables|Default|GetBiomeGroupWeights))
  (bind _value (Utilities|Map|Find _biomegroupweights Biome))
  (LocalVariables|SetValue (Math|Random|RandomFloatinRange 0.0 (.totalvalue _value)))
  (bind _keys (Utilities|Map|Keys (.groupweights _value)))
  (for _array_element _keys
    (if (< (LocalVariables|GetValue) (.Value (Utilities|Map|Find (.groupweights _value) _array_element)))
      (return (.OutItem (Utilities|Array|Random (.ismcs (.Value (Utilities|Map|Find (Variables|Default|GetISMCMap) _array_element))))))
      (else
        (LocalVariables|SetValue (- (LocalVariables|GetValue) (.Value (Utilities|Map|Find (.groupweights _value) _array_element))))))))

(fn RandomPointinHex
  (params (Center :type Vector) (Radius :type Float%20%28double-precision%29))
  ;[1 1 1] If I ever decide to switch to this - https://stackoverflow.com/questions/3239611/generating-random-points-within-a-hexagon-for-procedural-game-content
)

(fn RandomPointinRadius
  (params (Center :type Vector) (Radius :type Float%20%28double-precision%29))
  (bind (_x _y _z) (Class|KismetMathLibrary|BreakVector3f Center))
  (bind _returnvalue (Math|Random|RandomFloatinRange 0.0 3.6e+02))
  (bind _returnvalue_2 (Math|Random|RandomFloatinRange 0.0 Radius))
  (return (Math|Vector|MakeVector (+ _x (* (Math|Trig|Cos(Degrees) _returnvalue) _returnvalue_2)) (+ _y (* (Math|Trig|Sin(Degrees) _returnvalue) _returnvalue_2)) _z)))

(fn ClearFoliage
  (for _array_element (Variables|Default|GetISMCs)
    (Components|InstancedStaticMesh|ClearInstances _array_element)))