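; Tower placement actor for a tower defense map, spawning towers on instanced ghost tiles mapped to grid coordinates.
; Selection, tower preview and range meshes follow the hit tile, switching materials by validity.
; CanPlaceTower rejects occupied, path or blocked coordinates; placement spawns the tower actor and blocks its tile in TerrainGen.
; Hex-grid save and delayed-replay load remain, though live placement never fills their mesh maps and GenerateGrid is empty.
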(event Custom|AddToGrid
  (params (NewGrid :type Offset%20Coords%20Structure))
  (bind _transform (Default|FGetGroundTransform (Variables|Default|GetTerrainGen) NewGrid))
  (bind _returnvalue (Components|InstancedStaticMesh|AddInstance (Variables|Default|GetGhostTiles_ISM) _transform false))
  (Utilities|Map|Add (Variables|Default|GetGhostInstances) _returnvalue NewGrid))

(event Custom|RunTileActionDynamic
  ;[1 1 1] Run tile action, either adds or deletes
  (if (CallFunction|CanPlaceTower (Variables|Default|GetTileBeingManipulated))
    (CallFunction|AddTowertoSelectedwithAnimation)))

(event Custom|DisableGridBuilding_Event
  (Rendering|SetVisibility (Variables|Default|GetSelectionMesh) false true))

(event Custom|EnableGridBuilding_Event
  (Rendering|SetVisibility (Variables|Default|GetSelectionMesh) true true))

(event Custom|ClearGrid
  (Components|InstancedStaticMesh|ClearInstances (Variables|Default|GetGhostTiles_ISM))
  (Utilities|Map|Clear (Variables|Default|GetGhostInstances)))

(event Custom|UpdatePlacedTower
  (params (TowerData :type S%20Tower%20Data%20Struct%20Structure))
  (bind _towerselectionmesh (Variables|Default|GetTowerSelectionMesh))
  (bind _output_get (Variables|Default|SetTowerToSpawn TowerData))
  (Transformation|SetWorldScale3D (Variables|Default|GetRangeMesh) (Math|Vector|MakeVector (/ (.defaultrange _output_get) 1e+02) (/ (.defaultrange _output_get) 1e+02) 1e+01))
  (Components|StaticMesh|SetStaticMesh _towerselectionmesh (.placingmesh _output_get))
  (Transformation|SetRelativeTransform _towerselectionmesh (Math|Transform|MakeTransform "0, 0, 0" (.costomrotation _output_get) (- (.customscale _output_get) "0.010000,0.010000,0.010000")) false true)
  (for _index (range 0 (- (Rendering|Material|GetNumMaterials _towerselectionmesh) 1))
    (Rendering|Material|SetMaterial _towerselectionmesh _index (Variables|Default|GetTowerSelectionMaterial))))

(event Custom|GenerateGrid)

(event Custom|LoadExistingGridWithDelay
  (params (SaveFile :type Hex%20Grid%20Save%20Object%20Reference))
  ;[1 1 1] Here we load the grid from the save file
  (bind _result (Utilities|Set|ToArray (Variables|/HexGrids/HexGrids/Blueprints/HexGrid_Save.HexGrid_Save_C|GetInstancesUsed SaveFile)))
  (bind _element (Utilities|ForEachLoopwithDelay _result 0.1)
    (:Loop
      (Variables|Default|SetTileBeingManipulated _element)
      (if (.ReturnValue (Utilities|Map|Find (Variables|/HexGrids/HexGrids/Blueprints/HexGrid_Save.HexGrid_Save_C|GetMeshMap SaveFile) (.Value (Utilities|Map|Find (Variables|/HexGrids/HexGrids/Blueprints/HexGrid_Save.HexGrid_Save_C|GetGhostMap SaveFile) _element))))
        (Variables|Default|SetMeshToSpawn (.Value (Utilities|Map|Find (Variables|/HexGrids/HexGrids/Blueprints/HexGrid_Save.HexGrid_Save_C|GetMeshMap SaveFile) (.Value (Utilities|Map|Find (Variables|/HexGrids/HexGrids/Blueprints/HexGrid_Save.HexGrid_Save_C|GetGhostMap SaveFile) _element)))))
        (Variables|Default|SetMaterialForMeshToSpawn (.Value (Utilities|Map|Find (Variables|/HexGrids/HexGrids/Blueprints/HexGrid_Save.HexGrid_Save_C|GetMaterialMap SaveFile) (.Value (Utilities|Map|Find (Variables|/HexGrids/HexGrids/Blueprints/HexGrid_Save.HexGrid_Save_C|GetGhostMap SaveFile) _element)))))
        (CallFunction|RunTileActionDynamic)))))

(event EventBeginPlay
  (bind _asbp_gs_tower_defense (Utilities|Casting|CastToBP_GS_TowerDefense (Game|GetGameState)))
  (Variables|Default|SetGameState _asbp_gs_tower_defense)
  (CallFunction|GenerateGrid)
  (EventDispatchers|BindEventtoDisableGridBuilding (delegate Custom|DisableGridBuilding_Event))
  (EventDispatchers|BindEventtoEnableGridBuilding (delegate Custom|EnableGridBuilding_Event)))

(fn ConstructionScript)

(fn LoadGrid
  (params (SlotName :type String) (UserIndex :type Integer))
  (LocalVariables|SetSaveName SlotName)
  (LocalVariables|SetSaveIndex UserIndex)
  (bind _returnvalue (SaveGame|DoesSaveGameExist (LocalVariables|GetSaveName) (LocalVariables|GetSaveIndex)))
  (if _returnvalue
    (bind _returnvalue_2 (SaveGame|LoadGamefromSlot (LocalVariables|GetSaveName) (LocalVariables|GetSaveIndex)))
    (bind _ashex_grid_save (Utilities|Casting|CastToHexGrid_Save _returnvalue_2))
    (LocalVariables|SetGridSaveFile _ashex_grid_save)
    (Utilities|FlowControl|Sequence
      (:then_0
        (Variables|Default|SetGridScale (Variables|/HexGrids/HexGrids/Blueprints/HexGrid_Save.HexGrid_Save_C|GetGridScale (LocalVariables|GetGridSaveFile)))
        (Variables|Default|SetTileRotation (Variables|/HexGrids/HexGrids/Blueprints/HexGrid_Save.HexGrid_Save_C|GetTileRotation (LocalVariables|GetGridSaveFile)))
        (Variables|Default|SetTileScale (Variables|/HexGrids/HexGrids/Blueprints/HexGrid_Save.HexGrid_Save_C|GetTileScale (LocalVariables|GetGridSaveFile)))
        (CallFunction|GenerateGrid))
      (:then_1
        (CallFunction|LoadExistingGridwithDelay (LocalVariables|GetGridSaveFile))))
    (else
      (Development|PrintString "Error. Failed to find save file for loading grid" true true "(R=1.000000,G=0.000000,B=0.000000,A=1.000000)" 8.0))))

(fn SaveGrid
  (params (SlotName :type String) (UserIndex :type Integer))
  (Utilities|FlowControl|Sequence
    (:then_0
      (bind _returnvalue (SaveGame|CreateSaveGameObject "/HexGrids/HexGrids/Blueprints/HexGrid_Save.HexGrid_Save_C"))
      (LocalVariables|SetSaveFile _returnvalue)
      ;[1 1 1] Set all variables in save file
      (Utilities|FlowControl|Sequence
        (:then_0
          (Variables|/HexGrids/HexGrids/Blueprints/HexGrid_Save.HexGrid_Save_C|SetTileScale (LocalVariables|GetSaveFile) (Variables|Default|GetTileScale)))
        (:then_1
          (Variables|/HexGrids/HexGrids/Blueprints/HexGrid_Save.HexGrid_Save_C|SetTileRotation (LocalVariables|GetSaveFile) (Variables|Default|GetTileRotation)))
        (:then_2
          (Variables|/HexGrids/HexGrids/Blueprints/HexGrid_Save.HexGrid_Save_C|SetInstancesUsed (LocalVariables|GetSaveFile) (Variables|Default|GetInstancesUsed)))
        (:then_3
          (Variables|/HexGrids/HexGrids/Blueprints/HexGrid_Save.HexGrid_Save_C|SetGhostMap (LocalVariables|GetSaveFile) (Variables|Default|GetGhostInstances)))
        (:then_4
          (Variables|/HexGrids/HexGrids/Blueprints/HexGrid_Save.HexGrid_Save_C|SetMeshMap (LocalVariables|GetSaveFile) (Variables|Default|GetMeshMap)))
        (:then_5
          (Variables|/HexGrids/HexGrids/Blueprints/HexGrid_Save.HexGrid_Save_C|SetGridScale (LocalVariables|GetSaveFile) (Variables|Default|GetGridScale)))
        (:then_6
          (Variables|/HexGrids/HexGrids/Blueprints/HexGrid_Save.HexGrid_Save_C|SetMaterialMap (LocalVariables|GetSaveFile) (Variables|Default|GetMaterialMap)))
        (:then_8
          (Variables|/HexGrids/HexGrids/Blueprints/HexGrid_Save.HexGrid_Save_C|SetbUsesRuntimeGrid (LocalVariables|GetSaveFile) true))))
    (:then_1
      (SaveGame|SaveGametoSlot (LocalVariables|GetSaveFile) SlotName UserIndex))))

(fn DeleteSelectedTilewithAnimation
  (params (ID :type Integer))
  (bind _ghostinstances (Variables|Default|GetGhostInstances))
  (bind _value (Utilities|Map|Find _ghostinstances ID))
  (Utilities|Set|Remove (Variables|Default|GetInstancesUsed) ID)
  (Utilities|Set|Remove (Variables|Default|GetTowerSet) _value)
  (Utilities|Set|Remove (Variables|/Game/Blueprints/Map/BP_TerrainGen.BP_TerrainGen_C|GetBlocked (Variables|Default|GetTerrainGen)) _value))

(fn AddTowertoSelectedwithAnimation
  (bind _ghosttiles_ism (Variables|Default|GetGhostTiles_ISM))
  (bind _tilebeingmanipulated (Variables|Default|GetTileBeingManipulated))
  (bind _towertospawn (Variables|Default|GetTowerToSpawn))
  (bind _tilebeingmanipulated_2 (Variables|Default|GetTileBeingManipulated))
  (bind _ghostinstances (Variables|Default|GetGhostInstances))
  (bind (_towername _icon _desc _tower) (Utilities|Struct|BreakS_TowerDataStruct _towertospawn))
  (bind _outinstancetransform (Components|InstancedStaticMesh|GetInstanceTransform _ghosttiles_ism _tilebeingmanipulated false))
  (bind _value (Utilities|Map|Find _ghostinstances _tilebeingmanipulated_2))
  (bind (_location _rotation) (Math|Transform|BreakTransform _outinstancetransform))
  (Utilities|Set|Add (Variables|Default|GetInstancesUsed) _tilebeingmanipulated_2)
  (Utilities|Set|Add (Variables|Default|GetTowerSet) _value)
  (Game|SpawnActorfromClass _tower (Math|Transform|MakeTransform (+ _location (Math|Vector|MakeVector 0.0 0.0 (Variables|Default|GetAddedHeight))) _rotation) "AlwaysSpawn" (Variables|Default|GetCharRef) _towertospawn _icon _value _tilebeingmanipulated_2 0)
  (Utilities|Set|Add (Variables|/Game/Blueprints/Map/BP_TerrainGen.BP_TerrainGen_C|GetBlocked (Variables|Default|GetTerrainGen)) _value))

(fn UpdatePreviewMesh
  (params (HitID :type Integer))
  (bind _selectionmesh (Variables|Default|GetSelectionMesh))
  (bind _towerselectionmesh (Variables|Default|GetTowerSelectionMesh))
  (bind _returnvalue (Rendering|Material|GetNumMaterials _towerselectionmesh))
  (bind _returnvalue_2 (- _returnvalue 1))
  (Variables|Default|SetHitInstanceID HitID)
  (Utilities|FlowControl|Sequence
    (:then_0
      (Transformation|SetRelativeLocation (Variables|Default|GetSelectionMesh) (.location (.OutInstanceTransform (Components|InstancedStaticMesh|GetInstanceTransform (Variables|Default|GetGhostTiles_ISM) (Variables|Default|GetHitInstanceID) false))) false true)
      (Transformation|SetRelativeLocation (Variables|Default|GetTowerSelectionMesh) (+ (.location (.OutInstanceTransform (Components|InstancedStaticMesh|GetInstanceTransform (Variables|Default|GetGhostTiles_ISM) (Variables|Default|GetHitInstanceID) false))) (Math|Vector|MakeVector 0.0 0.0 (Variables|Default|GetAddedHeight))) false true)
      (Transformation|SetWorldLocation (Variables|Default|GetRangeMesh) (.location (.OutInstanceTransform (Components|InstancedStaticMesh|GetInstanceTransform (Variables|Default|GetGhostTiles_ISM) (Variables|Default|GetHitInstanceID) false))) false true))
    (:then_1
      (if (CallFunction|CanPlaceTower (Variables|Default|GetHitInstanceID))
        (Rendering|Material|SetMaterial _selectionmesh 0 "/Game/Assets/World/Tiles/materials/Selection.Selection")
        (for _index (range 0 _returnvalue_2)
          (Rendering|Material|SetMaterial _towerselectionmesh _index "/Game/Assets/Buildings/Towers/TowerRedesigns/M_TowerPlacementMat.M_TowerPlacementMat"))
        (else
          (Rendering|Material|SetMaterial _selectionmesh 0 "/Game/Assets/World/Tiles/materials/SelectionInvalid.SelectionInvalid")
          (for _index_2 (range 0 _returnvalue_2)
            (Rendering|Material|SetMaterial _towerselectionmesh _index_2 "/Game/Assets/Buildings/Towers/TowerRedesigns/MI_TowerPlacementMat_Invalid.MI_TowerPlacementMat_Invalid")))))))

(fn CanPlaceTower
  (params (ItemToFind :type Integer%20%28by%20ref%29))
  (bind _terraingen (Variables|Default|GetTerrainGen))
  (bind _ghostinstances (Variables|Default|GetGhostInstances))
  (bind _value (Utilities|Map|Find _ghostinstances ItemToFind))
  (return (and (not (Math|Boolean|ORBoolean (Utilities|Set|Contains (Variables|Default|GetTowerSet) _value) (Utilities|Set|Contains (Variables|/Game/Blueprints/Map/BP_TerrainGen.BP_TerrainGen_C|GetPaths _terraingen) _value) (Utilities|Set|Contains (Variables|/Game/Blueprints/Map/BP_TerrainGen.BP_TerrainGen_C|GetBlocked _terraingen) _value))) (Variables|Default|GetHitFound))))

(fn HideUnhideSelection
  (params (Hide :type Boolean))
  (bind _rangemesh (Variables|Default|GetRangeMesh))
  (if (and Hide (not (Variables|Default|GetSelectionHidden)))
    (Rendering|SetVisibility (Variables|Default|GetTowerSelectionMesh) false false)
    (Variables|Default|SetSelectionHidden true)
    (Variables|Default|SetHitFound false)
    (Rendering|SetVisibility _rangemesh false false)
    (elif (and (not Hide) (Variables|Default|GetSelectionHidden))
      (Rendering|SetVisibility (Variables|Default|GetSelectionMesh) true true)
      (Variables|Default|SetSelectionHidden false)
      (Variables|Default|SetHitFound true)
      (Rendering|SetVisibility _rangemesh true false))))

(fn OnTileSelectedbyUser
  (Variables|Default|SetTileBeingManipulated (Variables|Default|GetHitInstanceID))
  (if (CallFunction|CanPlaceTower (Variables|Default|GetTileBeingManipulated))
    (CallFunction|AddTowertoSelectedwithAnimation)
    (return true)
    (else
      (return false))))