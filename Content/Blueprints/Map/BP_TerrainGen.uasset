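; Procedurally generates the seeded hex-grid map for a tower defense game, rebuilding when the seed or den count changes.
; FastNoise layers drive biomes, height, mountains, path costs and den placement.
; Dens spawn on expanding rings around the base, each with an A* path back to it.
; Tiles render as per-biome instanced meshes with staggered animation, and drawing also feeds foliage, the tower placement grid and camera bounds.
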(event Custom|DrawTile
  (params (Offset%20Coords :type Offset%20Coords%20Structure))
  (bind _transform (Utilities|GetGroundTransform Offset%20Coords))
  (bind _returnvalue (Math|Transform|MakeTransform (.location _transform) (.rotation _transform) "0.010000,0.010000,0.010000"))
  (bind _hasbeendrawn (CallFunction|CheckifDrawn Offset%20Coords))
  (if (not _hasbeendrawn)
    (Utilities|Array|AddUnique (Variables|MapData|GetDrawnGrid) Offset%20Coords)
    (bind _biome (Foliage|GetBiome Offset%20Coords))
    (Utilities|FlowControl|Sequence
      (:then_0
        (Variables|Default|SetDrawDelay (Math|Random|RandomFloatinRange 0.0 1.0))
        (bind _returnvalue_2 (Components|InstancedStaticMesh|AddInstance (.Value (Utilities|Map|Find (Variables|Instances|GetInstancedGround) _biome)) _returnvalue false))
        (Utilities|Array|Add (Variables|Instances|GetGroundInstanceHolder) (Utilities|Struct|MakeMultiInstanceHolder Offset%20Coords (.Value (Utilities|Map|Find (Variables|Instances|GetInstancedGround) _biome)) _returnvalue_2))
        (AddComponent|AddACInstanceAnim (.Value (Utilities|Map|Find (Variables|Instances|GetInstancedGround) _biome)) _returnvalue_2 _returnvalue (Variables|Default|GetDrawDelay) 0.5 false))
      (:then_1
        (if (not (Utilities|Set|Contains (Variables|MapData|GetPaths) Offset%20Coords))
          (Utilities|FlowControl|Sequence
            (:then_0
              (bind _returnvalue_3 (Components|InstancedStaticMesh|AddInstance (.Value (Utilities|Map|Find (Variables|Instances|GetInstancedSurfaces) _biome)) _returnvalue false))
              (Utilities|Array|Add (Variables|Instances|GetSurfaceInstanceHolder) (Utilities|Struct|MakeMultiInstanceHolder Offset%20Coords (.Value (Utilities|Map|Find (Variables|Instances|GetInstancedSurfaces) _biome)) _returnvalue_3))
              (AddComponent|AddACInstanceAnim (.Value (Utilities|Map|Find (Variables|Instances|GetInstancedSurfaces) _biome)) _returnvalue_3 _returnvalue (Variables|Default|GetDrawDelay) 0.5 false))
            (:then_1
              (if (Utilities|Set|Contains (Variables|MapData|GetMountains) Offset%20Coords)
                (bind _output_get (Variables|Default|SetMountainToAdd (.OutItem (Utilities|Array|Random (Variables|Instances|GetMountainInstances)))))
                (bind _returnvalue_4 (Components|InstancedStaticMesh|AddInstance _output_get (Utilities|GetGroundTransform Offset%20Coords) false))
                (AddComponent|AddACInstanceAnim _output_get _returnvalue_4 _returnvalue (Variables|Default|GetDrawDelay) 0.5 false)
                (else
                  (Default|AddFoliage (Variables|Default|GetFoliageGen) (.location _transform) _biome (Variables|Default|GetDrawDelay))))))))
      (:then_2
        (CallFunction|UpdateCamBoundingVolume Offset%20Coords))
      (:then_3
        (Default|AddtoGrid (Variables|Default|GetTowerPlacer) Offset%20Coords)))))

(event Custom|DrawTiles
  (params (OffsetCoords :type Array%20of%20Offset%20Coords%20Structures))
  (for _array_element OffsetCoords
    (CallFunction|DrawTile _array_element)))

(event Custom|StartingDensChanged
  (params (StarterDens :type Integer))
  (Variables|MapData|SetStarterDens StarterDens)
  (CallFunction|CreateNewMap false))

(event Custom|AddPaths
  (params (Paths :type Array%20of%20Offset%20Coords%20Structures))
  (for _array_element Paths
    (CallFunction|AddPath _array_element)))

(event Custom|AddPath
  (params (Path :type Offset%20Coords%20Structure))
  (bind _gridscale (Variables|MapData|GetGridScale))
  (bind (_precise _returnvalue) (Class|GridsHex|ScaleandOffset Path _gridscale))
  (Utilities|Map|Add (Variables|MapData|GetMapCost) Path 0.0)
  (Utilities|Set|Add (Variables|MapData|GetPaths) Path)
  (Default|RemoveFoliage (Variables|Default|GetFoliageGen) (.location (Utilities|GetGroundTransform Path)) true)
  (bind _outhit (Collision|SphereTraceByChannel (Math|Conversions|ToVector(Vector2D) _precise 2e+03) (Class|GridsCore|ToVector(Offset) _returnvalue -2e+03) 1e+02 "TraceTypeQuery5" false 0 "None" false))
  (bind _values (Utilities|Map|Values (Variables|Instances|GetInstancedSurfaces)))
  (for _array_element _values
    (if (== _array_element (.HitComponent (Collision|BreakHitResult _outhit)))
      (AddComponent|AddACInstanceAnim _array_element (.HitItem (Collision|BreakHitResult _outhit)) (.OutInstanceTransform (Components|InstancedStaticMesh|GetInstanceTransform _array_element (.HitItem (Collision|BreakHitResult _outhit)) true)) 1.0 0.5 true))))

(event Custom|StartGame
  (for _array_element (Variables|Default|GetDenActors)
    (Variables|/Game/Blueprints/Mobs/BP_Path_Start.BP_Path_Start_C|SetAddProgressBool _array_element true)))

(event Custom|AddCost
  (params (Coords :type Offset%20Coords%20Structure))
  (bind (_col _row) (Utilities|Struct|BreakOffsetCoords Coords))
  (if (not (Utilities|Set|Contains (Variables|MapData|GetPaths) Coords))
    (Utilities|Map|Add (Variables|MapData|GetMapCost) Coords (+ (Class|FastNoiseWrapper|GetNoise2D (Variables|Noise|GetCellularNoise) (Math|Conversions|ToFloat(Integer) _col) (Math|Conversions|ToFloat(Integer) _row)) 1.0))))

(event Custom|AddToGrid
  (params (Coords :type Offset%20Coords%20Structure))
  (Utilities|Array|AddUnique (Variables|MapData|GetGeneratedGrid) Coords))

(event Custom|CreateNewMap
  (params (RandomSeed :type Boolean))
  (bind _foliagegen (Variables|Default|GetFoliageGen))
  (if RandomSeed
    (Default|ChangeSeed (Variables|Game|GetGameState) (Math|Random|RandomIntegerinRange -200000000 200000000))
    (else
      (Setup|ClearMap)
      (Setup|SetupNoise)
      (Default|ClearFoliage _foliagegen)
      (Default|SetupNoise _foliagegen)
      (Setup|SetupBase)
      (for _index (range 1 (Variables|MapData|GetStarterDens))
        (Dens|SpawnNewDen)))))

(event Custom|NewSeed
  (params (Seed :type Integer))
  (bind _output_get (Variables|Noise|SetSeed Seed))
  (Default|CallSeedChanged _output_get)
  (CallFunction|CreateNewMap false))

(event EventBeginPlay
  (bind _asbp_gs_tower_defense (Utilities|Casting|CastToBP_GS_TowerDefense (Game|GetGameState)))
  (bind _output_get (Variables|Game|SetGameState _asbp_gs_tower_defense))
  (EventDispatchers|BindEventtoNewSeed _output_get (delegate Custom|NewSeed))
  (EventDispatchers|BindEventtoDensNumberChanged _output_get (delegate Custom|StartingDensChanged))
  (if (Variables|Default|GetLoadGame)
    (Setup|LoadMap)
    (else
      (CallFunction|CreateNewMap true))))

(fn ConstructionScript
  (Variables|MapData|SetGridScale (Math|Vector2D|MakeVector2D (Class|GridsHex|HexWidth (.y (Variables|MapData|GetGridScale))) (.y (Variables|MapData|GetGridScale))))
  (Setup|SetupInstances))

(fn SetupNoise
  (bind _seed (Variables|Noise|GetSeed))
  (bind _returnvalue (Math|Random|MakeRandomStream _seed))
  (bind _returnvalue_2 (Game|ConstructObjectfromClass "/Script/FastNoiseGenerator.FastNoiseWrapper"))
  (bind _output_get (Variables|Noise|SetTempurature _returnvalue_2))
  (Class|FastNoiseWrapper|SetupFastNoise _output_get "Simplex" (Variables|Noise|GetSeed) 0.01 "Linear" "FBM" 3 2.0 5.0 0.45 "Euclidean" "Distance2")
  (bind _returnvalue_3 (Game|ConstructObjectfromClass "/Script/FastNoiseGenerator.FastNoiseWrapper"))
  (bind _output_get_2 (Variables|Noise|SetMagic _returnvalue_3))
  (Class|FastNoiseWrapper|SetupFastNoise _output_get_2 "Simplex" (Variables|Noise|GetSeed) 0.02 "Linear" "FBM" 4 2.0 5.0 0.45 "Euclidean" "Distance2")
  (bind _returnvalue_4 (Game|ConstructObjectfromClass "/Script/FastNoiseGenerator.FastNoiseWrapper"))
  (bind _output_get_3 (Variables|Noise|SetHeightMap _returnvalue_4))
  (Class|FastNoiseWrapper|SetupFastNoise _output_get_3 "Simplex" (Variables|Noise|GetSeed) 0.01 "Linear" "FBM" 3 2.0 1.0 0.45 "Euclidean" "Distance2")
  (bind _returnvalue_5 (Game|ConstructObjectfromClass "/Script/FastNoiseGenerator.FastNoiseWrapper"))
  (bind _output_get_4 (Variables|Noise|SetCellularNoise _returnvalue_5))
  (Class|FastNoiseWrapper|SetupFastNoise _output_get_4 "Cellular" (Variables|Noise|GetSeed) 0.5 "Linear" "FBM" 1 2.0 0.5 1.0 "Natural" "CellValue")
  (bind _returnvalue_6 (Game|ConstructObjectfromClass "/Script/FastNoiseGenerator.FastNoiseWrapper"))
  (bind _output_get_5 (Variables|Noise|SetDenNoise _returnvalue_6))
  (Class|FastNoiseWrapper|SetupFastNoise _output_get_5 "Simplex" (Variables|Noise|GetSeed) 2.0 "Linear" "FBM" 1 2.0 0.5 1.0 "Natural" "CellValue")
  (Variables|Noise|SetBiomeOffset (Utilities|Struct|MakeOffsetCoords (Class|KismetMathLibrary|RandomIntegerfromStream _returnvalue 10000000) (Class|KismetMathLibrary|RandomIntegerfromStream _returnvalue 10000000)))
  (Default|SetupNoise (Variables|Default|GetFoliageGen)))

(fn LoadMap
  (Setup|ClearMap)
  (Setup|SetupNoise))

(fn ClearMap
  (Utilities|FlowControl|Sequence
    (:then_0
      (bind _outactors (Actor|GetAllActorsOfClass "/Game/Blueprints/Mobs/BP_Path_End.BP_Path_End_C"))
      (for _array_element _outactors
        (Actor|DestroyActor _array_element)))
    (:then_1
      (bind _outactors_2 (Actor|GetAllActorsOfClass "/Game/Blueprints/Mobs/BP_Path_Start.BP_Path_Start_C"))
      (for _array_element_2 _outactors_2
        (Actor|DestroyActor _array_element_2)))
    (:then_2
      (bind _values (Utilities|Map|Values (Variables|Instances|GetInstancedGround)))
      (for _array_element_3 _values
        (Components|InstancedStaticMesh|ClearInstances _array_element_3)))
    (:then_3
      (bind _values_2 (Utilities|Map|Values (Variables|Instances|GetInstancedSurfaces)))
      (for _array_element_4 _values_2
        (Components|InstancedStaticMesh|ClearInstances _array_element_4))
      (for _array_element_5 (Variables|Instances|GetMountainInstances)
        (Components|InstancedStaticMesh|ClearInstances _array_element_5)))
    (:then_4
      (Default|ClearFoliage (Variables|Default|GetFoliageGen)))
    (:then_5
      (Utilities|Set|Clear (Variables|MapData|GetPaths))
      (Utilities|Set|Clear (Variables|MapData|GetDens))
      (Utilities|Set|Clear (Variables|MapData|GetBlocked))
      (Utilities|Array|Clear (Variables|MapData|GetGeneratedGrid))
      (Utilities|Array|Clear (Variables|MapData|GetDrawnGrid))
      (Utilities|Map|Clear (Variables|MapData|GetMapCost))
      (Variables|MapData|SetMinDenDistance (Variables|MapData|GetMinDenDistanceDEFAULT))
      (Utilities|Array|Clear (Variables|Default|GetDenActors))
      (Utilities|Set|Clear (Variables|MapData|GetMountains)))
    (:then_6
      (Variables|MapData|SetMinXIndex 0)
      (Variables|MapData|SetMaxXIndex 0)
      (Variables|MapData|SetMinYIndex 0)
      (Variables|MapData|SetMaxYIndex 0))
    (:then_7
      (Default|ClearGrid (Variables|Default|GetTowerPlacer)))))

(fn SetupInstances
  (bind _keys (Utilities|Map|Keys (Variables|Instances|GetGroundMaterials)))
  (for _array_element _keys
    (Utilities|FlowControl|Sequence
      (:then_0
        (bind _returnvalue (AddComponent|AddHierarchicalInstancedStaticMeshComponent false))
        (Components|StaticMesh|SetStaticMesh _returnvalue "/Game/Assets/World/Terrain/TerrainMeshes/SM_Ground.SM_Ground")
        (Rendering|Material|SetMaterial _returnvalue 0 "/Game/Assets/Materials/Landscape/MM_Ground.MM_Ground")
        (Components|InstancedStaticMesh|SetCullDistances _returnvalue 17500 17500)
        (Utilities|Map|Add (Variables|Instances|GetInstancedGround) _array_element _returnvalue))
      (:then_1
        (bind _returnvalue_2 (AddComponent|AddHierarchicalInstancedStaticMeshComponent false))
        (Components|StaticMesh|SetStaticMesh _returnvalue_2 "/Game/Assets/World/Terrain/TerrainMeshes/SM_Surface.SM_Surface")
        (Rendering|Material|SetMaterial _returnvalue_2 0 (.Value (Utilities|Map|Find (Variables|Instances|GetSurfaceMaterials) _array_element)))
        (Components|InstancedStaticMesh|SetCullDistances _returnvalue_2 17500 17500)
        (Utilities|Map|Add (Variables|Instances|GetInstancedSurfaces) _array_element _returnvalue_2))))
  (for _array_element_2 (Variables|Instances|GetMountainMeshes)
    (bind _returnvalue_3 (AddComponent|AddInstancedStaticMeshComponent false))
    (Components|StaticMesh|SetStaticMesh _returnvalue_3 _array_element_2)
    (Utilities|Array|Add (Variables|Instances|GetMountainInstances) _returnvalue_3)))

(fn GetBiome
  (params (Offset%20Coords :type Offset%20Coords%20Structure))
  (bind _tempurature (Variables|Noise|GetTempurature))
  (bind _biomeoffset (Variables|Noise|GetBiomeOffset))
  (bind _returnvalue (+ (.col Offset%20Coords) (.col _biomeoffset)))
  (bind _returnvalue_2 (+ (.row Offset%20Coords) (.row _biomeoffset)))
  (bind _returnvalue_3 (Math|Conversions|ToFloat(Integer) _returnvalue))
  (bind _returnvalue_4 (Math|Conversions|ToFloat(Integer) _returnvalue_2))
  (bind _returnvalue_5 (Class|FastNoiseWrapper|GetNoise2D _tempurature _returnvalue_3 _returnvalue_4))
  (if (< (Class|FastNoiseWrapper|GetNoise2D (Variables|Noise|GetMagic) _returnvalue_3 _returnvalue_4) 0.5)
    (if (< _returnvalue_5 0.5)
      (if (< _returnvalue_5 0.0)
        (if (< _returnvalue_5 -0.5)
          (return "NewEnumerator4")
          (else
            (return "NewEnumerator3")))
        (else
          (return "NewEnumerator2")))
      (else
        (return "NewEnumerator1")))
    (elif (< _returnvalue_5 0.5)
      (if (< _returnvalue_5 0.0)
        (if (< _returnvalue_5 -0.5)
          (return "NewEnumerator8")
          (else
            (return "NewEnumerator7")))
        (else
          (return "NewEnumerator6")))
      (else
        (return "NewEnumerator5")))))

(fn SetupBase
  (bind _basecoords (Variables|MapData|GetBaseCoords))
  (Utilities|FlowControl|Sequence
    (:then_0
      (Setup|SetupCosts _basecoords (Variables|MapData|GetInitialSetupRadius) false))
    (:then_1
      (CallFunction|AddPath _basecoords)
      (bind _offset (Class|GridsHex|SingleRing _basecoords 1))
      (CallFunction|AddPaths _offset)
      (Setup|DrawAroundBase))
    (:then_2
      (bind _returnvalue (Game|SpawnActorfromClass "/Game/Blueprints/Mobs/BP_Path_End.BP_Path_End_C" (Utilities|GetGroundTransform) "AlwaysSpawn" "OverrideRootScale" 0 _basecoords false 0 0 0 0))
      (Variables|Default|SetBase _returnvalue))))

(fn SpawnNewDen
  (bind _base (Variables|Default|GetBase))
  (bind (_denfound _newden _denpath) (Dens|GetNextDen))
  (if _denfound
    (Utilities|Set|Add (Variables|MapData|GetDens) _newden)
    (Setup|SetupCosts _newden 20 false)
    (bind _den (Dens|GetDenType _newden))
    (bind _returnvalue (Game|SpawnActorfromClass _den (Math|Transform|MakeTransform (.location (Utilities|GetGroundTransform _newden)) "0, 0, 0" "1.000000,1.000000,1.000000") "Undefined" "SelectDefaultAtRuntime" 0 (Utilities|Array|MakeArray _base) self _newden true _denpath _base (Variables|Default|GetGameDirector) 0))
    (Utilities|Array|Add (Variables|Default|GetDenActors) _returnvalue)))

(fn GetNextDen
  (bind _mindendistance (Variables|MapData|GetMinDenDistance))
  (bind _basecoords (Variables|MapData|GetBaseCoords))
  (while (>= (Variables|MapData|GetMaxDenDistance) (Variables|MapData|GetMinDenDistance))
    (Setup|SetupCosts _basecoords (+ (Variables|MapData|GetInitialSetupRadius) _mindendistance) true)
    (bind _offset (Class|GridsHex|SingleRing _basecoords _mindendistance))
    (for _array_element _offset
      (LocalVariables|SetDenTooClose false)
      (if (>= (Class|FastNoiseWrapper|GetNoise2D (Variables|Noise|GetDenNoise) (Math|Conversions|ToFloat(Integer) (.Col (Utilities|Struct|BreakOffsetCoords _array_element))) (Math|Conversions|ToFloat(Integer) (.Row (Utilities|Struct|BreakOffsetCoords _array_element)))) (Variables|MapData|GetDenThreshold))
        (bind _offset_2 (Class|GridsHex|SpiralRing _array_element 4))
        (bind _output_get (LocalVariables|SetTilesToCheck _offset_2))
        (Utilities|Array|Add _output_get _array_element)
        (for _array_element_2 _output_get
          (if (Utilities|Set|Contains (Variables|MapData|GetDens) _array_element_2)
            (LocalVariables|SetDenTooClose true)))
        (if (not (LocalVariables|GetDenTooClose))
          (bind _results (Class|GridsHex|AStarPathfinding :StartPoint (Variables|MapData|GetBaseCoords) :EndPoint _array_element :Grid (Variables|MapData|GetGeneratedGrid) :Cost (Variables|MapData|GetMapCost) :Blocked (Variables|MapData|GetBlocked)))
          (if (>= (Utilities|Array|Length _results) (LocalVariables|GetShortestDistanceAllowed))
            (return true _array_element (Class|GridsCore|ToOffsetArray(CubeArray) _results))))))
    (Math|Integer|IncrementInt (Variables|MapData|GetMinDenDistance)))
  (return false "(Col=0,Row=0)" 0))

(fn SetupCosts
  (params (Center :type Offset%20Coords%20Structure) (Radius :type Integer) (SingleRing :type Boolean))
  (bind _offset (Class|GridsHex|SingleRing Center Radius))
  (bind _offset_2 (Class|GridsHex|SpiralRing Center Radius))
  (bind _output_get (LocalVariables|SetCoordsToGenerate (select SingleRing _offset _offset_2)))
  (Utilities|Array|Add _output_get Center)
  (for _array_element _output_get
    (Utilities|FlowControl|Sequence
      (:then_0
        (CallFunction|AddtoGrid _array_element))
      (:then_1
        (if (not (Utilities|Set|Contains (Variables|MapData|GetPaths) _array_element))
          (Utilities|Map|Add (Variables|MapData|GetMapCost) _array_element (Utilities|GetPathingCost _array_element))))
      (:then_2
        (if (and (Variables|MapData|GetMountainsEnabled) (> (Class|FastNoiseWrapper|GetNoise2D (Variables|Noise|GetHeightMap) (Math|Conversions|ToFloat(Integer) (.Col (Utilities|Struct|BreakOffsetCoords _array_element))) (Math|Conversions|ToFloat(Integer) (.Row (Utilities|Struct|BreakOffsetCoords _array_element)))) (Variables|MapData|GetMountainThreshold)))
          (Utilities|Set|Add (Variables|MapData|GetBlocked) _array_element)
          (Utilities|Set|Add (Variables|MapData|GetMountains) _array_element)
          (CallFunction|DrawTile _array_element))))))

(fn CheckifDrawn
  (params (OffsetCoords :type Offset%20Coords%20Structure))
  (bind _gridscale (Variables|MapData|GetGridScale))
  (bind _precise (Class|GridsHex|ScaleandOffset OffsetCoords _gridscale))
  (bind _returnvalue (Collision|LineTraceByChannel (Math|Conversions|ToVector(Vector2D) _precise 2e+03) (Math|Conversions|ToVector(Vector2D) _precise -2e+03) "TraceTypeQuery5" false 0 "None" false))
  (return _returnvalue))

(fn UpdateCamBoundingVolume
  (params (OffsetCoords :type Offset%20Coords%20Structure))
  (Utilities|FlowControl|Sequence
    (:then_0
      (bind _output_get (Variables|MapData|SetMinXIndex (Math|Integer|Min(Integer) (.col OffsetCoords) (Variables|MapData|GetMinXIndex))))
      (Variables|MapData|SetMinX (.X (Math|Vector2D|BreakVector2D (.Precise (Class|GridsHex|ScaleandOffset (Utilities|Struct|MakeOffsetCoords _output_get 0) (Variables|MapData|GetGridScale)))))))
    (:then_1
      (bind _output_get_2 (Variables|MapData|SetMaxXIndex (Math|Integer|Max(Integer) (.col OffsetCoords) (Variables|MapData|GetMaxXIndex))))
      (Variables|MapData|SetMaxX (.X (Math|Vector2D|BreakVector2D (.Precise (Class|GridsHex|ScaleandOffset (Utilities|Struct|MakeOffsetCoords _output_get_2 0) (Variables|MapData|GetGridScale)))))))
    (:then_2
      (bind _output_get_3 (Variables|MapData|SetMinYIndex (Math|Integer|Min(Integer) (.row OffsetCoords) (Variables|MapData|GetMinYIndex))))
      (Variables|MapData|SetMinY (.Y (Math|Vector2D|BreakVector2D (.Precise (Class|GridsHex|ScaleandOffset (Utilities|Struct|MakeOffsetCoords 0 _output_get_3) (Variables|MapData|GetGridScale)))))))
    (:then_3
      (bind _output_get_4 (Variables|MapData|SetMaxYIndex (Math|Integer|Max(Integer) (.row OffsetCoords) (Variables|MapData|GetMaxYIndex))))
      (Variables|MapData|SetMaxY (.Y (Math|Vector2D|BreakVector2D (.Precise (Class|GridsHex|ScaleandOffset (Utilities|Struct|MakeOffsetCoords 0 _output_get_4) (Variables|MapData|GetGridScale)))))))
    (:then_4
      (bind _returnvalue (Actor|GetActorOfClass "/Script/OpenRTSCamera.RTSCameraBoundsVolume"))
      (Transformation|SetActorScale3D _returnvalue (Math|Vector|MakeVector (/ (- (Variables|MapData|GetMaxX) (Variables|MapData|GetMinX)) 2.5e+03) (/ (- (Variables|MapData|GetMaxY) (Variables|MapData|GetMinY)) 2.5e+03) 1.0))
      (Transformation|SetActorLocation _returnvalue (Math|Vector|MakeVector (/ (+ (Variables|MapData|GetMaxX) (Variables|MapData|GetMinX)) 2.0) (/ (+ (Variables|MapData|GetMaxY) (Variables|MapData|GetMinY)) 2.0) 0.0) false true))))

(fn FGetGroundTransform
  (params (Offset%20Coords :type Offset%20Coords%20Structure))
  (return (Utilities|GetGroundTransform Offset%20Coords)))

(fn DrawAroundBase
  (bind _basecoords (Variables|MapData|GetBaseCoords))
  (CallFunction|DrawTile _basecoords)
  (bind _offset (Class|GridsHex|SpiralRing _basecoords 3))
  (CallFunction|DrawTiles _offset))

(fn GetDenType
  (params (OffsetCoords :type Offset%20Coords%20Structure))
  (bind _biome (Foliage|GetBiome OffsetCoords))
  (return (.OutItem (Utilities|Array|RandomFromStream (.dens (.Value (Utilities|Map|Find (Variables|MapData|GetBiomesToDens) _biome))) (Variables|MapData|GetDenStream)))))