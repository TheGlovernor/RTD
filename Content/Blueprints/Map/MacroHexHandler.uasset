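; Procedurally generates the tower defense map as radius-4 macro hexes, starting from a walled base and expandable through spawned ExploreButton actors.
; Each new hex links neighboring path entrances to random exits with A*, occasionally splitting, or ends them centrally when exits run short.
; Exits determine the next explorable centers.
; Tiles render as per-type instanced ground and surface meshes, omitting surfaces on paths, with game-state noise driving button height.
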(event Custom|DrawExpandableButtons
  (bind _self self)
  (bind _newexplorablecenters (Variables|Map|GetNewExplorableCenters))
  (for _array_element (Variables|Map|GetNewExplorableCenters)
    (if (not (Utilities|Array|ContainsItem (Variables|Map|GetAlreadyDrawnButtons) _array_element))
      (Game|SpawnActorfromClass "/Game/Blueprints/Map/ExploreButton.ExploreButton_C" (Math|Transform|MakeTransform (Math|Conversions|ToVector(Vector2D) (.Precise (Class|GridsHex|ScaleandOffset _array_element (Variables|Map|GetGridScale))) (* (/ (Math|Conversions|ToFloat(Integer) (Math|Float|Ceil (* (Class|FastNoiseWrapper|GetNoise2D (Variables|Map|GetHeightMap) (Math|Conversions|ToFloat(Integer) (.Col (Utilities|Struct|BreakOffsetCoords _array_element))) (Math|Conversions|ToFloat(Integer) (.Row (Utilities|Struct|BreakOffsetCoords _array_element)))) 2e+01))) (/ 1e+01 (Math|Conversions|ToFloat(Integer) (Variables|Map|GetStepHeight)))) 1e+01)) "0, 0, 0" "2.000000,2.000000,2.000000") "Undefined" _self _array_element _self 0)))
  (Utilities|Array|AppendArray (Variables|Map|GetAlreadyDrawnButtons) _newexplorablecenters)
  (Utilities|Array|Clear _newexplorablecenters))

(event EventBeginPlay
  (CallFunction|DrawExpandableButtons))

(event Collision|EventActorBeginOverlap
  (params (OtherActor :type Actor%20Object%20Reference)))

(event EventTick
  (params (DeltaSeconds :type Float%20%28single-precision%29)))

(fn ConstructionScript
  (bind _returnvalue (Math|Random|RandomIntegerinRange -100000 100000))
  (bind _astower_defense_state (Utilities|Casting|CastToTowerDefenseState (Game|GetGameState)))
  (bind _output_get (Variables|Game|SetGameState _astower_defense_state))
  (Variables|Map|SetHeightMap (Variables|/Game/Blueprints/GM/TowerDefenseState.TowerDefenseState_C|Getheight _output_get))
  (CallFunction|SetTileMeshInstances)
  (CallFunction|DeleteGrid)
  (if (not (Variables|Game|GetLoadSave))
    (Variables|Game|SetSeed%20Rand%20Stream (Math|Random|MakeRandomStream _returnvalue))
    (Class|FastNoiseWrapper|SetSeed (Variables|Map|GetHeightMap) _returnvalue)
    (CallFunction|GenerateMacroHex true (Variables|/Game/Blueprints/GM/TowerDefenseState.TowerDefenseState_C|GetglobalPaths (Variables|Game|GetGameState)))))

(fn SetTileMeshInstances
  (Utilities|Map|Clear (Variables|Instances|GetInstancedGround))
  (bind _keys (Utilities|Map|Keys (Variables|Instances|GetGroundMeshes)))
  (for _array_element _keys
    (Utilities|FlowControl|Sequence
      (:then_0
        (bind _returnvalue (AddComponent|AddInstancedStaticMeshComponent false))
        (Components|StaticMesh|SetStaticMesh _returnvalue (.Value (Utilities|Map|Find (Variables|Instances|GetGroundMeshes) _array_element)))
        (Utilities|Map|Add (Variables|Instances|GetInstancedGround) _array_element _returnvalue))
      (:then_1
        (bind _returnvalue_2 (AddComponent|AddInstancedStaticMeshComponent false))
        (Components|StaticMesh|SetStaticMesh _returnvalue_2 (.Value (Utilities|Map|Find (Variables|Instances|GetSurfaceMeshes) _array_element)))
        (Utilities|Map|Add (Variables|Instances|GetInstancedSurfaces) _array_element _returnvalue_2)))))

(fn DeleteGrid)

(fn GenerateMacroHex
  (params (IsBase :type Boolean) (StartingPaths :type Integer) (Center :type Offset%20Coords%20Structure))
  (bind _newexplorablecenters (Variables|Map|GetNewExplorableCenters))
  (if IsBase
    (bind _potentialexits (CallFunction|GetPotentialExits Center))
    (bind (_newtiles _newpaths _nexexits) (CallFunction|SetupBase _potentialexits Center StartingPaths))
    (CallFunction|DrawGrid _newtiles _newpaths)
    (bind _newexplorablecenters_2 (CallFunction|SetAreastoExpandto _nexexits Center))
    (Utilities|Array|AppendArray _newexplorablecenters _newexplorablecenters_2)
    (Variables|Map|SetExploredCenter Center)
    (else
      (bind _potentialexits_2 (CallFunction|GetPotentialExits Center))
      (bind (_newtiles_2 _newpaths_2 _newexits) (CallFunction|SetupTiles _potentialexits_2 Center))
      (CallFunction|DrawGrid _newtiles_2 _newpaths_2)
      (bind _newexplorablecenters_3 (CallFunction|SetAreastoExpandto _newexits Center))
      (Utilities|Array|AppendArray _newexplorablecenters _newexplorablecenters_3)
      (Variables|Map|SetExploredCenter Center)
      (CallFunction|DrawExpandableButtons))))

(fn GetPotentialExits
  (params (Center :type Offset%20Coords%20Structure))
  (bind _returnvalue (Class|GridsCore|ToCube(Offset) Center))
  (bind _keys (Utilities|Map|Keys (Variables|Default|GetOuterToInnerMapMP)))
  (for _array_element _keys
    (if (not (Utilities|Set|Contains (Variables|Map|GetBlockedMap) (Class|GridsCore|ToOffset(Cube) (+ _array_element _returnvalue))))
      (Utilities|Array|AddUnique (LocalVariables|GetExits) (Class|GridsCore|ToOffset(Cube) (+ _returnvalue (.Value (Utilities|Map|Find (Variables|Default|GetOuterToInnerMapMP) _array_element)))))))
  (return (LocalVariables|GetExits)))

(fn SetExits
  (params (PotentialExits :type Array%20of%20Offset%20Coords%20Structures)))

(fn SetupBase
  (params (PotentialExits :type Array%20of%20Offset%20Coords%20Structures) (Origin :type Offset%20Coords%20Structure) (StarterPaths :type Integer))
  (LocalVariables|SetLocalPotentialExits PotentialExits)
  (bind _output_get (LocalVariables|SetLocalOrigin Origin))
  (bind _offset (Class|GridsHex|SpiralRing _output_get 4))
  (bind _output_get_2 (LocalVariables|SetLocalGrid _offset))
  (for _array_element _output_get_2
    (Utilities|Map|Add (LocalVariables|GetLocalTerrainMap) _array_element "NewEnumerator0"))
  (Utilities|FlowControl|Sequence
    (:then_0
      (for _index (range 1 StarterPaths)
        (bind _output_get_3 (LocalVariables|SetIndex (Class|KismetMathLibrary|RandomIntegerfromStream (Utilities|Array|Length (LocalVariables|GetLocalPotentialExits)) (Variables|Game|GetSeed%20Rand%20Stream))))
        (Utilities|FlowControl|Sequence
          (:then_0
            (Utilities|Array|Add (LocalVariables|GetLocalExits) (Utilities|Array|Get(acopy) (LocalVariables|GetLocalPotentialExits) _output_get_3)))
          (:then_1
            (Utilities|Array|RemoveItem (LocalVariables|GetLocalPotentialExits) (Utilities|Array|Get(acopy) (LocalVariables|GetLocalPotentialExits) _output_get_3))))))
    (:then_1
      (Utilities|Map|Add (LocalVariables|GetLocalTerrainMap) (LocalVariables|GetLocalOrigin) "NewEnumerator4")
      (Utilities|Set|Add (Variables|Map|GetBlockedMap) (LocalVariables|GetLocalOrigin))
      (for _array_element_2 (Class|GridsCore|ToOffsetArray(CubeArray) (LocalVariables|GetWallCoords))
        (Utilities|Map|Add (LocalVariables|GetLocalTerrainMap) (+ _array_element_2 (LocalVariables|GetLocalOrigin)) "NewEnumerator5")
        (Utilities|Set|Add (Variables|Map|GetBlockedMap) (+ _array_element_2 (LocalVariables|GetLocalOrigin)))))
    (:then_2
      (for _array_element_3 (LocalVariables|GetLocalExits)
        (bind _results (Class|GridsHex|AStarPathfinding :StartPoint (LocalVariables|GetLocalOrigin) :EndPoint _array_element_3 :Grid (LocalVariables|GetLocalGrid) :Blocked (Variables|Map|GetBlockedMap)))
        (Utilities|Set|AddItems (LocalVariables|GetLocalPaths) (Class|GridsCore|ToOffsetArray(CubeArray) _results))))
    (:then_3
      (Utilities|Set|AddItems (Variables|Map|GetBlockedMap) (LocalVariables|GetLocalGrid)))
    (:then_4
      (return (LocalVariables|GetLocalTerrainMap) (LocalVariables|GetLocalPaths) (LocalVariables|GetLocalExits)))))

(fn DrawGrid
  (params (NewTiles :type Map%20of%20Offset%20Coords%20Structures%20to%20Bytes) (NewPaths :type Set%20of%20Offset%20Coords%20Structures))
  (Utilities|FlowControl|Sequence
    (:then_0
      (bind _result (Utilities|Set|ToArray NewPaths))
      (Utilities|Set|AddItems (Variables|Map|GetPathMap) _result))
    (:then_1
      (bind _keys (Utilities|Map|Keys NewTiles))
      (bind _output_get (LocalVariables|SetCoords _keys))
      (Utilities|Set|AddItems (Variables|Map|GetBlockedMap) _output_get)
      (for _array_element _output_get
        (bind _returnvalue (Game|ConstructObjectfromClass "/Game/Assets/Tiles/TileDataAsset.TileDataAsset_C" (.Value (Utilities|Map|Find NewTiles _array_element)) (Utilities|Set|Contains NewPaths _array_element)))
        (Utilities|Map|Add (Variables|Map|GetMap) _array_element _returnvalue)
        (Utilities|FlowControl|Sequence
          (:then_0
            (bind _returnvalue_2 (Components|InstancedStaticMesh|AddInstance (.Value (Utilities|Map|Find (Variables|Instances|GetInstancedGround) (.Value (Utilities|Map|Find NewTiles _array_element)))) (|MakeGroundTransform _array_element) false))
            (Utilities|Array|Add (Variables|Map|GetGroundInstanceHolder) (Utilities|Struct|MakeMultiInstanceHolder _array_element (.Value (Utilities|Map|Find (Variables|Instances|GetInstancedGround) (.Value (Utilities|Map|Find NewTiles _array_element)))) _returnvalue_2)))
          (:then_1
            (if (not (Utilities|Set|Contains NewPaths _array_element))
              (bind _returnvalue_3 (Components|InstancedStaticMesh|AddInstance (.Value (Utilities|Map|Find (Variables|Instances|GetInstancedSurfaces) (.Value (Utilities|Map|Find NewTiles _array_element)))) (|MakeSurfaceTransform _array_element) false))
              (Utilities|Array|Add (Variables|Map|GetSurfaceInstanceHolder) (Utilities|Struct|MakeMultiInstanceHolder _array_element (.Value (Utilities|Map|Find (Variables|Instances|GetInstancedSurfaces) (.Value (Utilities|Map|Find NewTiles _array_element)))) _returnvalue_3)))))))))

(fn SetupTiles
  (params (PotentialExits :type Array%20of%20Offset%20Coords%20Structures) (Center :type Offset%20Coords%20Structure))
  (bind _exittoentrancemap (LocalVariables|GetExitToEntranceMap))
  (bind _blockedmap (Variables|Map|GetBlockedMap))
  (bind _localenterances (LocalVariables|GetLocalEnterances))
  (bind _localenterances_2 (LocalVariables|GetLocalEnterances))
  (bind _localpaths (LocalVariables|GetLocalPaths))
  (bind _returnvalue (Utilities|Array|Length _localenterances))
  (Utilities|FlowControl|Sequence
    (:then_0
      (bind _output_get (LocalVariables|SetLocalCenter Center)) ; Set Grid and Origin
      (bind _offset (Class|GridsHex|MovementRange _output_get 4))
      (bind _output_get_2 (LocalVariables|SetLocalGrid _offset))
      (Utilities|Array|Add _output_get_2 (LocalVariables|GetLocalCenter))
      (LocalVariables|SetLocalPotentialExits PotentialExits)
      (for _array_element (LocalVariables|GetLocalGrid)
        (Utilities|Map|Add (LocalVariables|GetLocalTerrainMap) _array_element "NewEnumerator0")))
    (:then_1
      (for _array_element_2 (Variables|Default|GetInnerMidpoints)
        (for _array_element_3 (Class|GridsHex|GetHexNeighbours (Class|GridsCore|ToOffset(Cube) (+ _array_element_2 (Class|GridsCore|ToCube(Offset) (LocalVariables|GetLocalCenter)))))
          (if (Utilities|Set|Contains (Variables|Map|GetPathMap) (Class|GridsCore|ToOffset(Cube) _array_element_3))
            (Utilities|Array|AddUnique (LocalVariables|GetLocalEnterances) (Class|GridsCore|ToOffset(Cube) (+ _array_element_2 (Class|GridsCore|ToCube(Offset) (LocalVariables|GetLocalCenter)))))))))
    (:then_2
      (for _array_element_4 (LocalVariables|GetLocalEnterances)
        (if (Utilities|Array|ContainsItem (LocalVariables|GetLocalPotentialExits) _array_element_4)
          (Utilities|Array|RemoveItem (LocalVariables|GetLocalPotentialExits) _array_element_4))))
    (:then_3
      (if (>= (Utilities|Array|Length (LocalVariables|GetLocalPotentialExits)) (Utilities|Array|Length (LocalVariables|GetLocalEnterances)))
        (Utilities|FlowControl|Sequence
          (:then_0
            (if (== _returnvalue 1)
              (Utilities|Map|Add (LocalVariables|GetExitToEntranceMap) (Utilities|Array|Get(acopy) (LocalVariables|GetLocalPotentialExits) (Math|Random|RandomIntegerinRangefromStream 0 (- (Utilities|Array|Length (LocalVariables|GetLocalPotentialExits)) 1) (Variables|Game|GetSeed%20Rand%20Stream))) (Utilities|Array|Get(acopy) (LocalVariables|GetLocalEnterances)))
              (if (and (Utilities|Array|IsNotEmpty (LocalVariables|GetLocalPotentialExits)) (> (Math|Float|Log (Variables|Default|GetChanceOfSplit) 1e+01) (Math|Random|RandomFloatfromStream (Variables|Game|GetSeed%20Rand%20Stream))))
                (Utilities|Map|Add (LocalVariables|GetExitToEntranceMap) (Utilities|Array|Get(acopy) (LocalVariables|GetLocalPotentialExits) (Math|Random|RandomIntegerinRangefromStream 0 (- (Utilities|Array|Length (LocalVariables|GetLocalPotentialExits)) 1) (Variables|Game|GetSeed%20Rand%20Stream))) (Utilities|Array|Get(acopy) (LocalVariables|GetLocalEnterances)))
                (Variables|Default|SetChanceOfSplit 1.0)
                (else
                  (bind _output_get_3 (Variables|Default|SetChanceOfSplit (+ (Variables|Default|GetChanceOfSplit) 0.5)))
                  (Development|PrintString (Utilities|String|ToString(Float) _output_get_3) true true "(R=1.000000,G=0.065753,B=0.000000,A=1.000000)" 1e+05)))))
          (:then_1
            (if (== _returnvalue 2)
              (if (!= (Utilities|Array|Length (LocalVariables|GetChosenExits)) (Utilities|Array|Length (LocalVariables|GetLocalEnterances))) :!label _label
                (Utilities|Array|AddUnique (LocalVariables|GetChosenExits) (Utilities|Array|Get(acopy) (LocalVariables|GetLocalPotentialExits) (Math|Random|RandomIntegerinRangefromStream 0 (- (Utilities|Array|Length (LocalVariables|GetLocalPotentialExits)) 1) (Variables|Game|GetSeed%20Rand%20Stream))))
                (goto _label)
                (else
                  (for (_array_element_5 _array_index) (LocalVariables|GetLocalEnterances)
                    (Utilities|Map|Add (LocalVariables|GetExitToEntranceMap) (Utilities|Array|Get(acopy) (LocalVariables|GetChosenExits) _array_index) _array_element_5))))))
          (:then_2
            (if (== _returnvalue 3)
              (goto _label))))
        (else
          (LocalVariables|SetBuildNormalPath false))))
    (:then_4
      (Utilities|FlowControl|Sequence
        (:then_0
          (bind _offset_2 (Class|GridsHex|SingleRing (LocalVariables|GetLocalCenter) 4))
          (Utilities|Set|AddItems (Variables|Map|GetBlockedMap) _offset_2)
          (bind _keys (Utilities|Map|Keys _exittoentrancemap))
          (bind _values (Utilities|Map|Values _exittoentrancemap))
          (Utilities|Set|RemoveItems _blockedmap _keys)
          (Utilities|Set|RemoveItems _blockedmap _values))
        (:then_1
          (if (LocalVariables|GetBuildNormalPath)
            (bind _keys_2 (Utilities|Map|Keys (LocalVariables|GetExitToEntranceMap)))
            (Development|PrintString (Utilities|String|ToString(Integer) (Utilities|Array|Length _keys_2)) true true "(R=0.000000,G=0.660000,B=1.000000,A=1.000000)" 1e+03)
            (for _array_element_6 _keys_2
              (Utilities|Set|Add _localpaths _array_element_6)
              (Utilities|Set|Add _localpaths (.Value (Utilities|Map|Find (LocalVariables|GetExitToEntranceMap) _array_element_6)))
              (bind (_bsuccess _results) (Class|GridsHex|AStarPathfinding :StartPoint _array_element_6 :EndPoint (.Value (Utilities|Map|Find (LocalVariables|GetExitToEntranceMap) _array_element_6)) :Grid (LocalVariables|GetLocalGrid) :Blocked (Variables|Map|GetBlockedMap)))
              (if _bsuccess
                _
                (else
                  (Development|PrintString "OOF" true true "(R=0.000000,G=0.660000,B=1.000000,A=1.000000)" 456456.0)))
              (Utilities|Set|AddItems (LocalVariables|GetLocalPaths) (Class|GridsCore|ToOffsetArray(CubeArray) _results)))
            (Utilities|Set|AddItems (Variables|Map|GetBlockedMap) _keys_2)
            (else
              (Utilities|Set|AddItems (LocalVariables|GetLocalPaths) _localenterances_2)
              (for _array_element_7 _localenterances_2
                (bind _results_2 (Class|GridsHex|AStarPathfinding :StartPoint _array_element_7 :EndPoint (LocalVariables|GetLocalCenter) :Grid (LocalVariables|GetLocalGrid) :Blocked (Variables|Map|GetBlockedMap)))
                (Utilities|Set|AddItems (LocalVariables|GetLocalPaths) (Class|GridsCore|ToOffsetArray(CubeArray) _results_2)))
              (bind _offset_3 (Class|GridsHex|SpiralRing (LocalVariables|GetLocalCenter) (Math|Integer|Clamp(Integer) (Utilities|Array|Length (LocalVariables|GetLocalEnterances)) 1 3)))
              (Utilities|Set|AddItems (LocalVariables|GetLocalPaths) _offset_3))))))
    (:then_5
      (bind _keys_3 (Utilities|Map|Keys (LocalVariables|GetExitToEntranceMap)))
      (return (LocalVariables|GetLocalTerrainMap) (LocalVariables|GetLocalPaths) _keys_3))))

(fn SetAreastoExpandto
  (params (Exits :type Array%20of%20Offset%20Coords%20Structures) (Center :type Offset%20Coords%20Structure))
  (bind _newcenters (LocalVariables|GetNewCenters))
  (for _array_element Exits
    (Utilities|FlowControl|Sequence
      (:then_0
        (if (Utilities|Operators|EqualEqual (Class|GridsCore|ToCube(Offset) (- _array_element Center)) "4.000000,-4.000000,0" 0.0)
          (Utilities|FlowControl|Sequence
            (:then_0
              (Utilities|Array|AddUnique _newcenters "5.000000,-9.000000,4.000000" :!label _label))
            (:then_1
              (Utilities|Array|AddUnique _newcenters "9.000000,-4.000000,-5.000000" :!label _label_2)))))
      (:then_1
        (if (Utilities|Operators|EqualEqual (Class|GridsCore|ToCube(Offset) (- _array_element Center)) "4.000000,-2.000000,-2.000000" 0.0)
          (goto _label_2)))
      (:then_2
        (if (Utilities|Operators|EqualEqual (Class|GridsCore|ToCube(Offset) (- _array_element Center)) "4.000000,0.000000,-4.000000" 0.0)
          (Utilities|FlowControl|Sequence
            (:then_0
              (goto _label_2))
            (:then_1
              (Utilities|Array|AddUnique _newcenters "4.000000,5.000000,-9.000000" :!label _label_3)))))
      (:then_3
        (if (Utilities|Operators|EqualEqual (Class|GridsCore|ToCube(Offset) (- _array_element Center)) "2.000000,2.000000,-4.000000" 0.0)
          (goto _label_3)))
      (:then_4
        (if (Utilities|Operators|EqualEqual (Class|GridsCore|ToCube(Offset) (- _array_element Center)) "0.000000,4.000000,-4.000000" 0.0)
          (Utilities|FlowControl|Sequence
            (:then_0
              (goto _label_3))
            (:then_1
              (Utilities|Array|AddUnique _newcenters "-5.000000,9.000000,-4.000000" :!label _label_4)))))
      (:then_5
        (if (Utilities|Operators|EqualEqual (Class|GridsCore|ToCube(Offset) (- _array_element Center)) "-2.000000,4.000000,-2.000000" 0.0)
          (goto _label_4)))
      (:then_6
        (if (Utilities|Operators|EqualEqual (Class|GridsCore|ToCube(Offset) (- _array_element Center)) "-4.000000,4.000000,0.000000" 0.0)
          (Utilities|FlowControl|Sequence
            (:then_0
              (goto _label_4))
            (:then_1
              (Utilities|Array|AddUnique _newcenters "-9.000000,4.000000,5.000000" :!label _label_5)))))
      (:then_7
        (if (Utilities|Operators|EqualEqual (Class|GridsCore|ToCube(Offset) (- _array_element Center)) "-4.000000,2.000000,2.000000" 0.0)
          (goto _label_5)))
      (:then_8
        (if (Utilities|Operators|EqualEqual (Class|GridsCore|ToCube(Offset) (- _array_element Center)) "-4.000000,0.000000,4.000000" 0.0)
          (Utilities|FlowControl|Sequence
            (:then_0
              (goto _label_5))
            (:then_1
              (Utilities|Array|AddUnique _newcenters "-4.000000,-5.000000,9.000000" :!label _label_6)))))
      (:then_9
        (if (Utilities|Operators|EqualEqual (Class|GridsCore|ToCube(Offset) (- _array_element Center)) "-2.000000,-2.000000,4.000000" 0.0)
          (goto _label_6)))
      (:then_10
        (if (Utilities|Operators|EqualEqual (Class|GridsCore|ToCube(Offset) (- _array_element Center)) "0.000000,-4.000000,4.000000" 0.0)
          (Utilities|FlowControl|Sequence
            (:then_0
              (goto _label_6))
            (:then_1
              (goto _label)))))
      (:then_11
        (if (Utilities|Operators|EqualEqual (Class|GridsCore|ToCube(Offset) (- _array_element Center)) "2.000000,-4.000000,2.000000" 0.0)
          (goto _label)))))
  (for _array_element_2 (LocalVariables|GetNewCenters)
    (Utilities|Array|Add (LocalVariables|GetOffsetCenters) (Class|GridsCore|ToOffset(Cube) (+ (Class|GridsCore|ToCube(Offset) Center) _array_element_2))))
  (return (LocalVariables|GetOffsetCenters)))