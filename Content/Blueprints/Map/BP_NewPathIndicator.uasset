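; BP_NewPathIndicator is a map actor that shows a clickable screen alert marking its world position, apparently for a new path.
; On BeginPlay it creates a CBB_Alert widget, then each tick projects a point above itself to the viewport, pinning the button to the screen edge when off-screen.
; Clicking briefly makes the RTS camera follow the actor.
; On destruction it unfollows the camera and removes the button.
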(event Custom|OpenTickGate
  (bind _returnvalue (Transformation|GetActorLocation))
  (bind _returnvalue_2 (+ _returnvalue "0.000000,0.000000,500.000000"))
  (Utilities|FlowControl|Gate true) ; enters at Open
)

(event Custom|Focus
  (bind _bp_openrtscamera (CallFunction|GetOpenRTSCamera))
  (bind _asbp_newcam (Utilities|Casting|CastToBP_NEWCAM _bp_openrtscamera))
  (Class|RTSCamera|FollowTarget (Variables|/OpenRTSCamera/BP_RTSCamera.BP_RTSCamera_C|GetRTSCamera _asbp_newcam) self)
  (Utilities|FlowControl|Delay 0.2)
  (Class|RTSCamera|UnFollowTarget (Variables|/OpenRTSCamera/BP_RTSCamera.BP_RTSCamera_C|GetRTSCamera _asbp_newcam)))

(event EventTick
  (params (DeltaSeconds :type Float%20%28single-precision%29))
  (bind _returnvalue (Transformation|GetActorLocation))
  (bind _returnvalue_2 (+ _returnvalue "0.000000,0.000000,500.000000"))
  (Utilities|FlowControl|Gate true
    (:Exit
      (bind _bonscreen (CallFunction|IsLocationonScreen _returnvalue_2))
      (if _bonscreen
        (Class|UserWidget|SetPositioninViewport (Variables|Default|GetAlertButton) (- (.ScreenLocation (Class|PlayerController|ProjectWorldLocationtoScreen (Game|GetPlayerController 0) _returnvalue_2 false)) "(X=32.000000,Y=32.000000)") true)
        (else
          (bind _screencoords (CallFunction|GetScreenEdgeCoords _returnvalue_2 0.9))
          (Class|UserWidget|SetPositioninViewport (Variables|Default|GetAlertButton) (- _screencoords "(X=32.000000,Y=32.000000)") true))))))

(event EventBeginPlay
  (bind _returnvalue (UserInterface|CreateWidget "/Game/Blueprints/UI/CBB_Alert.CBB_Alert_C" 0 0 true false false false false false false true false true false 0))
  (EventDispatchers|BindEventtoClicked _returnvalue (delegate Custom|Focus))
  (Class|UserWidget|SetDesiredSizeinViewport _returnvalue "(X=64.000000,Y=64.000000)")
  (UserInterface|Viewport|AddtoViewport _returnvalue -1)
  (Variables|Default|SetAlertButton _returnvalue)
  (CallFunction|OpenTickGate))

(event EventDestroyed
  (bind _bp_openrtscamera (CallFunction|GetOpenRTSCamera))
  (bind _asbp_newcam (Utilities|Casting|CastToBP_NEWCAM _bp_openrtscamera))
  (Class|RTSCamera|UnFollowTarget (Variables|/OpenRTSCamera/BP_RTSCamera.BP_RTSCamera_C|GetRTSCamera _asbp_newcam))
  (Widget|RemovefromParent (Variables|Default|GetAlertButton)))

(fn ConstructionScript)