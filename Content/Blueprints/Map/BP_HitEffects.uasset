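; BP_HitEffects batches armor and shield block and break hit effects into a single Niagara system.
; Add events for each of the four hit types queue non-zero locations, raised slightly on Z, into per-type position arrays.
; Every Tick it pushes the arrays to the HitEffects system as vector array parameters and clears them, so one component handles all hits that frame.
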(event Custom|AddShieldBlock
  (params (Location :type Vector))
  (if (Utilities|Operators|NotEqual(!=) :A Location :ErrorTolerance 0.1)
    (Utilities|Array|Add (Variables|Default|GetShieldBlockPositions) (+ Location "0.000000,0.000000,50.000000"))))

(event Custom|AddArmorBlock
  (params (Location :type Vector))
  (if (Utilities|Operators|NotEqual(!=) :A Location :ErrorTolerance 0.1)
    (Utilities|Array|Add (Variables|Default|GetArmorBlockPositions) (+ Location "0.000000,0.000000,50.000000"))))

(event Custom|AddArmorBreak
  (params (Location :type Vector))
  (if (Utilities|Operators|NotEqual(!=) :A Location :ErrorTolerance 0.1)
    (Utilities|Array|Add (Variables|Default|GetArmorBreakPositions) (+ Location "0.000000,0.000000,50.000000"))))

(event Custom|AddShieldBreak
  (params (Location :type Vector))
  (if (Utilities|Operators|NotEqual(!=) :A Location :ErrorTolerance 0.1)
    (Utilities|Array|Add (Variables|Default|GetShieldBreakPositions) (+ Location "0.000000,0.000000,50.000000"))))

(event EventTick
  (params (DeltaSeconds :type Float%20%28single-precision%29))
  (Class|NiagaraDataInterfaceArrayFunctionLibrary|SetNiagaraArrayVector (Variables|Default|GetHitEffects) "ArmorBlockPositions" (Variables|Default|GetArmorBlockPositions))
  (Utilities|Array|Clear (Variables|Default|GetArmorBlockPositions))
  (Class|NiagaraDataInterfaceArrayFunctionLibrary|SetNiagaraArrayVector (Variables|Default|GetHitEffects) "ArmorBreakPositions" (Variables|Default|GetArmorBreakPositions))
  (Utilities|Array|Clear (Variables|Default|GetArmorBreakPositions))
  (Class|NiagaraDataInterfaceArrayFunctionLibrary|SetNiagaraArrayVector (Variables|Default|GetHitEffects) "ShieldBlockPositions" (Variables|Default|GetShieldBlockPositions))
  (Utilities|Array|Clear (Variables|Default|GetShieldBlockPositions))
  (Class|NiagaraDataInterfaceArrayFunctionLibrary|SetNiagaraArrayVector (Variables|Default|GetHitEffects) "ShieldBreakPositions" (Variables|Default|GetShieldBreakPositions))
  (Utilities|Array|Clear (Variables|Default|GetShieldBreakPositions)))

(fn ConstructionScript)