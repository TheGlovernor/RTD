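; ExploreButton is a map actor with a widget button that expands the hex map when clicked.
; On begin play it hands itself to its ExploreButtonWidget, and each tick it rotates its root to face the player camera.
; Its Clicked function destroys the actor, debug-prints the cube coordinates and asks the Handler to generate a non-base macro hex centred on its stored coordinates.
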(event EventBeginPlay
  (bind _asexplore_button_widget (Utilities|Casting|CastToExploreButtonWidget (UserInterface|GetWidget (Variables|Default|GetWidget))))
  (Variables|/Game/Blueprints/Map/ExploreButtonWidget.ExploreButtonWidget_C|SetActor _asexplore_button_widget self))

(event EventTick
  (params (DeltaSeconds :type Float%20%28single-precision%29))
  (Transformation|SetWorldRotation (Variables|Default|GetDefaultSceneRoot) (Math|Rotator|FindLookatRotation (Transformation|GetWorldLocation (Variables|Default|GetDefaultSceneRoot)) (Transformation|GetActorLocation (Game|GetPlayerCameraManager 0))) false false))

(fn ConstructionScript)

(fn Clicked
  (Actor|DestroyActor)
  (Development|PrintString (Utilities|String|ToString(Vector) (Class|GridsCore|ToCube(Offset) (Variables|Default|GetCoords))) true true "(R=1.000000,G=0.135502,B=0.000000,A=1.000000)" 1e+07)
  (Default|GenerateMacroHex (Variables|Default|GetHandler) false 1 (Variables|Default|GetCoords)))