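; BP_SkyCycle drives a repeating day/night cycle by rotating a directional light.
; It caches BP_GS_TowerDefense on BeginPlay, then every Tick wraps the elapsed time of that object's Time timer by CycleLengthSeconds.
; NightPercentage splits the cycle, remapping day and night separately onto 180-degree pitch sweeps so each can last a different length.
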(event EventBeginPlay
  (bind _returnvalue (Actor|GetActorOfClass "/Game/Blueprints/GM/BP_GS_TowerDefense.BP_GS_TowerDefense_C"))
  (Variables|Default|SetState _returnvalue))

(event EventTick
  (params (DeltaSeconds :type Float%20%28single-precision%29))
  (bind _state (Variables|Default|GetState))
  (bind _cyclelengthseconds (Variables|Default|GetCycleLengthSeconds))
  (bind _nightpercentage (Variables|Default|GetNightPercentage))
  (bind _returnvalue (- 1.0 _nightpercentage))
  (bind _time (Variables|/Game/Blueprints/GM/BP_GS_TowerDefense.BP_GS_TowerDefense_C|GetTime _state))
  (bind _returnvalue_2 (Class|KismetSystemLibrary|GetTimerElapsedTimeHandle _time))
  (bind _returnvalue_3 (Math|Float|%(Float) _returnvalue_2 _cyclelengthseconds))
  (bind _returnvalue_4 (/ _returnvalue_3 _cyclelengthseconds))
  (if (> _returnvalue _returnvalue_4)
    (Transformation|SetWorldRotation (Variables|Default|GetDirectionalLight) (Math|Rotator|MakeRotator 0.1 (+ (* (/ _returnvalue_4 _returnvalue) 1.8e+02) 1.8e+02) 15.0) true false)
    (else
      (Transformation|SetWorldRotation (Variables|Default|GetDirectionalLight) (Math|Rotator|MakeRotator 0.1 (* (/ (- _returnvalue_4 _returnvalue) (Variables|Default|GetNightPercentage)) 1.8e+02) 15.0) true false))))

(fn ConstructionScript)