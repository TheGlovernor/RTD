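; BP_NoiseVisualizer previews BP_TerrainGen's noise as a hex map of instanced mesh tiles built ring by ring.
; Each tile stores cellular noise, which doubles as path cost, and den noise in custom data.
; High den-noise tiles beyond a minimum radius become dens, each given an A* path.
; Line traces find path tiles to flag, and their cost drops to near zero so later paths reuse them.
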(event Custom|DrawTile
  (params (Coords :type Offset%20Coords%20Structure))
  (bind _returnvalue (Class|GridsCore|ToVector2D(Offset) Coords))
  (bind _instancedstaticmesh (Variables|Default|GetInstancedStaticMesh))
  (bind _terraingenactor (Variables|Default|GetTerrainGenActor))
  (bind _cellularnoise (Variables|/Game/Blueprints/Map/BP_TerrainGen.BP_TerrainGen_C|GetCellularNoise _terraingenactor))
  (bind _dennoise (Variables|/Game/Blueprints/Map/BP_TerrainGen.BP_TerrainGen_C|GetDenNoise _terraingenactor))
  (bind _returnvalue_2 (Class|FastNoiseWrapper|GetNoise2D _cellularnoise (.x _returnvalue) (.y _returnvalue)))
  (bind _returnvalue_3 (Class|FastNoiseWrapper|GetNoise2D _dennoise (.x _returnvalue) (.y _returnvalue)))
  (bind _returnvalue_4 (+ _returnvalue_3 1.0))
  (bind _returnvalue_5 (+ _returnvalue_2 1.0))
  (bind _returnvalue_6 (Math|Float|Square _returnvalue_5))
  (bind _returnvalue_7 (/ _returnvalue_4 2.0))
  (bind _returnvalue_8 (Math|Float|Square _returnvalue_6))
  (bind _transform (Default|FGetGroundTransform (Variables|Default|GetTerrainGenActor) Coords))
  (bind _returnvalue_9 (Components|InstancedStaticMesh|AddInstance _instancedstaticmesh (Math|Transform|MakeTransform (+ (.location _transform) "0,0,1.000000") (.rotation _transform) (.scale _transform)) false))
  (Components|InstancedStaticMesh|SetCustomDataValue _instancedstaticmesh _returnvalue_9 0 _returnvalue_8 false)
  (Components|InstancedStaticMesh|SetCustomDataValue _instancedstaticmesh _returnvalue_9 1 _returnvalue_7 false)
  (Utilities|Array|AddUnique (Variables|Default|GetGrid) Coords)
  (Utilities|Map|Add (Variables|Default|GetCost) Coords _returnvalue_8)
  (if (and (>= _returnvalue_7 (Variables|Default|GetDenThreshold)) (> (Class|GridsHex|ManhattanDistanceOffset Coords) (Variables|Default|GetMinRadius)))
    (Utilities|Array|Add (Variables|Default|GetDens) Coords)))

(event Custom|Draw
  (CallFunction|ClearMap)
  (bind _returnvalue (Actor|GetActorOfClass "/Game/Blueprints/Map/BP_TerrainGen.BP_TerrainGen_C"))
  (bind _output_get (Variables|Default|SetTerrainGenActor _returnvalue))
  (Utilities|IsValid _output_get
    (:Is%20Valid
      (Variables|Default|SetGridScale (Variables|/Game/Blueprints/Map/BP_TerrainGen.BP_TerrainGen_C|GetGridScale _output_get))
      (Variables|Default|SetDenThreshold (Variables|/Game/Blueprints/Map/BP_TerrainGen.BP_TerrainGen_C|GetDenThreshold _output_get))
      (for _index (range 0 (Variables|Default|GetRadius))
        (bind _offset (Class|GridsHex|SingleRing "(Col=0,Row=0)" _index))
        (for _array_element _offset
          (CallFunction|DrawTile _array_element)))
      (CallFunction|ShowPaths))))

(event EventBeginPlay)

(fn ConstructionScript)

(fn ShowPaths
  (for _array_element (Variables|Default|GetDens)
    (bind _results (Class|GridsHex|AStarPathfinding :EndPoint _array_element :Grid (Variables|Default|GetGrid) :Cost (Variables|Default|GetCost) :bAllowInexact true))
    (for _array_element_2 (Class|GridsCore|ToOffsetArray(CubeArray) _results)
      (bind _outhit (Collision|LineTraceByChannel (Math|Conversions|ToVector(Vector2D) (.Precise (Class|GridsHex|ScaleandOffset _array_element_2 (Variables|Default|GetGridScale))) 1e+03) (Math|Conversions|ToVector(Vector2D) (.Precise (Class|GridsHex|ScaleandOffset _array_element_2 (Variables|Default|GetGridScale))) -1e+03) "TraceTypeQuery1" false 0 "None" false "(R=1.000000,G=0.000000,B=0.000000,A=1.000000)" "(R=0.000000,G=1.000000,B=0.000000,A=1.000000)" 6e+01))
      (Components|InstancedStaticMesh|SetCustomDataValue (Variables|Default|GetInstancedStaticMesh) (.HitItem (Collision|BreakHitResult _outhit)) 2 1.0 true)
      (Utilities|Map|Add (Variables|Default|GetCost) _array_element_2 0.0001))))

(fn ClearMap
  (Components|InstancedStaticMesh|ClearInstances (Variables|Default|GetInstancedStaticMesh))
  (Utilities|Array|Clear (Variables|Default|GetDens)))