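; BP_ScoutAreaButton is a world-placed widget button that reveals new map area in the tower defense game.
; On BeginPlay it links itself to its ScoutButton widget and hides if the game state is paused, then rotates to face the player camera every tick.
; Clicked flags the WaveDirector as game started, destroys the button and has its Handler generate a non-base macro hex at its Coords.
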(event EventBeginPlay
  (bind _asscout_button (Utilities|Casting|CastToScoutButton (UserInterface|GetWidget (Variables|Default|GetWidget))))
  (Variables|/Game/UI/ScoutButton.ScoutButton_C|Setactor _asscout_button self)
  (bind _asbp_gs_tower_defense (Utilities|Casting|CastToBP_GS_TowerDefense (Game|GetGameState)))
  (if (Variables|/Game/Blueprints/GM/BP_GS_TowerDefense.BP_GS_TowerDefense_C|GetPaused _asbp_gs_tower_defense)
    (Rendering|SetActorHiddenInGame true)
    (else
      (Rendering|SetActorHiddenInGame false))))

(event EventTick
  (params (DeltaSeconds :type Float%20%28single-precision%29))
  (Transformation|SetWorldRotation (Variables|Default|GetDefaultSceneRoot) (Math|Rotator|FindLookatRotation (Transformation|GetWorldLocation (Variables|Default|GetDefaultSceneRoot)) (Transformation|GetActorLocation (Game|GetPlayerCameraManager 0))) false false))

(fn ConstructionScript)

(fn Clicked
  (bind _asbp_gs_tower_defense (Utilities|Casting|CastToBP_GS_TowerDefense (Game|GetGameState))
    (:then
      (Variables|/Game/Blueprints/Mobs/BP_WaveDirector.BP_WaveDirector_C|SetGameStarted (Variables|/Game/Blueprints/GM/BP_GS_TowerDefense.BP_GS_TowerDefense_C|GetWaveDirector _asbp_gs_tower_defense) true))
    (:CastFailed
      _))
  (Actor|DestroyActor)
  (Default|GenerateMacroHex (Variables|Default|GetHandler) false 1 (Variables|Default|GetCoords)))