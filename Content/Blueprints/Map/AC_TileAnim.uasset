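; Actor component that animates the scale of one tile instance in an instanced static mesh, for a grow or shrink effect.
; After a random delay it zeroes the scale and opens a tick gate.
; Each tick samples a size curve over half a second, optionally reversed, and updates the instance transform.
; When the time is up it closes the gate and destroys itself.
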(event Custom|OpenTickGate
  (Utilities|FlowControl|Gate true) ; enters at Open
)

(event Custom|CloseTickGate
  (Utilities|FlowControl|Gate true) ; enters at Close
)

(event EventBeginPlay
  (Utilities|FlowControl|Delay (Math|Random|RandomFloatinRange 0.1 1.0))
  (Variables|Default|SetTransform (Math|Transform|MakeTransform (.location (Variables|Default|GetTransform)) (.rotation (Variables|Default|GetTransform)) "0.000000,0.000000,0.000000"))
  (CallFunction|OpenTickGate))

(event EventTick
  (params (DeltaSeconds :type Float%20%28single-precision%29))
  (Utilities|FlowControl|Gate true
    (:Exit
      (Variables|Default|SetLifetime (+ (Variables|Default|GetLifetime) DeltaSeconds))
      (Components|InstancedStaticMesh|UpdateInstanceTransform (Variables|Default|GetISMC) (Variables|Default|GetIndex) (Math|Transform|MakeTransform (.location (Variables|Default|GetTransform)) (.rotation (Variables|Default|GetTransform)) (Math|Conversions|ToVector(Float) (Math|Curves|GetFloatValue (Variables|Default|GetSizeCurve) (select (Variables|Default|GetReverse) (- 0.5 (Variables|Default|GetLifetime)) (Variables|Default|GetLifetime))))) false false false)
      (Variables|Default|SetTransform (Math|Transform|MakeTransform (.location (Variables|Default|GetTransform)) (.rotation (Variables|Default|GetTransform)) (Math|Conversions|ToVector(Float) (Math|Curves|GetFloatValue (Variables|Default|GetSizeCurve) (select (Variables|Default|GetReverse) (- 0.5 (Variables|Default|GetLifetime)) (Variables|Default|GetLifetime))))))
      (if (> (Variables|Default|GetLifetime) 0.5)
        (CallFunction|CloseTickGate)
        (Components|DestroyComponent)))))