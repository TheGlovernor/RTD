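; Runtime tower placer for the tower defense hex map, letting the player spawn tower actors on unoccupied tiles.
; It builds instanced ghost tiles from the GameState terrain grid, moves preview meshes to the hit instance and toggles their visibility with grid-building events.
; Selection spawns TowerToSpawn and records the used instance.
; HexGrid_Save supports saving and delayed replay loading, but the mesh placement filling its maps is unwired, as is deletion.
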(event Custom|OnTileSelectedByUser
  ;[1 1 1] On User Selection
  (Variables|Default|SetTileBeingManipulated (Variables|Default|GetHitInstanceID))
  (CallFunction|RunTileActionDynamic))

(event Custom|RunTileActionDynamic
  ;[1 1 1] Run tile action, either adds or deletes
  (if (not (CallFunction|DoesTileContainMesh (Variables|Default|GetTileBeingManipulated)))
    (CallFunction|AddTiletoSelectedwithAnimation)))

(event Custom|DisableGridBuilding_Event
  ;[1 1 1] Bind events to activate and deactivate. We just hide the meshes. Clearing and respawning them each time is another option. Its a balance between a single fps spike on generation, or a constant small memory cost.
  (Rendering|SetVisibility (Variables|Default|GetGhostTiles_ISM) false false))

(event Custom|EnableGridBuilding_Event
  ;[1 1 1] Bind events to activate and deactivate. We just hide the meshes. Clearing and respawning them each time is another option. Its a balance between a single fps spike on generation, or a constant small memory cost.
  (Rendering|SetVisibility (Variables|Default|GetGhostTiles_ISM) true false))

(event Custom|GenerateGrid
  ;[1 1 1] Generate Grid
  (Utilities|FlowControl|Sequence
    (:then_0
      ;[1 1 1] Calculate grid spacing
      (Variables|Default|SetGridScaleCalculated (Variables|/Game/Blueprints/GM/TowerDefenseState.TowerDefenseState_C|GetGrid%20Scale%202D (Variables|Default|GetGameState))))
    (:then_1
      (bind _output_get (Variables|Default|SetGrid (Variables|/Game/Blueprints/Map/terrainGrid.terrainGrid_C|GetGrid (Variables|/Game/Blueprints/GM/TowerDefenseState.TowerDefenseState_C|GetterrainGrid (Variables|Default|GetGameState)))))
      ;[1 1 1] Standard add instance setup as used in most other hex grid blueprints
      (for _array_element _output_get
        (bind _returnvalue (Components|InstancedStaticMesh|AddInstance (Variables|Default|GetGhostTiles_ISM) (Math|Transform|MakeTransform (Math|Conversions|ToVector(Vector2D) (.Precise (Class|GridsHex|ScaleandOffset _array_element (Variables|Default|GetGridScaleCalculated))) (|Gettileheight _array_element)) (Variables|Default|GetTileRotation) (Variables|Default|GetTileScale)) false))
        (Utilities|Map|Add (Variables|Default|GetGhostInstances) _returnvalue _array_element)))
    (:then_2
      ;[1 1 1] Bind events to activate and deactivate. We just hide the meshes. Clearing and respawning them each time is another option. Its a balance between a single fps spike on generation, or a constant small memory cost.
      (EventDispatchers|BindEventtoDisableGridBuilding (delegate Custom|DisableGridBuilding_Event))
      (EventDispatchers|BindEventtoEnableGridBuilding (delegate Custom|EnableGridBuilding_Event)))))

(event Custom|LoadExistingGridWithDelay
  (params (SaveFile :type Hex%20Grid%20Save%20Object%20Reference))
  ;[1 1 1] Here we load the grid from the save file
  (bind _result (Utilities|Set|ToArray (Variables|/HexGrids/HexGrids/Blueprints/HexGrid_Save.HexGrid_Save_C|GetInstancesUsed SaveFile)))
  (bind _element (Utilities|ForEachLoopwithDelay _result 0.1)
    (:Loop
      (Variables|Default|SetTileBeingManipulated _element)
      (if (.ReturnValue (Utilities|Map|Find (Variables|/HexGrids/HexGrids/Blueprints/HexGrid_Save.HexGrid_Save_C|GetMeshMap SaveFile) (.Value (Utilities|Map|Find (Variables|/HexGrids/HexGrids/Blueprints/HexGrid_Save.HexGrid_Save_C|GetGhostMap SaveFile) _element))))
        (Variables|Default|SetMeshToSpawn (.Value (Utilities|Map|Find (Variables|/HexGrids/HexGrids/Blueprints/HexGrid_Save.HexGrid_Save_C|GetMeshMap SaveFile) (.Value (Utilities|Map|Find (Variables|/HexGrids/HexGrids/Blueprints/HexGrid_Save.HexGrid_Save_C|GetGhostMap SaveFile) _element)))))
        (Variables|Default|SetMaterialForMeshToSpawn (.Value (Utilities|Map|Find (Variables|/HexGrids/HexGrids/Blueprints/HexGrid_Save.HexGrid_Save_C|GetMaterialMap SaveFile) (.Value (Utilities|Map|Find (Variables|/HexGrids/HexGrids/Blueprints/HexGrid_Save.HexGrid_Save_C|GetGhostMap SaveFile) _element)))))
        (CallFunction|RunTileActionDynamic)))))

(event EventBeginPlay
  (bind _astower_defense_state (Utilities|Casting|CastToTowerDefenseState (Game|GetGameState)))
  (bind _output_get (Variables|Default|SetGameState _astower_defense_state))
  (Variables|Default|SetHeight (Variables|/Game/Blueprints/GM/TowerDefenseState.TowerDefenseState_C|Getheight _output_get))
  ;[1 1 1] If Load is true, wait for user to call the load grid function
  (Utilities|FlowControl|Delay 0.2)
  (if (not (Variables|Default|GetLoadExistingGridFromSave))
    (CallFunction|GenerateGrid)))

(fn ConstructionScript)

(fn LoadGrid
  (params (SlotName :type String) (UserIndex :type Integer))
  (LocalVariables|SetSaveName SlotName)
  (LocalVariables|SetSaveIndex UserIndex)
  (bind _returnvalue (SaveGame|DoesSaveGameExist (LocalVariables|GetSaveName) (LocalVariables|GetSaveIndex)))
  (if _returnvalue
    (bind _returnvalue_2 (SaveGame|LoadGamefromSlot (LocalVariables|GetSaveName) (LocalVariables|GetSaveIndex)))
    (bind _ashex_grid_save (Utilities|Casting|CastToHexGrid_Save _returnvalue_2))
    (LocalVariables|SetGridSaveFile _ashex_grid_save)
    (Utilities|FlowControl|Sequence
      (:then_0
        (Variables|Default|SetGridScale (Variables|/HexGrids/HexGrids/Blueprints/HexGrid_Save.HexGrid_Save_C|GetGridScale (LocalVariables|GetGridSaveFile)))
        (Variables|Default|SetMaxGridSize (Variables|/HexGrids/HexGrids/Blueprints/HexGrid_Save.HexGrid_Save_C|GetMaxGridSize (LocalVariables|GetGridSaveFile)))
        (Variables|Default|SetTileRotation (Variables|/HexGrids/HexGrids/Blueprints/HexGrid_Save.HexGrid_Save_C|GetTileRotation (LocalVariables|GetGridSaveFile)))
        (Variables|Default|SetTileScale (Variables|/HexGrids/HexGrids/Blueprints/HexGrid_Save.HexGrid_Save_C|GetTileScale (LocalVariables|GetGridSaveFile)))
        (CallFunction|GenerateGrid))
      (:then_1
        (CallFunction|LoadExistingGridwithDelay (LocalVariables|GetGridSaveFile))))
    (else
      (Development|PrintString "Error. Failed to find save file for loading grid" true true "(R=1.000000,G=0.000000,B=0.000000,A=1.000000)" 8.0))))

(fn SaveGrid
  (params (SlotName :type String) (UserIndex :type Integer))
  (Utilities|FlowControl|Sequence
    (:then_0
      (bind _returnvalue (SaveGame|CreateSaveGameObject "/HexGrids/HexGrids/Blueprints/HexGrid_Save.HexGrid_Save_C"))
      (LocalVariables|SetSaveFile _returnvalue)
      ;[1 1 1] Set all variables in save file
      (Utilities|FlowControl|Sequence
        (:then_0
          (Variables|/HexGrids/HexGrids/Blueprints/HexGrid_Save.HexGrid_Save_C|SetTileScale (LocalVariables|GetSaveFile) (Variables|Default|GetTileScale)))
        (:then_1
          (Variables|/HexGrids/HexGrids/Blueprints/HexGrid_Save.HexGrid_Save_C|SetTileRotation (LocalVariables|GetSaveFile) (Variables|Default|GetTileRotation)))
        (:then_2
          (Variables|/HexGrids/HexGrids/Blueprints/HexGrid_Save.HexGrid_Save_C|SetInstancesUsed (LocalVariables|GetSaveFile) (Variables|Default|GetInstancesUsed)))
        (:then_3
          (Variables|/HexGrids/HexGrids/Blueprints/HexGrid_Save.HexGrid_Save_C|SetGhostMap (LocalVariables|GetSaveFile) (Variables|Default|GetGhostInstances)))
        (:then_4
          (Variables|/HexGrids/HexGrids/Blueprints/HexGrid_Save.HexGrid_Save_C|SetMeshMap (LocalVariables|GetSaveFile) (Variables|Default|GetMeshMap)))
        (:then_5
          (Variables|/HexGrids/HexGrids/Blueprints/HexGrid_Save.HexGrid_Save_C|SetGridScale (LocalVariables|GetSaveFile) (Variables|Default|GetGridScale)))
        (:then_6
          (Variables|/HexGrids/HexGrids/Blueprints/HexGrid_Save.HexGrid_Save_C|SetMaterialMap (LocalVariables|GetSaveFile) (Variables|Default|GetMaterialMap)))
        (:then_7
          (Variables|/HexGrids/HexGrids/Blueprints/HexGrid_Save.HexGrid_Save_C|SetMaxGridSize (LocalVariables|GetSaveFile) (Variables|Default|GetMaxGridSize)))
        (:then_8
          (Variables|/HexGrids/HexGrids/Blueprints/HexGrid_Save.HexGrid_Save_C|SetbUsesRuntimeGrid (LocalVariables|GetSaveFile) true))))
    (:then_1
      (SaveGame|SaveGametoSlot (LocalVariables|GetSaveFile) SlotName UserIndex))))

(fn DeleteSelectedTilewithAnimation
  (bind _tilebeingmanipulated (Variables|Default|GetTileBeingManipulated))
  (bind _ghostinstances (Variables|Default|GetGhostInstances))
  (bind _tilebeingmanipulated_2 (Variables|Default|GetTileBeingManipulated))
  (bind _value (Utilities|Map|Find _ghostinstances _tilebeingmanipulated))
  ;[1 1 1] Just a visually interesting deletion, use whatever you like.
  ; This node also destroys the static mesh component on completion, which is the simpliest method of timing the DestroyComponent.
  ; You could bind to the onComplete in the component, but the problem is if a second delete is called before the first has completed, the ref will be wrong
  (AddComponent|AddStaticMeshScaleTIleComponent "0.000000,0.000000,0.000000" 15.0 (.Value (Utilities|Map|Find (Variables|Default|GetInstanceToPlacedMeshMap) (Variables|Default|GetTileBeingManipulated))) true)
  ;[1 1 1] Remove mesh from various maps and mark the instance as a empty tile
  (Utilities|Map|Remove (Variables|Default|GetMeshes) _value)
  (Utilities|Map|Remove (Variables|Default|GetInstanceToPlacedMeshMap) _tilebeingmanipulated_2)
  (Utilities|Set|Remove (Variables|Default|GetInstancesUsed) _tilebeingmanipulated_2)
  (Utilities|Map|Remove (Variables|Default|GetMeshMap) _value)
  (Utilities|Map|Remove (Variables|Default|GetMaterialMap) _value))

(fn AddTiletoSelectedwithAnimation
  (bind _ghosttiles_ism (Variables|Default|GetGhostTiles_ISM))
  (bind _tilebeingmanipulated (Variables|Default|GetTileBeingManipulated))
  (bind _outinstancetransform (Components|InstancedStaticMesh|GetInstanceTransform _ghosttiles_ism _tilebeingmanipulated false))
  (bind (_location _rotation) (Math|Transform|BreakTransform _outinstancetransform))
  (Utilities|Set|Add (Variables|Default|GetInstancesUsed) (Variables|Default|GetTileBeingManipulated))
  (Game|SpawnActorfromClass (Utilities|GetClass (Variables|Default|GetTowerToSpawn)) (Math|Transform|MakeTransform _location _rotation "3.000000,3.000000,3.000000") "AlwaysSpawn" 0 (Game|Player|GetPlayerPawn 0)))

(fn UpdatePreviewMesh
  (params (HitID :type Integer))
  (bind _selectionmesh (Variables|Default|GetSelectionMesh))
  (Variables|Default|SetHitInstanceID HitID)
  (Utilities|FlowControl|Sequence
    (:then_0
      (Transformation|SetRelativeLocation (Variables|Default|GetSelectionMesh) (.location (.OutInstanceTransform (Components|InstancedStaticMesh|GetInstanceTransform (Variables|Default|GetGhostTiles_ISM) (Variables|Default|GetHitInstanceID) false))) false false)
      (Transformation|SetRelativeLocation (Variables|Default|GetTowerSelectionMesh) (.location (.OutInstanceTransform (Components|InstancedStaticMesh|GetInstanceTransform (Variables|Default|GetGhostTiles_ISM) (Variables|Default|GetHitInstanceID) false))) false false))
    (:then_1
      (if (CallFunction|DoesTileContainMesh (Variables|Default|GetHitInstanceID))
        (Rendering|Material|SetMaterial _selectionmesh 0 "/Engine/EngineDebugMaterials/M_SimpleUnlitTranslucent.M_SimpleUnlitTranslucent")
        (else
          (Rendering|Material|SetMaterial _selectionmesh 0 "/HexGrids/HexGrids/Materials/M_HexSelection.M_HexSelection"))))))

(fn DoesTileContainMesh
  (params (ItemToFind :type Integer%20%28by%20ref%29))
  (return (Utilities|Set|Contains (Variables|Default|GetInstancesUsed) ItemToFind)))