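; Paper2D tile map actor that draws the minimap from the PTM_minimap tile map asset.
; The construction script assigns the map and makes it editable.
; UpdateTiles reapplies it, resizes the grid to the given negative and positive extents, then sets tiles at Col/Row coordinates shifted into map space.
; The row offset depends on whether the total height is odd or even.
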(event EventBeginPlay)

(event Collision|EventActorBeginOverlap
  (params (OtherActor :type Actor%20Object%20Reference)))

(event EventTick
  (params (DeltaSeconds :type Float%20%28single-precision%29)))

(fn ConstructionScript
  (bind _rendercomponent (Variables|Default|GetRenderComponent))
  (Class|PaperTileMapComponent|SetTileMap _rendercomponent "/Game/Blueprints/Map/PTM_minimap.PTM_minimap")
  (Class|PaperTileMapComponent|MakeTileMapEditable _rendercomponent))

(fn UpdateTiles
  (params (Tiles :type Array%20of%20Offset%20Coords%20Structures) (NegativeX :type Integer) (NegativeY :type Integer) (PositiveX :type Integer) (PositiveY :type Integer))
  (bind _returnvalue (Math|Integer|Absolute(Integer) NegativeX))
  (bind _returnvalue_2 (Math|Integer|Absolute(Integer) NegativeY))
  (bind _rendercomponent (Variables|Default|GetRenderComponent))
  (bind _returnvalue_3 (+ _returnvalue_2 PositiveY))
  (Class|PaperTileMapComponent|SetTileMap _rendercomponent "/Game/Blueprints/Map/PTM_minimap.PTM_minimap")
  (Class|PaperTileMapComponent|MakeTileMapEditable _rendercomponent)
  (Class|PaperTileMapComponent|ResizeMap _rendercomponent (+ _returnvalue PositiveX) _returnvalue_3)
  (if (Class|GridsCore|IsOddInt _returnvalue_3)
    (for _array_element Tiles
      (Class|PaperTileMapComponent|SetTile _rendercomponent (+ (.Col (Utilities|Struct|BreakOffsetCoords _array_element)) _returnvalue) (+ (.Row (Utilities|Struct|BreakOffsetCoords _array_element)) _returnvalue_2) 0 (Variables|Default|GetNew%20Value)))
    (else
      (for _array_element_2 0
        (Class|PaperTileMapComponent|SetTile (Variables|Default|GetRenderComponent) (+ (.Col (Utilities|Struct|BreakOffsetCoords _array_element_2)) _returnvalue) (+ (.Row (Utilities|Struct|BreakOffsetCoords _array_element_2)) _returnvalue_3 -1) 0 (Variables|Default|GetNew%20Value))))))