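; Game state for a hex tower defense match, handling start, pause, game over, boss kills, map seed and starting den count.
; StartGame kicks off terrain and director spawning, then uses a near-endless timer as the match clock.
; Elapsed minutes drive curves for health, shield and armor scaling, plus an armor threshold broadcast every second.
; Game over stops spawning and saves survival time; demo builds force a fixed seed.
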(event Custom|timeisout)

(event Custom|SaveTimeSurvived
  (bind _outactors (Actor|GetAllActorsOfClass "/Game/Blueprints/Player/BP_Character_TD.BP_Character_TD_C"))
  (for _array_element _outactors
    (bind _returnvalue (Actor|GetActorOfClass "/Game/Blueprints/Map/BP_TerrainGen.BP_TerrainGen_C"))
    (Default|AddTime (Variables|/Game/Blueprints/Player/BP_Character_TD.BP_Character_TD_C|GetAC_StatTacker _array_element) (Variables|/Game/Blueprints/Map/BP_TerrainGen.BP_TerrainGen_C|GetStarterDens _returnvalue) (Class|KismetSystemLibrary|GetTimerElapsedTimeHandle (Variables|Default|GetTime)))))

(event Custom|GameOver_Event
  (Utilities|Time|PauseTimerbyHandle (Variables|Default|GetTime))
  (CallFunction|SaveTimeSurvived)
  (Default|StopSpawning (Variables|Default|GetGameDirector)))

(event Custom|UnpauseGame
  (Default|CallGameUnpaused))

(event Custom|StartGame
  (if (not (Variables|Default|GetHasBeenStarted))
    (Variables|Default|SetHasBeenStarted true)
    (bind _returnvalue (Actor|GetActorOfClass "/Game/Blueprints/Map/BP_TerrainGen.BP_TerrainGen_C"))
    (Default|StartGame _returnvalue)
    (bind _returnvalue_2 (Actor|GetActorOfClass "/Game/Blueprints/Mobs/BP_GameDirector.BP_GameDirector_C"))
    (Default|StartSpawning _returnvalue_2)
    (bind _returnvalue_3 (Utilities|Time|SetTimerbyEvent (delegate Custom|timeisout) 99999999999.0))
    (Variables|Default|SetTime _returnvalue_3)
    (Utilities|Time|SetTimerbyEvent (delegate Custom|UpdateArmorScaling) 1.0 true)))

(event Custom|BossKilled
  (Default|StartSpawningNewDens (Variables|Default|GetGameDirector)))

(event Custom|ChangeSeed
  (params (NewSeed :type Integer))
  (bind _output_get (Variables|Default|SetSeed (Math|Integer|SelectInt 12345678 NewSeed (Variables|Default|GetbIsDemo))))
  (Default|CallNewSeed _output_get))

(event Custom|ChangeTimeDilation
  (params (TimeDilation :type Float%20%28double-precision%29))
  (Utilities|Time|SetGlobalTimeDilation TimeDilation))

(event Custom|RestartGame_Event
  (Utilities|Time|ClearandInvalidateTimerbyHandle (Variables|Default|GetTime)))

(event Custom|ChangeStartingDens
  (params (Dens :type Integer))
  (bind _output_get (Variables|Default|SetStartingDens (Math|Integer|Clamp(Integer) Dens 1 6)))
  (Default|CallDensNumberChanged _output_get)
  (Default|CallNewSeed (Variables|Default|GetSeed)))

(event Custom|UpdateArmorScaling
  (bind _output_get (Variables|Default|SetArmorDamageThreshold (Math|Conversions|ToFloat(Integer) (Math|Float|Floor (Math|Curves|GetFloatValue (Variables|Default|GetArmorThresholdCurve) (/ (Class|KismetSystemLibrary|GetTimerElapsedTimeHandle (Variables|Default|GetTime)) 6e+01))))))
  (Default|CallArmorThresholdChanged _output_get))

(event Custom|PauseGame
  (CallFunction|ChangeTimeDilation 0.0)
  (Default|CallGamePaused))

(event EventBeginPlay
  (Game|SetGamePaused false)
  (bind _returnvalue (Actor|GetActorOfClass "/Game/Blueprints/Mobs/BP_GameDirector.BP_GameDirector_C"))
  (Variables|Default|SetGameDirector _returnvalue)
  (bind _asgi_hex_defense (Utilities|Casting|CastToGI_HexDefense (Game|GetGameInstance)))
  (Default|ResetAmounts _asgi_hex_defense)
  (EventDispatchers|BindEventtoGameOver (delegate Custom|GameOver_Event)))

(fn ConstructionScript
  (Variables|GridStorage|SetGrid%20Scale%202D (Math|Vector2D|MakeVector2D (Class|GridsHex|HexWidth (.y (Variables|GridStorage|GetGrid%20Scale%202D))) (.y (Variables|GridStorage|GetGrid%20Scale%202D))))
  (Variables|GlobalVars|SetglobalSeed (Math|Random|RandomIntegerinRange -1000000000 1000000000))
  (bind _returnvalue (Game|ConstructObjectfromClass "/Script/FastNoiseGenerator.FastNoiseWrapper"))
  (bind _output_get (Variables|noise|SetHeightMap _returnvalue))
  (Class|FastNoiseWrapper|SetupFastNoise _output_get "Cellular" (Variables|GlobalVars|GetglobalSeed) 0.025 "Linear" "FBM" 3 2.0 5.0 0.45 "Euclidean" "Distance2"))

(fn RedrawGrid
  (Actor|GetActorOfClass "/Game/Blueprints/Map/BP_TerrainGen.BP_TerrainGen_C"))

(fn StartPreGame
  (Variables|Default|SetPaused false)
  (bind _foundwidgets (Widget|GetAllWidgetsOfClass "/Game/UI/CUI_StartGame.CUI_StartGame_C" false))
  (for _array_element _foundwidgets
    (Widget|SetVisibility _array_element "Visible")))

(fn GetScaling
  (bind _time (Variables|Default|GetTime))
  (bind _returnvalue (Class|KismetSystemLibrary|GetTimerElapsedTimeHandle _time))
  (bind _returnvalue_2 (/ _returnvalue 6e+01))
  (return (Math|Curves|GetFloatValue (Variables|Default|GetHealthScalingCurve) _returnvalue_2) (Math|Curves|GetFloatValue (Variables|Default|GetShieldScalingCurve) _returnvalue_2) (Math|Curves|GetFloatValue (Variables|Default|GetArmorScalingCurve) _returnvalue_2)))