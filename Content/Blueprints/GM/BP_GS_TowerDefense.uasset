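; Game state for the tower defense mode that runs the match lifecycle and holds shared hex grid and noise setup.
; Construction derives hex grid scale, picks a random seed and builds a cellular FastNoise height map.
; Starting the game triggers terrain generation and director spawning, using a huge-duration timer as a stopwatch.
; Stopping pauses that timer, saves survival time to each character's stat tracker and stops the director.
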(event Custom|timeisout)

(event Custom|SaveTimeSurvived
  (bind _outactors (Actor|GetAllActorsOfClass "/Game/Blueprints/Player/BP_Character_TD.BP_Character_TD_C"))
  (for _array_element _outactors
    (bind _returnvalue (Actor|GetActorOfClass "/Game/Blueprints/Map/BP_TerrainGen.BP_TerrainGen_C"))
    (Default|AddTime (Variables|/Game/Blueprints/Player/BP_Character_TD.BP_Character_TD_C|GetAC_StatTacker _array_element) (Variables|/Game/Blueprints/Map/BP_TerrainGen.BP_TerrainGen_C|GetStarterDens _returnvalue) (Class|KismetSystemLibrary|GetTimerElapsedTimeHandle (Variables|Default|GetTime)))))

(event Custom|StartGame
  (if (not (Variables|Default|GetHasBeenStarted))
    (Variables|Default|SetHasBeenStarted true)
    (bind _returnvalue (Actor|GetActorOfClass "/Game/Blueprints/Map/BP_TerrainGen.BP_TerrainGen_C"))
    (Default|StartGame _returnvalue)
    (bind _returnvalue_2 (Actor|GetActorOfClass "/Game/Blueprints/Mobs/BP_GameDirector.BP_GameDirector_C"))
    (Default|StartSpawning _returnvalue_2)
    (bind _returnvalue_3 (Utilities|Time|SetTimerbyEvent (delegate Custom|timeisout) 99999999999.0))
    (Variables|Default|SetTime _returnvalue_3)))

(event Custom|StopGame
  (Utilities|Time|PauseTimerbyHandle (Variables|Default|GetTime))
  (CallFunction|SaveTimeSurvived)
  (Default|Stop (Variables|Default|GetGameDirector))
  (bind _foundwidgets (Widget|GetAllWidgetsOfClass "/Game/UI/CUI_StartScreen.CUI_StartScreen_C" false))
  (for _array_element _foundwidgets
    _))

(event Custom|ChangeTimeDilation
  (params (TimeDilation :type Float%20%28double-precision%29))
  (Utilities|Time|SetGlobalTimeDilation TimeDilation))

(event Custom|RestartGame_Event
  (Utilities|Time|ClearandInvalidateTimerbyHandle (Variables|Default|GetTime)))

(event EventBeginPlay
  (Game|SetGamePaused false)
  (bind _returnvalue (Actor|GetActorOfClass "/Game/Blueprints/Mobs/BP_GameDirector.BP_GameDirector_C"))
  (Variables|Default|SetGameDirector _returnvalue)
  (Utilities|FlowControl|Delay 0.1)
  (bind _foundwidgets (Widget|GetAllWidgetsOfClass "/Game/UI/CUI_TopBar.CUI_TopBar_C" false))
  (for _array_element _foundwidgets
    (Default|UpdateTime _array_element 0.0)))

(fn ConstructionScript
  (Variables|GridStorage|SetGrid%20Scale%202D (Math|Vector2D|MakeVector2D (Class|GridsHex|HexWidth (.y (Variables|GridStorage|GetGrid%20Scale%202D))) (.y (Variables|GridStorage|GetGrid%20Scale%202D))))
  (Variables|GlobalVars|SetglobalSeed (Math|Random|RandomIntegerinRange -1000000000 1000000000))
  (bind _returnvalue (Game|ConstructObjectfromClass "/Script/FastNoiseGenerator.FastNoiseWrapper"))
  (bind _output_get (Variables|noise|SetHeightMap _returnvalue))
  (Class|FastNoiseWrapper|SetupFastNoise _output_get "Cellular" (Variables|GlobalVars|GetglobalSeed) 0.025 "Linear" "FBM" 3 2.0 5.0 0.45 "Euclidean" "Distance2"))

(fn SpawnGridActor
  (bind _returnvalue (Game|SpawnActorfromClass "/Game/Blueprints/Map/BP_MacroHexHandler.BP_MacroHexHandler_C" (Math|Transform|MakeTransform "0, 0, 0") "AlwaysSpawn" 0 (Variables|GridStorage|GetGrid%20Scale%202D) 0))
  (bind _output_get (Variables|Default|SetMacroHexHandler _returnvalue))
  (return _output_get))

(fn RedrawGrid
  (Actor|GetActorOfClass "/Game/Blueprints/Map/BP_TerrainGen.BP_TerrainGen_C"))

(fn StartPreGame
  (Variables|Default|SetPaused false)
  (bind _foundwidgets (Widget|GetAllWidgetsOfClass "/Game/UI/CUI_StartGame.CUI_StartGame_C" false))
  (for _array_element _foundwidgets
    (Widget|SetVisibility _array_element "Visible")))