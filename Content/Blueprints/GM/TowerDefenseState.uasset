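; TowerDefenseState is the tower defense state Blueprint that sets up and spawns the hex terrain grid for the level.
; Its construction script derives the hex grid's X scale from Y and builds a cellular FastNoise height source (Distance2) from the global seed.
; On BeginPlay it spawns a TerrainGrid actor at the origin, passing in the seed, scale, noise and global paths, and keeps a reference to it.
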(event EventBeginPlay
  (|SpawnGridActor))

(event EventTick
  (params (DeltaSeconds :type Float%20%28single-precision%29)))

(fn ConstructionScript
  (Variables|Default|SetGrid%20Scale%202D (Math|Vector2D|MakeVector2D (Class|GridsHex|HexWidth (.y (Variables|Default|GetGrid%20Scale%202D))) (.y (Variables|Default|GetGrid%20Scale%202D))))
  (bind _returnvalue (Game|ConstructObjectfromClass "/Script/FastNoiseGenerator.FastNoiseWrapper"))
  (bind _output_get (Variables|noise|Setheight _returnvalue))
  (Class|FastNoiseWrapper|SetupFastNoise _output_get "Cellular" (Variables|GlobalVars|GetglobalSeed) 0.025 "Linear" "FBM" 3 2.0 5.0 0.45 "Euclidean" "Distance2"))