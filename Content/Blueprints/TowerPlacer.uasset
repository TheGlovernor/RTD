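; TowerPlacer is a runtime hex-grid builder that places or deletes tile meshes on user selection.
; It generates a hexagonal grid of ghost ISM instances, with a selection mesh colored by occupancy through a material parameter collection.
; Placed tiles are separate static mesh components animated by drop and scale components and tracked in maps.
; Those maps save to HexGrid_Save, and loading regenerates the grid and replays placements with a delay.
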(event Custom|OnTileSelectedByUser
  ;[1 1 1] On User Selection
  (Variables|Default|SetTileBeingManipulated (Variables|Default|GetHitInstanceID))
  (CallFunction|RunTileActionDynamic))

(event Custom|RunTileActionDynamic
  ;[1 1 1] Run tile action, either adds or deletes
  (if (CallFunction|DoesTileContainMesh (Variables|Default|GetTileBeingManipulated))
    (CallFunction|DeleteSelectedTilewithAnimation)
    (else
      (CallFunction|AddTiletoSelectedwithAnimation))))

(event Custom|DisableGridBuilding_Event
  ;[1 1 1] Bind events to activate and deactivate. We just hide the meshes. Clearing and respawning them each time is another option. Its a balance between a single fps spike on generation, or a constant small memory cost.
  (Rendering|SetVisibility (Variables|Default|GetGhostTiles_ISM) false false))

(event Custom|EnableGridBuilding_Event
  ;[1 1 1] Bind events to activate and deactivate. We just hide the meshes. Clearing and respawning them each time is another option. Its a balance between a single fps spike on generation, or a constant small memory cost.
  ;;[1 1 1] Comment
  (Rendering|SetVisibility (Variables|Default|GetGhostTiles_ISM) true false))

(event Custom|GenerateGrid
  (bind _gridscale (Variables|Default|GetGridScale))
  ;[1 1 1] Generate Grid
  (Utilities|FlowControl|Sequence
    (:then_0
      ;[1 1 1] Calculate grid spacing
      (Variables|Default|SetGridScaleCalculated (Math|Vector2D|MakeVector2D (Class|GridsHex|HexWidth (.y _gridscale)) (.y _gridscale))))
    (:then_1
      ;[1 1 1] If you want a different base grid shape, you can swap this node for one of the other generators
      (bind _returnvalue (Class|GridsHex|BuildHexagonArray (Variables|Default|GetMaxGridSize)))
      (bind _output_get (Variables|Default|SetGrid _returnvalue))
      ;[1 1 1] Standard add instance setup as used in most other hex grid blueprints
      (for _array_element _output_get
        (bind _returnvalue_2 (Components|InstancedStaticMesh|AddInstance (Variables|Default|GetGhostTiles_ISM) (Math|Transform|MakeTransform (Math|Conversions|ToVector(Vector2D) (.Precise (Class|GridsHex|ScaleandOffset _array_element (Variables|Default|GetGridScaleCalculated)))) (Variables|Default|GetTileRotation) (Variables|Default|GetTileScale)) false))
        (Utilities|Map|Add (Variables|Default|GetGhostInstances) _returnvalue_2 _array_element)))
    (:then_2
      ;[1 1 1] Bind events to activate and deactivate. We just hide the meshes. Clearing and respawning them each time is another option. Its a balance between a single fps spike on generation, or a constant small memory cost.
      (EventDispatchers|BindEventtoDisableGridBuilding (delegate Custom|DisableGridBuilding_Event))
      (EventDispatchers|BindEventtoEnableGridBuilding (delegate Custom|EnableGridBuilding_Event)))))

(event Custom|LoadExistingGridWithDelay
  (params (SaveFile :type Hex%20Grid%20Save%20Object%20Reference))
  ;[1 1 1] Here we load the grid from the save file
  (bind _result (Utilities|Set|ToArray (Variables|/HexGrids/HexGrids/Blueprints/HexGrid_Save.HexGrid_Save_C|GetInstancesUsed SaveFile)))
  (bind _element (Utilities|ForEachLoopwithDelay _result 0.1)
    (:Loop
      (Variables|Default|SetTileBeingManipulated _element)
      (if (.ReturnValue (Utilities|Map|Find (Variables|/HexGrids/HexGrids/Blueprints/HexGrid_Save.HexGrid_Save_C|GetMeshMap SaveFile) (.Value (Utilities|Map|Find (Variables|/HexGrids/HexGrids/Blueprints/HexGrid_Save.HexGrid_Save_C|GetGhostMap SaveFile) _element))))
        (Variables|Default|SetMeshToSpawn (.Value (Utilities|Map|Find (Variables|/HexGrids/HexGrids/Blueprints/HexGrid_Save.HexGrid_Save_C|GetMeshMap SaveFile) (.Value (Utilities|Map|Find (Variables|/HexGrids/HexGrids/Blueprints/HexGrid_Save.HexGrid_Save_C|GetGhostMap SaveFile) _element)))))
        (Variables|Default|SetMaterialForMeshToSpawn (.Value (Utilities|Map|Find (Variables|/HexGrids/HexGrids/Blueprints/HexGrid_Save.HexGrid_Save_C|GetMaterialMap SaveFile) (.Value (Utilities|Map|Find (Variables|/HexGrids/HexGrids/Blueprints/HexGrid_Save.HexGrid_Save_C|GetGhostMap SaveFile) _element)))))
        (CallFunction|RunTileActionDynamic)))))

(event EventBeginPlay
  ;[1 1 1] Begin Play
  ;[1 1 1] If Load is true, wait for user to call the load grid function
  (Utilities|FlowControl|Delay 0.2)
  (if (not (Variables|Default|GetLoadExistingGridFromSave))
    (CallFunction|GenerateGrid)))

(fn ConstructionScript)

(fn LoadGrid
  (params (SlotName :type String) (UserIndex :type Integer))
  (LocalVariables|SetSaveName SlotName)
  (LocalVariables|SetSaveIndex UserIndex)
  (bind _returnvalue (SaveGame|DoesSaveGameExist (LocalVariables|GetSaveName) (LocalVariables|GetSaveIndex)))
  (if _returnvalue
    (bind _returnvalue_2 (SaveGame|LoadGamefromSlot (LocalVariables|GetSaveName) (LocalVariables|GetSaveIndex)))
    (bind _ashex_grid_save (Utilities|Casting|CastToHexGrid_Save _returnvalue_2))
    (LocalVariables|SetGridSaveFile _ashex_grid_save)
    (Utilities|FlowControl|Sequence
      (:then_0
        (Variables|Default|SetGridScale (Variables|/HexGrids/HexGrids/Blueprints/HexGrid_Save.HexGrid_Save_C|GetGridScale (LocalVariables|GetGridSaveFile)))
        (Variables|Default|SetMaxGridSize (Variables|/HexGrids/HexGrids/Blueprints/HexGrid_Save.HexGrid_Save_C|GetMaxGridSize (LocalVariables|GetGridSaveFile)))
        (Variables|Default|SetTileRotation (Variables|/HexGrids/HexGrids/Blueprints/HexGrid_Save.HexGrid_Save_C|GetTileRotation (LocalVariables|GetGridSaveFile)))
        (Variables|Default|SetTileScale (Variables|/HexGrids/HexGrids/Blueprints/HexGrid_Save.HexGrid_Save_C|GetTileScale (LocalVariables|GetGridSaveFile)))
        (CallFunction|GenerateGrid))
      (:then_1
        (CallFunction|LoadExistingGridwithDelay (LocalVariables|GetGridSaveFile))))
    (else
      (Development|PrintString "Error. Failed to find save file for loading grid" true true "(R=1.000000,G=0.000000,B=0.000000,A=1.000000)" 8.0))))

(fn SaveGrid
  (params (SlotName :type String) (UserIndex :type Integer))
  (Utilities|FlowControl|Sequence
    (:then_0
      (bind _returnvalue (SaveGame|CreateSaveGameObject "/HexGrids/HexGrids/Blueprints/HexGrid_Save.HexGrid_Save_C"))
      (LocalVariables|SetSaveFile _returnvalue)
      ;[1 1 1] Set all variables in save file
      (Utilities|FlowControl|Sequence
        (:then_0
          (Variables|/HexGrids/HexGrids/Blueprints/HexGrid_Save.HexGrid_Save_C|SetTileScale (LocalVariables|GetSaveFile) (Variables|Default|GetTileScale)))
        (:then_1
          (Variables|/HexGrids/HexGrids/Blueprints/HexGrid_Save.HexGrid_Save_C|SetTileRotation (LocalVariables|GetSaveFile) (Variables|Default|GetTileRotation)))
        (:then_2
          (Variables|/HexGrids/HexGrids/Blueprints/HexGrid_Save.HexGrid_Save_C|SetInstancesUsed (LocalVariables|GetSaveFile) (Variables|Default|GetInstancesUsed)))
        (:then_3
          (Variables|/HexGrids/HexGrids/Blueprints/HexGrid_Save.HexGrid_Save_C|SetGhostMap (LocalVariables|GetSaveFile) (Variables|Default|GetGhostInstances)))
        (:then_4
          (Variables|/HexGrids/HexGrids/Blueprints/HexGrid_Save.HexGrid_Save_C|SetMeshMap (LocalVariables|GetSaveFile) (Variables|Default|GetMeshMap)))
        (:then_5
          (Variables|/HexGrids/HexGrids/Blueprints/HexGrid_Save.HexGrid_Save_C|SetGridScale (LocalVariables|GetSaveFile) (Variables|Default|GetGridScale)))
        (:then_6
          (Variables|/HexGrids/HexGrids/Blueprints/HexGrid_Save.HexGrid_Save_C|SetMaterialMap (LocalVariables|GetSaveFile) (Variables|Default|GetMaterialMap)))
        (:then_7
          (Variables|/HexGrids/HexGrids/Blueprints/HexGrid_Save.HexGrid_Save_C|SetMaxGridSize (LocalVariables|GetSaveFile) (Variables|Default|GetMaxGridSize)))
        (:then_8
          (Variables|/HexGrids/HexGrids/Blueprints/HexGrid_Save.HexGrid_Save_C|SetbUsesRuntimeGrid (LocalVariables|GetSaveFile) true))))
    (:then_1
      (SaveGame|SaveGametoSlot (LocalVariables|GetSaveFile) SlotName UserIndex))))

(fn DeleteSelectedTilewithAnimation
  (bind _tilebeingmanipulated (Variables|Default|GetTileBeingManipulated))
  (bind _ghostinstances (Variables|Default|GetGhostInstances))
  (bind _tilebeingmanipulated_2 (Variables|Default|GetTileBeingManipulated))
  (bind _value (Utilities|Map|Find _ghostinstances _tilebeingmanipulated))
  ;[1 1 1] Just a visually interesting deletion, use whatever you like.
  ; This node also destroys the static mesh component on completion, which is the simpliest method of timing the DestroyComponent.
  ; You could bind to the onComplete in the component, but the problem is if a second delete is called before the first has completed, the ref will be wrong
  (AddComponent|AddStaticMeshScaleTIleComponent "0.000000,0.000000,0.000000" 15.0 (.Value (Utilities|Map|Find (Variables|Default|GetInstanceToPlacedMeshMap) (Variables|Default|GetTileBeingManipulated))) true)
  ;[1 1 1] Remove mesh from various maps and mark the instance as a empty tile
  (Utilities|Map|Remove (Variables|Default|GetMeshes) _value)
  (Utilities|Map|Remove (Variables|Default|GetInstanceToPlacedMeshMap) _tilebeingmanipulated_2)
  (Utilities|Set|Remove (Variables|Default|GetInstancesUsed) _tilebeingmanipulated_2)
  (Utilities|Map|Remove (Variables|Default|GetMeshMap) _value)
  (Utilities|Map|Remove (Variables|Default|GetMaterialMap) _value))

(fn AddTiletoSelectedwithAnimation
  (bind _ghosttiles_ism (Variables|Default|GetGhostTiles_ISM))
  (bind _tilebeingmanipulated (Variables|Default|GetTileBeingManipulated))
  (bind _ghostinstances (Variables|Default|GetGhostInstances))
  (bind _tilebeingmanipulated_2 (Variables|Default|GetTileBeingManipulated))
  (bind _outinstancetransform (Components|InstancedStaticMesh|GetInstanceTransform _ghosttiles_ism _tilebeingmanipulated false))
  (bind (_value _returnvalue) (Utilities|Map|Find _ghostinstances _tilebeingmanipulated_2))
  (bind (_location _rotation _scale) (Math|Transform|BreakTransform _outinstancetransform))
  ;[1 1 1] If the instance is "empty" we spawn the actual mesh, with a little animation using the drop component, and update the various maps and sets
  (if _returnvalue
    ;;[1 1 1] Update my collision response to a custom trace for best results (See note at top)
    (bind _returnvalue_2 (AddComponent|AddStaticMeshComponent false (Math|Transform|MakeTransform (+ _location "0, 0,100.000000") _rotation _scale)))
    (bind _output_get (Variables|Default|SetLastSpawnStaticMeshComponent _returnvalue_2))
    ;;[1 1 1] If you have a UI for selecting your tile, you would set these variables to control what is spawned
    (Components|StaticMesh|SetStaticMesh _output_get (Variables|Default|GetMeshToSpawn))
    (Rendering|Material|SetMaterial (Variables|Default|GetLastSpawnStaticMeshComponent) 0 (Variables|Default|GetMaterialForMeshToSpawn))
    (Utilities|Map|Add (Variables|Default|GetMeshMap) _value (Variables|Default|GetMeshToSpawn))
    (Utilities|Map|Add (Variables|Default|GetMaterialMap) _value (Variables|Default|GetMaterialForMeshToSpawn))
    (AddComponent|AddStaticMeshDropTIleComponent 1e+02 2e+01 (Variables|Default|GetLastSpawnStaticMeshComponent))
    (Utilities|Map|Add (Variables|Default|GetMeshes) _value (Variables|Default|GetLastSpawnStaticMeshComponent))
    (Utilities|Set|Add (Variables|Default|GetInstancesUsed) (Variables|Default|GetTileBeingManipulated))
    (Utilities|Map|Add (Variables|Default|GetInstanceToPlacedMeshMap) (Variables|Default|GetTileBeingManipulated) (Variables|Default|GetLastSpawnStaticMeshComponent))))

(fn UpdatePreviewMesh
  (params (HitID :type Integer))
  (Variables|Default|SetHitInstanceID HitID)
  (Utilities|FlowControl|Sequence
    (:then_0
      (Transformation|SetRelativeLocation (Variables|Default|GetSelectionMesh) (.location (.OutInstanceTransform (Components|InstancedStaticMesh|GetInstanceTransform (Variables|Default|GetGhostTiles_ISM) (Variables|Default|GetHitInstanceID) false))) false false))
    (:then_1
      (if (CallFunction|DoesTileContainMesh (Variables|Default|GetHitInstanceID))
        (Rendering|Material|SetVectorParameterValue "/HexGrids/HexGrids/Materials/GhostTiles.GhostTiles" "SelectionBrushColor" (Utilities|Struct|MakeLinearColor 1.0 0.0 0.0 1.0) :!class /Script/Engine.KismetMaterialLibrary)
        (else
          (Rendering|Material|SetVectorParameterValue "/HexGrids/HexGrids/Materials/GhostTiles.GhostTiles" "SelectionBrushColor" (Utilities|Struct|MakeLinearColor 0.0 0.22 1.0 1.0) :!class /Script/Engine.KismetMaterialLibrary))))))

(fn DoesTileContainMesh
  (params (ItemToFind :type Integer%20%28by%20ref%29))
  (return (Utilities|Set|Contains (Variables|Default|GetInstancesUsed) ItemToFind)))