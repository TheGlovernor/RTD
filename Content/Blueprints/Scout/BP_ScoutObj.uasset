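; BP_ScoutObj is an object that gates a character's scouting behind a cooldown, with optional automatic scouting.
; TryScout consumes the CanScout flag, starts a one-shot timer of Interval length and returns whether it succeeded.
; ReadyToScout restores the flag and, if AutomaticScouting is on, restarts the cooldown and calls ScoutRandomArea on its outer BP_Character_TD.
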(event Custom|ReadyToScout
  (Variables|Default|SetCanScout true)
  (if (Variables|Default|GetAutomaticScouting)
    (CallFunction|TryScout)
    (bind _asbp_character_td (Utilities|Casting|CastToBP_Character_TD (Utilities|GetOuterObject self)))
    (Default|ScoutRandomArea _asbp_character_td)))

(fn TryScout
  (if (Variables|Default|GetCanScout)
    (Variables|Default|SetCanScout false)
    (bind _returnvalue (Utilities|Time|SetTimerbyEvent (EventDispatchers|CreateEvent :!event Custom|ReadyToScout) (Variables|Default|GetInterval)))
    (Variables|Default|SetTimer _returnvalue)
    (return true)
    (else
      (return false))))