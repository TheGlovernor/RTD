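; Base enemy mob that follows a chain of path-node splines toward a base, with health and a health bar widget.
; Tick advances it by MovementSpeed per frame, unscaled by delta time, carrying overshoot onto the next node's spline and destroying it when no valid spline remains.
; Move snaps position and rotation to the spline and decrements DistanceToBase.
; AnyDamage lowers Health, updating the bar or destroying the actor at zero.
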(event EventBeginPlay)

(event EventTick
  (params (DeltaSeconds :type Float%20%28single-precision%29))
  (Variables|Default|GetSpline
    (:then
      (if (>= (+ (Variables|Default|GetLocationOnCurrentSpline) (Variables|Default|GetMovementSpeed)) (Spline|GetSplineLength (Variables|Default|GetSpline)))
        (Variables|Default|SetprevSplineLength (Spline|GetSplineLength (Variables|Default|GetSpline)))
        (Variables|Default|SetSpline (Variables|/Game/Blueprints/Mobs/BP_Path_Node.BP_Path_Node_C|GetCurrentSplineComponent (Variables|Default|GetNextNode)))
        (Variables|Default|SetNextNode (Variables|/Game/Blueprints/Mobs/BP_Path_Node.BP_Path_Node_C|GetNextNode (Variables|Default|GetNextNode)))
        (CallFunction|Move (- (+ (Variables|Default|GetLocationOnCurrentSpline) (Variables|Default|GetMovementSpeed)) (Variables|Default|GetprevSplineLength)))
        (else
          (CallFunction|Move (+ (Variables|Default|GetLocationOnCurrentSpline) (Variables|Default|GetMovementSpeed))))))
    (:else
      (Actor|DestroyActor))))

(event Game|Damage|EventAnyDamage
  (params (Damage :type Float%20%28single-precision%29) (DamageType :type Damage%20Type%20Object%20Reference) (InstigatedBy :type Controller%20Object%20Reference) (DamageCauser :type Actor%20Object%20Reference))
  (bind _output_get (Variables|Default|SetHealth (- (Variables|Default|GetHealth) Damage)))
  (if (<= _output_get 0.0)
    (Actor|DestroyActor)
    (else
      (bind _aswbp_health_bar (Utilities|Casting|CastToWBP_HealthBar (UserInterface|GetWidget (Variables|Default|GetWidget))))
      (Default|SetPercent _aswbp_health_bar (/ (Variables|Default|GetHealth) (Variables|Default|GetMaxHealth))))))

(fn ConstructionScript
  (Variables|Default|SetHealth (Variables|Default|GetMaxHealth)))

(fn Move
  (params (Distance :type Float%20%28double-precision%29))
  (Transformation|AddActorWorldOffset (- (Spline|GetLocationatDistanceAlongSpline (Variables|Default|GetSpline) Distance "World") (Transformation|GetActorLocation)))
  (Transformation|SetActorRotation (Spline|GetRotationatDistanceAlongSpline (Variables|Default|GetSpline) Distance "Local"))
  (Variables|Default|SetLocationOnCurrentSpline Distance)
  (Variables|Default|SetDistanceToBase (- (Variables|Default|GetDistanceToBase) (Variables|Default|GetMovementSpeed))))