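; Enemy spawner node on a hex map that draws paths to its next nodes and spawns mobs onto them.
; On BeginPlay it runs A* to each next node and builds a spline just above the owning MacroHexHandler's surface, rendered with spline mesh segments.
; Each spline maps to its length plus that node's distance to base.
; SpawnEnemy spawns one enemy at every spline's start, passing it the spline and distance.
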(event EventBeginPlay
  (bind _asmacro_hex_handler (Utilities|Casting|CastToMacroHexHandler (Components|GetOwner)))
  (Variables|Default|SetMacroHexHandler _asmacro_hex_handler)
  (for _array_element (Variables|Default|GetNextNodes)
    (Utilities|FlowControl|Sequence
      (:then_0
        (bind _returnvalue (AddComponent|AddSplineComponent false (Math|Transform|MakeTransform "0, 0, 0")))
        (Variables|Default|SetCurrentSplineComponent _returnvalue))
      (:then_1
        (Spline|ClearSplinePoints (Variables|Default|GetCurrentSplineComponent) true))
      (:then_2
        (bind _results (Class|GridsHex|AStarPathfinding (Variables|Default|GetMyCoords) (Variables|/Game/Blueprints/Mobs/PathfindingNode.PathfindingNode_C|GetMyCoords _array_element) (Variables|Default|GetPath) 0 0 "(Col=0,Row=0)" true false))
        (bind _output_get (Variables|Default|SetCurrentPath (Class|GridsCore|ToOffsetArray(CubeArray) _results)))
        (Utilities|Array|Insert _output_get (Variables|Default|GetMyCoords))
        (Utilities|Array|Add _output_get (Variables|/Game/Blueprints/Mobs/PathfindingNode.PathfindingNode_C|GetMyCoords _array_element))
        (for _array_element_2 _output_get
          (bind _location (Default|SurfaceLocation (Variables|Default|GetMacroHexHandler) _array_element_2))
          (Spline|AddSplinePoint (Variables|Default|GetCurrentSplineComponent) (+ _location (Math|Vector|MakeVector 0.0 0.0 5.0)) "World" true)))
      (:then_3
        (for _index (range 0 (- (Spline|GetNumberOfSplinePoints (Variables|Default|GetCurrentSplineComponent)) 2))
          (bind _returnvalue_2 (AddComponent|AddSplineMeshComponent false (Math|Transform|MakeTransform "0, 0, 0")))
          (SplineMesh|SetStartandEnd _returnvalue_2 (.Location (Spline|GetLocationandTangentatSplinePoint (Variables|Default|GetCurrentSplineComponent) _index "Local")) (.Tangent (Spline|GetLocationandTangentatSplinePoint (Variables|Default|GetCurrentSplineComponent) _index "Local")) (.Location (Spline|GetLocationandTangentatSplinePoint (Variables|Default|GetCurrentSplineComponent) (+ _index 1) "Local")) (.Tangent (Spline|GetLocationandTangentatSplinePoint (Variables|Default|GetCurrentSplineComponent) (+ _index 1) "Local")) true :!class /Script/Engine.SplineMeshComponent)
          (Utilities|Array|Add (Variables|Default|GetSplineMeshComponents) _returnvalue_2))
        (Utilities|Map|Add (Variables|Default|GetSplineComponents) (Variables|Default|GetCurrentSplineComponent) (+ (Spline|GetSplineLength (Variables|Default|GetCurrentSplineComponent)) (Variables|/Game/Blueprints/Mobs/PathfindingNode.PathfindingNode_C|GetDistanceToBase _array_element)))))))

(event EventTick
  (params (DeltaSeconds :type Float%20%28single-precision%29)))

(event EventActorBeginOverlap
  (params (OtherActor :type Actor%20Object%20Reference)))

(fn ConstructionScript
  (|CallParentFunction))

(fn SpawnEnemy
  (params (Enemy :type TD%20Enemy%20Base%20Class%20Reference))
  (bind _splinecomponents (Variables|Default|GetSplineComponents))
  (bind _keys (Utilities|Map|Keys _splinecomponents))
  (bind _values (Utilities|Map|Values _splinecomponents))
  (for (_array_element _array_index) _keys
    (Game|SpawnActorfromClass Enemy (Math|Transform|MakeTransform (.Location (Spline|GetLocationandTangentatSplinePoint _array_element 0 "World")) (Math|Conversions|RotationFromXVector (.Tangent (Spline|GetLocationandTangentatSplinePoint _array_element 0 "World")))) "AlwaysSpawn" 0 _array_element (Utilities|Array|Get(acopy) _values _array_index) 0)))