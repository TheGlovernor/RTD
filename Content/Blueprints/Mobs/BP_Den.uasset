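; Enemy den for a hex-grid tower defense that grows a path over time and spawns enemies at its advancing tip.
; Tick drives a material percentage on spline mesh segments, revealing terrain tiles as each fills.
; A timer loop spawns queued or weighted-random tiered enemies with game-state scaling, paced by per-enemy cooldowns and GAS attributes.
; Completing the path reveals surrounding terrain, starts recurring boss spawns and applies a boss-cooldown effect.
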(event Custom|AddProgress
  (params (DeltaSeconds :type Float%20%28double-precision%29))
  (bind _currentsplinematerial (Variables|Default|GetCurrentSplineMaterial))
  ;[1 1 1] This is all post - macrohexgen
  (bind _output_get (Variables|Default|SetCurrentPercentage (+ (/ (select (Variables|Default|GetSetupDone) DeltaSeconds 0.0) (Class|GSCCoreComponent|GetCurrentAttributeValue (Variables|/Game/Blueprints/GM/GS_TowerDefense.GS_TowerDefense_C|GetGSCCore (Variables|Game|GetGameState)) "(AttributeName=\"DenExpandTime\",Attribute=/Script/RTD.GameDirector:DenExpandTime,AttributeOwner=\"/Script/CoreUObject.Class'/Script/RTD.GameDirector'\")")) (Variables|Default|GetCurrentPercentage))))
  (Utilities|IsValid _currentsplinematerial
    (:Is%20Valid
      (Rendering|Material|SetScalarParameterValue _currentsplinematerial "Percentage" _output_get :!class /Script/Engine.MaterialInstanceDynamic)
      (if (> _output_get 0.5)
        (if (Variables|Default|GetHasPassed50)
          (if (and (> (Variables|Default|GetCurrentPercentage) 1.0) (not (Variables|Default|GetHasPassed100)))
            (if (Variables|Default|GetLastMeshMade)
              (Variables|Default|SetbAddProgress false)
              (CallFunction|PathDoneBuilding)
              (else
                (Variables|Default|SetHasPassed100 true)
                (CallFunction|AddSplineMesh (Variables|Default|GetNextTile))
                (Variables|Default|SetCurrentPercentage 0.0)
                (Variables|Default|SetHasPassed100 false)
                (Variables|Default|SetHasPassed50 false))))
          (else
            (CallFunction|GenerateNextStepOfPath)
            (Variables|Default|SetHasPassed50 true)))))))

(event Custom|SpawnEnemiesIgnoringQueue
  (params (Enemy :type BP%20Enemy%20Base%2001%20Class%20Reference) (Num :type Integer))
  ;[1 1 1] This is all post - macrohexgen
  (for _index (range 1 Num)
    (CallFunction|SpawnEnemy Enemy -1)
    (Utilities|FlowControl|Delay 0.2)))

(event Custom|StopSpawning
  (bind _spawnspline (Variables|Default|GetSpawnSpline))
  (bind _currentpercentage (Variables|Default|GetCurrentPercentage))
  (bind _gamestate (Variables|Game|GetGameState))
  (bind _pathspline (Variables|Default|GetPathSpline))
  (bind _returnvalue (Spline|GetSplineLength _spawnspline))
  (bind (_goldscaling _healthscaling _shieldscaling _armorscaling) (Default|GetScaling _gamestate))
  (bind _returnvalue_2 (* _returnvalue _currentpercentage))
  (bind _returnvalue_3 (Spline|GetLocationatDistanceAlongSpline _spawnspline _returnvalue_2 "World"))
  ;[1 1 1] This is all post - macrohexgen
  (Utilities|FlowControl|Gate false) ; enters at Close
)

(event Custom|StartSpawning
  ;[1 1 1] This is all post - macrohexgen
  (Utilities|FlowControl|DoOnce false
    (:Completed
      (Variables|Default|SetSetupDone true)
      (CallFunction|SpawnEnemyfromQueue))))

(event Custom|SpawnEnemyFromQueue
  (bind _queue (Variables|Default|GetQueue))
  ;[1 1 1] This is all post - macrohexgen
  (if (Utilities|Array|IsEmpty (Variables|Default|GetQueue))
    (bind _enemy (CallFunction|ChooseEnemy))
    (bind _output_get (Variables|Default|SetEnemyToSpawn _enemy))
    (else
      (Variables|Default|SetEnemyToSpawn (Utilities|Array|Get(acopy) _queue))
      (Utilities|Array|RemoveIndex _queue)))
  (CallFunction|SpawnEnemy _output_get -1)
  (bind _cd (CallFunction|GetEnemyCooldown _output_get))
  (bind _returnvalue (Utilities|Time|SetTimerbyEvent (delegate Custom|SpawnEnemyFromQueue) (Math|Float|Max(Float) (* _cd (Class|GSCCoreComponent|GetCurrentAttributeValue (Variables|Default|GetGSCCore) "(AttributeName=\"NormalCooldownMultiplier\",Attribute=/Script/RTD.Den:NormalCooldownMultiplier,AttributeOwner=\"/Script/CoreUObject.Class'/Script/RTD.Den'\")")) 0.1)))
  (Variables|Default|SetSpawnTimer _returnvalue))

(event Custom|PathDoneBuilding
  (bind _path (Variables|Default|GetPath))
  ;[1 1 1] This is all post - macrohexgen
  (Utilities|FlowControl|DoOnce false
    (:Completed
      (Variables|Default|SetCanSpawnBosses true)
      (bind _offset (Class|GridsHex|SingleRing (Utilities|Array|Get(acopy) _path (- (Utilities|Array|Length _path) 1)) 3))
      (Default|DrawTiles (Variables|Default|GetTerrainGen) _offset)
      (for _array_element (Variables|Default|GetPath)
        (bind _offset_2 (Class|GridsHex|SingleRing _array_element 2))
        (Default|DrawTiles (Variables|Default|GetTerrainGen) _offset_2))
      (CallFunction|SpawnBoss)
      (GameplayEffects|ApplyGameplayEffectToSelf :self (Variables|Default|GetGSCAbilitySystem) :GameplayEffectClass "/Game/Blueprints/Mobs/Dens/GE_DenBossCooldownDecrease.GE_DenBossCooldownDecrease_C"))))

(event Custom|ExpandPreviousTiles
  (params (Index :type Integer) (Radius :type Integer))
  (bind _returnvalue (Math|Integer|Min(Integer) Radius 3))
  (bind _tilestogoback (Variables|Default|GetTilesToGoBack))
  (bind _returnvalue_2 (- Index _tilestogoback))
  ;[1 1 1] This is all post - macrohexgen
  (if (>= _returnvalue_2 0)
    (bind _offset (Class|GridsHex|SingleRing (Utilities|Array|Get(acopy) (Variables|Default|GetPath) _returnvalue_2) _returnvalue))
    (Default|DrawTiles (Variables|Default|GetTerrainGen) _offset)
    (CallFunction|ExpandPreviousTiles _returnvalue_2 (+ _returnvalue 1))))

(event Custom|AddToSpawnQueue
  (params (Enemy :type BP%20Enemy%20Base%2001%20Class%20Reference))
  ;[1 1 1] This is all post - macrohexgen
  (if (Utilities|IsValidClass Enemy)
    (Utilities|Array|Add (Variables|Default|GetQueue) Enemy)
    (else
      (bind _enemy (CallFunction|ChooseEnemy))
      (Utilities|Array|Add (Variables|Default|GetQueue) _enemy))))

(event Custom|SpawnEnemy
  (params (Enemy :type BP%20Enemy%20Base%2001%20Class%20Reference) (RushID :type Integer))
  (bind _spawnspline (Variables|Default|GetSpawnSpline))
  (bind _currentpercentage (Variables|Default|GetCurrentPercentage))
  (bind _gamestate (Variables|Game|GetGameState))
  (bind _pathspline (Variables|Default|GetPathSpline))
  (bind _returnvalue (Spline|GetSplineLength _spawnspline))
  (bind (_goldscaling _healthscaling _shieldscaling _armorscaling) (Default|GetScaling _gamestate))
  (bind _returnvalue_2 (* _returnvalue _currentpercentage))
  (bind _returnvalue_3 (Spline|GetLocationatDistanceAlongSpline _spawnspline _returnvalue_2 "World"))
  ;[1 1 1] This is all post - macrohexgen
  (Utilities|FlowControl|Gate false
    (:Exit
      (CallFunction|DenonSpawnEffects)
      (bind _returnvalue_4 (Game|SpawnActorfromClass Enemy (Math|Transform|MakeTransform _returnvalue_3 (Math|Conversions|RotationFromXVector (* (Spline|GetTangentatDistanceAlongSpline _spawnspline _returnvalue_2 "World") -1.0))) "AlwaysSpawn" "SelectDefaultAtRuntime" 0 _pathspline self (Class|SplineComponent|GetDistanceAlongSplineatSplineInputKey _pathspline (Class|SplineComponent|FindInputKeyClosesttoWorldLocation _pathspline _returnvalue_3)) (Variables|Default|GetNextNode) 0 false _goldscaling _healthscaling _shieldscaling _armorscaling (Variables|/Game/Blueprints/GM/GS_TowerDefense.GS_TowerDefense_C|GetArmorDamageThreshold _gamestate) "NewEnumerator0" true RushID 0))
      (Default|ApplyWorldEffectstoEnemy (Variables|Game|GetGameState) _returnvalue_4))))

(event Custom|SpawnBoss
  ;[1 1 1] This is all post - macrohexgen
  (if (Variables|Default|GetCanSpawnBosses)
    (bind _keys (Utilities|Map|Keys (Variables|Default|GetBoss)))
    (bind _output_get (Variables|Default|SetBossToSpawn (.OutItem (Utilities|Array|Random _keys))))
    (CallFunction|SpawnEnemy _output_get -1)
    (if true
      (bind _returnvalue (Utilities|Time|SetTimerbyEvent (delegate Custom|SpawnBoss) (* (.Value (Utilities|Map|Find (Variables|Default|GetBoss) _output_get)) (Class|GSCCoreComponent|GetCurrentAttributeValue (Variables|Default|GetGSCCore) "(AttributeName=\"BossCooldownMultiplier\",Attribute=/Script/RTD.Den:BossCooldownMultiplier,AttributeOwner=\"/Script/CoreUObject.Class'/Script/RTD.Den'\")"))))
      (Variables|Default|SetBossSpawnTimer _returnvalue))))

(event Custom|DenOnSpawnEffects
  ;[1 1 1] This is all post - macrohexgen
  (Variables|Default|SetSpawning true)
  (Utilities|FlowControl|Delay 0.2)
  (Variables|Default|SetSpawning false))

(event EventBeginPlay
  (bind _tiletodraw (Variables|Default|GetTileToDraw))
  (bind _mycoords (Variables|Default|GetMyCoords))
  (bind _mycoords_2 (Variables|Default|GetMyCoords))
  (bind _terraingen (Variables|Default|GetTerrainGen))
  (bind _mycoords_3 (Variables|Default|GetMyCoords))
  (bind _path (Variables|Default|GetPath))
  (bind _terraingen_2 (Variables|Default|GetTerrainGen))
  (bind _terraingen_3 (Variables|Default|GetTerrainGen))
  (bind _blocked (Variables|/Game/Blueprints/Map/BP_TerrainGen.BP_TerrainGen_C|GetBlocked _terraingen))
  (bind _asgs_tower_defense (Utilities|Casting|CastToGS_TowerDefense (Game|GetGameState)))
  (Variables|Game|SetGameState _asgs_tower_defense)
  ;[1 1 1] This is all post - macrohexgen
  (CallFunction|CustomDenEffects)
  (Default|StartScaling (Variables|Default|GetAC_EnemySpawn))
  (Default|AddPath _terraingen_2 _mycoords_3)
  (Class|GridsHex|SingleRing _mycoords_3 1)
  (Utilities|Set|AddItems (Variables|/Game/Blueprints/Map/BP_TerrainGen.BP_TerrainGen_C|GetBlocked _terraingen_2) 0)
  (Utilities|Array|Insert _path (Variables|/Game/Blueprints/Mobs/BP_PathNode.BP_PathNode_C|GetMyCoords (Variables|Default|GetNextNode)))
  (Default|AddPaths (Variables|Default|GetTerrainGen) _path)
  (bind _offset (Class|GridsHex|SpiralRing _mycoords_2 2))
  (Default|DrawTile _terraingen_3 _mycoords_2)
  (Default|DrawTiles _terraingen_3 _offset)
  (CallFunction|ConstructSpline)
  (CallFunction|FindFirstUniquePath)
  (for _index (range 1 (Variables|Default|GetNumStepsOnSpawn))
    (CallFunction|GenerateNextStepOfPath)
    (CallFunction|AddSplineMesh (Variables|Default|GetNextTile)))
  (Utilities|Set|Add _blocked _mycoords)
  (bind _offset_2 (Class|GridsHex|SingleRing _mycoords 1))
  (Utilities|Set|AddItems _blocked _offset_2)
  (if (Variables|/Game/Blueprints/GM/GS_TowerDefense.GS_TowerDefense_C|GetHasBeenStarted (Variables|Game|GetGameState))
    (bind _transform (Default|FGetGroundTransform (Variables|Default|GetTerrainGen) (select (and (== (.col _tiletodraw) 0) (== (.row _tiletodraw) 0)) (Variables|Default|GetMyCoords) (Variables|Default|GetTileToDraw))))
    (Game|SpawnActorfromClass "/Game/Blueprints/Map/BP_DangerIndicator.BP_DangerIndicator_C" _transform "Undefined" "MultiplyWithRoot" 0 0)
    (Utilities|Time|SetTimerbyEvent (delegate Custom|StartSpawning) 3e+01)))

(event EventTick
  (params (DeltaSeconds :type Float%20%28single-precision%29))
  ;[1 1 1] This is all post - macrohexgen
  (if (Variables|Default|GetbAddProgress)
    (CallFunction|AddProgress DeltaSeconds)))

(event EventApplyEffect
  (params (Source :type GSC%20Ability%20System%20Component%20Object%20Reference) (Effect :type Gameplay%20Effect%20Class%20Reference) (Power :type Float%20%28double-precision%29))
  (GameplayEffects|ApplyGameplayEffectToTarget :self Source :GameplayEffectClass Effect :Target (Variables|Default|GetGSCAbilitySystem)))

(fn ConstructionScript
  (|CallParentFunction)
  (bind _asgs_tower_defense (Utilities|Casting|CastToGS_TowerDefense (Game|GetGameState)))
  (Variables|Default|SetbAddProgress (Variables|/Game/Blueprints/GM/GS_TowerDefense.GS_TowerDefense_C|GetHasBeenStarted _asgs_tower_defense)))

(fn GenerateNextStepOfPath
  (bind _terraingen (Variables|Default|GetTerrainGen))
  (bind _path (Variables|Default|GetPath))
  (bind _mycoords (Variables|Default|GetMyCoords))
  (Default|DrawTile _terraingen (Variables|Default|GetTileToDraw))
  (Default|DrawTiles _terraingen (Class|GridsCore|ToOffsetArray(CubeArray) (Class|GridsHex|GetHexNeighbours (Variables|Default|GetTileToDraw))))
  (CallFunction|ExpandPreviousTiles (Utilities|Array|FindItem (Variables|Default|GetPath) (Variables|Default|GetTileToDraw)) 2)
  (bind _output_get (Variables|Default|SetTileToDraw (Variables|Default|GetNextTile)))
  (if (not (and (== (.Col (Utilities|Struct|BreakOffsetCoords _output_get)) (.col _mycoords)) (== (.Row (Utilities|Struct|BreakOffsetCoords _output_get)) (.row _mycoords))))
    (Variables|Default|SetNextTile (Utilities|Array|Get(acopy) _path (+ (Utilities|Array|FindItem _path _output_get) 1)))))

(fn FindFirstUniquePath
  (for _array_element (Variables|Default|GetPath)
    (bind _hasbeendrawn (Default|CheckifDrawn (Variables|Default|GetTerrainGen) _array_element))
    (if _hasbeendrawn
      (Default|DrawTiles (Variables|Default|GetTerrainGen) (Class|GridsCore|ToOffsetArray(CubeArray) (Class|GridsHex|GetHexNeighbours (Variables|Default|GetTileToDraw))))
      (bind _output_get (Variables|Default|SetTileToDraw _array_element))
      (CallFunction|AddSplineMesh _output_get)
      (else
        (bind _output_get_2 (Variables|Default|SetNextTile _array_element))
        (CallFunction|AddSplineMesh _output_get_2)
        (Default|DrawTiles (Variables|Default|GetTerrainGen) (Class|GridsCore|ToOffsetArray(CubeArray) (Class|GridsHex|GetHexNeighbours (Variables|Default|GetTileToDraw))))
        (return)))))

(fn ConstructSpline
  (Spline|ClearSplinePoints (Variables|Default|GetPathSpline) true)
  (for _array_element (Variables|Default|GetPath)
    (bind _transform (Default|FGetGroundTransform (Variables|Default|GetTerrainGen) _array_element))
    (Spline|AddSplinePoint (Variables|Default|GetPathSpline) (+ (.location _transform) "") "World" true)))

(fn AddSplineMesh
  (params (OffsetCoords :type Offset%20Coords%20Structure))
  (bind _pathspline (Variables|Default|GetPathSpline))
  (bind _spawnspline (Variables|Default|GetSpawnSpline))
  (bind _path (Variables|Default|GetPath))
  (bind _path_2 (Variables|Default|GetPath))
  (bind _returnvalue (Utilities|Array|FindItem _path_2 OffsetCoords))
  (bind (_location _tangent) (Spline|GetLocationandTangentatSplinePoint _pathspline _returnvalue "Local"))
  (bind _returnvalue_2 (- _returnvalue 1))
  (bind (_location_2 _tangent_2) (Spline|GetLocationandTangentatSplinePoint _pathspline _returnvalue_2 "Local"))
  (bind _keys (Utilities|Map|Keys (Variables|Default|GetSplineMeshes)))
  (if (not (or (Utilities|Array|ContainsItem _keys OffsetCoords) (== _returnvalue 0)))
    (Utilities|IsValid (Variables|Default|GetCurrentSplineMaterial)
      (:Is%20Valid
        (Rendering|Material|SetScalarParameterValue (Variables|Default|GetCurrentSplineMaterial) "Percentage" 1.0 :!class /Script/Engine.MaterialInstanceDynamic))
      (:Is%20Not%20Valid
        _))
    (bind _returnvalue_3 (AddComponent|AddSplineMeshComponent false (Math|Transform|MakeTransform "0, 0, 0")))
    (bind _returnvalue_4 (Rendering|Material|CreateDynamicMaterialInstance _returnvalue_3 0 "/Game/Assets/Materials/WorldHighlights/M_PathSpline.M_PathSpline" "None" :!class /Script/Engine.PrimitiveComponent))
    (Variables|Default|SetCurrentSplineMaterial _returnvalue_4)
    (SplineMesh|SetStartandEnd _returnvalue_3 (+ _location_2 "0,0,25.000000") _tangent_2 (+ _location "0,0,25.000000") _tangent true :!class /Script/Engine.SplineMeshComponent)
    (Spline|SetLocationatSplinePoint _spawnspline 0 _location_2 "Local" true)
    (Spline|SetTangentatSplinePoint _spawnspline 0 _tangent_2 "Local" true)
    (Spline|SetLocationatSplinePoint _spawnspline 1 _location "Local" true)
    (Spline|SetTangentatSplinePoint _spawnspline 1 _tangent "Local" true)
    (Utilities|Map|Add (Variables|Default|GetSplineMeshes) OffsetCoords _returnvalue_3)
    (Variables|Default|SetCurrentSplineMesh _returnvalue_3)
    (Rendering|Material|SetScalarParameterValue (Variables|Default|GetCurrentSplineMaterial) "Percentage" 0.0 :!class /Script/Engine.MaterialInstanceDynamic)
    (if (== (- (Utilities|Array|Length _path) 1) (Utilities|Array|FindItem _path OffsetCoords))
      (Variables|Default|SetLastMeshMade true))))

(fn CustomDenEffects)

(fn GetDenRotation
  (bind _path (Variables|Default|GetPath))
  (bind _returnvalue (Utilities|Array|Length _path))
  (return (Utilities|Select :Index (.Direction (Class|GridsHex|FindNeighbourfromAdjacentOffsets (Utilities|Array|Get(acopy) _path (- _returnvalue 1)) (Utilities|Array|Get(acopy) _path (- _returnvalue 2)) false)) :Option%200 "0,-60.000000, 0" :Option%201 "0, 0, 0" :Option%202 "0,60.000000, 0" :Option%203 "0,120.000000, 0" :Option%204 "0,180.000000, 0" :Option%205 "0,240.000000, 0")))

(fn GetEnemyCooldown
  (params (Enemy :type BP%20Enemy%20Base%2001%20Class%20Reference))
  (bind _t2enemy (Variables|Default|GetT2Enemy))
  (bind _t1enemy (Variables|Default|GetT1Enemy))
  (bind _foreignt1s (Variables|Default|GetForeignT1s))
  (bind _foreignt2s (Variables|Default|GetForeignT2s))
  (bind (_value _returnvalue) (Utilities|Map|Find _t1enemy Enemy))
  (bind (_value_2 _returnvalue_2) (Utilities|Map|Find _foreignt2s Enemy))
  (bind (_value_3 _returnvalue_3) (Utilities|Map|Find _t2enemy Enemy))
  (bind (_value_4 _returnvalue_4) (Utilities|Map|Find _foreignt1s Enemy))
  (if _returnvalue
    (return _value)
    (elif _returnvalue_3
      (return _value_3)
      (elif _returnvalue_4
        (return _value_4)
        (elif _returnvalue_2
          (return _value_2)
          (else
            (return 5.0)))))))

(fn ChooseEnemy
  (bind _gsccore (Variables|Default|GetGSCCore))
  (bind _foreignt1s (Variables|Default|GetForeignT1s))
  (bind _foreignt2s (Variables|Default|GetForeignT2s))
  (bind _returnvalue (Class|GSCCoreComponent|GetCurrentAttributeValue _gsccore "(AttributeName=\"T2Weight\",Attribute=/Script/RTD.Den:T2Weight,AttributeOwner=\"/Script/CoreUObject.Class'/Script/RTD.Den'\")"))
  (if (> _returnvalue 0.0)
    (bind _output_get (LocalVariables|SetTotalWeight (+ (Class|GSCCoreComponent|GetCurrentAttributeValue _gsccore "(AttributeName=\"T1Weight\",Attribute=/Script/RTD.Den:T1Weight,AttributeOwner=\"/Script/CoreUObject.Class'/Script/RTD.Den'\")") _returnvalue)))
    (bind _output_get_2 (LocalVariables|SetValue (Math|Random|RandomFloatinRange 0.0 _output_get)))
    (if (Math|Float|InRange(Float) _output_get_2 0.0 (Class|GSCCoreComponent|GetCurrentAttributeValue (Variables|Default|GetGSCCore) "(AttributeName=\"T1Weight\",Attribute=/Script/RTD.Den:T1Weight,AttributeOwner=\"/Script/CoreUObject.Class'/Script/RTD.Den'\")"))
      _
      (else
        (bind _keys (Utilities|Map|Keys (select (and (Utilities|Map|IsNotEmpty _foreignt2s) (< (Math|Random|RandomFloat) (Variables|Default|GetForeignEnemyChance))) _foreignt2s (Variables|Default|GetT2Enemy))))
        (return (.OutItem (Utilities|Array|Random _keys))))))
  (bind _keys_2 (Utilities|Map|Keys (select (and (Utilities|Map|IsNotEmpty _foreignt1s) (< (Math|Random|RandomFloat) (Variables|Default|GetForeignEnemyChance))) _foreignt1s (Variables|Default|GetT1Enemy))))
  (return (.OutItem (Utilities|Array|Random _keys_2))))

(fn SpawnBossRush
  (params (RushID :type Integer))
  (if (Variables|Default|GetCanSpawnBosses)
    (bind _keys (Utilities|Map|Keys (Variables|Default|GetBoss)))
    (bind _output_get (Variables|Default|SetBossToSpawn (.OutItem (Utilities|Array|Random _keys))))
    (CallFunction|SpawnEnemy _output_get -1)
    (return true)
    (else
      (return false))))