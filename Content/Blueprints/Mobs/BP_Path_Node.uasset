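; Enemy path node on the macro hex map that draws a route segment to NextNode and spawns enemies on it.
; On BeginPlay it builds a spline through the surface locations of its Path hexes and lays spline meshes along it, matching the last tangent to NextNode's first.
; DistanceToBase accumulates spline length from NextNode's value.
; SpawnEnemy places an enemy at the spline start, passing it the spline, distance and next node.
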(event EventBeginPlay
  (bind _asbp_macro_hex_handler (Utilities|Casting|CastToBP_MacroHexHandler (Components|GetOwner)))
  (Variables|Default|SetMacroHexHandler _asbp_macro_hex_handler)
  (Utilities|Array|Insert (Variables|Default|GetPath) (Variables|Default|GetMyCoords))
  (bind _nextnode (Variables|Default|GetNextNode)
    (:then
      (Utilities|Array|Add (Variables|Default|GetPath) (Variables|BP_Path_Node_C|GetMyCoords _nextnode)))
    (:else
      _))
  (Utilities|FlowControl|Sequence
    (:then_0
      (Variables|Default|GetCurrentSplineComponent
        (:then)
        (:else
          (bind _returnvalue (AddComponent|AddSplineComponent false (Math|Transform|MakeTransform "0, 0, 0")))
          (Variables|Default|SetCurrentSplineComponent _returnvalue))))
    (:then_1
      (Spline|ClearSplinePoints (Variables|Default|GetCurrentSplineComponent) true))
    (:then_2
      (for _array_element (Variables|Default|GetPath)
        (bind _location (Default|SurfaceLocation (Variables|Default|GetMacroHexHandler) _array_element))
        (Spline|AddSplinePoint (Variables|Default|GetCurrentSplineComponent) (+ _location (Math|Vector|MakeVector 0.0 0.0 1.0)) "World" true)))
    (:then_3
      (for _index (range 0 (- (Spline|GetNumberOfSplinePoints (Variables|Default|GetCurrentSplineComponent)) 2))
        (if (!= _index (- (Spline|GetNumberOfSplinePoints (Variables|Default|GetCurrentSplineComponent)) 2))
          (bind _returnvalue_2 (AddComponent|AddSplineMeshComponent false (Math|Transform|MakeTransform "0, 0, 0")))
          (SplineMesh|SetStartandEnd _returnvalue_2 (+ (.Location (Spline|GetLocationandTangentatSplinePoint (Variables|Default|GetCurrentSplineComponent) _index "Local")) "0,0,10.000000") (.Tangent (Spline|GetLocationandTangentatSplinePoint (Variables|Default|GetCurrentSplineComponent) _index "Local")) (+ (.Location (Spline|GetLocationandTangentatSplinePoint (Variables|Default|GetCurrentSplineComponent) (+ _index 1) "Local")) "0,0,10.000000") (.Tangent (Spline|GetLocationandTangentatSplinePoint (Variables|Default|GetCurrentSplineComponent) (+ _index 1) "Local")) true :!class /Script/Engine.SplineMeshComponent)
          (Utilities|Array|Add (Variables|Default|GetSplineMeshComponents) _returnvalue_2)
          (else
            (bind _returnvalue_3 (AddComponent|AddSplineMeshComponent false (Math|Transform|MakeTransform "0, 0, 0")))
            (SplineMesh|SetStartandEnd _returnvalue_3 (+ (.Location (Spline|GetLocationandTangentatSplinePoint (Variables|Default|GetCurrentSplineComponent) _index "Local")) "0.000000,0,10.000000") (.Tangent (Spline|GetLocationandTangentatSplinePoint (Variables|Default|GetCurrentSplineComponent) _index "Local")) (+ (.Location (Spline|GetLocationandTangentatSplinePoint (Variables|Default|GetCurrentSplineComponent) (+ _index 1) "Local")) "0,0,10.000000") (.Tangent (Spline|GetLocationandTangentatSplinePoint (Variables|BP_Path_Node_C|GetCurrentSplineComponent (Variables|Default|GetNextNode)) 0 "Local")) true :!class /Script/Engine.SplineMeshComponent)
            (Utilities|Array|Add (Variables|Default|GetSplineMeshComponents) _returnvalue_3)))))
    (:then_4
      (bind _nextnode_2 (Variables|Default|GetNextNode)
        (:then
          (Variables|Default|SetDistanceToBase (+ (Variables|BP_Path_Node_C|GetDistanceToBase _nextnode_2) (Spline|GetSplineLength (Variables|Default|GetCurrentSplineComponent)))))
        (:else)))))

(event Collision|EventActorBeginOverlap
  (params (OtherActor :type Actor%20Object%20Reference))
  (Utilities|Casting|CastToBP_Enemy_Base_01 OtherActor))

(fn ConstructionScript)

(fn SpawnEnemy
  (params (Enemy :type BP%20Enemy%20Base%2001%20Class%20Reference))
  (bind _currentsplinecomponent (Variables|Default|GetCurrentSplineComponent))
  (bind (_location _tangent) (Spline|GetLocationandTangentatSplinePoint _currentsplinecomponent 0 "World"))
  (Game|SpawnActorfromClass Enemy (Math|Transform|MakeTransform _location (Math|Conversions|RotationFromXVector _tangent) "0.500000,0.500000,0.500000") "AdjustIfPossibleButAlwaysSpawn" 0 (Variables|Default|GetCurrentSplineComponent) (Variables|Default|GetDistanceToBase) (Variables|Default|GetNextNode) 0))