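; Base tower-defense enemy that travels along a spline path and takes damage until destroyed.
; Each tick it advances a fixed step along the spline, matching position and rotation, and reduces its remaining distance to the base; without a valid spline it destroys itself.
; Damage lowers health, initialized to max at construction, then either destroys the actor or updates its health bar widget.
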(event EventBeginPlay)

(event EventTick
  (params (DeltaSeconds :type Float%20%28single-precision%29))
  (bind _spline (Variables|Default|GetSpline)
    (:then
      (Transformation|AddActorWorldOffset (- (Spline|GetLocationatDistanceAlongSpline _spline (+ (Variables|Default|GetLocationOnCurrentSpline) (Variables|Default|GetMovementSpeed)) "World") (Transformation|GetActorLocation)))
      (Transformation|SetActorRotation (Spline|GetRotationatDistanceAlongSpline _spline (+ (Variables|Default|GetLocationOnCurrentSpline) (Variables|Default|GetMovementSpeed)) "Local"))
      (Variables|Default|SetLocationOnCurrentSpline (+ (Variables|Default|GetLocationOnCurrentSpline) (Variables|Default|GetMovementSpeed)))
      (Variables|Default|SetDistanceToBase (- (Variables|Default|GetDistanceToBase) (Variables|Default|GetMovementSpeed))))
    (:else
      (Actor|DestroyActor))))

(event Game|Damage|EventAnyDamage
  (params (Damage :type Float%20%28single-precision%29) (DamageType :type Damage%20Type%20Object%20Reference) (InstigatedBy :type Controller%20Object%20Reference) (DamageCauser :type Actor%20Object%20Reference))
  (bind _output_get (Variables|Default|SetHealth (- (Variables|Default|GetHealth) Damage)))
  (if (<= _output_get 0.0)
    (Actor|DestroyActor)
    (else
      (bind _ashealth_bar (Utilities|Casting|CastToHealthBar (UserInterface|GetWidget (Variables|Default|GetWidget))))
      (Default|SetPercent _ashealth_bar (/ (Variables|Default|GetHealth) (Variables|Default|GetMaxHealth))))))

(fn ConstructionScript
  (Variables|Default|SetHealth (Variables|Default|GetMaxHealth)))