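; Enemy path start node on the hex grid that builds routes to its next nodes and spawns mobs onto them.
; On BeginPlay it turns A* hex paths into splines and spline meshes, blending the last tangent into the next node's spline.
; Each spline is stored with its total distance to base.
; SpawnEnemy spawns one enemy per spline, occasionally an enlarged elite, and applies difficulty scaling through a SetByCaller GameplayEffect.
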(event EventBeginPlay
  (bind _asbp_macro_hex_handler (Utilities|Casting|CastToBP_MacroHexHandler (Components|GetOwner)))
  (Variables|Default|SetMacroHexHandler _asbp_macro_hex_handler)
  (for _array_element (Variables|Default|GetNextNodes)
    (Utilities|FlowControl|Sequence
      (:then_0
        (bind _returnvalue (AddComponent|AddSplineComponent false (Math|Transform|MakeTransform "0, 0, 0")))
        (Variables|Default|SetCurrentSplineComponent _returnvalue))
      (:then_1
        (Spline|ClearSplinePoints (Variables|Default|GetCurrentSplineComponent) true))
      (:then_2
        (bind _results (Class|GridsHex|AStarPathfinding (Variables|Default|GetMyCoords) (Variables|/Game/Blueprints/Mobs/BP_Path_Node.BP_Path_Node_C|GetMyCoords _array_element) (Variables|Default|GetPath) 0 0 "(Col=0,Row=0)" true false))
        (bind _output_get (Variables|Default|SetCurrentPath (Class|GridsCore|ToOffsetArray(CubeArray) _results)))
        (Utilities|Array|Insert _output_get (Variables|Default|GetMyCoords))
        (Utilities|Array|Add _output_get (Variables|/Game/Blueprints/Mobs/BP_Path_Node.BP_Path_Node_C|GetMyCoords _array_element))
        (for _array_element_2 _output_get
          (bind _location (Default|TopOfSurfaceLocation (Variables|Default|GetMacroHexHandler) _array_element_2))
          (Spline|AddSplinePoint (Variables|Default|GetCurrentSplineComponent) (.location _location) "World" true)))
      (:then_3
        (for _index (range 0 (- (Spline|GetNumberOfSplinePoints (Variables|Default|GetCurrentSplineComponent)) 2))
          (if (!= _index (- (Spline|GetNumberOfSplinePoints (Variables|Default|GetCurrentSplineComponent)) 2))
            (bind _returnvalue_2 (AddComponent|AddSplineMeshComponent false (Math|Transform|MakeTransform "0, 0, 0")))
            (SplineMesh|SetStartandEnd _returnvalue_2 (+ (.Location (Spline|GetLocationandTangentatSplinePoint (Variables|Default|GetCurrentSplineComponent) _index "Local")) "0,0,20.000000") (.Tangent (Spline|GetLocationandTangentatSplinePoint (Variables|Default|GetCurrentSplineComponent) _index "Local")) (+ (.Location (Spline|GetLocationandTangentatSplinePoint (Variables|Default|GetCurrentSplineComponent) (+ _index 1) "Local")) "0,0,20.000000") (.Tangent (Spline|GetLocationandTangentatSplinePoint (Variables|Default|GetCurrentSplineComponent) (+ _index 1) "Local")) true :!class /Script/Engine.SplineMeshComponent)
            (Utilities|Array|Add (Variables|Default|GetSplineMeshComponents) _returnvalue_2)
            (else
              (bind _returnvalue_3 (AddComponent|AddSplineMeshComponent false (Math|Transform|MakeTransform "0, 0, 0")))
              (SplineMesh|SetStartandEnd _returnvalue_3 (+ (.Location (Spline|GetLocationandTangentatSplinePoint (Variables|Default|GetCurrentSplineComponent) _index "Local")) "0,0,20.000000") (.Tangent (Spline|GetLocationandTangentatSplinePoint (Variables|Default|GetCurrentSplineComponent) _index "Local")) (+ (.Location (Spline|GetLocationandTangentatSplinePoint (Variables|Default|GetCurrentSplineComponent) (+ _index 1) "Local")) "0,0,20.000000") (.Tangent (Spline|GetLocationandTangentatSplinePoint (Variables|/Game/Blueprints/Mobs/BP_Path_Node.BP_Path_Node_C|GetCurrentSplineComponent _array_element) 0 "Local")) true :!class /Script/Engine.SplineMeshComponent)
              (Utilities|Array|Add (Variables|Default|GetSplineMeshComponents) _returnvalue_3))))
        (Utilities|Map|Add (Variables|Default|GetSplineComponents) (Variables|Default|GetCurrentSplineComponent) (+ (Spline|GetSplineLength (Variables|Default|GetCurrentSplineComponent)) (Variables|/Game/Blueprints/Mobs/BP_Path_Node.BP_Path_Node_C|GetDistanceToBase _array_element)))))))

(event EventTick
  (params (DeltaSeconds :type Float%20%28single-precision%29)))

(event EventActorBeginOverlap
  (params (OtherActor :type Actor%20Object%20Reference)))

(fn ConstructionScript
  (|CallParentFunction))

(fn SpawnEnemy
  (bind _splinecomponents (Variables|Default|GetSplineComponents))
  (bind _gscabilitysystem (Variables|Default|GetGSCAbilitySystem))
  (bind _scaling (Variables|Default|GetScaling))
  (bind _keys (Utilities|Map|Keys _splinecomponents))
  (bind _values (Utilities|Map|Values _splinecomponents))
  (for (_array_element _array_index) _keys
    (bind _output_get (LocalVariables|SetElite (Math|Random|RandomBoolwithWeight 0.1)))
    (bind _enemyclass (CallFunction|ChooseEnemy))
    (bind _returnvalue (Game|SpawnActorfromClass :Class _enemyclass :SpawnTransform (Math|Transform|MakeTransform (.Location (Spline|GetLocationandTangentatSplinePoint _array_element 0 "World")) (Math|Conversions|RotationFromXVector (.Tangent (Spline|GetLocationandTangentatSplinePoint _array_element 0 "World"))) (Math|Conversions|ToVector(Float) (select _output_get 2.0 1.0))) :CollisionHandlingOverride "AlwaysSpawn" :Spline _array_element :DistanceToBase (Utilities|Array|Get(acopy) _values _array_index) :NextNode (Utilities|Array|Get(acopy) (Variables|Default|GetNextNodes) _array_index) :Instigator 0))
    (bind _returnvalue_2 (Ability|GameplayEffect|AssignTagSetbyCallerMagnitude (GameplayEffects|MakeOutgoingSpec :self _gscabilitysystem :GameplayEffectClass "/Game/Blueprints/Mobs/EnemyModifiers/GE_DifficultyScaling.GE_DifficultyScaling_C" :Level 1.0) "(TagName=\"EffectMagnitude\")" (select (LocalVariables|GetElite) (* _scaling 2.0) _scaling)))
    (Class|GASInterface|ApplySpec(Message) _returnvalue _gscabilitysystem _returnvalue_2)))