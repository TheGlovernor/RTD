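; BP_Yeti_King is a boss enemy Blueprint whose special ability applies the GE_Yeti_Inspire effect to actors around it.
; ActivateAbility resets the cooldown value, flags casting and runs a large capsule multi-trace at the boss's location, with debug drawing on.
; Each hit actor gets an apply-effect message sourced from GSCAbilitySystem.
; A short Delay inside the loop clears the casting flag, and construction defers to the parent.
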(event EventActivateAbility
  (bind _returnvalue (Transformation|GetActorLocation))
  (Variables|Default|SetCooldownValue 0.0)
  (Variables|Default|SetbCastingAbility true)
  (bind _outhits (Class|KismetSystemLibrary|CapsuleTraceMulti _returnvalue _returnvalue 1.5e+03 1e+03 "TraceTypeQuery6" false 0 "ForDuration" true))
  (for _array_element _outhits
    (Class|GASInterface|ApplyEffect(Message) (.HitActor (Collision|BreakHitResult _array_element)) (Variables|Default|GetGSCAbilitySystem) "/Game/Blueprints/Mobs/EnemyBPs/Bosses/GE_Yeti_Inspire.GE_Yeti_Inspire_C" 0.0)
    (Utilities|FlowControl|Delay 0.4)
    (Variables|Default|SetbCastingAbility false)))

(fn ConstructionScript
  (|CallParentFunction))