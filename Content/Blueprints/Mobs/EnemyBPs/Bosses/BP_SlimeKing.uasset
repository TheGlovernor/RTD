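; Slime King boss enemy that splits into smaller-generation copies of itself when destroyed, until the generation limit is reached.
; On Destroyed, a DoOnce gate spawns the offspring evenly across a spread around its current spline position, clamped to the spline's bounds.
; Each child inherits the path, next node, effects and scaling, with an incremented generation, an offspring flag and recomputed spline location and distance to base.
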(event EventDestroyed
  (Utilities|FlowControl|DoOnce false
    (:Completed
      (if (< (Variables|Default|GetGeneration) (Variables|Default|GetNumGenerations))
        (Variables|Default|SetStartSpawningAt (Math|Float|Max(Float) (- (Variables|Default|GetLocationOnCurrentSpline) (/ (Variables|Default|GetOffspringSpread) 2.0)) 0.0))
        (Variables|Default|SetSpawnDistanceToBase (+ (Variables|Default|GetDistanceToBase) (Math|Float|Min(Float) (Variables|Default|GetLocationOnCurrentSpline) (/ (Variables|Default|GetOffspringSpread) 2.0))))
        (for _index (range 0 (- (Variables|Default|GetNumOffspring) 1))
          (Game|SpawnActorfromClass "BP_SlimeKing_C" (Spline|GetTransformatDistanceAlongSpline (Variables|Default|GetSpline) (Math|Float|Clamp(Float) (+ (Variables|Default|GetStartSpawningAt) (* _index (/ (Variables|Default|GetOffspringSpread) (- (Variables|Default|GetNumOffspring) 1)))) 0.0 (Spline|GetSplineLength (Variables|Default|GetSpline))) "World" false) "AlwaysSpawn" 0 (+ (Variables|Default|GetGeneration) 1) (Variables|Default|GetNumGenerations) (Variables|Default|GetSpline) (Math|Float|Clamp(Float) (+ (Variables|Default|GetStartSpawningAt) (* _index (/ (Variables|Default|GetOffspringSpread) (- (Variables|Default|GetNumOffspring) 1)))) 0.0 (Spline|GetSplineLength (Variables|Default|GetSpline))) (+ (Math|Float|Clamp(Float) (+ (Variables|Default|GetStartSpawningAt) (* _index (/ (Variables|Default|GetOffspringSpread) (- (Variables|Default|GetNumOffspring) 1)))) 0.0 (Spline|GetSplineLength (Variables|Default|GetSpline))) (Variables|Default|GetSpawnDistanceToBase)) (Variables|Default|GetNextNode) (Variables|Default|GetBegginingEffects) true (Variables|Default|GetScaling) 0))))))

(fn ConstructionScript
  (|CallParentFunction))