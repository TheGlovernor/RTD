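; Projectile spawner that lobs a slime toward a target location and turns it into an offspring Slime King on arrival.
; BeginPlay starts scaling the mesh through ACEnemySpawn and launches ProjectileMovement on a computed high arc.
; A gated Tick detects arrival or a fall below a Z floor, then spawns BP_SlimeKing at the target with generation, spline path and stat data, and destroys the spawner.
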(event Custom|CloseGate
  (bind _returnvalue (Transformation|GetActorLocation))
  (Utilities|FlowControl|Gate false) ; enters at Close
)

(event EventBeginPlay
  (bind _returnvalue (Transformation|GetActorLocation))
  (bind _projectilemovement (Variables|Default|GetProjectileMovement))
  (bind _ac_enemyspawn (Variables|Default|GetAC_EnemySpawn))
  (bind _targetlocation (Variables|Default|GetTargetLocation))
  (bind _returnvalue_2 (Components|Movement|GetGravityZ _projectilemovement))
  (bind (_direction _velocity) (Utilities|GetInitialVelocitySimple _returnvalue _targetlocation 75.0 _returnvalue_2))
  (Variables|/Game/Blueprints/Mobs/EnemyBPs/AC_EnemySpawn.AC_EnemySpawn_C|SetTarget _ac_enemyspawn (Variables|Default|GetStaticMesh))
  (Default|StartScaling _ac_enemyspawn)
  (Variables|/Script/Engine.MovementComponent|SetVelocity _projectilemovement (* _direction _velocity))
  (Components|Activation|Activate _projectilemovement false))

(event EventTick
  (params (DeltaSeconds :type Float%20%28single-precision%29))
  (bind _returnvalue (Transformation|GetActorLocation))
  (Utilities|FlowControl|Gate false
    (:Exit
      (if (or (< (.Z (Math|Vector|BreakVector _returnvalue)) -1e+03) (Utilities|Operators|EqualEqual _returnvalue (Variables|Default|GetTargetLocation) 2e+01))
        (CallFunction|CloseGate)
        (Components|Activation|Deactivate (Variables|Default|GetProjectileMovement))
        (Game|SpawnActorfromClass "/Game/Blueprints/Mobs/EnemyBPs/Bosses/BP_SlimeKing.BP_SlimeKing_C" (Math|Conversions|ToTransform(Vector) (Variables|Default|GetTargetLocation)) "Undefined" "OverrideRootScale" 0 (Variables|Default|GetGeneration) (Variables|Default|GetNumGenerations) (Variables|Default|GetTargetScale) (Variables|Default|GetSpawnSpline) (Variables|Default|GetDen) (Variables|Default|GetLocationOnSpline) (Variables|Default|GetTargetNode) (Variables|Default|GetBeginningEffects) true (Variables|Default|GetScaling) (Variables|Default|GetArmor%20Damage%20Threshold) "NewEnumerator0" (Variables|Default|GetbCanCountAsKill) 0)
        (Actor|DestroyActor)))))

(fn ConstructionScript)