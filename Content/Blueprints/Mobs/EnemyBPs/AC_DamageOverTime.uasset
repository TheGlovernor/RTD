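; Actor component on enemies that applies fire, bleed and entangle damage over time.
; Fire and bleed stacks queue the source tower, whose attributes set each hit's damage; self-rescheduling timers consume one stack per hit, ticking faster as stacks grow.
; Entangle ticks down a counter at a fixed rate with an attribute-based chance to multiply damage.
; Fire and bleed changes refresh the enemy's health widget status effects.
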(event Custom|DoFireDamage
  (bind _onfire (Variables|Default|GetOnFire))
  (bind _onfire_2 (Variables|Default|GetOnFire))
  (bind _output (Utilities|Array|Get(acopy) _onfire))
  (bind _gsccore (Variables|/Game/Blueprints/Building/Tower/BP_Tower_1Parent.BP_Tower_1Parent_C|GetGSCCore _output))
  (if (Utilities|Array|IsNotEmpty (Variables|Default|GetOnFire))
    (Game|Damage|ApplyDamage (Components|GetOwner) (* (Class|GSCCoreComponent|GetCurrentAttributeValue _gsccore "(AttributeName=\"AttackPower\",Attribute=/Script/RTD.TowerAttributeSet:AttackPower,AttributeOwner=\"/Script/CoreUObject.Class'/Script/RTD.TowerAttributeSet'\")") (Class|GSCCoreComponent|GetCurrentAttributeValue _gsccore "(AttributeName=\"EngulfPower\",Attribute=/Script/RTD.TowerAttributeSet:EngulfPower,AttributeOwner=\"/Script/CoreUObject.Class'/Script/RTD.TowerAttributeSet'\")")) 0 _output "/Game/Blueprints/HealthDamage/DamageClasses/BP_FireDamage_DOT.BP_FireDamage_DOT_C")
    (Utilities|Array|RemoveIndex _onfire_2)
    (CallFunction|UpdateHealthWidget)
    (Utilities|Time|SetTimerbyEvent (delegate Custom|DoFireDamage) (/ 1.0 (Math|Conversions|ToFloat(Integer) (Math|Integer|Max(Integer) (Utilities|Array|Length _onfire_2) 1))))
    (else
      (Utilities|Time|SetTimerbyEvent (delegate Custom|DoFireDamage) 1.0))))

(event Custom|DoBleedDamage
  (bind _bleed (Variables|Default|GetBleed))
  (bind _bleed_2 (Variables|Default|GetBleed))
  (bind _output (Utilities|Array|Get(acopy) _bleed))
  (bind _gsccore (Variables|/Game/Blueprints/Building/Tower/BP_Tower_1Parent.BP_Tower_1Parent_C|GetGSCCore _output))
  (if (Utilities|Array|IsNotEmpty (Variables|Default|GetBleed))
    (bind _asbp_enemy_base_01 (Utilities|Casting|CastToBP_Enemy_Base_01 (Components|GetOwner)))
    (Game|Damage|ApplyDamage _asbp_enemy_base_01 (* (Class|GSCCoreComponent|GetCurrentAttributeValue _gsccore "(AttributeName=\"AttackPower\",Attribute=/Script/RTD.TowerAttributeSet:AttackPower,AttributeOwner=\"/Script/CoreUObject.Class'/Script/RTD.TowerAttributeSet'\")") (Class|GSCCoreComponent|GetCurrentAttributeValue _gsccore "(AttributeName=\"BleedPower\",Attribute=/Script/RTD.TowerAttributeSet:BleedPower,AttributeOwner=\"/Script/CoreUObject.Class'/Script/RTD.TowerAttributeSet'\")")) 0 _output "/Game/Blueprints/HealthDamage/DamageClasses/BP_BleedDamage_DOT.BP_BleedDamage_DOT_C")
    (Utilities|Array|RemoveIndex _bleed_2)
    (CallFunction|UpdateHealthWidget)
    (Utilities|Time|SetTimerbyEvent (delegate Custom|DoBleedDamage) (/ 1.0 (Math|Conversions|ToFloat(Integer) (Math|Integer|Max(Integer) (Utilities|Array|Length _bleed_2) 1))))
    (else
      (Utilities|Time|SetTimerbyEvent (delegate Custom|DoBleedDamage) 1.0))))

(event Custom|AddFireStack
  (params (Tower :type BP%20Tower%201%20Parent%20Object%20Reference))
  (Utilities|Array|Add (Variables|Default|GetOnFire) Tower)
  (CallFunction|UpdateHealthWidget))

(event Custom|AddBleedStack
  (params (Tower :type BP%20Tower%201%20Parent%20Object%20Reference))
  (Utilities|Array|Add (Variables|Default|GetBleed) Tower)
  (CallFunction|UpdateHealthWidget))

(event Custom|DoEntangleDamage
  (bind _entangledamage (Variables|Default|GetEntangleDamage))
  (bind _entangleactor (Variables|Default|GetEntangleActor))
  (bind _gsccore (Variables|/Game/Blueprints/Building/Tower/BP_Tower_1Parent.BP_Tower_1Parent_C|GetGSCCore _entangleactor))
  (if (> (Variables|Default|GetEntangleStacks) 0)
    (Game|Damage|ApplyDamage (Components|GetOwner) (Math|Float|SelectFloat (* (Class|GSCCoreComponent|GetCurrentAttributeValue _gsccore "(AttributeName=\"CritX\",Attribute=/Script/RTD.TowerAttributeSet:CritX,AttributeOwner=\"/Script/CoreUObject.Class'/Script/RTD.TowerAttributeSet'\")") _entangledamage) _entangledamage (> (Class|GSCCoreComponent|GetCurrentAttributeValue _gsccore "(AttributeName=\"CritChance\",Attribute=/Script/RTD.TowerAttributeSet:CritChance,AttributeOwner=\"/Script/CoreUObject.Class'/Script/RTD.TowerAttributeSet'\")") (Math|Random|RandomFloat))) 0 (Variables|Default|GetEntangleActor) "/Game/Blueprints/HealthDamage/DamageClasses/BP_PhysicalDamage_DOT.BP_PhysicalDamage_DOT_C")
    (Math|Integer|DecrementInt (Variables|Default|GetEntangleStacks)
      (:%20%20
        (Utilities|Time|SetTimerbyEvent (delegate Custom|DoEntangleDamage) 0.25)))
    (else
      (Utilities|Time|SetTimerbyEvent (delegate Custom|DoEntangleDamage) 0.1))))

(event Custom|UpdateHealthWidget
  (bind _asbp_enemy_base_01 (Utilities|Casting|CastToBP_Enemy_Base_01 (Components|GetOwner)))
  (bind _ashealth_widget (Utilities|Casting|CastToHealthWidget (UserInterface|GetWidget (Variables|/Game/Blueprints/Mobs/EnemyBPs/BP_Enemy_Base_01.BP_Enemy_Base_01_C|GetWidget _asbp_enemy_base_01))))
  (Default|UpdateNonTaggedStatusEffects _ashealth_widget self))

(event EventBeginPlay
  (CallFunction|DoFireDamage)
  (CallFunction|DoBleedDamage)
  (CallFunction|DoEntangleDamage))