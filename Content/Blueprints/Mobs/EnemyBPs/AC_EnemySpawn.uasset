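; AC_EnemySpawn animates a target component for enemy spawning, either growing it to full scale or dropping it to the ground.
; A gated Tick scales the target linearly up to TargetScale over ScaleInTime, then closes the gate.
; FallToGround switches Tick to an accelerating drop in relative Z, clamped at zero, which skips the validity check and never closes the gate itself.
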(event Custom|StartScaling
  (bind _target (Variables|Default|GetTarget))
  (bind _relativelocation (Variables|/Script/Engine.SceneComponent|GetRelativeLocation _target))
  (Utilities|FlowControl|Gate true) ; enters at Open
)

(event Custom|StopScaling
  (bind _target (Variables|Default|GetTarget))
  (bind _relativelocation (Variables|/Script/Engine.SceneComponent|GetRelativeLocation _target))
  (Utilities|FlowControl|Gate true) ; enters at Close
)

(event Custom|FallToGround
  (bind _target (Variables|Default|GetTarget))
  (bind _relativelocation (Variables|/Script/Engine.SceneComponent|GetRelativeLocation _target))
  (Variables|Default|SetbReverse true)
  (Utilities|FlowControl|Gate true) ; enters at Open
)

(event EventTick
  (params (DeltaSeconds :type Float%20%28single-precision%29))
  (bind _target (Variables|Default|GetTarget))
  (bind _relativelocation (Variables|/Script/Engine.SceneComponent|GetRelativeLocation _target))
  (Utilities|FlowControl|Gate true
    (:Exit
      (if (Variables|Default|GetbReverse)
        (Variables|Default|SetVelocity (+ (Variables|Default|GetVelocity) (* (Variables|Default|GetAcceleration) DeltaSeconds)))
        (Transformation|SetRelativeLocation (Variables|Default|GetTarget) (Math|Vector|MakeVector (.x _relativelocation) (.y _relativelocation) (Math|Float|Max(Float) (- (.z _relativelocation) (Variables|Default|GetVelocity)) 0.0)) false false)
        (else
          (bind _output_get (Variables|Default|SetValue (Math|Float|Clamp(Float) (+ (/ DeltaSeconds (Variables|Default|GetScaleInTime)) (Variables|Default|GetValue)))))
          (bind _target_2 (Variables|Default|GetTarget)
            (:then
              (Transformation|SetRelativeScale3D _target_2 (* (Math|Conversions|ToVector(Float) _output_get) (Variables|Default|GetTargetScale)))
              (if (== (Variables|Default|GetValue) 1.0)
                (CallFunction|StopScaling)))
            (:else)))))))