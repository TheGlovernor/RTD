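; Base enemy for a spline-path game with targeting: it walks toward distance zero, damages the home's health there, and exposes stats for target selection.
; Gameplay effects via GSC ability components drive spawn scaling, status effects and layered shield, armor and health damage, feeding a health widget and overlay material.
; Gates toggle movement and damage; death credits the killer and can trigger a necromancer ghost.
; Child classes can override empty hooks for abilities and effects.
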(event OnAttributeChange(GSCCore)
  (params (Attribute :type Gameplay%20Attribute%20Structure) (DeltaValue :type Float%20%28single-precision%29) (EventTags :type Gameplay%20Tag%20Container%20Structure))
  (CallFunction|UpdateUI))

(event OnGameplayTagChange(GSCCore)
  (params (GameplayTag :type Gameplay%20Tag%20Structure) (NewTagCount :type Integer))
  (bind _ashealth_widget (Utilities|Casting|CastToHealthWidget (UserInterface|GetWidget (Variables|Default|GetWidget))))
  (Default|UpdateStatusEffect _ashealth_widget GameplayTag NewTagCount))

(event Custom|ApplyHexDamage
  (Game|Damage|ApplyDamage self (Variables|Status|GetStoredDamage) 0 0 (Variables|status|GetHexDamageType)))

(event Custom|ActivateAbility)

(event Custom|ReachedDen)

(event Custom|Death
  (bind _overlappingactors (Collision|GetOverlappingActors "/Game/Blueprints/Mobs/EnemyBPs/Bosses/Enemy_Necromancer.Enemy_Necromancer_C" :!class /Script/Engine.Actor))
  (bind _skeletalmesh (Variables|Default|GetSkeletalMesh))
  (Game|SpawnActorfromClass "/Game/Blueprints/Mobs/EnemyBPs/BP_EnemyParticleDeath.BP_EnemyParticleDeath_C" (Math|Transform|MakeTransform (.location (Transformation|GetWorldTransform _skeletalmesh)) "0, 0, 0" "1.000000,1.000000,1.000000") "Undefined" "OverrideRootScale" 0 _skeletalmesh 0)
  (Utilities|FlowControl|Delay 0.05)
  (if (and (Variables|Default|GetbCanRessurect) (Utilities|Array|IsValidIndex _overlappingactors))
    (bind _asenemy_necromancer (Utilities|Casting|CastToEnemy_Necromancer (Utilities|Array|Get(acopy) _overlappingactors))
      (:then
        (Default|SpawnGhost _asenemy_necromancer (>= (Class|GSCCoreComponent|GetCurrentAttributeValue (Variables|Default|GetGSCCore) "(AttributeName=\"MaxArmor\",Attribute=/Script/RTD.EnemyAttribSet:MaxArmor,AttributeOwner=\"/Script/CoreUObject.Class'/Script/RTD.EnemyAttribSet'\")") 1.0) (Transformation|GetActorTransform) (Variables|Default|GetSpline) (Variables|Default|GetDen) (Variables|Default|GetLocationOnCurrentSpline)))
      (:CastFailed
        _)))
  (Actor|DestroyActor))

(event Custom|ArmorDamaged)

(event Custom|EnableDamage
  (Utilities|FlowControl|Gate true) ; enters at Open
)

(event Custom|EnableMovement
  (Utilities|FlowControl|Gate true) ; enters at Open
)

(event Custom|DisableDamage
  (Utilities|FlowControl|Gate true) ; enters at Close
)

(event Custom|DisableMovement
  (Utilities|FlowControl|Gate true) ; enters at Close
)

(event Custom|CalcAbilityCooldown
  (params (DeltaTime :type Float%20%28double-precision%29))
  (if (and (Variables|Default|GetbHasAbilityWithCooldown) (not (Variables|Default|GetbCastingAbility)))
    (bind _output_get (Variables|Default|SetCooldownValue (+ (Variables|Default|GetCooldownValue) (/ DeltaTime (Class|GSCCoreComponent|GetCurrentAttributeValue (Variables|Default|GetGSCCore) "(AttributeName=\"Cooldown\",Attribute=/Script/RTD.EnemyAbility:Cooldown,AttributeOwner=\"/Script/CoreUObject.Class'/Script/RTD.EnemyAbility'\")")))))
    (if (and (>= _output_get 1.0) (Variables|Default|GetbActivateAbilityOnCooldown))
      (CallFunction|ActivateAbility))))

(event Custom|Hit
  (GameplayEffects|ApplyGameplayEffectToSelf :self (Variables|Default|GetGSCAbilitySystem) :GameplayEffectClass "/Game/Blueprints/Mobs/EnemyBPs/GE_BlockRegeneration.GE_BlockRegeneration_C"))

(event EventBeginPlay
  (bind _ac_enemyspawn (Variables|Default|GetAC_EnemySpawn))
  (bind _skeletalmesh (Variables|Default|GetSkeletalMesh))
  (Variables|/Game/Blueprints/Mobs/EnemyBPs/AC_EnemySpawn.AC_EnemySpawn_C|SetTarget _ac_enemyspawn (Variables|Default|GetSkeletalMesh))
  (Variables|/Game/Blueprints/Mobs/EnemyBPs/AC_EnemySpawn.AC_EnemySpawn_C|SetTargetScale _ac_enemyspawn (Variables|/Script/Engine.SceneComponent|GetRelativeScale3D (Variables|Default|GetSkeletalMesh)))
  (Default|StartScaling _ac_enemyspawn)
  (CallFunction|UpdateUI)
  (Components|Animation|SetPosition (Variables|Default|GetSkeletalMesh) (Math|Random|RandomFloat) false)
  (CallFunction|CustomEffects)
  (for _array_element (Variables|Default|GetBegginingEffects)
    (GameplayEffects|ApplyGameplayEffectToSelf :self (Variables|Default|GetGSCAbilitySystem) :GameplayEffectClass _array_element)
    (if (== _array_element "/Game/Blueprints/Mobs/EnemyModifiers/GE_Heavy.GE_Heavy_C")
      (Transformation|SetWorldScale3D _skeletalmesh (* (Transformation|GetWorldScale _skeletalmesh) 1.5))))
  (CallFunction|ApplyScaling)
  (bind _ashealth_widget (Utilities|Casting|CastToHealthWidget (UserInterface|GetWidget (Variables|Default|GetWidget)))
    (:then
      (Default|Innit _ashealth_widget (Variables|Default|GetGSCCore) (Variables|Default|GetHealthType)))
    (:CastFailed
      _))
  (Actor|Tick|SetActorTickEnabled true)
  (CallFunction|EnableMovement)
  (CallFunction|EnableDamage)
  (Variables|Default|SetTargetable true)
  (Utilities|FlowControl|Delay 0.5)
  (Variables|Default|SetbSpawning false))

(event EventApplyEffect
  (params (Source :type GSC%20Ability%20System%20Component%20Object%20Reference) (Effect :type Gameplay%20Effect%20Class%20Reference) (Power :type Float%20%28double-precision%29))
  (GameplayEffects|ApplyGameplayEffectToTarget :self Source :GameplayEffectClass Effect :Target (Variables|Default|GetGSCAbilitySystem) :Level Power))

(event EventTick
  (params (DeltaSeconds :type Float%20%28single-precision%29))
  (Utilities|FlowControl|Gate true
    (:Exit
      (bind _output_get (Variables|Default|SetOverlayVisibility (- (Variables|Default|GetOverlayVisibility) (* DeltaSeconds 0.1))))
      (Rendering|Material|SetScalarParameterValue (Variables|Default|GetOverlayMaterial) "Opacity" _output_get :!class /Script/Engine.MaterialInstanceDynamic)
      (CallFunction|CalcAbilityCooldown DeltaSeconds)
      (if (GameplayTags|HasAnyMatchingGameplayTags (Variables|Default|GetGSCAbilitySystem) (Utilities|Struct|MakeGameplayTagContainer (Utilities|Array|MakeArray "(TagName=\"Effect.Entangled\")")))
        (Default|DoEntangleDamage (Variables|Default|GetAC_DamageOverTime) DeltaSeconds))
      (Variables|Default|GetSpline
        (:then
          (if (not (Game|IsActorBeingDestroyed))
            (CallFunction|Move DeltaSeconds)))
        (:else
          (Actor|DestroyActor))))))

(event EventHover
  (bind _ashealth_widget (Utilities|Casting|CastToHealthWidget (UserInterface|GetWidget (Variables|Default|GetWidget))))
  (Default|Hovered _ashealth_widget))

(event EventRemoveEffect
  (params (Source :type GSC%20Ability%20System%20Component%20Object%20Reference) (Effect :type Gameplay%20Effect%20Class%20Reference))
  (GameplayEffects|RemoveActiveGameplayEffectbySourceEffect (Variables|Default|GetGSCAbilitySystem) Effect Source -1))

(event EventApplySpec
  (params (Source :type GSC%20Ability%20System%20Component%20Object%20Reference) (Spec :type Gameplay%20Effect%20Spec%20Handle%20Structure))
  (GameplayEffects|ApplyGameplayEffectSpecToSelf (Variables|Default|GetGSCAbilitySystem) Spec))

(event Game|Damage|EventAnyDamage
  (params (Damage :type Float%20%28single-precision%29) (DamageType :type Damage%20Type%20Object%20Reference) (InstigatedBy :type Controller%20Object%20Reference) (DamageCauser :type Actor%20Object%20Reference))
  (Utilities|FlowControl|Gate true
    (:Exit
      (CallFunction|Hit)
      (if (< (Class|GSCCoreComponent|GetCurrentAttributeValue (Variables|Default|GetGSCCore) "(AttributeName=\"Armor\",Attribute=/Script/RTD.EnemyAttribSet:Armor,AttributeOwner=\"/Script/CoreUObject.Class'/Script/RTD.EnemyAttribSet'\")") 1.0)
        (if (< (Class|GSCCoreComponent|GetCurrentAttributeValue (Variables|Default|GetGSCCore) "(AttributeName=\"Shield\",Attribute=/Script/RTD.EnemyAttribSet:Shield,AttributeOwner=\"/Script/CoreUObject.Class'/Script/RTD.EnemyAttribSet'\")") 1.0)
          (Variables|Default|SetMostRecentDamageCauser DamageCauser)
          (bind _damagedone (Class|DamageInterface|CalculateDamage(Message) DamageType (Variables|Default|GetHealthType) Damage))
          (bind _returnvalue (Ability|GameplayEffect|AssignTagSetbyCallerMagnitude (GameplayEffects|MakeOutgoingSpec :self (Variables|Default|GetGSCAbilitySystem) :GameplayEffectClass "/Game/Blueprints/HealthDamage/GE_HealthDamage.GE_HealthDamage_C") "(TagName=\"DamageMagnitude\")" (* (* (Class|GSCCoreComponent|GetCurrentAttributeValue (Variables|Default|GetGSCCore) "(AttributeName=\"DamTakenModifier\",Attribute=/Script/RTD.EnemyAttribSet:DamTakenModifier,AttributeOwner=\"/Script/CoreUObject.Class'/Script/RTD.EnemyAttribSet'\")") _damagedone) -1.0)))
          (GameplayEffects|ApplyGameplayEffectSpecToSelf (Variables|Default|GetGSCAbilitySystem) _returnvalue)
          (Class|BPIDamageDealer|DamagedHealth(Message) (Variables|Default|GetMostRecentDamageCauser) (* (Class|GSCCoreComponent|GetCurrentAttributeValue (Variables|Default|GetGSCCore) "(AttributeName=\"DamTakenModifier\",Attribute=/Script/RTD.EnemyAttribSet:DamTakenModifier,AttributeOwner=\"/Script/CoreUObject.Class'/Script/RTD.EnemyAttribSet'\")") _damagedone) (Class|GSCCoreComponent|HasAnyMatchingGameplayTags (Variables|Default|GetGSCCore) "(GameplayTags=((TagName=\"Effect.Spotted\")))"))
          (if (<= (Class|GSCCoreComponent|GetCurrentAttributeValue (Variables|Default|GetGSCCore) "(AttributeName=\"Health\",Attribute=/Script/RTD.EnemyAttribSet:Health,AttributeOwner=\"/Script/CoreUObject.Class'/Script/RTD.EnemyAttribSet'\")") 0.0)
            (Utilities|FlowControl|Sequence
              (:then_0
                (GameplayEffects|ApplyGameplayEffectToSelf :self (Variables|Default|GetGSCAbilitySystem) :GameplayEffectClass "/Game/Blueprints/Mobs/EnemyBPs/GE_Death.GE_Death_C")
                (CallFunction|DisableDamage)
                (CallFunction|DisableMovement)
                (Components|DestroyComponent (Variables|Default|GetWidget)))
              (:then_1
                (Variables|Default|SetWasKilled true)
                (Actor|Tick|SetActorTickEnabled false)
                (if (and (Variables|Default|GetbCanCountAsKill) (Variables|Default|GetbIsLastGeneration))
                  (Class|BPIDamageDealer|GotKill(Message) (Variables|Default|GetMostRecentDamageCauser) (Math|Float|Floor (Class|GSCCoreComponent|GetCurrentAttributeValue (Variables|Default|GetGSCCore) "(AttributeName=\"KillValue\",Attribute=/Script/RTD.EnemyAttribSet:KillValue,AttributeOwner=\"/Script/CoreUObject.Class'/Script/RTD.EnemyAttribSet'\")")) (Variables|Default|GetEnemyGroups) (Class|GSCCoreComponent|HasAnyMatchingGameplayTags (Variables|Default|GetGSCCore) "(GameplayTags=((TagName=\"Effect.Spotted\")))") (select (and (Variables|Default|GetbCanCountAsKill) (Variables|Default|GetbIsLastGeneration)) (Class|GSCCoreComponent|GetCurrentAttributeValue (Variables|Default|GetGSCCore) "(AttributeName=\"ItemDropChance\",Attribute=/Script/RTD.EnemyAttribSet:ItemDropChance,AttributeOwner=\"/Script/CoreUObject.Class'/Script/RTD.EnemyAttribSet'\")") 0.0)))
                (Default|FalltoGround (Variables|Default|GetAC_EnemySpawn))
                (Utilities|FlowControl|Delay 1.0)
                (CallFunction|Death))))
          (else
            (bind _asbp_damage (Utilities|Casting|CastToBP_Damage DamageType))
            (if (Variables|/Game/Blueprints/HealthDamage/DamageClasses/BP_Damage.BP_Damage_C|GetCanDamageShields _asbp_damage)
              (bind _output_get (Variables|Default|SetMostRecentDamageCauser DamageCauser))
              (GameplayEffects|ApplyGameplayEffectToSelf :self (Variables|Default|GetGSCAbilitySystem) :GameplayEffectClass "/Game/Blueprints/HealthDamage/GE_ShieldDamage.GE_ShieldDamage_C")
              (Class|BPIDamageDealer|DamagedShield(Message) _output_get (Transformation|GetActorLocation))
              (else
                (Class|BPIDamageDealer|ShieldBlocked(Message) DamageCauser (Transformation|GetActorLocation))
                (Rendering|Material|SetScalarParameterValue (Variables|Default|GetOverlayMaterial) "ShieldValue" 0.5 :!class /Script/Engine.MaterialInstanceDynamic)
                (Variables|Default|SetOverlayVisibility 1.0)))))
        (else
          (bind _damagedone_2 (Class|DamageInterface|CalculateDamage(Message) DamageType "NewEnumerator4" Damage))
          (if (>= _damagedone_2 (Variables|Default|GetArmorDamageThreshold))
            (bind _output_get_2 (Variables|Default|SetMostRecentDamageCauser DamageCauser))
            (GameplayEffects|ApplyGameplayEffectToSelf :self (Variables|Default|GetGSCAbilitySystem) :GameplayEffectClass "/Game/Blueprints/HealthDamage/GE_ArmorDamage.GE_ArmorDamage_C")
            (Class|BPIDamageDealer|DamagedArmor(Message) _output_get_2 (Class|GSCCoreComponent|HasAnyMatchingGameplayTags (Variables|Default|GetGSCCore) "(GameplayTags=((TagName=\"Effect.Spotted\")))") (Transformation|GetActorLocation))
            (CallFunction|ArmorDamaged)
            (else
              (Class|BPIDamageDealer|ArmorBlocked(Message) DamageCauser (Transformation|GetActorLocation))
              (Rendering|Material|SetScalarParameterValue (Variables|Default|GetOverlayMaterial) "ShieldValue" 0.0 :!class /Script/Engine.MaterialInstanceDynamic)
              (Variables|Default|SetOverlayVisibility 0.5))))))))

(fn ConstructionScript
  (bind _returnvalue (Rendering|Material|CreateDynamicMaterialInstance "/Game/Assets/Materials/Overlays/M_EnemyOverlay.M_EnemyOverlay" "None" "None" :!class /Script/Engine.KismetMaterialLibrary))
  (bind _output_get (Variables|Default|SetOverlayMaterial _returnvalue))
  (Rendering|Material|SetOverlayMaterial (Variables|Default|GetSkeletalMesh) _output_get :!class /Script/Engine.MeshComponent))

(fn Move
  (params (DeltaTime :type Float%20%28double-precision%29))
  (bind _movespeed (Utilities|GetMoveSpeed))
  (bind _returnvalue (* DeltaTime _movespeed))
  (bind _output_get (Variables|Default|SetLocationOnCurrentSpline (Math|Float|Clamp(Float) (Math|Float|SelectFloat (+ (Variables|Default|GetLocationOnCurrentSpline) _returnvalue) (- (Variables|Default|GetLocationOnCurrentSpline) _returnvalue) (Variables|Default|GetbMovesBackwards)) 0.0 (Spline|GetSplineLength (Variables|Default|GetSpline)))))
  (Transformation|SetActorLocationAndRotation (Spline|GetLocationatDistanceAlongSpline (Variables|Default|GetSpline) _output_get "World") (Math|Conversions|RotationFromXVector (Math|Vector|SelectVector (Spline|GetTangentatDistanceAlongSpline (Variables|Default|GetSpline) _output_get "World") (* (Spline|GetTangentatDistanceAlongSpline (Variables|Default|GetSpline) _output_get "World") -1.0) (Variables|Default|GetbMovesBackwards))) true)
  (if (== (Variables|Default|GetLocationOnCurrentSpline) 0.0)
    (GameplayEffects|ApplyGameplayEffectToTarget :self (Variables|Default|GetGSCAbilitySystem) :GameplayEffectClass "/Game/Blueprints/Mobs/HomeBaseModifiers/GE_HomeHealth_Damage.GE_HomeHealth_Damage_C" :Target (Variables|/Game/Blueprints/Mobs/BP_PathNode.BP_PathNode_C|GetGSCAbilitySystem (Variables|Default|GetNextNode)))
    (Actor|DestroyActor)
    (elif (and (== (Variables|Default|GetLocationOnCurrentSpline) (Spline|GetSplineLength (Variables|Default|GetSpline))) (Variables|Default|GetbMovesBackwards))
      (CallFunction|ReachedDen))))

(fn CustomEffects)

(fn ApplyScaling
  (bind _returnvalue (Ability|GameplayEffect|AssignTagSetbyCallerMagnitude (GameplayEffects|MakeOutgoingSpec :self (Variables|Default|GetGSCAbilitySystem) :GameplayEffectClass "/Game/Blueprints/Mobs/EnemyModifiers/GE_DifficultyScaling.GE_DifficultyScaling_C") "(TagName=\"EffectMagnitude\")" (Variables|Default|GetScaling)))
  (GameplayEffects|ApplyGameplayEffectSpecToSelf (Variables|Default|GetGSCAbilitySystem) _returnvalue))

(fn UpdateUI
  (if (not (Game|IsActorBeingDestroyed))
    (bind _ashealth_widget (Utilities|Casting|CastToHealthWidget (UserInterface|GetWidget (Variables|Default|GetWidget))))
    (Default|UpdateValue _ashealth_widget (Variables|Default|GetGSCCore))))

(fn IsVisible
  (return (Math|Conversions|ToBoolean(Integer) (Math|Float|Truncate (Class|GSCCoreComponent|GetCurrentAttributeValue (Variables|Default|GetGSCCore) "(AttributeName=\"Visible\",Attribute=/Script/RTD.EnemyAttribSet:Visible,AttributeOwner=\"/Script/CoreUObject.Class'/Script/RTD.EnemyAttribSet'\")")))))

(fn ReportStatforTargeting
  (params (Mode :type ETargetMode%20Enum :default "NewEnumerator0"))
  (bind _gsccore (Variables|Default|GetGSCCore))
  (return (Utilities|Select :Index Mode :NewEnumerator0 (* (Variables|Default|GetLocationOnCurrentSpline) -1.0) :NewEnumerator1 (Class|GSCCoreComponent|GetCurrentAttributeValue _gsccore "(AttributeName=\"Health\",Attribute=/Script/RTD.EnemyAttribSet:Health,AttributeOwner=\"/Script/CoreUObject.Class'/Script/RTD.EnemyAttribSet'\")") :NewEnumerator3 (Utilities|GetMoveSpeed) :NewEnumerator2 (Math|Random|RandomFloat) :NewEnumerator4 (Class|GSCCoreComponent|GetCurrentAttributeValue _gsccore "(AttributeName=\"Shield\",Attribute=/Script/RTD.EnemyAttribSet:Shield,AttributeOwner=\"/Script/CoreUObject.Class'/Script/RTD.EnemyAttribSet'\")") :NewEnumerator5 (Class|GSCCoreComponent|GetCurrentAttributeValue _gsccore "(AttributeName=\"Armor\",Attribute=/Script/RTD.EnemyAttribSet:Armor,AttributeOwner=\"/Script/CoreUObject.Class'/Script/RTD.EnemyAttribSet'\")")) (Variables|Default|GetOverrideTargeting)))

(fn ReportTargetPoint
  (return (Transformation|GetWorldLocation (Variables|Default|GetDamageCapsule))))