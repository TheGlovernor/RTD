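; BP_Mush_King_Red is a mushroom enemy whose ability disables towers.
; ActivateAbility resets its cooldown, flags casting, then fires a Niagara effect after a short wind-up.
; A debug-drawn multi-sphere trace, centered DisableSize behind the actor with that same radius, sends GE_DisableTower to every hit actor via ApplyEffectMessage.
; The casting flag clears after a second delay; an older tower-cast path is left disconnected.
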(event EventActivateAbility
  (bind _returnvalue (Transformation|GetActorForwardVector))
  (bind _returnvalue_2 (Transformation|GetActorLocation))
  (bind _disablesize (Variables|Default|GetDisableSize))
  (bind _returnvalue_3 (* _returnvalue -1.0 _disablesize))
  (bind _returnvalue_4 (+ _returnvalue_2 _returnvalue_3))
  (Variables|Default|SetCooldownValue 0.0)
  (Variables|Default|SetbCastingAbility true)
  (Utilities|FlowControl|Delay 0.8)
  (Components|Activation|Activate (Variables|Default|GetNS) false)
  (bind _outhits (Collision|MultiSphereTraceByChannel _returnvalue_4 _returnvalue_4 _disablesize "TraceTypeQuery1" false 0 "ForDuration"))
  (for _array_element _outhits
    (Class|GASInterface|ApplyEffect(Message) (.hitactor _array_element) (Variables|Default|GetGSCAbilitySystem) "/Game/Blueprints/Mobs/EnemyBPs/Mush/GE_DisableTower.GE_DisableTower_C" 0.0))
  (Utilities|FlowControl|Delay 0.8)
  (Variables|Default|SetbCastingAbility false))

(fn ConstructionScript
  (|CallParentFunction))