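; PathingSpline is a mob-related Blueprint that builds a spline at runtime, presumably as a movement path, though nothing here moves along it.
; On BeginPlay it appends four hard-coded world-space points at a shared height to its SplineComponent without clearing existing points.
; The points ignore the actor's placement, and the construction script, overlap and tick events are empty.
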(event EventBeginPlay
  (Spline|AddSplinePoint (Variables|Default|GetSplineComponent) (Math|Vector|MakeVector 0.0 0.0 75.0) "World" true)
  (Spline|AddSplinePoint (Variables|Default|GetSplineComponent) (Math|Vector|MakeVector 5e+01 0.0 75.0) "World" true)
  (Spline|AddSplinePoint (Variables|Default|GetSplineComponent) (Math|Vector|MakeVector 75.0 25.0 75.0) "World" true)
  (Spline|AddSplinePoint (Variables|Default|GetSplineComponent) (Math|Vector|MakeVector 75.0 -25.0 75.0) "World" true))

(event Collision|EventActorBeginOverlap
  (params (OtherActor :type Actor%20Object%20Reference)))

(event EventTick
  (params (DeltaSeconds :type Float%20%28single-precision%29)))

(fn ConstructionScript)