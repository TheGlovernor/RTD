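; Mob path node that draws its link to the next node, tracks distance to base and picks random enemy spawn effects.
; BeginPlay starts spawn scaling, maps path coordinates onto BP_TerrainGen ground as spline points, and lays spline meshes, matching the last tangent to NextNode's spline.
; Distance accumulates from NextNode's distance plus spline length.
; ChooseOnSpawnEffects rolls Quick, Heavy, Bounty and Shielded effects against GameDirector attributes, with chance-based repeat rolls that can stack.
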(event Custom|AddPoints
  (params (ToAdd :type Float%20%28double-precision%29))
  (Variables|Default|SetPoints (+ ToAdd (Variables|Default|GetPoints))))

(event EventBeginPlay
  (Default|StartScaling (Variables|Default|GetAC_EnemySpawn))
  (Utilities|Array|Insert (Variables|Default|GetPath) (Variables|Default|GetMyCoords))
  (bind _nextnode (Variables|Default|GetNextNode)
    (:then
      (Utilities|Array|Add (Variables|Default|GetPath) (Variables|BP_PathNode_C|GetMyCoords _nextnode)))
    (:else
      _))
  (Utilities|FlowControl|Sequence
    (:then_0
      (Variables|Default|GetCurrentSplineComponent
        (:then)
        (:else
          (bind _returnvalue (AddComponent|AddSplineComponent false (Math|Transform|MakeTransform "0, 0, 0")))
          (Variables|Default|SetCurrentSplineComponent _returnvalue))))
    (:then_1
      (Spline|ClearSplinePoints (Variables|Default|GetCurrentSplineComponent) true))
    (:then_2
      (bind _returnvalue_2 (Actor|GetActorOfClass "/Game/Blueprints/Map/BP_TerrainGen.BP_TerrainGen_C"))
      (for _array_element (Variables|Default|GetPath)
        (bind _transform (Default|FGetGroundTransform _returnvalue_2 _array_element))
        (Spline|AddSplinePoint (Variables|Default|GetCurrentSplineComponent) (.location _transform) "World" true)))
    (:then_3
      (for _index (range 0 (- (Spline|GetNumberOfSplinePoints (Variables|Default|GetCurrentSplineComponent)) 2))
        (if (!= _index (- (Spline|GetNumberOfSplinePoints (Variables|Default|GetCurrentSplineComponent)) 2))
          (bind _returnvalue_3 (AddComponent|AddSplineMeshComponent false (Math|Transform|MakeTransform "0, 0, 0")))
          (SplineMesh|SetStartandEnd _returnvalue_3 (+ (.Location (Spline|GetLocationandTangentatSplinePoint (Variables|Default|GetCurrentSplineComponent) _index "Local")) "0,0,20.000000") (.Tangent (Spline|GetLocationandTangentatSplinePoint (Variables|Default|GetCurrentSplineComponent) _index "Local")) (+ (.Location (Spline|GetLocationandTangentatSplinePoint (Variables|Default|GetCurrentSplineComponent) (+ _index 1) "Local")) "0,0,20.000000") (.Tangent (Spline|GetLocationandTangentatSplinePoint (Variables|Default|GetCurrentSplineComponent) (+ _index 1) "Local")) true :!class /Script/Engine.SplineMeshComponent)
          (Utilities|Array|Add (Variables|Default|GetSplineMeshComponents) _returnvalue_3)
          (else
            (bind _returnvalue_4 (AddComponent|AddSplineMeshComponent false (Math|Transform|MakeTransform "0, 0,20.000000")))
            (SplineMesh|SetStartandEnd _returnvalue_4 (+ (.Location (Spline|GetLocationandTangentatSplinePoint (Variables|Default|GetCurrentSplineComponent) _index "Local")) "") (.Tangent (Spline|GetLocationandTangentatSplinePoint (Variables|Default|GetCurrentSplineComponent) _index "Local")) (+ (.Location (Spline|GetLocationandTangentatSplinePoint (Variables|Default|GetCurrentSplineComponent) (+ _index 1) "Local")) "") (.Tangent (Spline|GetLocationandTangentatSplinePoint (Variables|BP_PathNode_C|GetCurrentSplineComponent (Variables|Default|GetNextNode)) 0 "Local")) true :!class /Script/Engine.SplineMeshComponent)
            (Utilities|Array|Add (Variables|Default|GetSplineMeshComponents) _returnvalue_4)))))
    (:then_4
      (bind _nextnode_2 (Variables|Default|GetNextNode)
        (:then
          (Variables|Default|SetDistanceToBase (+ (Variables|BP_PathNode_C|GetDistanceToBase _nextnode_2) (Spline|GetSplineLength (Variables|Default|GetCurrentSplineComponent)))))
        (:else)))))

(fn ConstructionScript)

(fn ChooseonSpawnEffects
  (bind _gamedirector (Variables|Default|GetGameDirector)
    (:then
      _)
    (:else
      (bind _outactors (Actor|GetAllActorsOfClass "/Game/Blueprints/Mobs/BP_GameDirector.BP_GameDirector_C" :!label _label))
      (Utilities|IsValid (Utilities|Array|Get(acopy) _outactors)
        (:Is%20Valid
          (Variables|Default|SetGameDirector (Utilities|Array|Get(acopy) _outactors)))
        (:Is%20Not%20Valid
          (Development|PrintString "UH OH")
          (goto _label)))))
  (LocalVariables|SetMultipleRerollChance (Class|GSCCoreComponent|GetCurrentAttributeValue (Variables|/Game/Blueprints/Mobs/BP_GameDirector.BP_GameDirector_C|GetGSCCore _gamedirector) "(AttributeName=\"MultipleRollChance\",Attribute=/Script/RTD.GameDirector:MultipleRollChance,AttributeOwner=\"/Script/CoreUObject.Class'/Script/RTD.GameDirector'\")"))
  (Utilities|FlowControl|Sequence :!label _label_2
    (:then_0
      (if (> (Class|GSCCoreComponent|GetCurrentAttributeValue (Variables|/Game/Blueprints/Mobs/BP_GameDirector.BP_GameDirector_C|GetGSCCore (Variables|Default|GetGameDirector)) "(AttributeName=\"Quick\",Attribute=/Script/RTD.GameDirector:Quick,AttributeOwner=\"/Script/CoreUObject.Class'/Script/RTD.GameDirector'\")") (Math|Random|RandomFloat))
        (Utilities|Array|Add (LocalVariables|GetEffects) "/Game/Blueprints/Mobs/EnemyModifiers/GE_Quick.GE_Quick_C")))
    (:then_1
      (if (> (Class|GSCCoreComponent|GetCurrentAttributeValue (Variables|/Game/Blueprints/Mobs/BP_GameDirector.BP_GameDirector_C|GetGSCCore (Variables|Default|GetGameDirector)) "(AttributeName=\"Heavy\",Attribute=/Script/RTD.GameDirector:Heavy,AttributeOwner=\"/Script/CoreUObject.Class'/Script/RTD.GameDirector'\")") (Math|Random|RandomFloat))
        (Utilities|Array|Add (LocalVariables|GetEffects) "/Game/Blueprints/Mobs/EnemyModifiers/GE_Heavy.GE_Heavy_C")))
    (:then_2
      (if (> (Class|GSCCoreComponent|GetCurrentAttributeValue (Variables|/Game/Blueprints/Mobs/BP_GameDirector.BP_GameDirector_C|GetGSCCore (Variables|Default|GetGameDirector)) "(AttributeName=\"Bounty\",Attribute=/Script/RTD.GameDirector:Bounty,AttributeOwner=\"/Script/CoreUObject.Class'/Script/RTD.GameDirector'\")") (Math|Random|RandomFloat))
        (Utilities|Array|Add (LocalVariables|GetEffects) "/Game/Blueprints/Mobs/EnemyModifiers/IE_Bounty_Multiply.IE_Bounty_Multiply_C")))
    (:then_3
      (if (> (Class|GSCCoreComponent|GetCurrentAttributeValue (Variables|/Game/Blueprints/Mobs/BP_GameDirector.BP_GameDirector_C|GetGSCCore (Variables|Default|GetGameDirector)) "(AttributeName=\"Shielded\",Attribute=/Script/RTD.GameDirector:Shielded,AttributeOwner=\"/Script/CoreUObject.Class'/Script/RTD.GameDirector'\")") (Math|Random|RandomFloat))
        (Utilities|Array|Add (LocalVariables|GetEffects) "/Game/Blueprints/Mobs/EnemyModifiers/GE_Shielded.GE_Shielded_C")))
    (:then_4
      (if (> (LocalVariables|GetMultipleRerollChance) (Math|Random|RandomFloat))
        (Math|Float|DecrementFloat (LocalVariables|GetMultipleRerollChance)
          (:%20%20
            (goto _label_2)))
        (else
          (return (LocalVariables|GetEffects)))))))