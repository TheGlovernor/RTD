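; Wave manager for mobs that tracks the current wave number and holds a terrain grid reference.
; CalculateWave passes each of the grid's path heads to WaveSpawner with a map of one mob type and a fixed count.
; WaveSpawner derives a wave time from the largest count divided by the wave number, but spawns nothing yet.
; StartNextWave only increments the counter, without triggering the calculation.
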(event Custom|StartNextWave
  (Math|Integer|IncrementInt (Variables|Default|GetCurrentWave)))

(fn CalculateWave
  (bind _newparam (Default|GetPathHeads (Variables|Default|GetTerrain%20Grid)))
  (bind _result (Utilities|Set|ToArray _newparam))
  (for _array_element _result
    (bind _asmob_base (Utilities|Casting|CastToMob_Base (Variables|Default|GetMob)))
    (bind _output_get (Variables|Default|SetMob _asmob_base))
    (CallFunction|WaveSpawner _array_element (Utilities|Map|MakeMap _output_get (Class|KismetSystemLibrary|MakeLiteralInteger 10)))))

(fn InitWaveHandler
  (params (terrain%20Grid :type Terrain%20Grid%20Object%20Reference%20%28by%20ref%29))
  (Variables|Default|SetTerrain%20Grid terrain%20Grid))

(fn CalculateWaveTime
  (params (MostMobs :type Integer))
  (return (/ MostMobs (Variables|Default|GetCurrentWave))))

(fn WaveSpawner
  (params (Coords :type Offset%20Coords%20Structure%20%28by%20ref%29) (NewParam :type Map%20of%20Mob%20Base%20Object%20References%20to%20Integers))
  (Utilities|Map|Keys NewParam)
  (bind _values (Utilities|Map|Values NewParam))
  (bind _wavetime (CallFunction|CalculateWaveTime (.MaxValue (Math|Integer|MaxOfIntArray _values)))))