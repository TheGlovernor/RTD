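; Game director for the tower defense mode that paces enemy waves and den growth.
; StartSpawning starts a looping timer that makes every TerrainGen den spawn enemies, and opens a Tick gate that adds dens at an attribute-driven rate.
; GSCCore attribute changes are pushed to enemy-effect widgets, and GetScalingValue derives a multiplier from game time.
; Stop halts enemy waves but leaves den growth running; MacroHexHandler logic is unconnected.
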(event OnPreAttributeChange(GSCCore)
  (params (AttributeSet :type GSC%20Attribute%20Set%20Base%20Object%20Reference) (Attribute :type Gameplay%20Attribute%20Structure) (NewValue :type Float%20%28single-precision%29))
  (bind _foundwidgets (Widget|GetAllWidgetsOfClass "/Game/UI/CAW_EnemyEffectsHolder.CAW_EnemyEffectsHolder_C" false))
  (for _array_element _foundwidgets
    (Default|UpdateInfo _array_element Attribute NewValue)))

(event Custom|SpawnEnemies
  (Utilities|FlowControl|Gate false
    (:Exit
      (Variables|Default|GetTerrainGen
        (:then
          _)
        (:else
          (bind _returnvalue (Actor|GetActorOfClass "/Game/Blueprints/Map/BP_TerrainGen.BP_TerrainGen_C"))
          (Variables|Default|SetTerrainGen _returnvalue)))
      (for _array_element (Variables|/Game/Blueprints/Map/BP_TerrainGen.BP_TerrainGen_C|GetDenActors (Variables|Default|GetTerrainGen))
        (Default|SpawnEnemies _array_element)))))

(event Custom|Stop
  (Utilities|FlowControl|Sequence
    (:then_0
      (Utilities|FlowControl|Gate false) ; enters at Close
    )
    (:then_1
      (Utilities|Time|ClearandInvalidateTimerbyHandle (Variables|Default|GetSpawnerTimer)))))

(event Custom|StartSpawning
  (bind _returnvalue (Utilities|Time|SetTimerbyEvent (delegate Custom|SpawnEnemies) 5.0 true))
  (Variables|Default|SetSpawnerTimer _returnvalue)
  (Utilities|FlowControl|Gate true) ; enters at Open
)

(event EventTick
  (params (DeltaSeconds :type Float%20%28single-precision%29))
  (Utilities|FlowControl|Gate true
    (:Exit
      (bind _output_get (Variables|Default|SetNewDenProgress (+ (Variables|Default|GetNewDenProgress) (/ DeltaSeconds (Class|GSCCoreComponent|GetCurrentAttributeValue (Variables|Default|GetGSCCore) "(AttributeName=\"NewDenTime\",Attribute=/Script/RTD.GameDirector:NewDenTime,AttributeOwner=Class'\"/Script/RTD.GameDirector\"')")))))
      (if (> _output_get 1.0)
        (Utilities|FlowControl|DoOnce false :!label _label
          (:Completed
            (Default|SpawnNewDen (Variables|Default|GetTerrainGen))
            (Variables|Default|SetNewDenProgress 0.0)
            (goto _label Reset)))))))

(fn ConstructionScript)

(fn GetScalingValue
  (bind _asbp_gs_tower_defense (Utilities|Casting|CastToBP_GS_TowerDefense (Game|GetGameState))
    (:then
      (return (+ (/ (Class|KismetSystemLibrary|GetTimerElapsedTimeHandle (Variables|/Game/Blueprints/GM/BP_GS_TowerDefense.BP_GS_TowerDefense_C|GetTime _asbp_gs_tower_defense)) 6e+01) 1.0)))
    (:CastFailed
      (return 1.0))))