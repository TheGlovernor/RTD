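; Health component for mobs that calculates how damage depletes health stored as a map of separate pools.
; CalculateDamage walks the pools in map order, skipping near-empty ones and scaling damage by each key's Effectiveness multiplier.
; A pool that outlasts the hit stops the loop; otherwise it drops to zero and the scaled excess carries into the next.
; It returns the updated map; the event graph is empty.
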(event EventBeginPlay)

(event EventTick
  (params (DeltaSeconds :type Float%20%28single-precision%29)))

(fn CalculateDamage
  (params (Damage :type Float%20%28double-precision%29) (Effectiveness :type Map%20of%20EHealthTypes%20Enums%20to%20Reals :default "NewEnumerator0") (HealthIn :type Map%20of%20EHealthTypes%20Enums%20to%20Reals :default "NewEnumerator0"))
  (Variables|Default|SetDamageRemaining Damage)
  (Variables|Default|SetEffectiveness Effectiveness)
  (bind _output_get (Variables|Default|SetHealthReturn HealthIn))
  (bind _values (Utilities|Map|Values _output_get))
  (bind (_array_element _array_index) (Utilities|Array|ForEachLoopwithBreak _values :!label _label)
    (:LoopBody
      (if (not (Math|Float|NearlyEqual(Float) _array_element 0.0 0.1))
        (bind _keys (Utilities|Map|Keys (Variables|Default|GetHealthReturn)))
        (if (> _array_element (* (Variables|Default|GetDamageRemaining) (.Value (Utilities|Map|Find (Variables|Default|GetEffectiveness) (Utilities|Array|Get(acopy) _keys _array_index)))))
          (Utilities|Map|Add (Variables|Default|GetHealthReturn) (Utilities|Array|Get(acopy) _keys _array_index) (- _array_element (* (Variables|Default|GetDamageRemaining) (.Value (Utilities|Map|Find (Variables|Default|GetEffectiveness) (Utilities|Array|Get(acopy) _keys _array_index))))))
          (goto _label Break)
          (else
            (Variables|Default|SetDamageRemaining (- (* (Variables|Default|GetDamageRemaining) (.Value (Utilities|Map|Find (Variables|Default|GetEffectiveness) (Utilities|Array|Get(acopy) _keys _array_index)))) _array_element))
            (Utilities|Map|Add (Variables|Default|GetHealthReturn) (Utilities|Array|Get(acopy) _keys _array_index) 0.0)))))
    (:Completed
      (return (Variables|Default|GetHealthReturn)))))