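; Demo enemy that wanders a tile grid, repeatedly A* pathfinding to random clean tiles.
; The grid computes, visualises and builds a spline from each path, which a timeline follows at a play rate scaled by spline length for steady speed.
; MoveUsingNav switches to per-tile AI MoveTo, where Tick advances points by 2D proximity to avoid stutter; otherwise Tick records per-frame movement distance.
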(event Custom|NewPath
  (bind _grid (Variables|Default|GetGrid))
  (bind _grid_2 (Variables|Default|GetGrid))
  (bind _cleantiles (Variables|/HexGrids/HexGrids/Blueprints/ExampleContent/HexGrid_Demo_BaseFile.HexGrid_Demo_BaseFile_C|GetCleanTiles _grid))
  ;[0 0 0] This blueprint shows how to use A* Pathfinding to drive a character
  ; There are 3 solutions presented here.
  ;
  ; AI Movement using Nav Mesh and traditional AI Move To functions. Change MoveUsingNav to true to use this.
  ; VInterp System
  ; Spline Based Movement - We are currently using this for the demo.
  ;;[1 1 1] Choose a new path
  (Variables|Default|SetCurrentPathGoal (Utilities|Array|Get(acopy) _cleantiles (Math|Random|RandomIntegerinRange 0 (Utilities|Array|LastIndex _cleantiles))))
  (bind _results (Default|Pathfinder (Variables|Default|GetGrid) (Variables|Default|GetLastLocation) (Variables|Default|GetCurrentPathGoal))) ; We compressed pathfinding into a simple function for ease of use
  (Default|VisualiseGrid _grid_2 _results) ; Call the debug select method in grid so we can see the path\nPlug in to get the tiles to light up
  (bind _returnvalue (Class|GridsHex|AStartoWorldCoordinates _results (Math|Conversions|ToVector2D(Vector) (Variables|/HexGrids/HexGrids/Blueprints/ExampleContent/HexGrid_Demo_BaseFile.HexGrid_Demo_BaseFile_C|GetGridScaleCalculated _grid_2)) (Variables|Default|GetGrid))) ; This function scale and offsets the grid, then\nperforms a TransformLocation to conver to world space
  (bind _output_get (Variables|Default|SetWorldPositions _returnvalue))
  (Default|GenerateSplinePath _grid_2 _output_get)
  (if (Variables|Default|GetMoveUsingNav)
    (CallFunction|NextPathPoint) ; Move Using AI Moves and NavMeshes
    (else
      (CallFunction|MoveAIAlongSpline))))

(event Custom|MoveAIAlongSpline
  (bind _grid (Variables|Default|GetGrid))
  (bind _splinecomponent (Variables|/HexGrids/HexGrids/Blueprints/ExampleContent/HexGrid_Demo_BaseFile.HexGrid_Demo_BaseFile_C|GetSplineComponent _grid))
  ;[0 0 0] This blueprint shows how to use A* Pathfinding to drive a character
  ; There are 3 solutions presented here.
  ;
  ; AI Movement using Nav Mesh and traditional AI Move To functions. Change MoveUsingNav to true to use this.
  ; VInterp System
  ; Spline Based Movement - We are currently using this for the demo.
  ;;[1 1 1] For this demo, we are using the spline based movement, new as of the 4.20 update. Simplier to use and control, and does not require any nav mesh
  (Utilities|IsValid (Variables|/HexGrids/HexGrids/Blueprints/ExampleContent/HexGrid_Demo_BaseFile.HexGrid_Demo_BaseFile_C|GetSplineComponent (Variables|Default|GetGrid))
    (:Is%20Valid
      (Components|Timeline|SetPlayRate (Variables|Default|GetMoveAlongSpline) (Math|Float|Clamp(Float) (CallFunction|CalculatePlayRateonSplineLength) 0.1 1e+01))
      (bind _newtrack_0 (Timeline|MoveAlongSpline PlayFromStart) ; Must be a 0-1 output
        (:Update
          (Transformation|SetActorTransform (Math|Transform|MakeTransform (Math|Vector|MakeVector (.X (Math|Vector|BreakVector (Spline|GetLocationatDistanceAlongSpline _splinecomponent (* _newtrack_0 (Spline|GetSplineLength _splinecomponent)) "World"))) (.Y (Math|Vector|BreakVector (Spline|GetLocationatDistanceAlongSpline _splinecomponent (* _newtrack_0 (Spline|GetSplineLength _splinecomponent)) "World"))) (.z (Transformation|GetActorLocation))) (Spline|GetRotationatDistanceAlongSpline _splinecomponent (* _newtrack_0 (Spline|GetSplineLength _splinecomponent)) "World"))))
        (:Finished
          (Utilities|FlowControl|Delay 1.0)
          (Variables|Default|SetLastLocation (Variables|Default|GetCurrentPathGoal))
          (CallFunction|NewPath))))))

(event Custom|NextPathPoint
  ;[0 0 0] This blueprint shows how to use A* Pathfinding to drive a character
  ; There are 3 solutions presented here.
  ;
  ; AI Movement using Nav Mesh and traditional AI Move To functions. Change MoveUsingNav to true to use this.
  ; VInterp System
  ; Spline Based Movement - We are currently using this for the demo.
  ;;[1 1 1] When called, performs AI-MoveTo using a path point, This position is moving just a single tile per call
  (AI|AIMoveTo self (Utilities|Array|Get(acopy) (Variables|Default|GetWorldPositions) (Variables|Default|GetCurrentPathIndex)) 0 5.0 false))

(event EventBeginPlay
  ;[0 0 0] This blueprint shows how to use A* Pathfinding to drive a character
  ; There are 3 solutions presented here.
  ;
  ; AI Movement using Nav Mesh and traditional AI Move To functions. Change MoveUsingNav to true to use this.
  ; VInterp System
  ; Spline Based Movement - We are currently using this for the demo.
  ;;[1 1 1] Begin Play / Init
  (Utilities|FlowControl|Delay 0.2)
  (Variables|Default|SetLastLocation (Utilities|Struct|MakeOffsetCoords 0 5))
  (CallFunction|NewPath))

(event EventTick
  (params (DeltaSeconds :type Float%20%28single-precision%29))
  ;[0 0 0] This blueprint shows how to use A* Pathfinding to drive a character
  ; There are 3 solutions presented here.
  ;
  ; AI Movement using Nav Mesh and traditional AI Move To functions. Change MoveUsingNav to true to use this.
  ; VInterp System
  ; Spline Based Movement - We are currently using this for the demo.
  ;;[1 1 1] On Tick, we check if we have nearly reached our destination, and if so, move to the next point, unless we have reached the final point, in which case, wait 2 seconds, then choose a new destination
  ;; Alternatively, You can use the "OnSuccess" Pin from the MoveTo, but this causes a small stutter as the character comes to a halt on each point.
  (if (Variables|Default|GetMoveUsingNav) ; Tick is only required for AI Move to version, and only if you dont wish to use the OnSuccess. See the reroute from OnSuccess for notes on this
    (if (Math|Vector|Equal(Vector) (Math|Conversions|ToVector2D(Vector) (Transformation|GetActorLocation)) (Math|Conversions|ToVector2D(Vector) (Utilities|Array|Get(acopy) (Variables|Default|GetWorldPositions) (Variables|Default|GetCurrentPathIndex))) 5.0)
      (if (== (Variables|Default|GetCurrentPathIndex) (Utilities|Array|LastIndex (Variables|Default|GetWorldPositions))) ; Are we at last point in array (end of path)
        (Variables|Default|SetCurrentPathIndex 0)
        (Utilities|FlowControl|Delay 2.0)
        (Variables|Default|SetLastLocation (Variables|Default|GetCurrentPathGoal))
        (CallFunction|NewPath)
        (else
          (Math|Integer|IncrementInt (Variables|Default|GetCurrentPathIndex)
            (:%20%20
              (CallFunction|NextPathPoint)
              (Default|DestroyNextSplinePoint (Variables|Default|GetGrid)) ; You could change how this function works to be 1 behind if you liked, so the visuals are a bit different.
            )))))
    (else
      (CallFunction|CalculateDelta))))

(fn ConstructionScript)

(fn CalculatePlayRateonSplineLength
  (return (/ (Variables|Default|GetSplineWalkStandardSpeed%28CM/S%29) (Spline|GetSplineLength (Variables|/HexGrids/HexGrids/Blueprints/ExampleContent/HexGrid_Demo_BaseFile.HexGrid_Demo_BaseFile_C|GetSplineComponent (Variables|Default|GetGrid))))))

(fn CalculateDelta
  (Variables|Default|SetDelta (Math|Vector|VectorLength (- (Variables|Default|GetLocationLastFrame) (Transformation|GetActorLocation))))
  (Variables|Default|SetLocationLastFrame (Transformation|GetActorLocation)))