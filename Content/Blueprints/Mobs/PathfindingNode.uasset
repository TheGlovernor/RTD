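; PathfindingNode is a hex-map node, owned by a MacroHexHandler, that builds a spline mesh along its path at BeginPlay.
; It prepends its own coordinates to Path, then places spline points slightly above each hex's surface location from the handler.
; A spline mesh component is added and stored for each segment between consecutive points.
; The NextNode validity check does nothing on either branch.
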(event EventBeginPlay
  (bind _asmacro_hex_handler (Utilities|Casting|CastToMacroHexHandler (Components|GetOwner)))
  (Variables|Default|SetMacroHexHandler _asmacro_hex_handler)
  (Utilities|Array|Insert (Variables|Default|GetPath) (Variables|Default|GetMyCoords))
  (Variables|Default|GetNextNode
    (:then
      _)
    (:else
      _))
  (Utilities|FlowControl|Sequence
    (:then_0
      (Variables|Default|GetCurrentSplineComponent
        (:then)
        (:else
          (bind _returnvalue (AddComponent|AddSplineComponent false (Math|Transform|MakeTransform "0, 0, 0")))
          (Variables|Default|SetCurrentSplineComponent _returnvalue))))
    (:then_1
      (Spline|ClearSplinePoints (Variables|Default|GetCurrentSplineComponent) true))
    (:then_2
      (for _array_element (Variables|Default|GetPath)
        (bind _location (Default|SurfaceLocation (Variables|Default|GetMacroHexHandler) _array_element))
        (Spline|AddSplinePoint (Variables|Default|GetCurrentSplineComponent) (+ _location (Math|Vector|MakeVector 0.0 0.0 25.0)) "World" true)))
    (:then_3
      (for _index (range 0 (- (Spline|GetNumberOfSplinePoints (Variables|Default|GetCurrentSplineComponent)) 2))
        (bind _returnvalue_2 (AddComponent|AddSplineMeshComponent false (Math|Transform|MakeTransform "0, 0, 0")))
        (SplineMesh|SetStartandEnd _returnvalue_2 (.Location (Spline|GetLocationandTangentatSplinePoint (Variables|Default|GetCurrentSplineComponent) _index "Local")) (.Tangent (Spline|GetLocationandTangentatSplinePoint (Variables|Default|GetCurrentSplineComponent) _index "Local")) (.Location (Spline|GetLocationandTangentatSplinePoint (Variables|Default|GetCurrentSplineComponent) (+ _index 1) "Local")) (.Tangent (Spline|GetLocationandTangentatSplinePoint (Variables|Default|GetCurrentSplineComponent) (+ _index 1) "Local")) true :!class /Script/Engine.SplineMeshComponent)
        (Utilities|Array|Add (Variables|Default|GetSplineMeshComponents) _returnvalue_2)))))

(event Collision|EventActorBeginOverlap
  (params (OtherActor :type Actor%20Object%20Reference)))

(event EventTick
  (params (DeltaSeconds :type Float%20%28single-precision%29)))

(fn ConstructionScript)