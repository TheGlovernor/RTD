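; Ground loot actor that rolls a random-style item on spawn and displays it with a hover tooltip.
; BeginPlay asks the BP_Character_TD loot table component to choose loot, constructs that item, and copies its icon, name and description into the tooltip widget.
; RotatingMovement spins the ChestCylinder component.
; Hover shows the widget, using a short retriggerable delay to hide it once hover calls stop.
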(event EventBeginPlay
  (bind _returnvalue (Actor|GetActorOfClass "/Game/Blueprints/Player/BP_Character_TD.BP_Character_TD_C"))
  (bind _item (Default|ChooseLoot (Variables|/Game/Blueprints/Player/BP_Character_TD.BP_Character_TD_C|GetAC_LootTable _returnvalue)))
  (bind _returnvalue_2 (Game|ConstructObjectfromClass _item))
  (bind _output_get (Variables|Default|SetItem _returnvalue_2))
  (bind _ascui_tooltip (Utilities|Casting|CastToCUI_Tooltip (UserInterface|GetWidget (Variables|Default|GetWidget))))
  (Class|Image|SetBrush (Variables|/Game/UI/CUI_Tooltip.CUI_Tooltip_C|GetIcon _ascui_tooltip) (Class|WidgetBlueprintLibrary|MakeBrushfromTexture (Variables|/Game/Blueprints/Item/BP_Item.BP_Item_C|GetIcon _output_get) 128 128))
  (Rendering|Components|TextRender|SetText (Variables|/Game/UI/CUI_Tooltip.CUI_Tooltip_C|GetItemName _ascui_tooltip) (Variables|/Game/Blueprints/Item/BP_Item.BP_Item_C|GetItemName _output_get))
  (Rendering|Components|TextRender|SetText (Variables|/Game/UI/CUI_Tooltip.CUI_Tooltip_C|GetItemDesc _ascui_tooltip) (Variables|/Game/Blueprints/Item/BP_Item.BP_Item_C|GetDescriptiveText _output_get))
  (Components|Movement|SetUpdatedComponent (Variables|Default|GetRotatingMovement) (Variables|Default|Getchest_Cylinder)))

(event EventHover
  (bind _widget (Variables|Default|GetWidget))
  (Rendering|SetVisibility _widget true false)
  (Utilities|FlowControl|RetriggerableDelay 0.1)
  (Rendering|SetVisibility _widget false false))

(fn ConstructionScript)