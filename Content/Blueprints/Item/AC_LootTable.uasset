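; AC_LootTable is a loot component that randomly grants items in the HexDefense game.
; SpawnNewItem rolls against the given chance, checks that GI_HexDefense has unlocked items, then picks randomly from its EnabledItems.
; Nested random rolls select one of three rarity tiers, weighted toward the lowest.
; AddItem increments the item's amount at that rarity and fires the NewItem dispatcher only the first time an item appears, tracked in ItemsAddedToUI.
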(event Custom|AddItem
  (params (Item :type DA%20Tower%20Item%20Object%20Reference) (Rarity :type E_ItemRarities%20Enum :default "NewEnumerator0"))
  (Class|BPIListObject|IncrementAmount(Message) Item Rarity)
  (if (not (Utilities|Array|ContainsItem (Variables|Default|GetItemsAddedToUI) Item))
    (Default|CallNewItem Item)
    (Utilities|Array|Add (Variables|Default|GetItemsAddedToUI) Item)))

(event Custom|SpawnNewItem
  (params (Chance :type Float%20%28double-precision%29))
  (bind _returnvalue (Math|Random|RandomFloat))
  (bind _gameinstance (Variables|Default|GetGameInstance))
  (bind _unlockeditems (Variables|/Game/Blueprints/GM/GI_HexDefense.GI_HexDefense_C|GetUnlockedItems _gameinstance))
  (if (> Chance (Math|Random|RandomFloat))
    (if (!= (Utilities|Set|Length _unlockeditems) 0)
      (Utilities|Set|ToArray _unlockeditems)
      (CallFunction|AddItem (.OutItem (Utilities|Array|Random (Variables|/Game/Blueprints/GM/GI_HexDefense.GI_HexDefense_C|GetEnabledItems _gameinstance))) (select (> _returnvalue 0.95) "NewEnumerator2" (select (> _returnvalue 0.8) "NewEnumerator1" "NewEnumerator0"))))))

(event EventBeginPlay
  (bind _asgi_hex_defense (Utilities|Casting|CastToGI_HexDefense (Game|GetGameInstance)))
  (Variables|Default|SetGameInstance _asgi_hex_defense))