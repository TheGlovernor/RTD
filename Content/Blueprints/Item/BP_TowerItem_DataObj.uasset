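; BP_TowerItem_DataObj is a data object for a tower item, exposing the item's name, icon and query functions.
; ReportNameIcon returns the ItemName and ItemIcon variables with an empty description, marked as not buyable at zero price.
; GetEffects, GetOnKillEffects, GetOverride and GetTags are empty stubs that return no values here, which suggests a base class for specific items to override.
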(fn GetEffects
  (return 0))

(fn GetonKillEffects
  (return 0))

(fn GetOverride
  (return 0))

(fn GetTags
  (return "" ""))

(fn ReportNameIcon
  (return (Variables|Default|GetItemName) (Variables|Default|GetItemIcon) "" false 0))