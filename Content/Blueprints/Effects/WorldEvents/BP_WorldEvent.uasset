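; Timed world event actor that applies gameplay effects to enemies and offers the same for dens.
; On BeginPlay it records its starting duration attribute and, if enemy effects are set, applies them to every existing enemy.
; Each enemy also receives a bounty-change effect whose spec level carries the bounty increase.
; Attribute changes drive expiry: at zero it calls TimeIsUp and destroys itself; den effects have no caller here.
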(event OnAttributeChange(GSCCore)
  (params (Attribute :type Gameplay%20Attribute%20Structure) (DeltaValue :type Float%20%28single-precision%29) (EventTags :type Gameplay%20Tag%20Container%20Structure))
  (|SwitchGameplayAttribute Attribute
    (:Duration
      (if (<= (Class|GSCCoreComponent|GetCurrentAttributeValue (Variables|Default|GetGSCCore) "(AttributeName=\"Duration\",Attribute=/Script/RTD.WorldEvent:Duration,AttributeOwner=\"/Script/CoreUObject.Class'/Script/RTD.WorldEvent'\")") 0.0)
        (Default|CallTimeIsUp)
        (Actor|DestroyActor)))))

(event Custom|ApplyEffectsToEnemy
  (params (Enemy :type BP%20Enemy%20Base%2001%20Object%20Reference))
  (bind _gscabilitysystem (Variables|/Game/Blueprints/Mobs/EnemyBPs/BP_Enemy_Base_01.BP_Enemy_Base_01_C|GetGSCAbilitySystem Enemy))
  (for _array_element (Variables|Default|GetEffectsToEnemies)
    (Default|ApplyEffect Enemy (Variables|Default|GetGSCAbilitySystem) _array_element 0.0))
  (bind _returnvalue (Class|AbilitySystemBlueprintLibrary|AssignSetbyCallerMagnitude (GameplayEffects|MakeOutgoingSpec :self _gscabilitysystem :GameplayEffectClass "/Game/Blueprints/Effects/WorldEvents/EventModifiers/WE_BountyChange.WE_BountyChange_C" :Level (Variables|Default|GetBountyIncrease)) "None" 0.0))
  (GameplayEffects|ApplyGameplayEffectSpecToSelf _gscabilitysystem _returnvalue))

(event Custom|ApplyEffectsToDen
  (params (Den :type BP%20Den%20Object%20Reference))
  (for _array_element (Variables|Default|GetEffectsToDens)
    (Default|ApplyEffect Den (Variables|Default|GetGSCAbilitySystem) _array_element 0.0)))

(event EventBeginPlay
  (Variables|Default|SetStartDuration (Class|GSCCoreComponent|GetCurrentAttributeValue (Variables|Default|GetGSCCore) "(AttributeName=\"Duration\",Attribute=/Script/RTD.WorldEvent:Duration,AttributeOwner=\"/Script/CoreUObject.Class'/Script/RTD.WorldEvent'\")"))
  (if (Utilities|Array|IsNotEmpty (Variables|Default|GetEffectsToEnemies))
    (bind _outactors (Actor|GetAllActorsOfClass "/Game/Blueprints/Mobs/EnemyBPs/BP_Enemy_Base_01.BP_Enemy_Base_01_C"))
    (for _array_element _outactors
      (CallFunction|ApplyEffectstoEnemy _array_element))))

(fn ConstructionScript)