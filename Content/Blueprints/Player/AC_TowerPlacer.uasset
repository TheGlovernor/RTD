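; Player component that drives grid-based tower placement through a BP_TowerPlacer grid actor found in the level.
; While build mode is on, Tick traces under the cursor to update the grid's preview mesh and feed the hit location to the ghost-tile material parameter collection.
; Events forward tile clicks, mesh changes and grid save, load and reset to that actor.
; The dispatcher bindings for these events sit in unconnected nodes that never run.
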(event Custom|ActivateGridBuilderMode
  (params (SpawnTransform :type Transform))
  ;[1 1 1] Activate grid builder mode - spawns the grid
  (Variables|Default|GetGridBuilder ; If this is valid, we use the previous grid. If you want to support multiple grids, then remove this and always spawn
    (:then
      _)
    (:else
      (bind _returnvalue (Actor|GetActorOfClass "/Game/Blueprints/Map/BP_TowerPlacer.BP_TowerPlacer_C"))
      (Variables|Default|SetGridBuilder _returnvalue)))
  ;[1 1 1] Enable system bool, enable tick, and call enable on the grid builder
  (Variables|Default|SetbMapBuilder true)
  (Components|Tick|SetComponentTickEnabled true)
  (Default|CallEnableGridBuilding (Variables|Default|GetGridBuilder)))

(event Custom|ClearOldGridAndReset
  ;[1 1 1] Delete Old Grid
  (Default|CallDeactivateGridBuilder)
  (bind _gridbuilder (Variables|Default|GetGridBuilder)
    (:then
      (Actor|DestroyActor _gridbuilder))
    (:else)))

(event Custom|SaveGrid_Internal
  (params (SlotName :type String) (UserIndex :type Integer))
  ;[1 1 1] Save Grid
  (bind _gridbuilder (Variables|Default|GetGridBuilder)
    (:then
      (Default|SaveGrid _gridbuilder SlotName UserIndex)
      (Development|PrintString "Saving Grid"))
    (:else)))

(event Custom|TileInteraction_Internal
  ;[1 1 1] On Tile interaction, inform grid
  (if (Variables|Default|GetbMapBuilder)
    (Default|OnTileSelectedbyUser (Variables|Default|GetGridBuilder))))

(event Custom|ChangePlacedMesh_Internal
  (params (NextMesh :type Static%20Mesh%20Object%20Reference))
  ;[1 1 1] Change Mesh to spawn
  (Variables|/Game/Blueprints/Map/BP_TowerPlacer.BP_TowerPlacer_C|SetMeshToSpawn (Variables|Default|GetGridBuilder) NextMesh))

(event Custom|LoadGrid_Internal
  (params (SlotName :type String) (UserIndex :type Integer))
  ;[1 1 1] Load Grid
  (CallFunction|ClearOldGridandReset)
  (Default|CallActivateGridBuilderSystem)
  (Variables|/Game/Blueprints/Map/BP_TowerPlacer.BP_TowerPlacer_C|SetLoadExistingGridFromSave (Variables|Default|GetGridBuilder) false)
  (Default|LoadGrid (Variables|Default|GetGridBuilder) SlotName UserIndex)
  (Development|PrintString "Loading Grid"))

(event Custom|DeactivateGridBuilderMode
  ;[1 1 1] Deactivate the grid. Stops the ticking, and passes stop into the grid
  (Variables|Default|SetbMapBuilder false)
  (Components|Tick|SetComponentTickEnabled false)
  (bind _gridbuilder (Variables|Default|GetGridBuilder)
    (:then
      (Default|CallDisableGridBuilding _gridbuilder))
    (:else)))

(event EventBeginPlay
  (bind _astower_defense_state (Utilities|Casting|CastToBP_GS_TowerDefense (Game|GetGameState)))
  (Variables|Default|SetGameState _astower_defense_state)
  (bind _ascharacter (Utilities|Casting|CastToCharacter (Components|GetOwner)))
  (Variables|Default|SetCharacterRef _ascharacter))

(event EventTick
  (params (DeltaSeconds :type Float%20%28single-precision%29))
  (bind _returnvalue (Game|GetPlayerController 0))
  (bind _hitresult (Game|Player|GetHitResultUnderCursorbyChannel _returnvalue "TraceTypeQuery3" false))
  (bind (_bblockinghit _binitialoverlap _time _distance _location _impactpoint _normal _impactnormal _physmat _hitactor _hitcomponent _hitbonename _bonename _hititem) (Collision|BreakHitResult _hitresult))
  (if (Variables|Default|GetbMapBuilder)
    (if _bblockinghit
      (if (== _hitactor (Variables|Default|GetGridBuilder))
        (Default|HideUnhideSelection (Variables|Default|GetGridBuilder) false)
        (Utilities|FlowControl|Sequence
          (:then_0
            (Default|UpdatePreviewMesh (Variables|Default|GetGridBuilder) _hititem))
          (:then_1
            (Rendering|Material|SetVectorParameterValue "/HexGrids/HexGrids/Materials/GhostTiles.GhostTiles" "MouseTraceLocWS" (Math|Conversions|ToLinearColor(Vector) _location) :!class /Script/Engine.KismetMaterialLibrary) ; Update the hit location in the ghost material
          )))
      (else
        (Default|HideUnhideSelection (Variables|Default|GetGridBuilder) true)))))