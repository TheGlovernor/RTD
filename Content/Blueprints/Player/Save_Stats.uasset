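; Save_Stats keeps the player's tower defense statistics: survival time, money, towers built, kills, damage and boss rushes.
; Events add to counters and class-keyed maps, some tracking records such as longest survival, highest damage and most enemies hit at once.
; Spotted kills, health damage and armor hits also credit BP_Tower_Spotter, while damage types roll up into five base classes.
; Most changes fire CallStatsUpdated, but tower builds and boss rushes do not.
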(event Custom|AddTowerKill
  (params (Tower :type BP%20Tower%201%20Parent%20Class%20Reference) (Spotted :type Boolean))
  (bind _towerkills (Variables|Default|GetTowerKills))
  (Utilities|FlowControl|Sequence
    (:then_0
      (Utilities|Map|Add (Variables|Default|GetTowerKills) Tower (+ (.Value (Utilities|Map|Find (Variables|Default|GetTowerKills) Tower)) 1)))
    (:then_1
      (if Spotted
        (Utilities|Map|Add _towerkills "/Game/Blueprints/Building/Tower/BP_Tower_Spotter.BP_Tower_Spotter_C" (+ (.Value (Utilities|Map|Find _towerkills "/Game/Blueprints/Building/Tower/BP_Tower_Spotter.BP_Tower_Spotter_C")) 1))))
    (:then_2
      (Default|CallStatsUpdated))))

(event Custom|AddHealthDamage
  (params (Tower :type BP%20Tower%201%20Parent%20Class%20Reference) (Damage :type Float%20%28double-precision%29) (Spotted :type Boolean))
  (bind _towerdamage (Variables|Default|GetTowerDamage))
  (bind _towerdamage_2 (Variables|Default|GetTowerDamage))
  (bind (_value _returnvalue) (Utilities|Map|Find _towerdamage_2 Tower))
  (Utilities|FlowControl|Sequence
    (:then_0
      (if Spotted
        (Utilities|Map|Add _towerdamage "/Game/Blueprints/Building/Tower/BP_Tower_Spotter.BP_Tower_Spotter_C" (+ (.Value (Utilities|Map|Find _towerdamage "/Game/Blueprints/Building/Tower/BP_Tower_Spotter.BP_Tower_Spotter_C")) Damage))))
    (:then_1
      (if _returnvalue
        (Utilities|Map|Add (Variables|Default|GetTowerDamage) Tower (+ Damage _value))
        (if (> Damage (.Value (Utilities|Map|Find (Variables|Default|GetTowerHighestDamage) Tower)))
          (Utilities|Map|Add (Variables|Default|GetTowerHighestDamage) Tower Damage))
        (else
          (Utilities|Map|Add (Variables|Default|GetTowerDamage) Tower Damage)
          (Utilities|Map|Add (Variables|Default|GetTowerHighestDamage) Tower Damage))))
    (:then_2
      (Default|CallStatsUpdated))))

(event Custom|TowerBuilt
  (params (Tower :type BP%20Tower%201%20Parent%20Class%20Reference))
  (bind _towersbuilt (Variables|Default|GetTowersBuilt))
  (Utilities|Map|Add _towersbuilt Tower (+ (.Value (Utilities|Map|Find _towersbuilt Tower)) 1)))

(event Custom|BossRushSurvived
  (Math|Integer|IncrementInt (Variables|Default|GetBossRushesSurvived)))

(event Custom|AddTime
  (params (Dens :type Integer) (Time :type Float%20%28double-precision%29))
  (bind _timesurvived (Variables|Default|GetTimeSurvived))
  (bind (_value _returnvalue) (Utilities|Map|Find _timesurvived Dens))
  (if _returnvalue
    (Utilities|Map|Add (Variables|Default|GetTimeSurvived) Dens (+ Time _value))
    (if (> Time (.Value (Utilities|Map|Find (Variables|Default|GetLongestTimeSurvived) Dens)))
      (Utilities|Map|Add (Variables|Default|GetLongestTimeSurvived) Dens Time)
      (Default|CallStatsUpdated))
    (else
      (Utilities|Map|Add (Variables|Default|GetTimeSurvived) Dens Time)
      (Utilities|Map|Add (Variables|Default|GetLongestTimeSurvived) Dens Time)
      (Default|CallStatsUpdated))))

(event Custom|AddArmorDamage
  (params (Tower :type BP%20Tower%201%20Parent%20Class%20Reference%20%28by%20ref%29) (Spotted :type Boolean))
  (bind _towerarmordamage (Variables|Default|GetTowerArmorDamage))
  (Utilities|FlowControl|Sequence
    (:then_0
      (if Spotted
        (Utilities|Map|Add _towerarmordamage "/Game/Blueprints/Building/Tower/BP_Tower_Spotter.BP_Tower_Spotter_C" (+ (.Value (Utilities|Map|Find _towerarmordamage "/Game/Blueprints/Building/Tower/BP_Tower_Spotter.BP_Tower_Spotter_C")) 1))))
    (:then_1
      (if (.ReturnValue (Utilities|Map|Find (Variables|Default|GetTowerArmorDamage) Tower))
        (Utilities|Map|Add (Variables|Default|GetTowerArmorDamage) Tower (+ (.Value (Utilities|Map|Find (Variables|Default|GetTowerArmorDamage) Tower)) 1))
        (else
          (Utilities|Map|Add (Variables|Default|GetTowerArmorDamage) Tower 1))))
    (:then_2
      (Default|CallStatsUpdated))))

(event Custom|AddShieldDamage
  (params (Tower :type BP%20Tower%201%20Parent%20Class%20Reference%20%28by%20ref%29) (Amount :type Integer))
  (if (.ReturnValue (Utilities|Map|Find (Variables|Default|GetTowerShieldDamage) Tower))
    (Utilities|Map|Add (Variables|Default|GetTowerShieldDamage) Tower (+ (.Value (Utilities|Map|Find (Variables|Default|GetTowerShieldDamage) Tower)) Amount))
    (Default|CallStatsUpdated)
    (else
      (Utilities|Map|Add (Variables|Default|GetTowerShieldDamage) Tower Amount)
      (Default|CallStatsUpdated))))

(event Custom|AddEnemiesHitAtOnce
  (params (Tower :type BP%20Tower%201%20Parent%20Class%20Reference) (EnemiesHit :type Integer))
  (if (> EnemiesHit (.Value (Utilities|Map|Find (Variables|Default|GetEnemiesHitAtOnce) Tower)))
    (Utilities|Map|Add (Variables|Default|GetEnemiesHitAtOnce) Tower EnemiesHit)
    (Default|CallStatsUpdated)))

(event Custom|AddMoneyEarned
  (params (Money :type Float%20%28double-precision%29))
  (Variables|Default|SetMoneyEarned (+ (Math|Float|Absolute(Float) Money) (Variables|Default|GetMoneyEarned)))
  (Default|CallStatsUpdated))

(event Custom|AddEnemyKill
  (params (Groups :type Array%20of%20EnemyGroup%20Enums :default "NewEnumerator4") (bShielded :type Boolean) (bArmored :type Boolean))
  (Utilities|FlowControl|Sequence
    (:then_0
      (for _array_element Groups
        (Utilities|Map|Add (Variables|Default|GetEnemiesKilled) _array_element (+ (.Value (Utilities|Map|Find (Variables|Default|GetEnemiesKilled) _array_element)) 1))
        (Default|CallStatsUpdated)))
    (:then_1
      (if bShielded
        (Math|Integer|IncrementInt (Variables|Default|GetShieldedEnemyKills))))
    (:then_2
      (if bArmored
        (Math|Integer|IncrementInt (Variables|Default|GetArmoredEnemyKills))))))

(event Custom|AddMoneySpent
  (params (Money :type Float%20%28double-precision%29))
  (Variables|Default|SetMoneySpent (+ (Math|Float|Absolute(Float) Money) (Variables|Default|GetMoneySpent)))
  (Default|CallStatsUpdated))

(event Custom|AddDamageType
  (params (DamageType :type BP%20Damage%20Class%20Reference%20%28by%20ref%29) (Amount :type Float%20%28double-precision%29))
  (bind _damagebytype (Variables|Default|GetDamageByType))
  (bind _damagebytype_2 (Variables|Default|GetDamageByType))
  (bind _damagebytype_3 (Variables|Default|GetDamageByType))
  (bind _damagebytype_4 (Variables|Default|GetDamageByType))
  (bind _damagebytype_5 (Variables|Default|GetDamageByType))
  (if (or (Utilities|ClassIsChildOf DamageType "/Game/Blueprints/HealthDamage/DamageClasses/BP_BleedDamage.BP_BleedDamage_C") (== DamageType "/Game/Blueprints/HealthDamage/DamageClasses/BP_BleedDamage.BP_BleedDamage_C"))
    (Utilities|Map|Add _damagebytype "/Game/Blueprints/HealthDamage/DamageClasses/BP_BleedDamage.BP_BleedDamage_C" (+ (.Value (Utilities|Map|Find _damagebytype "/Game/Blueprints/HealthDamage/DamageClasses/BP_BleedDamage.BP_BleedDamage_C")) Amount))
    (Default|CallStatsUpdated)
    (elif (or (Utilities|ClassIsChildOf DamageType "/Game/Blueprints/HealthDamage/DamageClasses/BP_FireDamage.BP_FireDamage_C") (== DamageType "/Game/Blueprints/HealthDamage/DamageClasses/BP_FireDamage.BP_FireDamage_C"))
      (Utilities|Map|Add _damagebytype_3 "/Game/Blueprints/HealthDamage/DamageClasses/BP_FireDamage.BP_FireDamage_C" (+ (.Value (Utilities|Map|Find _damagebytype_3 "/Game/Blueprints/HealthDamage/DamageClasses/BP_FireDamage.BP_FireDamage_C")) Amount))
      (Default|CallStatsUpdated)
      (elif (or (Utilities|ClassIsChildOf DamageType "/Game/Blueprints/HealthDamage/DamageClasses/BP_FrostDamage.BP_FrostDamage_C") (== DamageType "/Game/Blueprints/HealthDamage/DamageClasses/BP_FrostDamage.BP_FrostDamage_C"))
        (Utilities|Map|Add _damagebytype_4 "/Game/Blueprints/HealthDamage/DamageClasses/BP_FrostDamage.BP_FrostDamage_C" (+ (.Value (Utilities|Map|Find _damagebytype_4 "/Game/Blueprints/HealthDamage/DamageClasses/BP_FrostDamage.BP_FrostDamage_C")) Amount))
        (Default|CallStatsUpdated)
        (elif (or (Utilities|ClassIsChildOf DamageType "/Game/Blueprints/HealthDamage/DamageClasses/BP_ShockDamage.BP_ShockDamage_C") (== DamageType "/Game/Blueprints/HealthDamage/DamageClasses/BP_ShockDamage.BP_ShockDamage_C"))
          (Utilities|Map|Add _damagebytype_5 "/Game/Blueprints/HealthDamage/DamageClasses/BP_ShockDamage.BP_ShockDamage_C" (+ (.Value (Utilities|Map|Find _damagebytype_5 "/Game/Blueprints/HealthDamage/DamageClasses/BP_ShockDamage.BP_ShockDamage_C")) Amount))
          (Default|CallStatsUpdated)
          (elif (or (Utilities|ClassIsChildOf DamageType "/Game/Blueprints/HealthDamage/DamageClasses/BP_Damage_Physical.BP_Damage_Physical_C") (== DamageType "/Game/Blueprints/HealthDamage/DamageClasses/BP_Damage_Physical.BP_Damage_Physical_C"))
            (Utilities|Map|Add _damagebytype_2 "/Game/Blueprints/HealthDamage/DamageClasses/BP_Damage_Physical.BP_Damage_Physical_C" (+ (.Value (Utilities|Map|Find _damagebytype_2 "/Game/Blueprints/HealthDamage/DamageClasses/BP_Damage_Physical.BP_Damage_Physical_C")) Amount))
            (Default|CallStatsUpdated)))))))