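; Player character for a tower defense game: a flying pawn that owns the start screen UI, money and scouts.
; Left-click either places a tower through CharacterTowerPlacerComponent, charging its cost, or selects the actor under the cursor via select/deselect messages.
; StartGame fills the tower list from unlocked DT_TowerData rows plus hardcoded items, while Enter toggles automatic scouting.
; Legacy camera movement, zoom, rotation and cursor logic remains but is disconnected.
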(event Custom|scrollArm
  ;[1 1 1] On Tick Events
)

(event Custom|Rotate
  ;[1 1 1] On Tick Events
)

(event Custom|Move)

(event EventBeginPlay
  (bind _returnvalue (Game|GetPlayerController 0))
  (CallFunction|CreateStartScreen)
  (Pawn|Components|CharacterMovement|SetMovementMode (Variables|Character|GetCharacterMovement) "MOVE_Flying" 0)
  (Variables|/Script/Engine.PlayerController|SetbShowMouseCursor _returnvalue true)
  (Input|SetInputModeGameandUI _returnvalue 0 "DoNotLock" false)
  (CallFunction|ChangeMoney 5000)
  (CallFunction|AddScout))

(event Collision|EventActorBeginOverlap
  (params (OtherActor :type Actor%20Object%20Reference)))

(event EventTick
  (params (DeltaSeconds :type Float%20%28single-precision%29)))

(event Collision|EventActorEndOverlap
  (params (OtherActor :type Actor%20Object%20Reference)))

(event EventChangeMoney
  (params (DeltaDosh :type Integer))
  (bind _output_get (Variables|Default|SetMoney (+ DeltaDosh (Variables|Default|GetMoney))))
  (Default|UpdateGold (Variables|/Game/UI/CUI_StartScreen.CUI_StartScreen_C|GetCUI_TOPINFO (Variables|Default|GetStartScreen)) _output_get))

(event EventRemoveTower
  (params (ID :type Integer))
  (Variables|Default|SetSelectedObject 0)
  (Default|RemoveTower (Variables|Default|GetCharacterTowerPlacerComponent) ID))

(event Input|MouseEvents|MouseWheelAxis
  (params (AxisValue :type Float%20%28single-precision%29))
  ;[1 1 1] Mouse and Key Events
)

(event Input|MouseEvents|MouseX
  (params (AxisValue :type Float%20%28single-precision%29))
  ;[1 1 1] Mouse and Key Events
)

(event Input|MouseEvents|MouseY
  (params (AxisValue :type Float%20%28single-precision%29))
  ;[1 1 1] Mouse and Key Events
)

(event Input|KeyboardEvents|W
  (params (Key :type Key%20Structure))
  ;[1 1 1] Mouse and Key Events
)

(event Input|KeyboardEvents|A
  (params (Key :type Key%20Structure))
  ;[1 1 1] Mouse and Key Events
)

(event Input|KeyboardEvents|Enter
  (params (Key :type Key%20Structure))
  ;[1 1 1] Mouse and Key Events
  (:Released
    (if (Variables|Default|Getautoscout)
      (for _array_element (Variables|Default|GetScouts)
        (Variables|/Game/Blueprints/Scout/BP_ScoutObj.BP_ScoutObj_C|SetAutomaticScouting _array_element false))
      (Variables|Default|Setautoscout false)
      (else
        (for _array_element_2 (Variables|Default|GetScouts)
          (Variables|/Game/Blueprints/Scout/BP_ScoutObj.BP_ScoutObj_C|SetAutomaticScouting _array_element_2 true))
        (Variables|Default|Setautoscout true)))))

(event Input|KeyboardEvents|S
  (params (Key :type Key%20Structure))
  ;[1 1 1] Mouse and Key Events
)

(event Input|KeyboardEvents|D
  (params (Key :type Key%20Structure))
  ;[1 1 1] Mouse and Key Events
)

(event Input|KeyboardEvents|Q
  (params (Key :type Key%20Structure))
  ;[1 1 1] Mouse and Key Events
)

(event Input|KeyboardEvents|E
  (params (Key :type Key%20Structure))
  ;[1 1 1] Mouse and Key Events
)

(event Input|MouseEvents|LeftMouseButton
  (params (Key :type Key%20Structure))
  (bind _towercost (Variables|Default|GetTowerCost))
  (bind _charactertowerplacercomponent (Variables|Default|GetCharacterTowerPlacerComponent))
  ;[1 1 1] Mouse and Key Events
  (:Released
    (if (Variables|/Game/Blueprints/Player/AC_TowerPlacer.AC_TowerPlacer_C|GetbMapBuilder _charactertowerplacercomponent)
      (if (>= (Variables|Default|GetMoney) _towercost)
        (Default|TileInteractionInternal _charactertowerplacercomponent)
        (CallFunction|ChangeMoney (* _towercost -1)))
      (else
        (CallFunction|SelectObject)))))

(event Input|MouseEvents|RightMouseButton
  (params (Key :type Key%20Structure))
  ;[1 1 1] Mouse and Key Events
)

(event Input|MouseEvents|MiddleMouseButton
  (params (Key :type Key%20Structure))
  ;[1 1 1] Mouse and Key Events
  (:Pressed
    (Variables|ButtonBools|SetmouseWheelDown true)
    (CallFunction|CursorTypeHandler :!label _label))
  (:Released
    (Variables|ButtonBools|SetmouseWheelDown false)
    (goto _label)))

(event Input|MouseEvents|Mouse2D
  (params (AxisValue :type Vector :default "0, 0, 0"))
  ;[1 1 1] Mouse and Key Events
)

(fn ConstructionScript)

(fn CursorTypeHandler)

(fn InitTowerList
  (Variables|Default|SetTowerTileView (Variables|/Game/UI/CUI_StartScreen.CUI_StartScreen_C|GetCommonTileView_Towers (Variables|Default|GetStartScreen)))
  (bind _outrownames (DataTable|GetDataTableRowNames "/Game/Blueprints/Building/Tower/DataAndEnums/DT_TowerData.DT_TowerData"))
  (for _array_element _outrownames
    (bind _returnvalue (Utilities|GetDataTableRow "/Game/Blueprints/Building/Tower/DataAndEnums/DT_TowerData.DT_TowerData" _array_element)
      (:then
        (if (and (.Unlocked (Utilities|Struct|BreakS_TowerDataStruct _returnvalue)) (.Enabled (Utilities|Struct|BreakS_TowerDataStruct _returnvalue)))
          (bind _returnvalue_2 (Game|ConstructObjectfromClass "/Game/Blueprints/Building/Tower/DataAndEnums/BP_Tower_DataObj.BP_Tower_DataObj_C" _returnvalue))
          (Class|ListView|AddItem (Variables|Default|GetTowerTileView) _returnvalue_2)))
      (:RowNotFound
        (Development|PrintString "Hello"))))
  (for _index (range 0 11)
    (bind _returnvalue_3 (Game|ConstructObjectfromClass "/Game/Blueprints/Item/TowerItems/Item_CursedLens.Item_CursedLens_C"))
    (Class|ListView|AddItem (Variables|/Game/UI/CUI_StartScreen.CUI_StartScreen_C|GetCommonTileView_Items (Variables|Default|GetStartScreen)) _returnvalue_3)
    (bind _returnvalue_4 (Game|ConstructObjectfromClass "/Game/Blueprints/Item/TowerItems/Item_GATBLEED.Item_GATBLEED_C"))
    (Class|ListView|AddItem (Variables|/Game/UI/CUI_StartScreen.CUI_StartScreen_C|GetCommonTileView_Items (Variables|Default|GetStartScreen)) _returnvalue_4)))

(fn EnsurePlacerActive
  (bind _charactertowerplacercomponent (Variables|Default|GetCharacterTowerPlacerComponent))
  (if (not (Variables|/Game/Blueprints/Player/AC_TowerPlacer.AC_TowerPlacer_C|GetbMapBuilder _charactertowerplacercomponent))
    (Default|ActivateGridBuilderMode _charactertowerplacercomponent)))

(fn SelectObject
  (bind _returnvalue (Game|GetPlayerController 0))
  (bind _hitresult (Game|Player|GetHitResultUnderCursorbyChannel _returnvalue "TraceTypeQuery5" false))
  (bind _hitactor (Collision|BreakHitResult _hitresult))
  (Class|BPISelectable|Deselect(Message) (Variables|Default|GetSelectedObject) (Variables|Default|GetStartScreen))
  (if (!= (Variables|Default|GetSelectedObject) _hitactor)
    (bind _output_get (Variables|Default|SetSelectedObject _hitactor))
    (Class|BPISelectable|Select(Message) _output_get (Variables|Default|GetStartScreen))
    (else
      (Variables|Default|SetSelectedObject 0))))

(fn CreateStartScreen
  (bind _returnvalue (UserInterface|CreateWidget "/Game/UI/CUI_StartScreen.CUI_StartScreen_C" (Game|GetPlayerController 0)))
  (bind _output_get (Variables|Default|SetStartScreen _returnvalue))
  (UserInterface|Viewport|AddtoPlayerScreen _output_get))

(fn StartGame
  (CallFunction|InitTowerList)
  (Input|EnableInput self 0)
  (Variables|Default|SetGameStarted true)
  (Game|SetGamePaused false))

(fn AddScout
  (bind _startscreen (Variables|Default|GetStartScreen))
  (bind _commontileview_scouts (Variables|/Game/UI/CUI_StartScreen.CUI_StartScreen_C|GetCommonTileView_Scouts _startscreen))
  (bind _returnvalue (Game|ConstructObjectfromClass "/Game/Blueprints/Scout/BP_ScoutObj.BP_ScoutObj_C"))
  (Utilities|Array|Add (Variables|Default|GetScouts) _returnvalue)
  (Class|ListView|AddItem _commontileview_scouts _returnvalue)
  (Default|UpdateScouts (Variables|/Game/UI/CUI_StartScreen.CUI_StartScreen_C|GetCUI_TOPINFO _startscreen) (Class|ListView|GetNumItems _commontileview_scouts)))

(fn ScoutRandomArea
  (bind _outactors (Actor|GetAllActorsOfClass "/Game/Blueprints/Map/BP_ScoutAreaButton.BP_ScoutAreaButton_C"))
  (if (Utilities|Array|IsNotEmpty _outactors)
    (Default|Clicked (Utilities|Array|Get(acopy) _outactors (Math|Random|RandomIntegerinRange 0 (- (Utilities|Array|Length _outactors) 1))))))

(fn GetMoney
  (return (Variables|Default|GetMoney)))