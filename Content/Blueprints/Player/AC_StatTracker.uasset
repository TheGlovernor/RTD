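; Player component that records tower-defense combat, economy and time stats into the game instance's stats save object.
; Damage, kill, build and money events forward to matching save functions, while shield and armor hits and blocks also trigger effects on the level's BP_HitEffects actor.
; Kills of one enemy group notify GS_TowerDefense of a boss kill.
; GetTowerStat reads a tower's saved value for a given challenge type.
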(event Custom|GotKill
  (params (Tower :type BP%20Tower%201%20Parent%20Class%20Reference) (EnemyGroups :type Array%20of%20EnemyGroup%20Enums :default "NewEnumerator4") (Spotted :type Boolean) (bShielded :type Boolean) (bArmored :type Boolean))
  (Default|AddTowerKill (Variables|Default|GetStatsSaveGame) Tower Spotted)
  (Default|AddEnemyKill (Variables|Default|GetStatsSaveGame) EnemyGroups bShielded bArmored)
  (if (Utilities|Array|ContainsItem EnemyGroups "NewEnumerator4")
    (bind _asgs_tower_defense (Utilities|Casting|CastToGS_TowerDefense (Game|GetGameState)))
    (Default|BossKilled _asgs_tower_defense)))

(event Custom|DamagedHealth
  (params (Tower :type BP%20Tower%201%20Parent%20Class%20Reference) (DamageType :type BP%20Damage%20Class%20Reference) (DamageDone :type Float%20%28double-precision%29) (Spotted :type Boolean))
  (Default|AddHealthDamage (Variables|Default|GetStatsSaveGame) Tower DamageDone Spotted)
  (Default|AddDamageType (Variables|Default|GetStatsSaveGame) DamageType DamageDone))

(event Custom|ShieldBlock
  (params (Location :type Vector))
  (Default|AddShieldBlock (Variables|Default|GetHitEffects) Location))

(event Custom|BossRushSurvived
  (Default|BossRushSurvived (Variables|Default|GetStatsSaveGame)))

(event Custom|AddTime
  (params (StarterDens :type Integer) (Time :type Float%20%28double-precision%29))
  (Default|AddTime (Variables|Default|GetStatsSaveGame) StarterDens Time))

(event Custom|SpentMoney
  (params (Money :type Float%20%28double-precision%29))
  (Default|AddMoneySpent (Variables|Default|GetStatsSaveGame) Money))

(event Custom|EarnedMoney
  (params (Money :type Float%20%28double-precision%29))
  (Default|AddMoneyEarned (Variables|Default|GetStatsSaveGame) Money))

(event Custom|TowerBuilt
  (params (Tower :type BP%20Tower%201%20Parent%20Class%20Reference))
  (Default|TowerBuilt (Variables|Default|GetStatsSaveGame) Tower))

(event Custom|DamagedArmor
  (params (Tower :type BP%20Tower%201%20Parent%20Class%20Reference) (Spotted :type Boolean) (Location :type Vector))
  (Default|AddArmorDamage (Variables|Default|GetStatsSaveGame) Tower Spotted)
  (Default|AddArmorBreak (Variables|Default|GetHitEffects) Location))

(event Custom|DamagedShield
  (params (Tower :type BP%20Tower%201%20Parent%20Class%20Reference) (Amount :type Integer) (Location :type Vector))
  (Default|AddShieldDamage (Variables|Default|GetStatsSaveGame) Tower Amount)
  (Default|AddShieldBreak (Variables|Default|GetHitEffects) Location))

(event Custom|EnemiesHitAtOnce
  (params (Tower :type BP%20Tower%201%20Parent%20Class%20Reference) (EnemiesHit :type Integer))
  (Default|AddEnemiesHitatOnce (Variables|Default|GetStatsSaveGame) Tower EnemiesHit))

(event Custom|ArmorBlock
  (params (Location :type Vector))
  (Default|AddArmorBlock (Variables|Default|GetHitEffects) Location))

(event EventBeginPlay
  (bind _asgi_hex_defense (Utilities|Casting|CastToGI_HexDefense (Game|GetGameInstance)))
  (bind _output_get (Variables|Game|SetGameInstance _asgi_hex_defense))
  (Variables|Default|SetStatsSaveGame (Variables|/Game/Blueprints/GM/GI_HexDefense.GI_HexDefense_C|GetSave_Stats _output_get))
  (bind _returnvalue (Actor|GetActorOfClass "/Game/Blueprints/Map/BP_HitEffects.BP_HitEffects_C"))
  (Variables|Default|SetHitEffects _returnvalue))

(fn GetTowerStat
  (params (Tower :type BP%20Tower%201%20Parent%20Class%20Reference) (Challenge :type E_ChallengeType%20Enum :default "NewEnumerator0"))
  (bind _statssavegame (Variables|Default|GetStatsSaveGame))
  (return (Utilities|Select :Index Challenge :NewEnumerator7 0.0 :NewEnumerator0 (Math|Conversions|ToFloat(Integer) (.Value (Utilities|Map|Find (Variables|/Game/Blueprints/Player/Save_Stats.Save_Stats_C|GetTowerKills _statssavegame) Tower))) :NewEnumerator1 (.Value (Utilities|Map|Find (Variables|/Game/Blueprints/Player/Save_Stats.Save_Stats_C|GetTowerDamage _statssavegame) Tower)) :NewEnumerator2 (.Value (Utilities|Map|Find (Variables|/Game/Blueprints/Player/Save_Stats.Save_Stats_C|GetTowerHighestDamage _statssavegame) Tower)) :NewEnumerator3 (Math|Conversions|ToFloat(Integer) (.Value (Utilities|Map|Find (Variables|/Game/Blueprints/Player/Save_Stats.Save_Stats_C|GetTowerShieldDamage _statssavegame) Tower))) :NewEnumerator4 (Math|Conversions|ToFloat(Integer) (.Value (Utilities|Map|Find (Variables|/Game/Blueprints/Player/Save_Stats.Save_Stats_C|GetTowerArmorDamage _statssavegame) Tower))) :NewEnumerator6 (Math|Conversions|ToFloat(Integer) (.Value (Utilities|Map|Find (Variables|/Game/Blueprints/Player/Save_Stats.Save_Stats_C|GetEnemiesHitAtOnce _statssavegame) Tower))))))