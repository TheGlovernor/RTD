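; Player selection component that tracks selected and hovered towers, tower data assets and tower item assets.
; Selection, hover and clear events cast the incoming object, update a SelectionType state and broadcast changes.
; Unhover uses a retriggerable delay and a gate, closed by new hovers, to debounce state resets.
; It also inserts items into the selected tower, decrementing the item's amount on success and printing the failure reason otherwise.
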(event Custom|NewSelection
  (params (SelectedObject :type Object%20Object%20Reference))
  (Utilities|IsValid SelectedObject
    (:Is%20Valid
      (bind _asda_tower_item (Utilities|Casting|CastToDA_TowerItem SelectedObject)
        (:then
          (if (Utilities|ClassIsChildOf (Utilities|GetClass (Variables|Selection|GetCurrentSelection)) "/Game/Blueprints/Building/Tower/BP_Tower_1Parent.BP_Tower_1Parent_C")
            (Variables|Selection|SetSelectedItem _asda_tower_item)
            (Variables|Selection|SetSelectionType "NewEnumerator5")
            (else
              (CallFunction|ClearSelection)))
          (Default|CallSelectionTypeChanged))
        (:CastFailed
          (bind _asda_tower (Utilities|Casting|CastToDA_Tower SelectedObject)
            (:then
              (Variables|Selection|SetCurrentSelection _asda_tower)
              (Variables|Selection|SetSelectionType "NewEnumerator2")
              (Default|CallSelectionTypeChanged))
            (:CastFailed
              (bind _asbp_tower_1parent (Utilities|Casting|CastToBP_Tower_1Parent SelectedObject)
                (:then
                  (Class|BPISelectable|Deselect(Message) (Variables|Selection|GetCurrentSelection))
                  (Variables|Selection|SetCurrentSelection _asbp_tower_1parent)
                  (switch Utilities|FlowControl|Switch|SwitchonESelectionType (Variables|Selection|GetSelectionType)
                    (:NewEnumerator0
                      (Variables|Selection|SetSelectionType "NewEnumerator1" :!label _label)
                      (Default|CallSelectionTypeChanged))
                    (:NewEnumerator1
                      (goto _label))
                    (:NewEnumerator6
                      (goto _label))
                    (:NewEnumerator2
                      (goto _label))
                    (:NewEnumerator3
                      (goto _label))
                    (:NewEnumerator5
                      (Variables|Selection|SetSelectionType "NewEnumerator4")
                      (Default|CallSelectionTypeChanged))
                    (:NewEnumerator7
                      (goto _label))))
                (:CastFailed
                  (CallFunction|ClearSelection))))))))
    (:Is%20Not%20Valid
      (CallFunction|ClearSelection))))

(event Custom|ClearSelection
  (switch Utilities|FlowControl|Switch|SwitchonESelectionType (Variables|Selection|GetSelectionType)
    (:NewEnumerator0
      (Class|BPISelectable|Deselect(Message) (Variables|Selection|GetCurrentSelection) :!label _label)
      (Variables|Selection|SetSelectionType "NewEnumerator0" :!label _label_2)
      (Variables|Selection|SetCurrentSelection 0)
      (Default|CallSelectionTypeChanged))
    (:NewEnumerator1
      (goto _label))
    (:NewEnumerator6
      (goto _label_2))
    (:NewEnumerator2
      (Default|CallDeselectDATower)
      (goto _label))
    (:NewEnumerator3
      (goto _label_2))
    (:NewEnumerator4
      (goto _label))
    (:NewEnumerator5
      (Default|CallDeselectDATowerItem)
      (Variables|Selection|SetSelectionType "NewEnumerator4")
      (Variables|Selection|SetSelectedItem 0)
      (Default|CallSelectionTypeChanged))
    (:NewEnumerator7
      (goto _label_2))))

(event Custom|NewHover
  (params (HoveredObject :type Object%20Object%20Reference))
  (CallFunction|CloseUnhoverGate)
  (switch Utilities|FlowControl|Switch|SwitchonESelectionType (Variables|Selection|GetSelectionType)
    (:NewEnumerator0
      _)
    (:NewEnumerator1
      _)
    (:NewEnumerator6
      _)
    (:NewEnumerator2
      _)
    (:NewEnumerator3
      _)
    (:NewEnumerator4
      _)
    (:NewEnumerator7
      _))
  (bind _currentselection (Variables|Selection|GetCurrentSelection)
    (:then
      (Utilities|Casting|CastToBP_Tower_1Parent _currentselection)
      (bind _asda_tower_item (Utilities|Casting|CastToDA_TowerItem HoveredObject))
      (Variables|Selection|SetHoveredObject _asda_tower_item)
      (Variables|Selection|SetSelectionType "NewEnumerator4")
      (Default|CallSelectionTypeChanged))
    (:else
      (bind _asda_tower (Utilities|Casting|CastToDA_Tower HoveredObject)
        (:then
          (Variables|Selection|SetHoveredObject _asda_tower)
          (Variables|Selection|SetSelectionType "NewEnumerator6")
          (Default|CallSelectionTypeChanged))
        (:CastFailed
          (bind _asda_tower_item_2 (Utilities|Casting|CastToDA_TowerItem HoveredObject)
            (:then
              (Variables|Selection|SetHoveredObject _asda_tower_item_2)
              (Variables|Selection|SetSelectionType "NewEnumerator3")
              (Default|CallSelectionTypeChanged))
            (:CastFailed
              (Default|CallSelectionTypeChanged))))))))

(event Custom|Unhover
  (CallFunction|OpenUnhoverGate)
  (Utilities|FlowControl|RetriggerableDelay 0.2)
  (Utilities|FlowControl|Gate false
    (:Exit
      (switch Utilities|FlowControl|Switch|SwitchonESelectionType (Variables|Selection|GetSelectionType)
        (:NewEnumerator0
          (Variables|Selection|SetSelectionType "NewEnumerator0" :!label _label)
          (Default|CallSelectionTypeChanged))
        (:NewEnumerator1
          (Variables|Selection|SetSelectionType "NewEnumerator1" :!label _label_2)
          (Default|CallSelectionTypeChanged))
        (:NewEnumerator6
          (goto _label))
        (:NewEnumerator3
          (goto _label))
        (:NewEnumerator4
          (goto _label_2))
        (:NewEnumerator7
          (goto _label))))))

(event Custom|OpenUnhoverGate
  (Utilities|FlowControl|Gate false) ; enters at Open
)

(event Custom|CloseUnhoverGate
  (Utilities|FlowControl|Gate false) ; enters at Close
)

(event Custom|Back
  (CallFunction|ClearSelection))

(event Custom|InsertItemToSelectedTower
  (params (Item :type DA%20Tower%20Item%20Object%20Reference) (Rarity :type E_ItemRarities%20Enum :default "NewEnumerator0"))
  (bind _amount (Class|BPIListObject|GetAmount(Message) Item Rarity))
  (if (> _amount 0)
    (if (Utilities|ClassIsChildOf (Utilities|GetClass (Variables|Selection|GetCurrentSelection)) "/Game/Blueprints/Building/Tower/BP_Tower_1Parent.BP_Tower_1Parent_C")
      (bind (_inserted _reason) (Class|BPITower|InsertItem(Message) (Variables|Selection|GetCurrentSelection) Item Rarity))
      (if _inserted
        (Class|BPIListObject|DecrementAmount(Message) Item Rarity)
        (Default|CallReturntoItem)
        (else
          (CallFunction|ItemInsertionFailed _reason)))
      (else
        (CallFunction|ItemInsertionFailed "NewEnumerator0")))
    (else
      (CallFunction|ItemInsertionFailed "NewEnumerator3"))))

(event Custom|ItemInsertionFailed
  (params (Reason :type E_ItemErrors%20Enum :default "NewEnumerator4"))
  (Development|PrintString (Utilities|String|EnumtoString Reason)))

(event Custom|NewWorldHover
  (params (HoveredObject :type Object%20Object%20Reference))
  (bind _asbp_tower_1parent (Utilities|Casting|CastToBP_Tower_1Parent HoveredObject)
    (:then
      (CallFunction|CloseUnhoverGate)
      (if (!= HoveredObject (Variables|Selection|GetWorldHoveredObject))
        (switch Utilities|FlowControl|Switch|SwitchonESelectionType (Variables|Selection|GetSelectionType)
          (:NewEnumerator0
            _)
          (:NewEnumerator6
            _)
          (:NewEnumerator3
            _)
          (:NewEnumerator7
            _))
        (Variables|Selection|SetWorldHoveredObject _asbp_tower_1parent)
        (Variables|Selection|SetSelectionType "NewEnumerator7")
        (Default|CallSelectionTypeChanged)))
    (:CastFailed
      (Variables|Selection|GetWorldHoveredObject
        (:then
          (Variables|Selection|SetWorldHoveredObject 0)
          (CallFunction|Unhover))
        (:else)))))