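; Tower defense player character acting as a flying RTS-style camera, with a start screen that leads into the tower placement UI.
; Keys and mouse drive movement plus decelerating rotation and zoom velocities on Tick, with arm length setting pitch and fly speed.
; Left click either forwards tile interaction to CharacterTowerPlayerComponent or selects towers, toggling range indicators and updating the UI.
; Overlapping enemies show their widgets, and cursor shape follows mouse drag state.
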(event Custom|scrollArm
  ;[1 1 1] On Tick Events
  (bind _output_get (|UpdateLength))
  (|UpdateAngle _output_get
    (:out
      (|UpdateVelocity))))

(event Custom|Rotate
  ;[1 1 1] On Tick Events
  (Utilities|FlowControl|Sequence
    (:then_0
      (if (Variables|ButtonBools|GetholdE)
        (|IncRotationSpeed)
        (elif (Variables|ButtonBools|GetholdQ)
          (|DecRotationSpeed))))
    (:then_1
      (|UpdateRotation)
      (|MoveRotationSpeedto0))))

(event Custom|Move
  (Pawn|Input|AddMovementInput (+ (* (Math|Vector|GetForwardVector (Variables|Collision|GetCapsuleComponent)) (Variables|Camera|GetForwards)) (* (Math|Vector|GetRightVector (Variables|Collision|GetCapsuleComponent)) (Variables|Camera|GetSideways))) 1.0 false))

(event EventBeginPlay
  (bind _returnvalue (Game|GetPlayerController 0))
  (CallFunction|CreateStartScreen)
  (Pawn|Components|CharacterMovement|SetMovementMode (Variables|Character|GetCharacterMovement) "MOVE_Flying" 0)
  (Transformation|SetRelativeRotation (Variables|Camera|GetSpringArm) (Math|Rotator|MakeRotator 0.0 (Variables|Camera|GetCameraAngle) 0.0) false false)
  (Variables|/Script/Engine.PlayerController|SetbShowMouseCursor _returnvalue true)
  (Input|SetInputModeGameandUI _returnvalue 0 "DoNotLock" false)
  (Variables|/Script/Engine.SpringArmComponent|SetTargetArmLength (Variables|Camera|GetSpringArm) (Variables|Camera|GetMinArmLength))
  (Transformation|SetActorLocation "0, 0,300.000000" false false))

(event Collision|EventActorBeginOverlap
  (params (OtherActor :type Actor%20Object%20Reference))
  (bind _astd_enemy_base (Utilities|Casting|CastToTD_enemy_base OtherActor))
  (Rendering|SetVisibility (Variables|/Game/Blueprints/Mobs/TD_enemy_base.TD_enemy_base_C|GetWidget _astd_enemy_base) true true))

(event EventTick
  (params (DeltaSeconds :type Float%20%28single-precision%29))
  (CallFunction|Move)
  (CallFunction|Rotate)
  (CallFunction|ScrollArm))

(event Collision|EventActorEndOverlap
  (params (OtherActor :type Actor%20Object%20Reference))
  (bind _astd_enemy_base (Utilities|Casting|CastToTD_enemy_base OtherActor))
  (Rendering|SetVisibility (Variables|/Game/Blueprints/Mobs/TD_enemy_base.TD_enemy_base_C|GetWidget _astd_enemy_base) false true))

(event Input|MouseEvents|MouseWheelAxis
  (params (AxisValue :type Float%20%28single-precision%29))
  ;[1 1 1] Mouse and Key Events
  (|AddVelocity AxisValue))

(event Input|MouseEvents|MouseX
  (params (AxisValue :type Float%20%28single-precision%29))
  ;[1 1 1] Mouse and Key Events
  (if (Variables|ButtonBools|GetholdRightMouse)
    (Variables|Camera|SetRotationSpeed (Math|Float|Clamp(Float) (+ (Variables|Camera|GetRotationSpeed) (* AxisValue 1.0)) (Variables|Camera|GetMinRotationSpeed) (Variables|Camera|GetMaxRotationSpeed)))))

(event Input|MouseEvents|MouseY
  (params (AxisValue :type Float%20%28single-precision%29))
  ;[1 1 1] Mouse and Key Events
  (if (Variables|ButtonBools|GetmouseWheelDown)
    (Variables|Camera|SetArmLengthVelocity (+ (* AxisValue -1.5 (Variables|Camera|GetZoomScalar)) (Variables|Camera|GetArmLengthVelocity)))))

(event Input|KeyboardEvents|W
  (params (Key :type Key%20Structure))
  ;[1 1 1] Mouse and Key Events
  (:Pressed
    (Variables|Camera|SetForwards 1.0))
  (:Released
    (Variables|Camera|SetForwards 0.0)))

(event Input|KeyboardEvents|A
  (params (Key :type Key%20Structure))
  ;[1 1 1] Mouse and Key Events
  (:Pressed
    (Variables|Camera|SetSideways -1.0))
  (:Released
    (Variables|Camera|SetSideways 0.0)))

(event Input|KeyboardEvents|S
  (params (Key :type Key%20Structure))
  ;[1 1 1] Mouse and Key Events
  (:Pressed
    (Variables|Camera|SetForwards -1.0))
  (:Released
    (Variables|Camera|SetForwards 0.0)))

(event Input|KeyboardEvents|D
  (params (Key :type Key%20Structure))
  ;[1 1 1] Mouse and Key Events
  (:Pressed
    (Variables|Camera|SetSideways 1.0))
  (:Released
    (Variables|Camera|SetSideways 0.0)))

(event Input|KeyboardEvents|Q
  (params (Key :type Key%20Structure))
  ;[1 1 1] Mouse and Key Events
  (:Pressed
    (Variables|ButtonBools|SetholdQ true))
  (:Released
    (Variables|ButtonBools|SetholdQ false)))

(event Input|KeyboardEvents|E
  (params (Key :type Key%20Structure))
  ;[1 1 1] Mouse and Key Events
  (:Pressed
    (Variables|ButtonBools|SetholdE true))
  (:Released
    (Variables|ButtonBools|SetholdE false)))

(event Input|MouseEvents|LeftMouseButton
  (params (Key :type Key%20Structure))
  (bind _charactertowerplayercomponent (Variables|Default|GetCharacterTowerPlayerComponent))
  ;[1 1 1] Mouse and Key Events
  (:Released
    (if (Variables|/Game/Blueprints/Player/CharacterTowerPlacerComponent.CharacterTowerPlacerComponent_C|GetbMapBuilder _charactertowerplayercomponent)
      (Default|TileInteractionInternal _charactertowerplayercomponent)
      (else
        (CallFunction|SelectObject)))))

(event Input|MouseEvents|RightMouseButton
  (params (Key :type Key%20Structure))
  ;[1 1 1] Mouse and Key Events
  (:Pressed
    (Variables|ButtonBools|SetholdRightMouse true)
    (CallFunction|CursorTypeHandler :!label _label))
  (:Released
    (Variables|ButtonBools|SetholdRightMouse false)
    (goto _label)))

(event Input|MouseEvents|MiddleMouseButton
  (params (Key :type Key%20Structure))
  ;[1 1 1] Mouse and Key Events
  (:Pressed
    (Variables|ButtonBools|SetmouseWheelDown true)
    (CallFunction|CursorTypeHandler :!label _label))
  (:Released
    (Variables|ButtonBools|SetmouseWheelDown false)
    (goto _label)))

(event Input|MouseEvents|Mouse2D
  (params (AxisValue :type Vector :default "0, 0, 0"))
  ;[1 1 1] Mouse and Key Events
)

(fn ConstructionScript)

(fn CursorTypeHandler
  (bind _returnvalue (Game|GetPlayerController 0))
  (if (Variables|TowerPlacing|GetplaceTower)
    (Variables|/Script/Engine.PlayerController|SetCurrentMouseCursor _returnvalue "None")
    (elif (Variables|ButtonBools|GetholdLeftMouse)
      (Variables|/Script/Engine.PlayerController|SetCurrentMouseCursor _returnvalue "GrabHandClosed")
      (elif (Variables|ButtonBools|GetholdRightMouse)
        (Variables|/Script/Engine.PlayerController|SetCurrentMouseCursor _returnvalue "ResizeLeftRight")
        (elif (Variables|ButtonBools|GetmouseWheelDown)
          (Variables|/Script/Engine.PlayerController|SetCurrentMouseCursor _returnvalue "ResizeUpDown")
          (else
            (Variables|/Script/Engine.PlayerController|SetCurrentMouseCursor _returnvalue "GrabHand")))))))

(fn InitTowerList
  (bind _returnvalue (UserInterface|CreateWidget "/Game/Blueprints/Player/UI/TowerPlacerUI.TowerPlacerUI_C" (Game|GetPlayerController 0)))
  (bind _output_get (Variables|TowerPlacing|SetTowerPlacerUI _returnvalue))
  (UserInterface|Viewport|AddtoPlayerScreen _output_get)
  (Variables|TowerPlacing|SetTower%20List%20View (Variables|/Game/Blueprints/Player/UI/TowerPlacerUI.TowerPlacerUI_C|GetTowerListView _output_get))
  (bind _returnvalue_2 (Game|ConstructObjectfromClass "/Game/Blueprints/Building/Tower/TowerTypeData.TowerTypeData_C"))
  (bind _output_get_2 (Variables|Default|SetTowerTypeData _returnvalue_2))
  (Default|InitData _output_get_2)
  (for _array_element (Variables|TowerPlacing|GetavailableTowers)
    (bind _newparam (Default|GetTowerDatafromEnum (Variables|Default|GetTowerTypeData) _array_element))
    (Class|ListView|AddItem (Variables|TowerPlacing|GetTower%20List%20View) _newparam)))

(fn EnsurePlacerActive
  (bind _charactertowerplayercomponent (Variables|Default|GetCharacterTowerPlayerComponent))
  (if (not (Variables|/Game/Blueprints/Player/CharacterTowerPlacerComponent.CharacterTowerPlacerComponent_C|GetbMapBuilder _charactertowerplayercomponent))
    (Default|ActivateGridBuilderMode _charactertowerplayercomponent)))

(fn SelectObject
  (bind _returnvalue (Game|GetPlayerController 0))
  (bind _hitresult (Game|Player|GetHitResultUnderCursorbyChannel _returnvalue "TraceTypeQuery5" false))
  (bind (_bblockinghit _binitialoverlap _time _distance _location _impactpoint _normal _impactnormal _physmat _hitactor) (Collision|BreakHitResult _hitresult))
  (Variables|TowerPlacing|GetTowerPlacerUI
    (:then
      (bind _selectedobject (Variables|Default|GetSelectedObject)
        (:then
          (bind _asbase_tower (Utilities|Casting|CastToBaseTower _selectedobject)
            (:then
              (Default|ToggleRangeIndicator _asbase_tower false))
            (:CastFailed
              _)))
        (:else
          _))
      (if _bblockinghit
        (bind _asbase_tower_2 (Utilities|Casting|CastToBaseTower _hitactor)
          (:then
            (Default|ToggleRangeIndicator _asbase_tower_2 true)
            (Variables|Default|SetSelectedObject _asbase_tower_2)
            (Default|TowerSelected (Variables|TowerPlacing|GetTowerPlacerUI) _asbase_tower_2))
          (:CastFailed
            (Variables|Default|SetSelectedObject 0 :!label _label)
            (Default|ChangetoHoverView (Variables|TowerPlacing|GetTowerPlacerUI))))
        (else
          (Development|PrintString "Hello")
          (goto _label))))
    (:else)))

(fn CreateStartScreen
  (bind _returnvalue (UserInterface|CreateWidget "/Game/Blueprints/Player/UI/StartScreen.StartScreen_C" (Game|GetPlayerController 0)))
  (bind _output_get (Variables|Default|SetStartScreen _returnvalue))
  (UserInterface|Viewport|AddtoPlayerScreen _output_get))

(fn StartGame
  (Widget|SetVisibility (Variables|Default|GetStartScreen) "Collapsed")
  (CallFunction|InitTowerList))