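; BP_HexDefenseCamera is the player camera for the hex tower defense game, moved through an RTSCamera component.
; On begin play it applies CameraSpeed to that component and binds to the time dilation change event of GS_TowerDefense.
; Each change divides CameraSpeed by the global time dilation, so camera movement keeps the same real-time speed when game speed changes.
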(event Custom|UpdateCameraSpeed
  (Variables|/Script/OpenRTSCamera.RTSCamera|SetMoveSpeed (Variables|Default|GetRTSCamera) (/ (Variables|Default|GetCameraSpeed) (Class|GameplayStatics|GetGlobalTimeDilation))))

(event EventBeginPlay
  (Variables|/Script/OpenRTSCamera.RTSCamera|SetMoveSpeed (Variables|Default|GetRTSCamera) (Variables|Default|GetCameraSpeed))
  (bind _asgs_tower_defense (Utilities|Casting|CastToGS_TowerDefense (Game|GetGameState)))
  (EventDispatchers|BindEventtoTimeDilationChanged _asgs_tower_defense (delegate Custom|UpdateCameraSpeed)))

(fn ConstructionScript
  (|CallParentFunction))