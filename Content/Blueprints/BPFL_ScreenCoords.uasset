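; Blueprint function library for off-screen indicators, placing a marker at the screen edge toward a world location.
; GetScreenEdgeCoords projects a point just ahead of the deprojected view center toward the target, then scales that direction to the edge by Margin, returning DPI-adjusted coordinates and an angle.
; IsLocationOnScreen tests whether a location projects inside the visible area.
; Both exclude the side selectables panel and input bar, using UIStyle sizes from GI_HexDefense.
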(fn GetScreenEdgeCoords
  (params (TargetLocation :type Vector) (Margin :type Float%20%28double-precision%29))
  (bind _returnvalue (Game|GetPlayerController 0))
  (bind _returnvalue_2 (Class|WidgetLayoutLibrary|GetViewportScale))
  (bind (_sizex _sizey) (HUD|GetViewportSize _returnvalue))
  (bind _asgi_hex_defense (Utilities|Casting|CastToGI_HexDefense (Game|GetGameInstance)))
  (LocalVariables|SetMarginValue Margin)
  (LocalVariables|SetHalfScreenWidth (* (- _sizex (Variables|/Game/Blueprints/UI/Styles/DA_Style.DA_Style_C|GetSelectablesWidthMinusSrollBar (Variables|/Game/Blueprints/GM/GI_HexDefense.GI_HexDefense_C|GetUIStyle _asgi_hex_defense))) 0.5))
  (LocalVariables|SetHalfScreenHeight (* (- _sizey (Variables|/Game/Blueprints/UI/Styles/DA_Style.DA_Style_C|GetInputBarHeight (Variables|/Game/Blueprints/GM/GI_HexDefense.GI_HexDefense_C|GetUIStyle _asgi_hex_defense))) 0.5))
  (return (Math|Vector2D|MakeVector2D (+ (* (* (/ (- (.x (.ScreenLocation (Class|PlayerController|ProjectWorldLocationtoScreen _returnvalue (+ (Math|Vector|GetForwardVector (Math|Rotator|FindLookatRotation (+ (.WorldLocation (Class|PlayerController|DeprojectScreenPositiontoWorld _returnvalue (* (- _sizex (Variables|/Game/Blueprints/UI/Styles/DA_Style.DA_Style_C|GetSelectablesWidthMinusSrollBar (Variables|/Game/Blueprints/GM/GI_HexDefense.GI_HexDefense_C|GetUIStyle _asgi_hex_defense))) 0.5) (* (- _sizey (Variables|/Game/Blueprints/UI/Styles/DA_Style.DA_Style_C|GetInputBarHeight (Variables|/Game/Blueprints/GM/GI_HexDefense.GI_HexDefense_C|GetUIStyle _asgi_hex_defense))) 0.5))) (* (.WorldDirection (Class|PlayerController|DeprojectScreenPositiontoWorld _returnvalue (* (- _sizex (Variables|/Game/Blueprints/UI/Styles/DA_Style.DA_Style_C|GetSelectablesWidthMinusSrollBar (Variables|/Game/Blueprints/GM/GI_HexDefense.GI_HexDefense_C|GetUIStyle _asgi_hex_defense))) 0.5) (* (- _sizey (Variables|/Game/Blueprints/UI/Styles/DA_Style.DA_Style_C|GetInputBarHeight (Variables|/Game/Blueprints/GM/GI_HexDefense.GI_HexDefense_C|GetUIStyle _asgi_hex_defense))) 0.5))) 1e+01)) TargetLocation)) (+ (.WorldLocation (Class|PlayerController|DeprojectScreenPositiontoWorld _returnvalue (* (- _sizex (Variables|/Game/Blueprints/UI/Styles/DA_Style.DA_Style_C|GetSelectablesWidthMinusSrollBar (Variables|/Game/Blueprints/GM/GI_HexDefense.GI_HexDefense_C|GetUIStyle _asgi_hex_defense))) 0.5) (* (- _sizey (Variables|/Game/Blueprints/UI/Styles/DA_Style.DA_Style_C|GetInputBarHeight (Variables|/Game/Blueprints/GM/GI_HexDefense.GI_HexDefense_C|GetUIStyle _asgi_hex_defense))) 0.5))) (* (.WorldDirection (Class|PlayerController|DeprojectScreenPositiontoWorld _returnvalue (* (- _sizex (Variables|/Game/Blueprints/UI/Styles/DA_Style.DA_Style_C|GetSelectablesWidthMinusSrollBar (Variables|/Game/Blueprints/GM/GI_HexDefense.GI_HexDefense_C|GetUIStyle _asgi_hex_defense))) 0.5) (* (- _sizey (Variables|/Game/Blueprints/UI/Styles/DA_Style.DA_Style_C|GetInputBarHeight (Variables|/Game/Blueprints/GM/GI_HexDefense.GI_HexDefense_C|GetUIStyle _asgi_hex_defense))) 0.5))) 1e+01))) false))) (LocalVariables|GetHalfScreenWidth)) (Math|Float|Absolute(Float) (+ (- (.x (.ScreenLocation (Class|PlayerController|ProjectWorldLocationtoScreen _returnvalue (+ (Math|Vector|GetForwardVector (Math|Rotator|FindLookatRotation (+ (.WorldLocation (Class|PlayerController|DeprojectScreenPositiontoWorld _returnvalue (* (- _sizex (Variables|/Game/Blueprints/UI/Styles/DA_Style.DA_Style_C|GetSelectablesWidthMinusSrollBar (Variables|/Game/Blueprints/GM/GI_HexDefense.GI_HexDefense_C|GetUIStyle _asgi_hex_defense))) 0.5) (* (- _sizey (Variables|/Game/Blueprints/UI/Styles/DA_Style.DA_Style_C|GetInputBarHeight (Variables|/Game/Blueprints/GM/GI_HexDefense.GI_HexDefense_C|GetUIStyle _asgi_hex_defense))) 0.5))) (* (.WorldDirection (Class|PlayerController|DeprojectScreenPositiontoWorld _returnvalue (* (- _sizex (Variables|/Game/Blueprints/UI/Styles/DA_Style.DA_Style_C|GetSelectablesWidthMinusSrollBar (Variables|/Game/Blueprints/GM/GI_HexDefense.GI_HexDefense_C|GetUIStyle _asgi_hex_defense))) 0.5) (* (- _sizey (Variables|/Game/Blueprints/UI/Styles/DA_Style.DA_Style_C|GetInputBarHeight (Variables|/Game/Blueprints/GM/GI_HexDefense.GI_HexDefense_C|GetUIStyle _asgi_hex_defense))) 0.5))) 1e+01)) TargetLocation)) (+ (.WorldLocation (Class|PlayerController|DeprojectScreenPositiontoWorld _returnvalue (* (- _sizex (Variables|/Game/Blueprints/UI/Styles/DA_Style.DA_Style_C|GetSelectablesWidthMinusSrollBar (Variables|/Game/Blueprints/GM/GI_HexDefense.GI_HexDefense_C|GetUIStyle _asgi_hex_defense))) 0.5) (* (- _sizey (Variables|/Game/Blueprints/UI/Styles/DA_Style.DA_Style_C|GetInputBarHeight (Variables|/Game/Blueprints/GM/GI_HexDefense.GI_HexDefense_C|GetUIStyle _asgi_hex_defense))) 0.5))) (* (.WorldDirection (Class|PlayerController|DeprojectScreenPositiontoWorld _returnvalue (* (- _sizex (Variables|/Game/Blueprints/UI/Styles/DA_Style.DA_Style_C|GetSelectablesWidthMinusSrollBar (Variables|/Game/Blueprints/GM/GI_HexDefense.GI_HexDefense_C|GetUIStyle _asgi_hex_defense))) 0.5) (* (- _sizey (Variables|/Game/Blueprints/UI/Styles/DA_Style.DA_Style_C|GetInputBarHeight (Variables|/Game/Blueprints/GM/GI_HexDefense.GI_HexDefense_C|GetUIStyle _asgi_hex_defense))) 0.5))) 1e+01))) false))) (LocalVariables|GetHalfScreenWidth)) (- (.y (.ScreenLocation (Class|PlayerController|ProjectWorldLocationtoScreen _returnvalue (+ (Math|Vector|GetForwardVector (Math|Rotator|FindLookatRotation (+ (.WorldLocation (Class|PlayerController|DeprojectScreenPositiontoWorld _returnvalue (* (- _sizex (Variables|/Game/Blueprints/UI/Styles/DA_Style.DA_Style_C|GetSelectablesWidthMinusSrollBar (Variables|/Game/Blueprints/GM/GI_HexDefense.GI_HexDefense_C|GetUIStyle _asgi_hex_defense))) 0.5) (* (- _sizey (Variables|/Game/Blueprints/UI/Styles/DA_Style.DA_Style_C|GetInputBarHeight (Variables|/Game/Blueprints/GM/GI_HexDefense.GI_HexDefense_C|GetUIStyle _asgi_hex_defense))) 0.5))) (* (.WorldDirection (Class|PlayerController|DeprojectScreenPositiontoWorld _returnvalue (* (- _sizex (Variables|/Game/Blueprints/UI/Styles/DA_Style.DA_Style_C|GetSelectablesWidthMinusSrollBar (Variables|/Game/Blueprints/GM/GI_HexDefense.GI_HexDefense_C|GetUIStyle _asgi_hex_defense))) 0.5) (* (- _sizey (Variables|/Game/Blueprints/UI/Styles/DA_Style.DA_Style_C|GetInputBarHeight (Variables|/Game/Blueprints/GM/GI_HexDefense.GI_HexDefense_C|GetUIStyle _asgi_hex_defense))) 0.5))) 1e+01)) TargetLocation)) (+ (.WorldLocation (Class|PlayerController|DeprojectScreenPositiontoWorld _returnvalue (* (- _sizex (Variables|/Game/Blueprints/UI/Styles/DA_Style.DA_Style_C|GetSelectablesWidthMinusSrollBar (Variables|/Game/Blueprints/GM/GI_HexDefense.GI_HexDefense_C|GetUIStyle _asgi_hex_defense))) 0.5) (* (- _sizey (Variables|/Game/Blueprints/UI/Styles/DA_Style.DA_Style_C|GetInputBarHeight (Variables|/Game/Blueprints/GM/GI_HexDefense.GI_HexDefense_C|GetUIStyle _asgi_hex_defense))) 0.5))) (* (.WorldDirection (Class|PlayerController|DeprojectScreenPositiontoWorld _returnvalue (* (- _sizex (Variables|/Game/Blueprints/UI/Styles/DA_Style.DA_Style_C|GetSelectablesWidthMinusSrollBar (Variables|/Game/Blueprints/GM/GI_HexDefense.GI_HexDefense_C|GetUIStyle _asgi_hex_defense))) 0.5) (* (- _sizey (Variables|/Game/Blueprints/UI/Styles/DA_Style.DA_Style_C|GetInputBarHeight (Variables|/Game/Blueprints/GM/GI_HexDefense.GI_HexDefense_C|GetUIStyle _asgi_hex_defense))) 0.5))) 1e+01))) false))) (LocalVariables|GetHalfScreenHeight))))) (Math|Float|Min(Float) (Math|Float|Absolute(Float) (/ (LocalVariables|GetHalfScreenWidth) (/ (- (.x (.ScreenLocation (Class|PlayerController|ProjectWorldLocationtoScreen _returnvalue (+ (Math|Vector|GetForwardVector (Math|Rotator|FindLookatRotation (+ (.WorldLocation (Class|PlayerController|DeprojectScreenPositiontoWorld _returnvalue (* (- _sizex (Variables|/Game/Blueprints/UI/Styles/DA_Style.DA_Style_C|GetSelectablesWidthMinusSrollBar (Variables|/Game/Blueprints/GM/GI_HexDefense.GI_HexDefense_C|GetUIStyle _asgi_hex_defense))) 0.5) (* (- _sizey (Variables|/Game/Blueprints/UI/Styles/DA_Style.DA_Style_C|GetInputBarHeight (Variables|/Game/Blueprints/GM/GI_HexDefense.GI_HexDefense_C|GetUIStyle _asgi_hex_defense))) 0.5))) (* (.WorldDirection (Class|PlayerController|DeprojectScreenPositiontoWorld _returnvalue (* (- _sizex (Variables|/Game/Blueprints/UI/Styles/DA_Style.DA_Style_C|GetSelectablesWidthMinusSrollBar (Variables|/Game/Blueprints/GM/GI_HexDefense.GI_HexDefense_C|GetUIStyle _asgi_hex_defense))) 0.5) (* (- _sizey (Variables|/Game/Blueprints/UI/Styles/DA_Style.DA_Style_C|GetInputBarHeight (Variables|/Game/Blueprints/GM/GI_HexDefense.GI_HexDefense_C|GetUIStyle _asgi_hex_defense))) 0.5))) 1e+01)) TargetLocation)) (+ (.WorldLocation (Class|PlayerController|DeprojectScreenPositiontoWorld _returnvalue (* (- _sizex (Variables|/Game/Blueprints/UI/Styles/DA_Style.DA_Style_C|GetSelectablesWidthMinusSrollBar (Variables|/Game/Blueprints/GM/GI_HexDefense.GI_HexDefense_C|GetUIStyle _asgi_hex_defense))) 0.5) (* (- _sizey (Variables|/Game/Blueprints/UI/Styles/DA_Style.DA_Style_C|GetInputBarHeight (Variables|/Game/Blueprints/GM/GI_HexDefense.GI_HexDefense_C|GetUIStyle _asgi_hex_defense))) 0.5))) (* (.WorldDirection (Class|PlayerController|DeprojectScreenPositiontoWorld _returnvalue (* (- _sizex (Variables|/Game/Blueprints/UI/Styles/DA_Style.DA_Style_C|GetSelectablesWidthMinusSrollBar (Variables|/Game/Blueprints/GM/GI_HexDefense.GI_HexDefense_C|GetUIStyle _asgi_hex_defense))) 0.5) (* (- _sizey (Variables|/Game/Blueprints/UI/Styles/DA_Style.DA_Style_C|GetInputBarHeight (Variables|/Game/Blueprints/GM/GI_HexDefense.GI_HexDefense_C|GetUIStyle _asgi_hex_defense))) 0.5))) 1e+01))) false))) (LocalVariables|GetHalfScreenWidth)) (Math|Float|Absolute(Float) (+ (- (.x (.ScreenLocation (Class|PlayerController|ProjectWorldLocationtoScreen _returnvalue (+ (Math|Vector|GetForwardVector (Math|Rotator|FindLookatRotation (+ (.WorldLocation (Class|PlayerController|DeprojectScreenPositiontoWorld _returnvalue (* (- _sizex (Variables|/Game/Blueprints/UI/Styles/DA_Style.DA_Style_C|GetSelectablesWidthMinusSrollBar (Variables|/Game/Blueprints/GM/GI_HexDefense.GI_HexDefense_C|GetUIStyle _asgi_hex_defense))) 0.5) (* (- _sizey (Variables|/Game/Blueprints/UI/Styles/DA_Style.DA_Style_C|GetInputBarHeight (Variables|/Game/Blueprints/GM/GI_HexDefense.GI_HexDefense_C|GetUIStyle _asgi_hex_defense))) 0.5))) (* (.WorldDirection (Class|PlayerController|DeprojectScreenPositiontoWorld _returnvalue (* (- _sizex (Variables|/Game/Blueprints/UI/Styles/DA_Style.DA_Style_C|GetSelectablesWidthMinusSrollBar (Variables|/Game/Blueprints/GM/GI_HexDefense.GI_HexDefense_C|GetUIStyle _asgi_hex_defense))) 0.5) (* (- _sizey (Variables|/Game/Blueprints/UI/Styles/DA_Style.DA_Style_C|GetInputBarHeight (Variables|/Game/Blueprints/GM/GI_HexDefense.GI_HexDefense_C|GetUIStyle _asgi_hex_defense))) 0.5))) 1e+01)) TargetLocation)) (+ (.WorldLocation (Class|PlayerController|DeprojectScreenPositiontoWorld _returnvalue (* (- _sizex (Variables|/Game/Blueprints/UI/Styles/DA_Style.DA_Style_C|GetSelectablesWidthMinusSrollBar (Variables|/Game/Blueprints/GM/GI_HexDefense.GI_HexDefense_C|GetUIStyle _asgi_hex_defense))) 0.5) (* (- _sizey (Variables|/Game/Blueprints/UI/Styles/DA_Style.DA_Style_C|GetInputBarHeight (Variables|/Game/Blueprints/GM/GI_HexDefense.GI_HexDefense_C|GetUIStyle _asgi_hex_defense))) 0.5))) (* (.WorldDirection (Class|PlayerController|DeprojectScreenPositiontoWorld _returnvalue (* (- _sizex (Variables|/Game/Blueprints/UI/Styles/DA_Style.DA_Style_C|GetSelectablesWidthMinusSrollBar (Variables|/Game/Blueprints/GM/GI_HexDefense.GI_HexDefense_C|GetUIStyle _asgi_hex_defense))) 0.5) (* (- _sizey (Variables|/Game/Blueprints/UI/Styles/DA_Style.DA_Style_C|GetInputBarHeight (Variables|/Game/Blueprints/GM/GI_HexDefense.GI_HexDefense_C|GetUIStyle _asgi_hex_defense))) 0.5))) 1e+01))) false))) (LocalVariables|GetHalfScreenWidth)) (- (.y (.ScreenLocation (Class|PlayerController|ProjectWorldLocationtoScreen _returnvalue (+ (Math|Vector|GetForwardVector (Math|Rotator|FindLookatRotation (+ (.WorldLocation (Class|PlayerController|DeprojectScreenPositiontoWorld _returnvalue (* (- _sizex (Variables|/Game/Blueprints/UI/Styles/DA_Style.DA_Style_C|GetSelectablesWidthMinusSrollBar (Variables|/Game/Blueprints/GM/GI_HexDefense.GI_HexDefense_C|GetUIStyle _asgi_hex_defense))) 0.5) (* (- _sizey (Variables|/Game/Blueprints/UI/Styles/DA_Style.DA_Style_C|GetInputBarHeight (Variables|/Game/Blueprints/GM/GI_HexDefense.GI_HexDefense_C|GetUIStyle _asgi_hex_defense))) 0.5))) (* (.WorldDirection (Class|PlayerController|DeprojectScreenPositiontoWorld _returnvalue (* (- _sizex (Variables|/Game/Blueprints/UI/Styles/DA_Style.DA_Style_C|GetSelectablesWidthMinusSrollBar (Variables|/Game/Blueprints/GM/GI_HexDefense.GI_HexDefense_C|GetUIStyle _asgi_hex_defense))) 0.5) (* (- _sizey (Variables|/Game/Blueprints/UI/Styles/DA_Style.DA_Style_C|GetInputBarHeight (Variables|/Game/Blueprints/GM/GI_HexDefense.GI_HexDefense_C|GetUIStyle _asgi_hex_defense))) 0.5))) 1e+01)) TargetLocation)) (+ (.WorldLocation (Class|PlayerController|DeprojectScreenPositiontoWorld _returnvalue (* (- _sizex (Variables|/Game/Blueprints/UI/Styles/DA_Style.DA_Style_C|GetSelectablesWidthMinusSrollBar (Variables|/Game/Blueprints/GM/GI_HexDefense.GI_HexDefense_C|GetUIStyle _asgi_hex_defense))) 0.5) (* (- _sizey (Variables|/Game/Blueprints/UI/Styles/DA_Style.DA_Style_C|GetInputBarHeight (Variables|/Game/Blueprints/GM/GI_HexDefense.GI_HexDefense_C|GetUIStyle _asgi_hex_defense))) 0.5))) (* (.WorldDirection (Class|PlayerController|DeprojectScreenPositiontoWorld _returnvalue (* (- _sizex (Variables|/Game/Blueprints/UI/Styles/DA_Style.DA_Style_C|GetSelectablesWidthMinusSrollBar (Variables|/Game/Blueprints/GM/GI_HexDefense.GI_HexDefense_C|GetUIStyle _asgi_hex_defense))) 0.5) (* (- _sizey (Variables|/Game/Blueprints/UI/Styles/DA_Style.DA_Style_C|GetInputBarHeight (Variables|/Game/Blueprints/GM/GI_HexDefense.GI_HexDefense_C|GetUIStyle _asgi_hex_defense))) 0.5))) 1e+01))) false))) (LocalVariables|GetHalfScreenHeight))))))) (Math|Float|Absolute(Float) (/ (LocalVariables|GetHalfScreenHeight) (/ (- (.y (.ScreenLocation (Class|PlayerController|ProjectWorldLocationtoScreen _returnvalue (+ (Math|Vector|GetForwardVector (Math|Rotator|FindLookatRotation (+ (.WorldLocation (Class|PlayerController|DeprojectScreenPositiontoWorld _returnvalue (* (- _sizex (Variables|/Game/Blueprints/UI/Styles/DA_Style.DA_Style_C|GetSelectablesWidthMinusSrollBar (Variables|/Game/Blueprints/GM/GI_HexDefense.GI_HexDefense_C|GetUIStyle _asgi_hex_defense))) 0.5) (* (- _sizey (Variables|/Game/Blueprints/UI/Styles/DA_Style.DA_Style_C|GetInputBarHeight (Variables|/Game/Blueprints/GM/GI_HexDefense.GI_HexDefense_C|GetUIStyle _asgi_hex_defense))) 0.5))) (* (.WorldDirection (Class|PlayerController|DeprojectScreenPositiontoWorld _returnvalue (* (- _sizex (Variables|/Game/Blueprints/UI/Styles/DA_Style.DA_Style_C|GetSelectablesWidthMinusSrollBar (Variables|/Game/Blueprints/GM/GI_HexDefense.GI_HexDefense_C|GetUIStyle _asgi_hex_defense))) 0.5) (* (- _sizey (Variables|/Game/Blueprints/UI/Styles/DA_Style.DA_Style_C|GetInputBarHeight (Variables|/Game/Blueprints/GM/GI_HexDefense.GI_HexDefense_C|GetUIStyle _asgi_hex_defense))) 0.5))) 1e+01)) TargetLocation)) (+ (.WorldLocation (Class|PlayerController|DeprojectScreenPositiontoWorld _returnvalue (* (- _sizex (Variables|/Game/Blueprints/UI/Styles/DA_Style.DA_Style_C|GetSelectablesWidthMinusSrollBar (Variables|/Game/Blueprints/GM/GI_HexDefense.GI_HexDefense_C|GetUIStyle _asgi_hex_defense))) 0.5) (* (- _sizey (Variables|/Game/Blueprints/UI/Styles/DA_Style.DA_Style_C|GetInputBarHeight (Variables|/Game/Blueprints/GM/GI_HexDefense.GI_HexDefense_C|GetUIStyle _asgi_hex_defense))) 0.5))) (* (.WorldDirection (Class|PlayerController|DeprojectScreenPositiontoWorld _returnvalue (* (- _sizex (Variables|/Game/Blueprints/UI/Styles/DA_Style.DA_Style_C|GetSelectablesWidthMinusSrollBar (Variables|/Game/Blueprints/GM/GI_HexDefense.GI_HexDefense_C|GetUIStyle _asgi_hex_defense))) 0.5) (* (- _sizey (Variables|/Game/Blueprints/UI/Styles/DA_Style.DA_Style_C|GetInputBarHeight (Variables|/Game/Blueprints/GM/GI_HexDefense.GI_HexDefense_C|GetUIStyle _asgi_hex_defense))) 0.5))) 1e+01))) false))) (LocalVariables|GetHalfScreenHeight)) (Math|Float|Absolute(Float) (+ (- (.x (.ScreenLocation (Class|PlayerController|ProjectWorldLocationtoScreen _returnvalue (+ (Math|Vector|GetForwardVector (Math|Rotator|FindLookatRotation (+ (.WorldLocation (Class|PlayerController|DeprojectScreenPositiontoWorld _returnvalue (* (- _sizex (Variables|/Game/Blueprints/UI/Styles/DA_Style.DA_Style_C|GetSelectablesWidthMinusSrollBar (Variables|/Game/Blueprints/GM/GI_HexDefense.GI_HexDefense_C|GetUIStyle _asgi_hex_defense))) 0.5) (* (- _sizey (Variables|/Game/Blueprints/UI/Styles/DA_Style.DA_Style_C|GetInputBarHeight (Variables|/Game/Blueprints/GM/GI_HexDefense.GI_HexDefense_C|GetUIStyle _asgi_hex_defense))) 0.5))) (* (.WorldDirection (Class|PlayerController|DeprojectScreenPositiontoWorld _returnvalue (* (- _sizex (Variables|/Game/Blueprints/UI/Styles/DA_Style.DA_Style_C|GetSelectablesWidthMinusSrollBar (Variables|/Game/Blueprints/GM/GI_HexDefense.GI_HexDefense_C|GetUIStyle _asgi_hex_defense))) 0.5) (* (- _sizey (Variables|/Game/Blueprints/UI/Styles/DA_Style.DA_Style_C|GetInputBarHeight (Variables|/Game/Blueprints/GM/GI_HexDefense.GI_HexDefense_C|GetUIStyle _asgi_hex_defense))) 0.5))) 1e+01)) TargetLocation)) (+ (.WorldLocation (Class|PlayerController|DeprojectScreenPositiontoWorld _returnvalue (* (- _sizex (Variables|/Game/Blueprints/UI/Styles/DA_Style.DA_Style_C|GetSelectablesWidthMinusSrollBar (Variables|/Game/Blueprints/GM/GI_HexDefense.GI_HexDefense_C|GetUIStyle _asgi_hex_defense))) 0.5) (* (- _sizey (Variables|/Game/Blueprints/UI/Styles/DA_Style.DA_Style_C|GetInputBarHeight (Variables|/Game/Blueprints/GM/GI_HexDefense.GI_HexDefense_C|GetUIStyle _asgi_hex_defense))) 0.5))) (* (.WorldDirection (Class|PlayerController|DeprojectScreenPositiontoWorld _returnvalue (* (- _sizex (Variables|/Game/Blueprints/UI/Styles/DA_Style.DA_Style_C|GetSelectablesWidthMinusSrollBar (Variables|/Game/Blueprints/GM/GI_HexDefense.GI_HexDefense_C|GetUIStyle _asgi_hex_defense))) 0.5) (* (- _sizey (Variables|/Game/Blueprints/UI/Styles/DA_Style.DA_Style_C|GetInputBarHeight (Variables|/Game/Blueprints/GM/GI_HexDefense.GI_HexDefense_C|GetUIStyle _asgi_hex_defense))) 0.5))) 1e+01))) false))) (LocalVariables|GetHalfScreenWidth)) (- (.y (.ScreenLocation (Class|PlayerController|ProjectWorldLocationtoScreen _returnvalue (+ (Math|Vector|GetForwardVector (Math|Rotator|FindLookatRotation (+ (.WorldLocation (Class|PlayerController|DeprojectScreenPositiontoWorld _returnvalue (* (- _sizex (Variables|/Game/Blueprints/UI/Styles/DA_Style.DA_Style_C|GetSelectablesWidthMinusSrollBar (Variables|/Game/Blueprints/GM/GI_HexDefense.GI_HexDefense_C|GetUIStyle _asgi_hex_defense))) 0.5) (* (- _sizey (Variables|/Game/Blueprints/UI/Styles/DA_Style.DA_Style_C|GetInputBarHeight (Variables|/Game/Blueprints/GM/GI_HexDefense.GI_HexDefense_C|GetUIStyle _asgi_hex_defense))) 0.5))) (* (.WorldDirection (Class|PlayerController|DeprojectScreenPositiontoWorld _returnvalue (* (- _sizex (Variables|/Game/Blueprints/UI/Styles/DA_Style.DA_Style_C|GetSelectablesWidthMinusSrollBar (Variables|/Game/Blueprints/GM/GI_HexDefense.GI_HexDefense_C|GetUIStyle _asgi_hex_defense))) 0.5) (* (- _sizey (Variables|/Game/Blueprints/UI/Styles/DA_Style.DA_Style_C|GetInputBarHeight (Variables|/Game/Blueprints/GM/GI_HexDefense.GI_HexDefense_C|GetUIStyle _asgi_hex_defense))) 0.5))) 1e+01)) TargetLocation)) (+ (.WorldLocation (Class|PlayerController|DeprojectScreenPositiontoWorld _returnvalue (* (- _sizex (Variables|/Game/Blueprints/UI/Styles/DA_Style.DA_Style_C|GetSelectablesWidthMinusSrollBar (Variables|/Game/Blueprints/GM/GI_HexDefense.GI_HexDefense_C|GetUIStyle _asgi_hex_defense))) 0.5) (* (- _sizey (Variables|/Game/Blueprints/UI/Styles/DA_Style.DA_Style_C|GetInputBarHeight (Variables|/Game/Blueprints/GM/GI_HexDefense.GI_HexDefense_C|GetUIStyle _asgi_hex_defense))) 0.5))) (* (.WorldDirection (Class|PlayerController|DeprojectScreenPositiontoWorld _returnvalue (* (- _sizex (Variables|/Game/Blueprints/UI/Styles/DA_Style.DA_Style_C|GetSelectablesWidthMinusSrollBar (Variables|/Game/Blueprints/GM/GI_HexDefense.GI_HexDefense_C|GetUIStyle _asgi_hex_defense))) 0.5) (* (- _sizey (Variables|/Game/Blueprints/UI/Styles/DA_Style.DA_Style_C|GetInputBarHeight (Variables|/Game/Blueprints/GM/GI_HexDefense.GI_HexDefense_C|GetUIStyle _asgi_hex_defense))) 0.5))) 1e+01))) false))) (LocalVariables|GetHalfScreenHeight))))))))) (/ (LocalVariables|GetMarginValue) _returnvalue_2)) (/ (LocalVariables|GetHalfScreenWidth) _returnvalue_2)) (+ (* (* (Math|Float|Min(Float) (Math|Float|Absolute(Float) (/ (LocalVariables|GetHalfScreenWidth) (/ (- (.x (.ScreenLocation (Class|PlayerController|ProjectWorldLocationtoScreen _returnvalue (+ (Math|Vector|GetForwardVector (Math|Rotator|FindLookatRotation (+ (.WorldLocation (Class|PlayerController|DeprojectScreenPositiontoWorld _returnvalue (* (- _sizex (Variables|/Game/Blueprints/UI/Styles/DA_Style.DA_Style_C|GetSelectablesWidthMinusSrollBar (Variables|/Game/Blueprints/GM/GI_HexDefense.GI_HexDefense_C|GetUIStyle _asgi_hex_defense))) 0.5) (* (- _sizey (Variables|/Game/Blueprints/UI/Styles/DA_Style.DA_Style_C|GetInputBarHeight (Variables|/Game/Blueprints/GM/GI_HexDefense.GI_HexDefense_C|GetUIStyle _asgi_hex_defense))) 0.5))) (* (.WorldDirection (Class|PlayerController|DeprojectScreenPositiontoWorld _returnvalue (* (- _sizex (Variables|/Game/Blueprints/UI/Styles/DA_Style.DA_Style_C|GetSelectablesWidthMinusSrollBar (Variables|/Game/Blueprints/GM/GI_HexDefense.GI_HexDefense_C|GetUIStyle _asgi_hex_defense))) 0.5) (* (- _sizey (Variables|/Game/Blueprints/UI/Styles/DA_Style.DA_Style_C|GetInputBarHeight (Variables|/Game/Blueprints/GM/GI_HexDefense.GI_HexDefense_C|GetUIStyle _asgi_hex_defense))) 0.5))) 1e+01)) TargetLocation)) (+ (.WorldLocation (Class|PlayerController|DeprojectScreenPositiontoWorld _returnvalue (* (- _sizex (Variables|/Game/Blueprints/UI/Styles/DA_Style.DA_Style_C|GetSelectablesWidthMinusSrollBar (Variables|/Game/Blueprints/GM/GI_HexDefense.GI_HexDefense_C|GetUIStyle _asgi_hex_defense))) 0.5) (* (- _sizey (Variables|/Game/Blueprints/UI/Styles/DA_Style.DA_Style_C|GetInputBarHeight (Variables|/Game/Blueprints/GM/GI_HexDefense.GI_HexDefense_C|GetUIStyle _asgi_hex_defense))) 0.5))) (* (.WorldDirection (Class|PlayerController|DeprojectScreenPositiontoWorld _returnvalue (* (- _sizex (Variables|/Game/Blueprints/UI/Styles/DA_Style.DA_Style_C|GetSelectablesWidthMinusSrollBar (Variables|/Game/Blueprints/GM/GI_HexDefense.GI_HexDefense_C|GetUIStyle _asgi_hex_defense))) 0.5) (* (- _sizey (Variables|/Game/Blueprints/UI/Styles/DA_Style.DA_Style_C|GetInputBarHeight (Variables|/Game/Blueprints/GM/GI_HexDefense.GI_HexDefense_C|GetUIStyle _asgi_hex_defense))) 0.5))) 1e+01))) false))) (LocalVariables|GetHalfScreenWidth)) (Math|Float|Absolute(Float) (+ (- (.x (.ScreenLocation (Class|PlayerController|ProjectWorldLocationtoScreen _returnvalue (+ (Math|Vector|GetForwardVector (Math|Rotator|FindLookatRotation (+ (.WorldLocation (Class|PlayerController|DeprojectScreenPositiontoWorld _returnvalue (* (- _sizex (Variables|/Game/Blueprints/UI/Styles/DA_Style.DA_Style_C|GetSelectablesWidthMinusSrollBar (Variables|/Game/Blueprints/GM/GI_HexDefense.GI_HexDefense_C|GetUIStyle _asgi_hex_defense))) 0.5) (* (- _sizey (Variables|/Game/Blueprints/UI/Styles/DA_Style.DA_Style_C|GetInputBarHeight (Variables|/Game/Blueprints/GM/GI_HexDefense.GI_HexDefense_C|GetUIStyle _asgi_hex_defense))) 0.5))) (* (.WorldDirection (Class|PlayerController|DeprojectScreenPositiontoWorld _returnvalue (* (- _sizex (Variables|/Game/Blueprints/UI/Styles/DA_Style.DA_Style_C|GetSelectablesWidthMinusSrollBar (Variables|/Game/Blueprints/GM/GI_HexDefense.GI_HexDefense_C|GetUIStyle _asgi_hex_defense))) 0.5) (* (- _sizey (Variables|/Game/Blueprints/UI/Styles/DA_Style.DA_Style_C|GetInputBarHeight (Variables|/Game/Blueprints/GM/GI_HexDefense.GI_HexDefense_C|GetUIStyle _asgi_hex_defense))) 0.5))) 1e+01)) TargetLocation)) (+ (.WorldLocation (Class|PlayerController|DeprojectScreenPositiontoWorld _returnvalue (* (- _sizex (Variables|/Game/Blueprints/UI/Styles/DA_Style.DA_Style_C|GetSelectablesWidthMinusSrollBar (Variables|/Game/Blueprints/GM/GI_HexDefense.GI_HexDefense_C|GetUIStyle _asgi_hex_defense))) 0.5) (* (- _sizey (Variables|/Game/Blueprints/UI/Styles/DA_Style.DA_Style_C|GetInputBarHeight (Variables|/Game/Blueprints/GM/GI_HexDefense.GI_HexDefense_C|GetUIStyle _asgi_hex_defense))) 0.5))) (* (.WorldDirection (Class|PlayerController|DeprojectScreenPositiontoWorld _returnvalue (* (- _sizex (Variables|/Game/Blueprints/UI/Styles/DA_Style.DA_Style_C|GetSelectablesWidthMinusSrollBar (Variables|/Game/Blueprints/GM/GI_HexDefense.GI_HexDefense_C|GetUIStyle _asgi_hex_defense))) 0.5) (* (- _sizey (Variables|/Game/Blueprints/UI/Styles/DA_Style.DA_Style_C|GetInputBarHeight (Variables|/Game/Blueprints/GM/GI_HexDefense.GI_HexDefense_C|GetUIStyle _asgi_hex_defense))) 0.5))) 1e+01))) false))) (LocalVariables|GetHalfScreenWidth)) (- (.y (.ScreenLocation (Class|PlayerController|ProjectWorldLocationtoScreen _returnvalue (+ (Math|Vector|GetForwardVector (Math|Rotator|FindLookatRotation (+ (.WorldLocation (Class|PlayerController|DeprojectScreenPositiontoWorld _returnvalue (* (- _sizex (Variables|/Game/Blueprints/UI/Styles/DA_Style.DA_Style_C|GetSelectablesWidthMinusSrollBar (Variables|/Game/Blueprints/GM/GI_HexDefense.GI_HexDefense_C|GetUIStyle _asgi_hex_defense))) 0.5) (* (- _sizey (Variables|/Game/Blueprints/UI/Styles/DA_Style.DA_Style_C|GetInputBarHeight (Variables|/Game/Blueprints/GM/GI_HexDefense.GI_HexDefense_C|GetUIStyle _asgi_hex_defense))) 0.5))) (* (.WorldDirection (Class|PlayerController|DeprojectScreenPositiontoWorld _returnvalue (* (- _sizex (Variables|/Game/Blueprints/UI/Styles/DA_Style.DA_Style_C|GetSelectablesWidthMinusSrollBar (Variables|/Game/Blueprints/GM/GI_HexDefense.GI_HexDefense_C|GetUIStyle _asgi_hex_defense))) 0.5) (* (- _sizey (Variables|/Game/Blueprints/UI/Styles/DA_Style.DA_Style_C|GetInputBarHeight (Variables|/Game/Blueprints/GM/GI_HexDefense.GI_HexDefense_C|GetUIStyle _asgi_hex_defense))) 0.5))) 1e+01)) TargetLocation)) (+ (.WorldLocation (Class|PlayerController|DeprojectScreenPositiontoWorld _returnvalue (* (- _sizex (Variables|/Game/Blueprints/UI/Styles/DA_Style.DA_Style_C|GetSelectablesWidthMinusSrollBar (Variables|/Game/Blueprints/GM/GI_HexDefense.GI_HexDefense_C|GetUIStyle _asgi_hex_defense))) 0.5) (* (- _sizey (Variables|/Game/Blueprints/UI/Styles/DA_Style.DA_Style_C|GetInputBarHeight (Variables|/Game/Blueprints/GM/GI_HexDefense.GI_HexDefense_C|GetUIStyle _asgi_hex_defense))) 0.5))) (* (.WorldDirection (Class|PlayerController|DeprojectScreenPositiontoWorld _returnvalue (* (- _sizex (Variables|/Game/Blueprints/UI/Styles/DA_Style.DA_Style_C|GetSelectablesWidthMinusSrollBar (Variables|/Game/Blueprints/GM/GI_HexDefense.GI_HexDefense_C|GetUIStyle _asgi_hex_defense))) 0.5) (* (- _sizey (Variables|/Game/Blueprints/UI/Styles/DA_Style.DA_Style_C|GetInputBarHeight (Variables|/Game/Blueprints/GM/GI_HexDefense.GI_HexDefense_C|GetUIStyle _asgi_hex_defense))) 0.5))) 1e+01))) false))) (LocalVariables|GetHalfScreenHeight))))))) (Math|Float|Absolute(Float) (/ (LocalVariables|GetHalfScreenHeight) (/ (- (.y (.ScreenLocation (Class|PlayerController|ProjectWorldLocationtoScreen _returnvalue (+ (Math|Vector|GetForwardVector (Math|Rotator|FindLookatRotation (+ (.WorldLocation (Class|PlayerController|DeprojectScreenPositiontoWorld _returnvalue (* (- _sizex (Variables|/Game/Blueprints/UI/Styles/DA_Style.DA_Style_C|GetSelectablesWidthMinusSrollBar (Variables|/Game/Blueprints/GM/GI_HexDefense.GI_HexDefense_C|GetUIStyle _asgi_hex_defense))) 0.5) (* (- _sizey (Variables|/Game/Blueprints/UI/Styles/DA_Style.DA_Style_C|GetInputBarHeight (Variables|/Game/Blueprints/GM/GI_HexDefense.GI_HexDefense_C|GetUIStyle _asgi_hex_defense))) 0.5))) (* (.WorldDirection (Class|PlayerController|DeprojectScreenPositiontoWorld _returnvalue (* (- _sizex (Variables|/Game/Blueprints/UI/Styles/DA_Style.DA_Style_C|GetSelectablesWidthMinusSrollBar (Variables|/Game/Blueprints/GM/GI_HexDefense.GI_HexDefense_C|GetUIStyle _asgi_hex_defense))) 0.5) (* (- _sizey (Variables|/Game/Blueprints/UI/Styles/DA_Style.DA_Style_C|GetInputBarHeight (Variables|/Game/Blueprints/GM/GI_HexDefense.GI_HexDefense_C|GetUIStyle _asgi_hex_defense))) 0.5))) 1e+01)) TargetLocation)) (+ (.WorldLocation (Class|PlayerController|DeprojectScreenPositiontoWorld _returnvalue (* (- _sizex (Variables|/Game/Blueprints/UI/Styles/DA_Style.DA_Style_C|GetSelectablesWidthMinusSrollBar (Variables|/Game/Blueprints/GM/GI_HexDefense.GI_HexDefense_C|GetUIStyle _asgi_hex_defense))) 0.5) (* (- _sizey (Variables|/Game/Blueprints/UI/Styles/DA_Style.DA_Style_C|GetInputBarHeight (Variables|/Game/Blueprints/GM/GI_HexDefense.GI_HexDefense_C|GetUIStyle _asgi_hex_defense))) 0.5))) (* (.WorldDirection (Class|PlayerController|DeprojectScreenPositiontoWorld _returnvalue (* (- _sizex (Variables|/Game/Blueprints/UI/Styles/DA_Style.DA_Style_C|GetSelectablesWidthMinusSrollBar (Variables|/Game/Blueprints/GM/GI_HexDefense.GI_HexDefense_C|GetUIStyle _asgi_hex_defense))) 0.5) (* (- _sizey (Variables|/Game/Blueprints/UI/Styles/DA_Style.DA_Style_C|GetInputBarHeight (Variables|/Game/Blueprints/GM/GI_HexDefense.GI_HexDefense_C|GetUIStyle _asgi_hex_defense))) 0.5))) 1e+01))) false))) (LocalVariables|GetHalfScreenHeight)) (Math|Float|Absolute(Float) (+ (- (.x (.ScreenLocation (Class|PlayerController|ProjectWorldLocationtoScreen _returnvalue (+ (Math|Vector|GetForwardVector (Math|Rotator|FindLookatRotation (+ (.WorldLocation (Class|PlayerController|DeprojectScreenPositiontoWorld _returnvalue (* (- _sizex (Variables|/Game/Blueprints/UI/Styles/DA_Style.DA_Style_C|GetSelectablesWidthMinusSrollBar (Variables|/Game/Blueprints/GM/GI_HexDefense.GI_HexDefense_C|GetUIStyle _asgi_hex_defense))) 0.5) (* (- _sizey (Variables|/Game/Blueprints/UI/Styles/DA_Style.DA_Style_C|GetInputBarHeight (Variables|/Game/Blueprints/GM/GI_HexDefense.GI_HexDefense_C|GetUIStyle _asgi_hex_defense))) 0.5))) (* (.WorldDirection (Class|PlayerController|DeprojectScreenPositiontoWorld _returnvalue (* (- _sizex (Variables|/Game/Blueprints/UI/Styles/DA_Style.DA_Style_C|GetSelectablesWidthMinusSrollBar (Variables|/Game/Blueprints/GM/GI_HexDefense.GI_HexDefense_C|GetUIStyle _asgi_hex_defense))) 0.5) (* (- _sizey (Variables|/Game/Blueprints/UI/Styles/DA_Style.DA_Style_C|GetInputBarHeight (Variables|/Game/Blueprints/GM/GI_HexDefense.GI_HexDefense_C|GetUIStyle _asgi_hex_defense))) 0.5))) 1e+01)) TargetLocation)) (+ (.WorldLocation (Class|PlayerController|DeprojectScreenPositiontoWorld _returnvalue (* (- _sizex (Variables|/Game/Blueprints/UI/Styles/DA_Style.DA_Style_C|GetSelectablesWidthMinusSrollBar (Variables|/Game/Blueprints/GM/GI_HexDefense.GI_HexDefense_C|GetUIStyle _asgi_hex_defense))) 0.5) (* (- _sizey (Variables|/Game/Blueprints/UI/Styles/DA_Style.DA_Style_C|GetInputBarHeight (Variables|/Game/Blueprints/GM/GI_HexDefense.GI_HexDefense_C|GetUIStyle _asgi_hex_defense))) 0.5))) (* (.WorldDirection (Class|PlayerController|DeprojectScreenPositiontoWorld _returnvalue (* (- _sizex (Variables|/Game/Blueprints/UI/Styles/DA_Style.DA_Style_C|GetSelectablesWidthMinusSrollBar (Variables|/Game/Blueprints/GM/GI_HexDefense.GI_HexDefense_C|GetUIStyle _asgi_hex_defense))) 0.5) (* (- _sizey (Variables|/Game/Blueprints/UI/Styles/DA_Style.DA_Style_C|GetInputBarHeight (Variables|/Game/Blueprints/GM/GI_HexDefense.GI_HexDefense_C|GetUIStyle _asgi_hex_defense))) 0.5))) 1e+01))) false))) (LocalVariables|GetHalfScreenWidth)) (- (.y (.ScreenLocation (Class|PlayerController|ProjectWorldLocationtoScreen _returnvalue (+ (Math|Vector|GetForwardVector (Math|Rotator|FindLookatRotation (+ (.WorldLocation (Class|PlayerController|DeprojectScreenPositiontoWorld _returnvalue (* (- _sizex (Variables|/Game/Blueprints/UI/Styles/DA_Style.DA_Style_C|GetSelectablesWidthMinusSrollBar (Variables|/Game/Blueprints/GM/GI_HexDefense.GI_HexDefense_C|GetUIStyle _asgi_hex_defense))) 0.5) (* (- _sizey (Variables|/Game/Blueprints/UI/Styles/DA_Style.DA_Style_C|GetInputBarHeight (Variables|/Game/Blueprints/GM/GI_HexDefense.GI_HexDefense_C|GetUIStyle _asgi_hex_defense))) 0.5))) (* (.WorldDirection (Class|PlayerController|DeprojectScreenPositiontoWorld _returnvalue (* (- _sizex (Variables|/Game/Blueprints/UI/Styles/DA_Style.DA_Style_C|GetSelectablesWidthMinusSrollBar (Variables|/Game/Blueprints/GM/GI_HexDefense.GI_HexDefense_C|GetUIStyle _asgi_hex_defense))) 0.5) (* (- _sizey (Variables|/Game/Blueprints/UI/Styles/DA_Style.DA_Style_C|GetInputBarHeight (Variables|/Game/Blueprints/GM/GI_HexDefense.GI_HexDefense_C|GetUIStyle _asgi_hex_defense))) 0.5))) 1e+01)) TargetLocation)) (+ (.WorldLocation (Class|PlayerController|DeprojectScreenPositiontoWorld _returnvalue (* (- _sizex (Variables|/Game/Blueprints/UI/Styles/DA_Style.DA_Style_C|GetSelectablesWidthMinusSrollBar (Variables|/Game/Blueprints/GM/GI_HexDefense.GI_HexDefense_C|GetUIStyle _asgi_hex_defense))) 0.5) (* (- _sizey (Variables|/Game/Blueprints/UI/Styles/DA_Style.DA_Style_C|GetInputBarHeight (Variables|/Game/Blueprints/GM/GI_HexDefense.GI_HexDefense_C|GetUIStyle _asgi_hex_defense))) 0.5))) (* (.WorldDirection (Class|PlayerController|DeprojectScreenPositiontoWorld _returnvalue (* (- _sizex (Variables|/Game/Blueprints/UI/Styles/DA_Style.DA_Style_C|GetSelectablesWidthMinusSrollBar (Variables|/Game/Blueprints/GM/GI_HexDefense.GI_HexDefense_C|GetUIStyle _asgi_hex_defense))) 0.5) (* (- _sizey (Variables|/Game/Blueprints/UI/Styles/DA_Style.DA_Style_C|GetInputBarHeight (Variables|/Game/Blueprints/GM/GI_HexDefense.GI_HexDefense_C|GetUIStyle _asgi_hex_defense))) 0.5))) 1e+01))) false))) (LocalVariables|GetHalfScreenHeight)))))))) (/ (- (.y (.ScreenLocation (Class|PlayerController|ProjectWorldLocationtoScreen _returnvalue (+ (Math|Vector|GetForwardVector (Math|Rotator|FindLookatRotation (+ (.WorldLocation (Class|PlayerController|DeprojectScreenPositiontoWorld _returnvalue (* (- _sizex (Variables|/Game/Blueprints/UI/Styles/DA_Style.DA_Style_C|GetSelectablesWidthMinusSrollBar (Variables|/Game/Blueprints/GM/GI_HexDefense.GI_HexDefense_C|GetUIStyle _asgi_hex_defense))) 0.5) (* (- _sizey (Variables|/Game/Blueprints/UI/Styles/DA_Style.DA_Style_C|GetInputBarHeight (Variables|/Game/Blueprints/GM/GI_HexDefense.GI_HexDefense_C|GetUIStyle _asgi_hex_defense))) 0.5))) (* (.WorldDirection (Class|PlayerController|DeprojectScreenPositiontoWorld _returnvalue (* (- _sizex (Variables|/Game/Blueprints/UI/Styles/DA_Style.DA_Style_C|GetSelectablesWidthMinusSrollBar (Variables|/Game/Blueprints/GM/GI_HexDefense.GI_HexDefense_C|GetUIStyle _asgi_hex_defense))) 0.5) (* (- _sizey (Variables|/Game/Blueprints/UI/Styles/DA_Style.DA_Style_C|GetInputBarHeight (Variables|/Game/Blueprints/GM/GI_HexDefense.GI_HexDefense_C|GetUIStyle _asgi_hex_defense))) 0.5))) 1e+01)) TargetLocation)) (+ (.WorldLocation (Class|PlayerController|DeprojectScreenPositiontoWorld _returnvalue (* (- _sizex (Variables|/Game/Blueprints/UI/Styles/DA_Style.DA_Style_C|GetSelectablesWidthMinusSrollBar (Variables|/Game/Blueprints/GM/GI_HexDefense.GI_HexDefense_C|GetUIStyle _asgi_hex_defense))) 0.5) (* (- _sizey (Variables|/Game/Blueprints/UI/Styles/DA_Style.DA_Style_C|GetInputBarHeight (Variables|/Game/Blueprints/GM/GI_HexDefense.GI_HexDefense_C|GetUIStyle _asgi_hex_defense))) 0.5))) (* (.WorldDirection (Class|PlayerController|DeprojectScreenPositiontoWorld _returnvalue (* (- _sizex (Variables|/Game/Blueprints/UI/Styles/DA_Style.DA_Style_C|GetSelectablesWidthMinusSrollBar (Variables|/Game/Blueprints/GM/GI_HexDefense.GI_HexDefense_C|GetUIStyle _asgi_hex_defense))) 0.5) (* (- _sizey (Variables|/Game/Blueprints/UI/Styles/DA_Style.DA_Style_C|GetInputBarHeight (Variables|/Game/Blueprints/GM/GI_HexDefense.GI_HexDefense_C|GetUIStyle _asgi_hex_defense))) 0.5))) 1e+01))) false))) (LocalVariables|GetHalfScreenHeight)) (Math|Float|Absolute(Float) (+ (- (.x (.ScreenLocation (Class|PlayerController|ProjectWorldLocationtoScreen _returnvalue (+ (Math|Vector|GetForwardVector (Math|Rotator|FindLookatRotation (+ (.WorldLocation (Class|PlayerController|DeprojectScreenPositiontoWorld _returnvalue (* (- _sizex (Variables|/Game/Blueprints/UI/Styles/DA_Style.DA_Style_C|GetSelectablesWidthMinusSrollBar (Variables|/Game/Blueprints/GM/GI_HexDefense.GI_HexDefense_C|GetUIStyle _asgi_hex_defense))) 0.5) (* (- _sizey (Variables|/Game/Blueprints/UI/Styles/DA_Style.DA_Style_C|GetInputBarHeight (Variables|/Game/Blueprints/GM/GI_HexDefense.GI_HexDefense_C|GetUIStyle _asgi_hex_defense))) 0.5))) (* (.WorldDirection (Class|PlayerController|DeprojectScreenPositiontoWorld _returnvalue (* (- _sizex (Variables|/Game/Blueprints/UI/Styles/DA_Style.DA_Style_C|GetSelectablesWidthMinusSrollBar (Variables|/Game/Blueprints/GM/GI_HexDefense.GI_HexDefense_C|GetUIStyle _asgi_hex_defense))) 0.5) (* (- _sizey (Variables|/Game/Blueprints/UI/Styles/DA_Style.DA_Style_C|GetInputBarHeight (Variables|/Game/Blueprints/GM/GI_HexDefense.GI_HexDefense_C|GetUIStyle _asgi_hex_defense))) 0.5))) 1e+01)) TargetLocation)) (+ (.WorldLocation (Class|PlayerController|DeprojectScreenPositiontoWorld _returnvalue (* (- _sizex (Variables|/Game/Blueprints/UI/Styles/DA_Style.DA_Style_C|GetSelectablesWidthMinusSrollBar (Variables|/Game/Blueprints/GM/GI_HexDefense.GI_HexDefense_C|GetUIStyle _asgi_hex_defense))) 0.5) (* (- _sizey (Variables|/Game/Blueprints/UI/Styles/DA_Style.DA_Style_C|GetInputBarHeight (Variables|/Game/Blueprints/GM/GI_HexDefense.GI_HexDefense_C|GetUIStyle _asgi_hex_defense))) 0.5))) (* (.WorldDirection (Class|PlayerController|DeprojectScreenPositiontoWorld _returnvalue (* (- _sizex (Variables|/Game/Blueprints/UI/Styles/DA_Style.DA_Style_C|GetSelectablesWidthMinusSrollBar (Variables|/Game/Blueprints/GM/GI_HexDefense.GI_HexDefense_C|GetUIStyle _asgi_hex_defense))) 0.5) (* (- _sizey (Variables|/Game/Blueprints/UI/Styles/DA_Style.DA_Style_C|GetInputBarHeight (Variables|/Game/Blueprints/GM/GI_HexDefense.GI_HexDefense_C|GetUIStyle _asgi_hex_defense))) 0.5))) 1e+01))) false))) (LocalVariables|GetHalfScreenWidth)) (- (.y (.ScreenLocation (Class|PlayerController|ProjectWorldLocationtoScreen _returnvalue (+ (Math|Vector|GetForwardVector (Math|Rotator|FindLookatRotation (+ (.WorldLocation (Class|PlayerController|DeprojectScreenPositiontoWorld _returnvalue (* (- _sizex (Variables|/Game/Blueprints/UI/Styles/DA_Style.DA_Style_C|GetSelectablesWidthMinusSrollBar (Variables|/Game/Blueprints/GM/GI_HexDefense.GI_HexDefense_C|GetUIStyle _asgi_hex_defense))) 0.5) (* (- _sizey (Variables|/Game/Blueprints/UI/Styles/DA_Style.DA_Style_C|GetInputBarHeight (Variables|/Game/Blueprints/GM/GI_HexDefense.GI_HexDefense_C|GetUIStyle _asgi_hex_defense))) 0.5))) (* (.WorldDirection (Class|PlayerController|DeprojectScreenPositiontoWorld _returnvalue (* (- _sizex (Variables|/Game/Blueprints/UI/Styles/DA_Style.DA_Style_C|GetSelectablesWidthMinusSrollBar (Variables|/Game/Blueprints/GM/GI_HexDefense.GI_HexDefense_C|GetUIStyle _asgi_hex_defense))) 0.5) (* (- _sizey (Variables|/Game/Blueprints/UI/Styles/DA_Style.DA_Style_C|GetInputBarHeight (Variables|/Game/Blueprints/GM/GI_HexDefense.GI_HexDefense_C|GetUIStyle _asgi_hex_defense))) 0.5))) 1e+01)) TargetLocation)) (+ (.WorldLocation (Class|PlayerController|DeprojectScreenPositiontoWorld _returnvalue (* (- _sizex (Variables|/Game/Blueprints/UI/Styles/DA_Style.DA_Style_C|GetSelectablesWidthMinusSrollBar (Variables|/Game/Blueprints/GM/GI_HexDefense.GI_HexDefense_C|GetUIStyle _asgi_hex_defense))) 0.5) (* (- _sizey (Variables|/Game/Blueprints/UI/Styles/DA_Style.DA_Style_C|GetInputBarHeight (Variables|/Game/Blueprints/GM/GI_HexDefense.GI_HexDefense_C|GetUIStyle _asgi_hex_defense))) 0.5))) (* (.WorldDirection (Class|PlayerController|DeprojectScreenPositiontoWorld _returnvalue (* (- _sizex (Variables|/Game/Blueprints/UI/Styles/DA_Style.DA_Style_C|GetSelectablesWidthMinusSrollBar (Variables|/Game/Blueprints/GM/GI_HexDefense.GI_HexDefense_C|GetUIStyle _asgi_hex_defense))) 0.5) (* (- _sizey (Variables|/Game/Blueprints/UI/Styles/DA_Style.DA_Style_C|GetInputBarHeight (Variables|/Game/Blueprints/GM/GI_HexDefense.GI_HexDefense_C|GetUIStyle _asgi_hex_defense))) 0.5))) 1e+01))) false))) (LocalVariables|GetHalfScreenHeight)))))) (/ (LocalVariables|GetMarginValue) _returnvalue_2)) (/ (LocalVariables|GetHalfScreenHeight) _returnvalue_2))) (Class|KismetMathLibrary|DegAtan2 (/ (- (.x (.ScreenLocation (Class|PlayerController|ProjectWorldLocationtoScreen _returnvalue (+ (Math|Vector|GetForwardVector (Math|Rotator|FindLookatRotation (+ (.WorldLocation (Class|PlayerController|DeprojectScreenPositiontoWorld _returnvalue (* (- _sizex (Variables|/Game/Blueprints/UI/Styles/DA_Style.DA_Style_C|GetSelectablesWidthMinusSrollBar (Variables|/Game/Blueprints/GM/GI_HexDefense.GI_HexDefense_C|GetUIStyle _asgi_hex_defense))) 0.5) (* (- _sizey (Variables|/Game/Blueprints/UI/Styles/DA_Style.DA_Style_C|GetInputBarHeight (Variables|/Game/Blueprints/GM/GI_HexDefense.GI_HexDefense_C|GetUIStyle _asgi_hex_defense))) 0.5))) (* (.WorldDirection (Class|PlayerController|DeprojectScreenPositiontoWorld _returnvalue (* (- _sizex (Variables|/Game/Blueprints/UI/Styles/DA_Style.DA_Style_C|GetSelectablesWidthMinusSrollBar (Variables|/Game/Blueprints/GM/GI_HexDefense.GI_HexDefense_C|GetUIStyle _asgi_hex_defense))) 0.5) (* (- _sizey (Variables|/Game/Blueprints/UI/Styles/DA_Style.DA_Style_C|GetInputBarHeight (Variables|/Game/Blueprints/GM/GI_HexDefense.GI_HexDefense_C|GetUIStyle _asgi_hex_defense))) 0.5))) 1e+01)) TargetLocation)) (+ (.WorldLocation (Class|PlayerController|DeprojectScreenPositiontoWorld _returnvalue (* (- _sizex (Variables|/Game/Blueprints/UI/Styles/DA_Style.DA_Style_C|GetSelectablesWidthMinusSrollBar (Variables|/Game/Blueprints/GM/GI_HexDefense.GI_HexDefense_C|GetUIStyle _asgi_hex_defense))) 0.5) (* (- _sizey (Variables|/Game/Blueprints/UI/Styles/DA_Style.DA_Style_C|GetInputBarHeight (Variables|/Game/Blueprints/GM/GI_HexDefense.GI_HexDefense_C|GetUIStyle _asgi_hex_defense))) 0.5))) (* (.WorldDirection (Class|PlayerController|DeprojectScreenPositiontoWorld _returnvalue (* (- _sizex (Variables|/Game/Blueprints/UI/Styles/DA_Style.DA_Style_C|GetSelectablesWidthMinusSrollBar (Variables|/Game/Blueprints/GM/GI_HexDefense.GI_HexDefense_C|GetUIStyle _asgi_hex_defense))) 0.5) (* (- _sizey (Variables|/Game/Blueprints/UI/Styles/DA_Style.DA_Style_C|GetInputBarHeight (Variables|/Game/Blueprints/GM/GI_HexDefense.GI_HexDefense_C|GetUIStyle _asgi_hex_defense))) 0.5))) 1e+01))) false))) (LocalVariables|GetHalfScreenWidth)) (Math|Float|Absolute(Float) (+ (- (.x (.ScreenLocation (Class|PlayerController|ProjectWorldLocationtoScreen _returnvalue (+ (Math|Vector|GetForwardVector (Math|Rotator|FindLookatRotation (+ (.WorldLocation (Class|PlayerController|DeprojectScreenPositiontoWorld _returnvalue (* (- _sizex (Variables|/Game/Blueprints/UI/Styles/DA_Style.DA_Style_C|GetSelectablesWidthMinusSrollBar (Variables|/Game/Blueprints/GM/GI_HexDefense.GI_HexDefense_C|GetUIStyle _asgi_hex_defense))) 0.5) (* (- _sizey (Variables|/Game/Blueprints/UI/Styles/DA_Style.DA_Style_C|GetInputBarHeight (Variables|/Game/Blueprints/GM/GI_HexDefense.GI_HexDefense_C|GetUIStyle _asgi_hex_defense))) 0.5))) (* (.WorldDirection (Class|PlayerController|DeprojectScreenPositiontoWorld _returnvalue (* (- _sizex (Variables|/Game/Blueprints/UI/Styles/DA_Style.DA_Style_C|GetSelectablesWidthMinusSrollBar (Variables|/Game/Blueprints/GM/GI_HexDefense.GI_HexDefense_C|GetUIStyle _asgi_hex_defense))) 0.5) (* (- _sizey (Variables|/Game/Blueprints/UI/Styles/DA_Style.DA_Style_C|GetInputBarHeight (Variables|/Game/Blueprints/GM/GI_HexDefense.GI_HexDefense_C|GetUIStyle _asgi_hex_defense))) 0.5))) 1e+01)) TargetLocation)) (+ (.WorldLocation (Class|PlayerController|DeprojectScreenPositiontoWorld _returnvalue (* (- _sizex (Variables|/Game/Blueprints/UI/Styles/DA_Style.DA_Style_C|GetSelectablesWidthMinusSrollBar (Variables|/Game/Blueprints/GM/GI_HexDefense.GI_HexDefense_C|GetUIStyle _asgi_hex_defense))) 0.5) (* (- _sizey (Variables|/Game/Blueprints/UI/Styles/DA_Style.DA_Style_C|GetInputBarHeight (Variables|/Game/Blueprints/GM/GI_HexDefense.GI_HexDefense_C|GetUIStyle _asgi_hex_defense))) 0.5))) (* (.WorldDirection (Class|PlayerController|DeprojectScreenPositiontoWorld _returnvalue (* (- _sizex (Variables|/Game/Blueprints/UI/Styles/DA_Style.DA_Style_C|GetSelectablesWidthMinusSrollBar (Variables|/Game/Blueprints/GM/GI_HexDefense.GI_HexDefense_C|GetUIStyle _asgi_hex_defense))) 0.5) (* (- _sizey (Variables|/Game/Blueprints/UI/Styles/DA_Style.DA_Style_C|GetInputBarHeight (Variables|/Game/Blueprints/GM/GI_HexDefense.GI_HexDefense_C|GetUIStyle _asgi_hex_defense))) 0.5))) 1e+01))) false))) (LocalVariables|GetHalfScreenWidth)) (- (.y (.ScreenLocation (Class|PlayerController|ProjectWorldLocationtoScreen _returnvalue (+ (Math|Vector|GetForwardVector (Math|Rotator|FindLookatRotation (+ (.WorldLocation (Class|PlayerController|DeprojectScreenPositiontoWorld _returnvalue (* (- _sizex (Variables|/Game/Blueprints/UI/Styles/DA_Style.DA_Style_C|GetSelectablesWidthMinusSrollBar (Variables|/Game/Blueprints/GM/GI_HexDefense.GI_HexDefense_C|GetUIStyle _asgi_hex_defense))) 0.5) (* (- _sizey (Variables|/Game/Blueprints/UI/Styles/DA_Style.DA_Style_C|GetInputBarHeight (Variables|/Game/Blueprints/GM/GI_HexDefense.GI_HexDefense_C|GetUIStyle _asgi_hex_defense))) 0.5))) (* (.WorldDirection (Class|PlayerController|DeprojectScreenPositiontoWorld _returnvalue (* (- _sizex (Variables|/Game/Blueprints/UI/Styles/DA_Style.DA_Style_C|GetSelectablesWidthMinusSrollBar (Variables|/Game/Blueprints/GM/GI_HexDefense.GI_HexDefense_C|GetUIStyle _asgi_hex_defense))) 0.5) (* (- _sizey (Variables|/Game/Blueprints/UI/Styles/DA_Style.DA_Style_C|GetInputBarHeight (Variables|/Game/Blueprints/GM/GI_HexDefense.GI_HexDefense_C|GetUIStyle _asgi_hex_defense))) 0.5))) 1e+01)) TargetLocation)) (+ (.WorldLocation (Class|PlayerController|DeprojectScreenPositiontoWorld _returnvalue (* (- _sizex (Variables|/Game/Blueprints/UI/Styles/DA_Style.DA_Style_C|GetSelectablesWidthMinusSrollBar (Variables|/Game/Blueprints/GM/GI_HexDefense.GI_HexDefense_C|GetUIStyle _asgi_hex_defense))) 0.5) (* (- _sizey (Variables|/Game/Blueprints/UI/Styles/DA_Style.DA_Style_C|GetInputBarHeight (Variables|/Game/Blueprints/GM/GI_HexDefense.GI_HexDefense_C|GetUIStyle _asgi_hex_defense))) 0.5))) (* (.WorldDirection (Class|PlayerController|DeprojectScreenPositiontoWorld _returnvalue (* (- _sizex (Variables|/Game/Blueprints/UI/Styles/DA_Style.DA_Style_C|GetSelectablesWidthMinusSrollBar (Variables|/Game/Blueprints/GM/GI_HexDefense.GI_HexDefense_C|GetUIStyle _asgi_hex_defense))) 0.5) (* (- _sizey (Variables|/Game/Blueprints/UI/Styles/DA_Style.DA_Style_C|GetInputBarHeight (Variables|/Game/Blueprints/GM/GI_HexDefense.GI_HexDefense_C|GetUIStyle _asgi_hex_defense))) 0.5))) 1e+01))) false))) (LocalVariables|GetHalfScreenHeight))))) (/ (- (.y (.ScreenLocation (Class|PlayerController|ProjectWorldLocationtoScreen _returnvalue (+ (Math|Vector|GetForwardVector (Math|Rotator|FindLookatRotation (+ (.WorldLocation (Class|PlayerController|DeprojectScreenPositiontoWorld _returnvalue (* (- _sizex (Variables|/Game/Blueprints/UI/Styles/DA_Style.DA_Style_C|GetSelectablesWidthMinusSrollBar (Variables|/Game/Blueprints/GM/GI_HexDefense.GI_HexDefense_C|GetUIStyle _asgi_hex_defense))) 0.5) (* (- _sizey (Variables|/Game/Blueprints/UI/Styles/DA_Style.DA_Style_C|GetInputBarHeight (Variables|/Game/Blueprints/GM/GI_HexDefense.GI_HexDefense_C|GetUIStyle _asgi_hex_defense))) 0.5))) (* (.WorldDirection (Class|PlayerController|DeprojectScreenPositiontoWorld _returnvalue (* (- _sizex (Variables|/Game/Blueprints/UI/Styles/DA_Style.DA_Style_C|GetSelectablesWidthMinusSrollBar (Variables|/Game/Blueprints/GM/GI_HexDefense.GI_HexDefense_C|GetUIStyle _asgi_hex_defense))) 0.5) (* (- _sizey (Variables|/Game/Blueprints/UI/Styles/DA_Style.DA_Style_C|GetInputBarHeight (Variables|/Game/Blueprints/GM/GI_HexDefense.GI_HexDefense_C|GetUIStyle _asgi_hex_defense))) 0.5))) 1e+01)) TargetLocation)) (+ (.WorldLocation (Class|PlayerController|DeprojectScreenPositiontoWorld _returnvalue (* (- _sizex (Variables|/Game/Blueprints/UI/Styles/DA_Style.DA_Style_C|GetSelectablesWidthMinusSrollBar (Variables|/Game/Blueprints/GM/GI_HexDefense.GI_HexDefense_C|GetUIStyle _asgi_hex_defense))) 0.5) (* (- _sizey (Variables|/Game/Blueprints/UI/Styles/DA_Style.DA_Style_C|GetInputBarHeight (Variables|/Game/Blueprints/GM/GI_HexDefense.GI_HexDefense_C|GetUIStyle _asgi_hex_defense))) 0.5))) (* (.WorldDirection (Class|PlayerController|DeprojectScreenPositiontoWorld _returnvalue (* (- _sizex (Variables|/Game/Blueprints/UI/Styles/DA_Style.DA_Style_C|GetSelectablesWidthMinusSrollBar (Variables|/Game/Blueprints/GM/GI_HexDefense.GI_HexDefense_C|GetUIStyle _asgi_hex_defense))) 0.5) (* (- _sizey (Variables|/Game/Blueprints/UI/Styles/DA_Style.DA_Style_C|GetInputBarHeight (Variables|/Game/Blueprints/GM/GI_HexDefense.GI_HexDefense_C|GetUIStyle _asgi_hex_defense))) 0.5))) 1e+01))) false))) (LocalVariables|GetHalfScreenHeight)) (Math|Float|Absolute(Float) (+ (- (.x (.ScreenLocation (Class|PlayerController|ProjectWorldLocationtoScreen _returnvalue (+ (Math|Vector|GetForwardVector (Math|Rotator|FindLookatRotation (+ (.WorldLocation (Class|PlayerController|DeprojectScreenPositiontoWorld _returnvalue (* (- _sizex (Variables|/Game/Blueprints/UI/Styles/DA_Style.DA_Style_C|GetSelectablesWidthMinusSrollBar (Variables|/Game/Blueprints/GM/GI_HexDefense.GI_HexDefense_C|GetUIStyle _asgi_hex_defense))) 0.5) (* (- _sizey (Variables|/Game/Blueprints/UI/Styles/DA_Style.DA_Style_C|GetInputBarHeight (Variables|/Game/Blueprints/GM/GI_HexDefense.GI_HexDefense_C|GetUIStyle _asgi_hex_defense))) 0.5))) (* (.WorldDirection (Class|PlayerController|DeprojectScreenPositiontoWorld _returnvalue (* (- _sizex (Variables|/Game/Blueprints/UI/Styles/DA_Style.DA_Style_C|GetSelectablesWidthMinusSrollBar (Variables|/Game/Blueprints/GM/GI_HexDefense.GI_HexDefense_C|GetUIStyle _asgi_hex_defense))) 0.5) (* (- _sizey (Variables|/Game/Blueprints/UI/Styles/DA_Style.DA_Style_C|GetInputBarHeight (Variables|/Game/Blueprints/GM/GI_HexDefense.GI_HexDefense_C|GetUIStyle _asgi_hex_defense))) 0.5))) 1e+01)) TargetLocation)) (+ (.WorldLocation (Class|PlayerController|DeprojectScreenPositiontoWorld _returnvalue (* (- _sizex (Variables|/Game/Blueprints/UI/Styles/DA_Style.DA_Style_C|GetSelectablesWidthMinusSrollBar (Variables|/Game/Blueprints/GM/GI_HexDefense.GI_HexDefense_C|GetUIStyle _asgi_hex_defense))) 0.5) (* (- _sizey (Variables|/Game/Blueprints/UI/Styles/DA_Style.DA_Style_C|GetInputBarHeight (Variables|/Game/Blueprints/GM/GI_HexDefense.GI_HexDefense_C|GetUIStyle _asgi_hex_defense))) 0.5))) (* (.WorldDirection (Class|PlayerController|DeprojectScreenPositiontoWorld _returnvalue (* (- _sizex (Variables|/Game/Blueprints/UI/Styles/DA_Style.DA_Style_C|GetSelectablesWidthMinusSrollBar (Variables|/Game/Blueprints/GM/GI_HexDefense.GI_HexDefense_C|GetUIStyle _asgi_hex_defense))) 0.5) (* (- _sizey (Variables|/Game/Blueprints/UI/Styles/DA_Style.DA_Style_C|GetInputBarHeight (Variables|/Game/Blueprints/GM/GI_HexDefense.GI_HexDefense_C|GetUIStyle _asgi_hex_defense))) 0.5))) 1e+01))) false))) (LocalVariables|GetHalfScreenWidth)) (- (.y (.ScreenLocation (Class|PlayerController|ProjectWorldLocationtoScreen _returnvalue (+ (Math|Vector|GetForwardVector (Math|Rotator|FindLookatRotation (+ (.WorldLocation (Class|PlayerController|DeprojectScreenPositiontoWorld _returnvalue (* (- _sizex (Variables|/Game/Blueprints/UI/Styles/DA_Style.DA_Style_C|GetSelectablesWidthMinusSrollBar (Variables|/Game/Blueprints/GM/GI_HexDefense.GI_HexDefense_C|GetUIStyle _asgi_hex_defense))) 0.5) (* (- _sizey (Variables|/Game/Blueprints/UI/Styles/DA_Style.DA_Style_C|GetInputBarHeight (Variables|/Game/Blueprints/GM/GI_HexDefense.GI_HexDefense_C|GetUIStyle _asgi_hex_defense))) 0.5))) (* (.WorldDirection (Class|PlayerController|DeprojectScreenPositiontoWorld _returnvalue (* (- _sizex (Variables|/Game/Blueprints/UI/Styles/DA_Style.DA_Style_C|GetSelectablesWidthMinusSrollBar (Variables|/Game/Blueprints/GM/GI_HexDefense.GI_HexDefense_C|GetUIStyle _asgi_hex_defense))) 0.5) (* (- _sizey (Variables|/Game/Blueprints/UI/Styles/DA_Style.DA_Style_C|GetInputBarHeight (Variables|/Game/Blueprints/GM/GI_HexDefense.GI_HexDefense_C|GetUIStyle _asgi_hex_defense))) 0.5))) 1e+01)) TargetLocation)) (+ (.WorldLocation (Class|PlayerController|DeprojectScreenPositiontoWorld _returnvalue (* (- _sizex (Variables|/Game/Blueprints/UI/Styles/DA_Style.DA_Style_C|GetSelectablesWidthMinusSrollBar (Variables|/Game/Blueprints/GM/GI_HexDefense.GI_HexDefense_C|GetUIStyle _asgi_hex_defense))) 0.5) (* (- _sizey (Variables|/Game/Blueprints/UI/Styles/DA_Style.DA_Style_C|GetInputBarHeight (Variables|/Game/Blueprints/GM/GI_HexDefense.GI_HexDefense_C|GetUIStyle _asgi_hex_defense))) 0.5))) (* (.WorldDirection (Class|PlayerController|DeprojectScreenPositiontoWorld _returnvalue (* (- _sizex (Variables|/Game/Blueprints/UI/Styles/DA_Style.DA_Style_C|GetSelectablesWidthMinusSrollBar (Variables|/Game/Blueprints/GM/GI_HexDefense.GI_HexDefense_C|GetUIStyle _asgi_hex_defense))) 0.5) (* (- _sizey (Variables|/Game/Blueprints/UI/Styles/DA_Style.DA_Style_C|GetInputBarHeight (Variables|/Game/Blueprints/GM/GI_HexDefense.GI_HexDefense_C|GetUIStyle _asgi_hex_defense))) 0.5))) 1e+01))) false))) (LocalVariables|GetHalfScreenHeight))))))))

(fn IsLocationonScreen
  (params (Location :type Vector))
  (bind _returnvalue (Game|GetPlayerController 0))
  (bind _returnvalue_2 (Viewport|GetViewportSize))
  (bind _screenlocation (Class|PlayerController|ProjectWorldLocationtoScreen _returnvalue Location false))
  (bind _asgi_hex_defense (Utilities|Casting|CastToGI_HexDefense (Game|GetGameInstance)))
  (return (Math|Boolean|ANDBoolean (> (.x _screenlocation) 0.0) (> (.y _screenlocation) 0.0) (< (.x _screenlocation) (- (.x _returnvalue_2) (Variables|/Game/Blueprints/UI/Styles/DA_Style.DA_Style_C|GetSelectablesWidthMinusSrollBar (Variables|/Game/Blueprints/GM/GI_HexDefense.GI_HexDefense_C|GetUIStyle _asgi_hex_defense)))) (< (.y _screenlocation) (- (.y _returnvalue_2) (Variables|/Game/Blueprints/UI/Styles/DA_Style.DA_Style_C|GetInputBarHeight (Variables|/Game/Blueprints/GM/GI_HexDefense.GI_HexDefense_C|GetUIStyle _asgi_hex_defense)))))))