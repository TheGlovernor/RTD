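; Music player actor that plays a playlist through an audio component, using volume and shuffle settings from the game config save.
; BeginPlay creates the save if missing, forces shuffle on in it, and starts the first track.
; UpdateSettings reapplies saved settings and rebuilds the track order, keeping the current track's position.
; Each finished track advances to the next, wrapping at the end and reshuffling if enabled.
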(event OnAudioFinished(Audio)
  (CallFunction|MovetoNextTrack))

(event Custom|UpdateSettings
  (bind _audio (Variables|Default|GetAudio))
  (bind _returnvalue (SaveGame|DoesSaveGameExist (Variables|Default|GetConfigSaveName)))
  (if _returnvalue
    (bind _returnvalue_2 (SaveGame|LoadGamefromSlot (Variables|Default|GetConfigSaveName)))
    (bind _assave_game_config (Utilities|Casting|CastToSave_GameConfig _returnvalue_2))
    (Audio|Components|Audio|SetVolumeMultiplier _audio (* (Variables|/Game/Blueprints/Saves/Save_GameConfig.Save_GameConfig_C|GetMainVol _assave_game_config) (Variables|/Game/Blueprints/Saves/Save_GameConfig.Save_GameConfig_C|GetMusicVol _assave_game_config)) :!class /Script/Engine.AudioComponent)
    (bind _output_get (Variables|Default|SetShuffle (Variables|/Game/Blueprints/Saves/Save_GameConfig.Save_GameConfig_C|GetShuffleTracks _assave_game_config)))
    (CallFunction|ShuffleTrackList _output_get)
    (switch Utilities|FlowControl|Switch|SwitchonEAudioComponentPlayState (Audio|Components|Audio|GetPlayState _audio)
      (:Stopped
        (Audio|Components|Audio|Play _audio 0.0))
      (:Paused
        (Class|AudioComponent|SetPaused _audio true)))))

(event Custom|ShuffleTrackList
  (params (Shuffle :type Boolean))
  (bind _output_get (Variables|Default|SetTrackOrder (Variables|Default|GetTracks)))
  (if Shuffle
    (Utilities|Array|Shuffle _output_get))
  (bind (_array_element _array_index) (Utilities|Array|ForEachLoopwithBreak (Variables|Default|GetTrackOrder) :!label _label)
    (:LoopBody
      (if (== _array_element (Variables|Default|GetCurrentTrack))
        (Variables|Default|SetCurrentTrackIndex _array_index)
        (goto _label Break)))))

(event Custom|MoveToNextTrack
  (bind _audio (Variables|Default|GetAudio))
  (Audio|Components|Audio|Stop (Variables|Default|GetAudio))
  (bind _result (Math|Integer|IncrementInt (Variables|Default|GetCurrentTrackIndex))
    (:%20%20
      (if (>= _result (Utilities|Array|Length (Variables|Default|GetTrackOrder)))
        (Variables|Default|SetCurrentTrackIndex 0)
        (if (Variables|Default|GetShuffle)
          (Utilities|Array|Shuffle (Variables|Default|GetTrackOrder))))
      (Audio|Components|Audio|SetSound _audio (Utilities|Array|Get(acopy) (Variables|Default|GetTrackOrder) (Variables|Default|GetCurrentTrackIndex)))
      (Audio|Components|Audio|Play _audio 0.0))))

(event EventBeginPlay
  (bind _configsavename (Variables|Default|GetConfigSaveName))
  (bind _audio (Variables|Default|GetAudio))
  (bind _returnvalue (SaveGame|DoesSaveGameExist (Variables|Default|GetConfigSaveName)))
  (if _returnvalue
    _
    (else
      (bind _returnvalue_2 (SaveGame|CreateSaveGameObject "/Game/Blueprints/Saves/Save_GameConfig.Save_GameConfig_C"))
      (SaveGame|SaveGametoSlot _returnvalue_2 _configsavename)))
  (bind _returnvalue_3 (SaveGame|LoadGamefromSlot (Variables|Default|GetConfigSaveName)))
  (bind _assave_game_config (Utilities|Casting|CastToSave_GameConfig _returnvalue_3))
  (Variables|/Game/Blueprints/Saves/Save_GameConfig.Save_GameConfig_C|SetShuffleTracks _assave_game_config true)
  (SaveGame|SaveGametoSlot _assave_game_config _configsavename)
  (Audio|Components|Audio|SetVolumeMultiplier (Variables|Default|GetAudio) (* (Variables|/Game/Blueprints/Saves/Save_GameConfig.Save_GameConfig_C|GetMainVol _assave_game_config) (Variables|/Game/Blueprints/Saves/Save_GameConfig.Save_GameConfig_C|GetMusicVol _assave_game_config)) :!class /Script/Engine.AudioComponent)
  (bind _output_get (Variables|Default|SetCurrentTrack (Utilities|Array|Get(acopy) (Variables|Default|GetTracks))))
  (Audio|Components|Audio|SetSound _audio _output_get)
  (Audio|Components|Audio|Play _audio 0.0)
  (Variables|Default|SetShuffle (Variables|/Game/Blueprints/Saves/Save_GameConfig.Save_GameConfig_C|GetShuffleTracks _assave_game_config)))

(fn ConstructionScript)