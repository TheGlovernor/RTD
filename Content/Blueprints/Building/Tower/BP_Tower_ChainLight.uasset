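; Chain lightning tower that fires BP_ChainProj bolts from its barrel, which jump between enemies.
; Attack fires at the first targetable once aimed and re-arms its timer from an attribute, or retries shortly when it cannot fire.
; Stats are GAS Companion attributes: LevelUp applies GE_Chain_LevelUp, and post-effect handling clamps values and updates range.
; ReportStats pushes stats and a rich-text description to the selection widget after attribute changes.
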(event OnPostGameplayEffectExecute(GSCCore)
  (params (Attribute :type Gameplay%20Attribute%20Structure) (SourceActor :type Actor%20Object%20Reference) (TargetActor :type Actor%20Object%20Reference) (SourceTags :type Gameplay%20Tag%20Container%20Structure%20%28by%20ref%29) (Payload :type GSC%20Gameplay%20Effect%20Execute%20Data%20Structure))
  (|SwitchGameplayAttribute Attribute
    (:Level
      (Class|GSCCoreComponent|ClampAttributeValue (Variables|Default|GetGSCCore) "(AttributeName=\"Level\",Attribute=/Script/RTD.TowerAttributeSet:Level,AttributeOwner=Class'\"/Script/RTD.TowerAttributeSet\"')" 0.0 1e+08))
    (:AttackPower
      (Class|GSCCoreComponent|ClampAttributeValue (Variables|Default|GetGSCCore) "(AttributeName=\"AttackPower\",Attribute=/Script/RTD.TowerAttributeSet:AttackPower,AttributeOwner=Class'\"/Script/RTD.TowerAttributeSet\"')" 0.0 1e+08))
    (:AttackSpeed
      (Class|GSCCoreComponent|ClampAttributeValue (Variables|Default|GetGSCCore) "(AttributeName=\"AttackSpeed\",Attribute=/Script/RTD.TowerAttributeSet:AttackSpeed,AttributeOwner=Class'\"/Script/RTD.TowerAttributeSet\"')" 0.01 1e+08))
    (:Range
      (Class|GSCCoreComponent|ClampAttributeValue (Variables|Default|GetGSCCore) "(AttributeName=\"Range\",Attribute=/Script/RTD.TowerAttributeSet:Range,AttributeOwner=Class'\"/Script/RTD.TowerAttributeSet\"')" 0.0 1e+08)
      (CallFunction|UpdateRange))
    (:CurrentTargets
      (Class|GSCCoreComponent|ClampAttributeValue (Variables|Default|GetGSCCore) "(AttributeName=\"CurrentTargets\",Attribute=/Script/RTD.TowerAttributeSet:CurrentTargets,AttributeOwner=Class'\"/Script/RTD.TowerAttributeSet\"')" 0.0 1e+08))
    (:MaxTargets
      (Class|GSCCoreComponent|ClampAttributeValue (Variables|Default|GetGSCCore) "(AttributeName=\"MaxTargets\",Attribute=/Script/RTD.TowerAttributeSet:MaxTargets,AttributeOwner=Class'\"/Script/RTD.TowerAttributeSet\"')" 0.0 1e+08))
    (:CritChance
      (Class|GSCCoreComponent|ClampAttributeValue (Variables|Default|GetGSCCore) "(AttributeName=\"CritChance\",Attribute=/Script/RTD.TowerAttributeSet:CritChance,AttributeOwner=Class'\"/Script/RTD.TowerAttributeSet\"')" 0.0 1e+08))
    (:CritX
      (Class|GSCCoreComponent|ClampAttributeValue (Variables|Default|GetGSCCore) "(AttributeName=\"CritX\",Attribute=/Script/RTD.TowerAttributeSet:CritX,AttributeOwner=Class'\"/Script/RTD.TowerAttributeSet\"')" 1.0 1e+08))
    (:MaxItems
      (Class|GSCCoreComponent|ClampAttributeValue (Variables|Default|GetGSCCore) "(AttributeName=\"MaxItems\",Attribute=/Script/RTD.TowerAttributeSet:MaxItems,AttributeOwner=Class'\"/Script/RTD.TowerAttributeSet\"')" 0.0 1e+08))
    (:BuyValue
      (Class|GSCCoreComponent|ClampAttributeValue (Variables|Default|GetGSCCore) "(AttributeName=\"BuyValue\",Attribute=/Script/RTD.TowerAttributeSet:BuyValue,AttributeOwner=Class'\"/Script/RTD.TowerAttributeSet\"')" 0.0 1e+08))
    (:UpgradeValue
      (Class|GSCCoreComponent|ClampAttributeValue (Variables|Default|GetGSCCore) "(AttributeName=\"UpgradeValue\",Attribute=/Script/RTD.TowerAttributeSet:UpgradeValue,AttributeOwner=Class'\"/Script/RTD.TowerAttributeSet\"')" 0.0 1e+08))
    (:SellValue
      (Class|GSCCoreComponent|ClampAttributeValue (Variables|Default|GetGSCCore) "(AttributeName=\"SellValue\",Attribute=/Script/RTD.TowerAttributeSet:SellValue,AttributeOwner=Class'\"/Script/RTD.TowerAttributeSet\"')" 0.0 1e+08)))
  (CallFunction|ReportStats))

(event EventBeginPlay
  (|CallParentFunction) ; This node is disabled and will not be called.\nDrag off pins to build functionality.
)

(event Collision|EventActorBeginOverlap
  (params (OtherActor :type Actor%20Object%20Reference))
  (|CallParentFunction OtherActor) ; This node is disabled and will not be called.\nDrag off pins to build functionality.
)

(event EventTick
  (params (DeltaSeconds :type Float%20%28single-precision%29))
  (|CallParentFunction DeltaSeconds))

(event EventAttack
  (if (and (Utilities|Array|IsValidIndex (Variables|Default|GetTargetables)) (Variables|Default|GetAimed))
    (Game|SpawnActorfromClass "/Game/Blueprints/Building/Tower/Projs_Beams/BP_ChainProj.BP_ChainProj_C" (Math|Conversions|ToTransform(Vector) (Transformation|GetSocketLocation (Variables|Default|GetChain) "BarrelEnd")) "AlwaysSpawn" 0 (Utilities|Array|Get(acopy) (Variables|Default|GetTargetables)) (Class|GSCCoreComponent|GetCurrentAttributeValue (Variables|Default|GetGSCCore) "(AttributeName=\"AttackPower\",Attribute=/Script/RTD.TowerAttributeSet:AttackPower,AttributeOwner=Class'\"/Script/RTD.TowerAttributeSet\"')") (Math|Float|Floor (Class|GSCCoreComponent|GetCurrentAttributeValue (Variables|Default|GetGSCCore) "(AttributeName=\"CurrentTargets\",Attribute=/Script/RTD.TowerAttributeSet:CurrentTargets,AttributeOwner=Class'\"/Script/RTD.TowerAttributeSet\"')")) (Variables|Default|GetDamageTypeClass) 0)
    (bind _returnvalue (Utilities|Time|SetTimerbyEvent (delegate EventAttack) (Class|GSCCoreComponent|GetCurrentAttributeValue (Variables|Default|GetGSCCore) "(AttributeName=\"AttackSpeed\",Attribute=/Script/RTD.TowerAttributeSet:AttackSpeed,AttributeOwner=Class'\"/Script/RTD.TowerAttributeSet\"')")))
    (Variables|Default|SetAttack%20Timer _returnvalue)
    (else
      (bind _returnvalue_2 (Utilities|Time|SetTimerbyEvent (delegate EventAttack) 0.1))
      (Variables|Default|SetAttack%20Timer _returnvalue_2))))

(event EventLevelUp
  (|CallParentFunction)
  (GameplayEffects|ApplyGameplayEffectToSelf :self (Variables|Default|GetGSCAbilitySystem) :GameplayEffectClass "/Game/Blueprints/Building/Tower/Stats/GE_Chain_LevelUp.GE_Chain_LevelUp_C" :Level 1.0))

(fn ConstructionScript
  (|CallParentFunction))

(fn ReportStats
  (bind _gsccore (Variables|Default|GetGSCCore))
  (bind _gsccore_2 (Variables|Default|GetGSCCore))
  (bind _rowname (CallFunction|GetDisplayData (Variables|Default|GetDamageTypeClass)))
  (Class|BPISelectionWidget|ReportStats(Message) (UserInterface|GetWidget (Variables|Default|GetSelectionWidget)) self (Components|GetOwner) (Variables|Default|GetTowerName) (Variables|Default|GetIcon) (Utilities|Array|MakeArray (Utilities|Text|ToText(String) (Utilities|String|Replace (Utilities|String|Replace (Utilities|String|Replace (Utilities|String|ToString(Text) (Utilities|Text|MakeLiteralText "Fires a bolt of lightning that jumps to a max total of <RichText.Emphasis>TARGETS</> enemies, dealing <img id=\"ROW\"/><RichText.ROW> DMG</> damage to each.")) "ROW" _rowname "CaseSensitive") "DMG" (Utilities|String|ToString(Float) (Class|GSCCoreComponent|GetCurrentAttributeValue _gsccore "(AttributeName=\"AttackPower\",Attribute=/Script/RTD.TowerAttributeSet:AttackPower,AttributeOwner=Class'\"/Script/RTD.TowerAttributeSet\"')")) "CaseSensitive") "TARGETS" (Utilities|String|ToString(Integer) (Math|Float|Round (Class|GSCCoreComponent|GetCurrentAttributeValue _gsccore "(AttributeName=\"CurrentTargets\",Attribute=/Script/RTD.TowerAttributeSet:CurrentTargets,AttributeOwner=Class'\"/Script/RTD.TowerAttributeSet\"')"))) "CaseSensitive"))) (Math|Float|Truncate (Class|GSCCoreComponent|GetCurrentAttributeValue _gsccore_2 "(AttributeName=\"Level\",Attribute=/Script/RTD.TowerAttributeSet:Level,AttributeOwner=Class'\"/Script/RTD.TowerAttributeSet\"')")) (Class|GSCCoreComponent|GetCurrentAttributeValue _gsccore_2 "(AttributeName=\"AttackPower\",Attribute=/Script/RTD.TowerAttributeSet:AttackPower,AttributeOwner=Class'\"/Script/RTD.TowerAttributeSet\"')") (Class|GSCCoreComponent|GetCurrentAttributeValue _gsccore_2 "(AttributeName=\"AttackSpeed\",Attribute=/Script/RTD.TowerAttributeSet:AttackSpeed,AttributeOwner=Class'\"/Script/RTD.TowerAttributeSet\"')") (Class|GSCCoreComponent|GetCurrentAttributeValue _gsccore_2 "(AttributeName=\"Range\",Attribute=/Script/RTD.TowerAttributeSet:Range,AttributeOwner=Class'\"/Script/RTD.TowerAttributeSet\"')") (Class|GSCCoreComponent|GetCurrentAttributeValue _gsccore_2 "(AttributeName=\"CritChance\",Attribute=/Script/RTD.TowerAttributeSet:CritChance,AttributeOwner=Class'\"/Script/RTD.TowerAttributeSet\"')") 0 (Variables|Default|GetUpgradeCost) (Variables|Default|GetSellValue) (Variables|Default|GetItems) (Variables|Default|GetAvailableModes) (Variables|Default|GetTargetingMode) (Variables|Default|GetTargetingPriority)))