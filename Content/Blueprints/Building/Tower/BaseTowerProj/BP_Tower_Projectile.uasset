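; Projectile tower Blueprint that attacks its current target by firing basic projectiles.
; On each Tick with a valid Target, it spawns a scaled-up BP_Projectile_Basic at its PointLight, passing the Target and AttackPower as damage.
; Without a valid Target, it calls GetNewTarget instead of firing.
; The graph has no cooldown check, so the firing rate follows the actor's tick rate.
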(event EventBeginPlay
  (|CallParentFunction) ; This node is disabled and will not be called.\nDrag off pins to build functionality.
)

(event Collision|EventActorBeginOverlap
  (params (OtherActor :type Actor%20Object%20Reference))
  (|CallParentFunction OtherActor) ; This node is disabled and will not be called.\nDrag off pins to build functionality.
)

(event EventTick
  (params (DeltaSeconds :type Float%20%28single-precision%29))
  (bind _target (Variables|Default|GetTarget)
    (:then
      (Game|SpawnActorfromClass "/Game/Blueprints/Building/Projectiles/BP_Projectile_Basic.BP_Projectile_Basic_C" (Math|Transform|MakeTransform (Transformation|GetWorldLocation (Variables|Default|GetPointLight)) "0, 0, 0" "5.000000,5.000000,5.000000") "Undefined" self _target (Variables|Default|GetAttackPower) 0))
    (:else
      (bind _newtarget (CallFunction|GetNewTarget))
      (Variables|Default|SetTarget _newtarget))))

(fn ConstructionScript
  (|CallParentFunction))