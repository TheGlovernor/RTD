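; Basic tower projectile that homes in on a Target actor.
; Each tick it caches the target's location, so it keeps heading to the last known point if the target becomes invalid, and moves MovementSpeed units toward it without delta-time scaling or sweep.
; A distance check against MovementSpeed then either rotates it toward that point or destroys it.
; Overlapping the Target also disables tick and destroys it, with no damage applied here.
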(event EventBeginPlay)

(event Collision|EventActorBeginOverlap
  (params (OtherActor :type Actor%20Object%20Reference))
  (if (== OtherActor (Variables|Default|GetTarget))
    (Actor|Tick|SetActorTickEnabled false)
    (Actor|DestroyActor)))

(event EventTick
  (params (DeltaSeconds :type Float%20%28single-precision%29))
  (bind _defaultsceneroot (Variables|Default|GetDefaultSceneRoot))
  (bind _movementspeed (Variables|Default|GetMovementSpeed))
  (bind _returnvalue (Transformation|GetWorldLocation _defaultsceneroot))
  (Utilities|IsValid (Variables|Default|GetTarget)
    (:Is%20Valid
      (Variables|Default|SetLastKnownLocation (Transformation|GetWorldLocation (Variables|/Game/Blueprints/Mobs/BP_Enemy_Base_01.BP_Enemy_Base_01_C|GetDefaultSceneRoot (Variables|Default|GetTarget)))))
    (:Is%20Not%20Valid
      _))
  (Transformation|AddActorWorldOffset (* _movementspeed (Math|Vector|GetUnitDirection(Vector) _returnvalue (Variables|Default|GetLastKnownLocation))))
  (if (< (Math|Vector|Distance(Vector) _returnvalue (Variables|Default|GetLastKnownLocation)) _movementspeed)
    (if (Class|Actor|IsActorTickEnabled)
      (Transformation|SetActorRotation (Math|Conversions|RotationFromXVector (Math|Vector|GetUnitDirection(Vector) _returnvalue (Variables|Default|GetLastKnownLocation)))))
    (else
      (Actor|Tick|SetActorTickEnabled false)
      (Actor|DestroyActor))))

(fn ConstructionScript)