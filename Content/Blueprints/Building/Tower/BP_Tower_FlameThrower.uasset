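; Flamethrower tower that burns enemies in a line ahead of it, applying a status effect and damage with a chance-based damage multiplier.
; Attack loops on short delays while a target exists, sphere-tracing along the flame's forward vector and hitting each unique actor; otherwise it switches the flame off.
; UpdateRange scales Niagara particle velocity from GSCCore attributes.
; ReportStats fills the selection widget with attribute-driven rich text describing damage and stacking ignite.
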(event EventAttack
  (bind _targetables (Variables|Default|GetTargetables))
  (bind _flame (Variables|Default|Getflame))
  (bind _niagara (Variables|Default|GetNiagara))
  (bind _gsccore (Variables|Default|GetGSCCore))
  (bind _hitactors (Variables|Default|GetHitActors))
  (bind _returnvalue (Class|GSCCoreComponent|GetCurrentAttributeValue _gsccore "(AttributeName=\"AttackPower\",Attribute=/Script/RTD.TowerAttributeSet:AttackPower,AttributeOwner=Class'\"/Script/RTD.TowerAttributeSet\"')"))
  (bind _returnvalue_2 (Transformation|GetWorldLocation _niagara))
  (bind _returnvalue_3 (Math|Vector|GetForwardVector _flame))
  (Utilities|Array|Clear (Variables|Default|GetHitActors))
  (if (Utilities|Array|IsValidIndex _targetables)
    (Utilities|IsValid (Utilities|Array|Get(acopy) _targetables)
      (:Is%20Valid
        (Components|Activation|Activate _niagara false)
        (bind _outhits (Collision|MultiSphereTraceByChannel _returnvalue_2 (+ _returnvalue_2 (* _returnvalue_3 (Class|GSCCoreComponent|GetCurrentAttributeValue (Variables|Default|GetGSCCore) "(AttributeName=\"Range\",Attribute=/Script/RTD.TowerAttributeSet:Range,AttributeOwner=Class'\"/Script/RTD.TowerAttributeSet\"')") "1.000000,1.000000,0.000000") (* _returnvalue_3 "-1.000000,-1.000000,0.000000" "250.000000,250.000000,0")) 1.5e+02 "TraceTypeQuery6" false 0 "ForDuration"))
        (for _array_element _outhits
          (Utilities|Array|AddUnique _hitactors (.HitActor (Collision|BreakHitResult _array_element))))
        (for _array_element_2 _hitactors
          (CallFunction|ApplyStatusEffect _array_element_2)
          (Game|Damage|ApplyDamage _array_element_2 (select (> (Class|GSCCoreComponent|GetCurrentAttributeValue _gsccore "(AttributeName=\"CritChance\",Attribute=/Script/RTD.TowerAttributeSet:CritChance,AttributeOwner=Class'\"/Script/RTD.TowerAttributeSet\"')") (Math|Random|RandomFloat)) (* _returnvalue (Class|GSCCoreComponent|GetCurrentAttributeValue _gsccore "(AttributeName=\"CritX\",Attribute=/Script/RTD.TowerAttributeSet:CritX,AttributeOwner=Class'\"/Script/RTD.TowerAttributeSet\"')")) _returnvalue) 0 0 (Variables|Default|GetDamageTypeClass)))
        (Utilities|FlowControl|Delay (/ 1.0 4.0))
        (CallFunction|Attack))
      (:Is%20Not%20Valid
        (Components|Activation|Deactivate (Variables|Default|GetNiagara) :!label _label)
        (Utilities|FlowControl|Delay 0.1)
        (CallFunction|Attack)))
    (else
      (goto _label))))

(fn ConstructionScript
  (|CallParentFunction)
  (CallFunction|CalculateTowerStats)
  (CallFunction|ToggleSelect false))

(fn ReportStats
  (bind _gsccore (Variables|Default|GetGSCCore))
  (bind _returnvalue (Class|GSCCoreComponent|GetCurrentAttributeValue _gsccore "(AttributeName=\"AttackPower\",Attribute=/Script/RTD.TowerAttributeSet:AttackPower,AttributeOwner=Class'\"/Script/RTD.TowerAttributeSet\"')"))
  (bind _rowname (CallFunction|GetDisplayData (Variables|Default|GetDamageTypeClass)))
  (Class|BPISelectionWidget|ReportStats(Message) (UserInterface|GetWidget (Variables|Default|GetSelectionWidget)) self (Components|GetOwner) (Variables|Default|GetTowerName) (Variables|Default|GetIcon) (Utilities|Array|MakeArray (Utilities|Text|ToText(String) (Utilities|String|Replace (Utilities|String|Replace (Utilities|String|Replace (Utilities|String|Replace (Utilities|String|ToString(Text) (Utilities|Text|MakeLiteralText "Shoots flames at it's target, dealing <img id=\"ROW\"/><RichText.ROW>DMG</> to any enemies caught in it. Has a <RichText.Emphasis>CHANCE</> chance to ignite the enemy, dealing <img id=\"ROW\"/><RichText.ROW>EFFDAM</> damage every 1s for 3s, Can stack.")) "CHANCE" (Utilities|String|ToString(Text) (Class|KismetTextLibrary|AsPercentFloat (Class|GSCCoreComponent|GetCurrentAttributeValue _gsccore "(AttributeName=\"EngulfChance\",Attribute=/Script/RTD.TowerAttributeSet:EngulfChance,AttributeOwner=Class'\"/Script/RTD.TowerAttributeSet\"')") "HalfToEven")) "CaseSensitive") "EFFDAM" (Utilities|String|ToString(Float) (* (Class|GSCCoreComponent|GetCurrentAttributeValue _gsccore "(AttributeName=\"EngulfPower\",Attribute=/Script/RTD.TowerAttributeSet:EngulfPower,AttributeOwner=Class'\"/Script/RTD.TowerAttributeSet\"')") _returnvalue)) "CaseSensitive") "ROW" _rowname "CaseSensitive") "DMG" (Utilities|String|ToString(Float) _returnvalue) "CaseSensitive"))) (Variables|Default|GetUpgradeCost) (Variables|Default|GetSellValue) (Variables|Default|GetItems) (Variables|Default|GetAvailableModes) (Variables|Default|GetTargetingMode) (Variables|Default|GetTargetingPriority)))

(fn UpdateRange
  (bind _niagara (Variables|Default|GetNiagara))
  (bind _gsccore (Variables|Default|GetGSCCore))
  (bind _returnvalue (Class|GSCCoreComponent|GetCurrentAttributeValue _gsccore "(AttributeName=\"Range\",Attribute=/Script/RTD.TowerAttributeSet:Range,AttributeOwner=Class'\"/Script/RTD.TowerAttributeSet\"')"))
  (bind _returnvalue_2 (Math|Float|MapRangeUnclamped _returnvalue 1e+03 8e+03 0.5 1.0))
  (bind _returnvalue_3 (* _returnvalue _returnvalue_2))
  (|CallParentFunction)
  (Effects|Components|ParticleSystem|SetFloatParameter _niagara "User.MinInitVelocity" (- _returnvalue_3 1e+02))
  (Effects|Components|ParticleSystem|SetFloatParameter _niagara "User.MaxInitVelocity" _returnvalue_3))