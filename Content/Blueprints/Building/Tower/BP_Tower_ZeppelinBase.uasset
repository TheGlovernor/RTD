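; Tower Blueprint that attacks through a spawned BP_Zeppelin, overriding its own attack events as empty.
; On BeginPlay it spawns the zeppelin above itself with damage and attack rate from GAS attributes, then a re-arming timer hands it the first acquired target.
; Leveling applies a gameplay effect.
; Attribute changes are clamped, reported to the selection widget and pushed to the zeppelin, with Range also updating the tower's range.
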(event EventLevelUp
  (|CallParentFunction)
  (GameplayEffects|ApplyGameplayEffectToSelf :self (Variables|Default|GetGSCAbilitySystem) :GameplayEffectClass "/Game/Blueprints/Building/Tower/Stats/GE_GAT_LevelUp.GE_GAT_LevelUp_C" :Level 1.0))

(event EventBeginPlay
  (bind _gsccore (Variables|Default|GetGSCCore))
  (|CallParentFunction)
  (bind _returnvalue (Game|SpawnActorfromClass "/Game/Blueprints/Building/Tower/Projs_Beams/BP_Zeppelin.BP_Zeppelin_C" (Math|Conversions|ToTransform(Vector) (+ (Transformation|GetWorldLocation (Variables|Default|GetDefaultSceneRoot)) "0,0,50.000000")) "Undefined" 0 0 (Variables|Default|GetDamageTypeClass) (Class|GSCCoreComponent|GetCurrentAttributeValue _gsccore "(AttributeName=\"AttackPower\",Attribute=/Script/RTD.TowerAttributeSet:AttackPower,AttributeOwner=Class'\"/Script/RTD.TowerAttributeSet\"')") (Class|GSCCoreComponent|GetCurrentAttributeValue _gsccore "(AttributeName=\"AttackSpeed\",Attribute=/Script/RTD.TowerAttributeSet:AttackSpeed,AttributeOwner=Class'\"/Script/RTD.TowerAttributeSet\"')") 25.0 0))
  (Variables|Default|SetZeppelins _returnvalue)
  (Utilities|Time|SetTimerbyEvent (delegate EventGetTargets) 0.5))

(event EventGetTargets
  (bind _targetableenemies (CallFunction|AcquireTargets))
  (bind _output_get (Variables|Default|SetTargetables _targetableenemies))
  (if (Utilities|Array|IsNotEmpty _output_get)
    (Utilities|Time|SetTimerbyEvent (delegate EventGetTargets) 1.0)
    (Variables|/Game/Blueprints/Building/Tower/Projs_Beams/BP_Zeppelin.BP_Zeppelin_C|SetTarget (Variables|Default|GetZeppelins) (Utilities|Array|Get(acopy) (Variables|Default|GetTargetables)))
    (else
      (Utilities|Time|SetTimerbyEvent (delegate EventGetTargets) 0.1))))

(event EventAttemptAttack)

(event EventAttack)

(event OnPostGameplayEffectExecute(GSCCore)
  (params (Attribute :type Gameplay%20Attribute%20Structure) (SourceActor :type Actor%20Object%20Reference) (TargetActor :type Actor%20Object%20Reference) (SourceTags :type Gameplay%20Tag%20Container%20Structure%20%28by%20ref%29) (Payload :type GSC%20Gameplay%20Effect%20Execute%20Data%20Structure))
  (bind _gsccore (Variables|Default|GetGSCCore))
  (|SwitchGameplayAttribute Attribute
    (:Level
      (Class|GSCCoreComponent|ClampAttributeValue (Variables|Default|GetGSCCore) "(AttributeName=\"Level\",Attribute=/Script/RTD.TowerAttributeSet:Level,AttributeOwner=Class'\"/Script/RTD.TowerAttributeSet\"')" 0.0 1e+08))
    (:AttackPower
      (Class|GSCCoreComponent|ClampAttributeValue (Variables|Default|GetGSCCore) "(AttributeName=\"AttackPower\",Attribute=/Script/RTD.TowerAttributeSet:AttackPower,AttributeOwner=Class'\"/Script/RTD.TowerAttributeSet\"')" 0.0 1e+08))
    (:AttackSpeed
      (Class|GSCCoreComponent|ClampAttributeValue (Variables|Default|GetGSCCore) "(AttributeName=\"AttackSpeed\",Attribute=/Script/RTD.TowerAttributeSet:AttackSpeed,AttributeOwner=Class'\"/Script/RTD.TowerAttributeSet\"')" 0.01 1e+08))
    (:Range
      (Class|GSCCoreComponent|ClampAttributeValue (Variables|Default|GetGSCCore) "(AttributeName=\"Range\",Attribute=/Script/RTD.TowerAttributeSet:Range,AttributeOwner=Class'\"/Script/RTD.TowerAttributeSet\"')" 0.0 1e+08)
      (CallFunction|UpdateRange))
    (:CurrentTargets
      (Class|GSCCoreComponent|ClampAttributeValue (Variables|Default|GetGSCCore) "(AttributeName=\"CurrentTargets\",Attribute=/Script/RTD.TowerAttributeSet:CurrentTargets,AttributeOwner=Class'\"/Script/RTD.TowerAttributeSet\"')" 0.0 1e+08))
    (:MaxTargets
      (Class|GSCCoreComponent|ClampAttributeValue (Variables|Default|GetGSCCore) "(AttributeName=\"MaxTargets\",Attribute=/Script/RTD.TowerAttributeSet:MaxTargets,AttributeOwner=Class'\"/Script/RTD.TowerAttributeSet\"')" 0.0 1e+08))
    (:CritChance
      (Class|GSCCoreComponent|ClampAttributeValue (Variables|Default|GetGSCCore) "(AttributeName=\"CritChance\",Attribute=/Script/RTD.TowerAttributeSet:CritChance,AttributeOwner=Class'\"/Script/RTD.TowerAttributeSet\"')" 0.0 1e+08))
    (:CritX
      (Class|GSCCoreComponent|ClampAttributeValue (Variables|Default|GetGSCCore) "(AttributeName=\"CritX\",Attribute=/Script/RTD.TowerAttributeSet:CritX,AttributeOwner=Class'\"/Script/RTD.TowerAttributeSet\"')" 1.0 1e+08))
    (:MaxItems
      (Class|GSCCoreComponent|ClampAttributeValue (Variables|Default|GetGSCCore) "(AttributeName=\"MaxItems\",Attribute=/Script/RTD.TowerAttributeSet:MaxItems,AttributeOwner=Class'\"/Script/RTD.TowerAttributeSet\"')" 0.0 1e+08))
    (:BuyValue
      (Class|GSCCoreComponent|ClampAttributeValue (Variables|Default|GetGSCCore) "(AttributeName=\"BuyValue\",Attribute=/Script/RTD.TowerAttributeSet:BuyValue,AttributeOwner=Class'\"/Script/RTD.TowerAttributeSet\"')" 0.0 1e+08))
    (:UpgradeValue
      (Class|GSCCoreComponent|ClampAttributeValue (Variables|Default|GetGSCCore) "(AttributeName=\"UpgradeValue\",Attribute=/Script/RTD.TowerAttributeSet:UpgradeValue,AttributeOwner=Class'\"/Script/RTD.TowerAttributeSet\"')" 0.0 1e+08))
    (:SellValue
      (Class|GSCCoreComponent|ClampAttributeValue (Variables|Default|GetGSCCore) "(AttributeName=\"SellValue\",Attribute=/Script/RTD.TowerAttributeSet:SellValue,AttributeOwner=Class'\"/Script/RTD.TowerAttributeSet\"')" 0.0 1e+08)))
  (CallFunction|ReportStats)
  (bind _zeppelins (Variables|Default|GetZeppelins)
    (:then
      (Default|UpdateStats _zeppelins (Variables|Default|GetDamageTypeClass) (Class|GSCCoreComponent|GetCurrentAttributeValue _gsccore "(AttributeName=\"AttackPower\",Attribute=/Script/RTD.TowerAttributeSet:AttackPower,AttributeOwner=Class'\"/Script/RTD.TowerAttributeSet\"')") (Class|GSCCoreComponent|GetCurrentAttributeValue _gsccore "(AttributeName=\"AttackSpeed\",Attribute=/Script/RTD.TowerAttributeSet:AttackSpeed,AttributeOwner=Class'\"/Script/RTD.TowerAttributeSet\"')")))
    (:else)))

(fn ConstructionScript
  (|CallParentFunction)
  (CallFunction|CalculateTowerStats)
  (CallFunction|ToggleSelect false))

(fn ReportStats
  (bind _gsccore (Variables|Default|GetGSCCore))
  (Class|BPISelectionWidget|ReportStats(Message) (UserInterface|GetWidget (Variables|Default|GetSelectionWidget)) self (Components|GetOwner) (Variables|Default|GetTowerName) (Variables|Default|GetIcon) (Utilities|Array|MakeArray "") (Math|Float|Truncate (Class|GSCCoreComponent|GetCurrentAttributeValue _gsccore "(AttributeName=\"Level\",Attribute=/Script/RTD.TowerAttributeSet:Level,AttributeOwner=Class'\"/Script/RTD.TowerAttributeSet\"')")) (Class|GSCCoreComponent|GetCurrentAttributeValue _gsccore "(AttributeName=\"AttackPower\",Attribute=/Script/RTD.TowerAttributeSet:AttackPower,AttributeOwner=Class'\"/Script/RTD.TowerAttributeSet\"')") (Class|GSCCoreComponent|GetCurrentAttributeValue _gsccore "(AttributeName=\"AttackSpeed\",Attribute=/Script/RTD.TowerAttributeSet:AttackSpeed,AttributeOwner=Class'\"/Script/RTD.TowerAttributeSet\"')") (Class|GSCCoreComponent|GetCurrentAttributeValue _gsccore "(AttributeName=\"Range\",Attribute=/Script/RTD.TowerAttributeSet:Range,AttributeOwner=Class'\"/Script/RTD.TowerAttributeSet\"')") (Class|GSCCoreComponent|GetCurrentAttributeValue _gsccore "(AttributeName=\"CritChance\",Attribute=/Script/RTD.TowerAttributeSet:CritChance,AttributeOwner=Class'\"/Script/RTD.TowerAttributeSet\"')") 0 (Variables|Default|GetUpgradeCost) (Variables|Default|GetSellValue) (Variables|Default|GetItems) (Variables|Default|GetAvailableModes) (Variables|Default|GetTargetingMode) (Variables|Default|GetTargetingPriority)))