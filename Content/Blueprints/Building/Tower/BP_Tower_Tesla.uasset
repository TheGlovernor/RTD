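; Tesla tower Blueprint that shocks targeted enemies with lightning, with chances to crit and stun per its tooltip.
; Attack re-invokes itself on attribute-driven delays, giving each entry in Targetables a short-lived Niagara beam, crit-rolled damage and a status effect.
; GSCCore attribute changes are clamped, refresh range when relevant, and trigger ReportStats.
; ReportStats sends the selection widget tower data and a rich-text description built by token replacement.
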(event OnPostGameplayEffectExecute(GSCCore)
  (params (Attribute :type Gameplay%20Attribute%20Structure) (SourceActor :type Actor%20Object%20Reference) (TargetActor :type Actor%20Object%20Reference) (SourceTags :type Gameplay%20Tag%20Container%20Structure%20%28by%20ref%29) (Payload :type GSC%20Gameplay%20Effect%20Execute%20Data%20Structure))
  (Utilities|FlowControl|Sequence
    (:then_0
      (|SwitchGameplayAttribute Attribute
        (:Level
          (Class|GSCCoreComponent|ClampAttributeValue (Variables|Default|GetGSCCore) "(AttributeName=\"Level\",Attribute=/Script/RTD.TowerAttributeSet:Level,AttributeOwner=Class'\"/Script/RTD.TowerAttributeSet\"')" 0.0 1e+08))
        (:AttackPower
          (Class|GSCCoreComponent|ClampAttributeValue (Variables|Default|GetGSCCore) "(AttributeName=\"AttackPower\",Attribute=/Script/RTD.TowerAttributeSet:AttackPower,AttributeOwner=Class'\"/Script/RTD.TowerAttributeSet\"')" 0.0 1e+08))
        (:AttackSpeed
          (Class|GSCCoreComponent|ClampAttributeValue (Variables|Default|GetGSCCore) "(AttributeName=\"AttackSpeed\",Attribute=/Script/RTD.TowerAttributeSet:AttackSpeed,AttributeOwner=Class'\"/Script/RTD.TowerAttributeSet\"')" 0.05 1e+08))
        (:Range
          (Class|GSCCoreComponent|ClampAttributeValue (Variables|Default|GetGSCCore) "(AttributeName=\"Range\",Attribute=/Script/RTD.TowerAttributeSet:Range,AttributeOwner=Class'\"/Script/RTD.TowerAttributeSet\"')" 0.0 1e+08)
          (CallFunction|UpdateRange))
        (:CurrentTargets
          (Class|GSCCoreComponent|ClampAttributeValue (Variables|Default|GetGSCCore) "(AttributeName=\"CurrentTargets\",Attribute=/Script/RTD.TowerAttributeSet:CurrentTargets,AttributeOwner=Class'\"/Script/RTD.TowerAttributeSet\"')" 0.0 1e+08))
        (:MaxTargets
          (Class|GSCCoreComponent|ClampAttributeValue (Variables|Default|GetGSCCore) "(AttributeName=\"MaxTargets\",Attribute=/Script/RTD.TowerAttributeSet:MaxTargets,AttributeOwner=Class'\"/Script/RTD.TowerAttributeSet\"')" 0.0 1e+08))
        (:CritChance
          (Class|GSCCoreComponent|ClampAttributeValue (Variables|Default|GetGSCCore) "(AttributeName=\"CritChance\",Attribute=/Script/RTD.TowerAttributeSet:CritChance,AttributeOwner=Class'\"/Script/RTD.TowerAttributeSet\"')" 0.0 1e+08))
        (:MaxItems
          (Class|GSCCoreComponent|ClampAttributeValue (Variables|Default|GetGSCCore) "(AttributeName=\"MaxItems\",Attribute=/Script/RTD.TowerAttributeSet:MaxItems,AttributeOwner=Class'\"/Script/RTD.TowerAttributeSet\"')" 0.0 1e+08))
        (:BuyValue
          (Class|GSCCoreComponent|ClampAttributeValue (Variables|Default|GetGSCCore) "(AttributeName=\"BuyValue\",Attribute=/Script/RTD.TowerAttributeSet:BuyValue,AttributeOwner=Class'\"/Script/RTD.TowerAttributeSet\"')" 0.0 1e+08))
        (:UpgradeValue
          (Class|GSCCoreComponent|ClampAttributeValue (Variables|Default|GetGSCCore) "(AttributeName=\"UpgradeValue\",Attribute=/Script/RTD.TowerAttributeSet:UpgradeValue,AttributeOwner=Class'\"/Script/RTD.TowerAttributeSet\"')" 0.0 1e+08))
        (:SellValue
          (Class|GSCCoreComponent|ClampAttributeValue (Variables|Default|GetGSCCore) "(AttributeName=\"SellValue\",Attribute=/Script/RTD.TowerAttributeSet:SellValue,AttributeOwner=Class'\"/Script/RTD.TowerAttributeSet\"')" 0.0 1e+08))
        (:CritX
          (Class|GSCCoreComponent|ClampAttributeValue (Variables|Default|GetGSCCore) "(AttributeName=\"CritX\",Attribute=/Script/RTD.TowerAttributeSet:CritX,AttributeOwner=Class'\"/Script/RTD.TowerAttributeSet\"')" 0.0 1e+08))))
    (:then_1
      (CallFunction|ReportStats))))

(event EventBeginPlay
  (|CallParentFunction))

(event EventAttack
  (bind _targetables (Variables|Default|GetTargetables))
  (bind _gsccore (Variables|Default|GetGSCCore))
  (bind _returnvalue (Class|GSCCoreComponent|GetCurrentAttributeValue _gsccore "(AttributeName=\"AttackPower\",Attribute=/Script/RTD.TowerAttributeSet:AttackPower,AttributeOwner=Class'\"/Script/RTD.TowerAttributeSet\"')"))
  (if (Utilities|Array|IsNotEmpty _targetables)
    (for _array_element _targetables
      (Utilities|IsValid _array_element
        (:Is%20Valid
          (bind _location (Class|EnemyInterface|ReportTargetPoint(Message) _array_element))
          (bind _returnvalue_2 (AddComponent|AddNiagaraComponent false))
          (Effects|Components|ParticleSystem|SetVectorParameter _returnvalue_2 "User.BeamStartpoint" (+ (Transformation|GetActorLocation) "0,0,400.000000"))
          (Effects|Components|ParticleSystem|SetVectorParameter _returnvalue_2 "User.BeamEndpoint" _location)
          (Components|Activation|Activate _returnvalue_2 false)
          (Game|Damage|ApplyDamage _array_element (Math|Float|SelectFloat _returnvalue (* _returnvalue (Class|GSCCoreComponent|GetCurrentAttributeValue _gsccore "(AttributeName=\"CritX\",Attribute=/Script/RTD.TowerAttributeSet:CritX,AttributeOwner=Class'\"/Script/RTD.TowerAttributeSet\"')")) (> (Class|GSCCoreComponent|GetCurrentAttributeValue _gsccore "(AttributeName=\"CritChance\",Attribute=/Script/RTD.TowerAttributeSet:CritChance,AttributeOwner=Class'\"/Script/RTD.TowerAttributeSet\"')") (Math|Random|RandomFloat))) (Game|GetPlayerController 0) self (Variables|Default|GetDamageTypeClass))
          (CallFunction|ApplyStatusEffect _array_element)
          (Utilities|FlowControl|Delay 0.2)
          (Components|DestroyComponent _returnvalue_2))))
    (Utilities|FlowControl|Delay (/ 1.0 (Class|GSCCoreComponent|GetCurrentAttributeValue (Variables|Default|GetGSCCore) "(AttributeName=\"AttackSpeed\",Attribute=/Script/RTD.TowerAttributeSet:AttackSpeed,AttributeOwner=Class'\"/Script/RTD.TowerAttributeSet\"')")))
    (CallFunction|Attack)
    (else
      (Utilities|FlowControl|Delay 0.1)
      (CallFunction|Attack))))

(fn ConstructionScript
  (|CallParentFunction))

(fn ReportStats
  (bind _gsccore (Variables|Default|GetGSCCore))
  (bind _gsccore_2 (Variables|Default|GetGSCCore))
  (bind _rowname (CallFunction|GetDisplayData (Variables|Default|GetDamageTypeClass)))
  (Class|BPISelectionWidget|ReportStats(Message) (UserInterface|GetWidget (Variables|Default|GetSelectionWidget)) self (Components|GetOwner) (Variables|Default|GetTowerName) (Variables|Default|GetIcon) (Utilities|Array|MakeArray (Utilities|Text|ToText(String) (Utilities|String|Replace (Utilities|String|Replace (Utilities|String|Replace (Utilities|String|Replace (Utilities|String|Replace (Utilities|String|Replace (Utilities|String|Replace (Utilities|String|Replace (Utilities|String|ToString(Text) (Utilities|Text|MakeLiteralText "Every <RichText.Emphasis>TIME</>s randomly shocks up to <RichText.Emphasis>TARGETS</> enemies in it's range, dealing <img id=\"ROW\"/><RichText.ROW> DMG</> damage to each with a <RichText.Emphasis>STUNCHANCE</>% chance to <img id=\"Stun\"/><RichText.Stun>stun</> for <RichText.Emphasis>STUNDURATION</>s. This tower has a <RichText.Emphasis>CRITCHANCE</> chance to crit, dealing <RichText.Emphasis>CRITX</>x the damage.")) "ROW" _rowname "CaseSensitive") "DMG" (Utilities|String|ToString(Float) (Math|Float|SnapToGrid(Float) (Class|GSCCoreComponent|GetCurrentAttributeValue _gsccore "(AttributeName=\"AttackPower\",Attribute=/Script/RTD.TowerAttributeSet:AttackPower,AttributeOwner=Class'\"/Script/RTD.TowerAttributeSet\"')") 0.1)) "CaseSensitive") "TIME" (Utilities|String|ToString(Float) (Math|Float|SnapToGrid(Float) (/ 1.0 (Class|GSCCoreComponent|GetCurrentAttributeValue _gsccore "(AttributeName=\"AttackSpeed\",Attribute=/Script/RTD.TowerAttributeSet:AttackSpeed,AttributeOwner=Class'\"/Script/RTD.TowerAttributeSet\"')")) 0.01)) "CaseSensitive") "STUNCHANCE" (Utilities|String|ToString(Float) (Math|Float|SnapToGrid(Float) (* (Class|GSCCoreComponent|GetCurrentAttributeValue _gsccore "(AttributeName=\"StunChance\",Attribute=/Script/RTD.TowerAttributeSet:StunChance,AttributeOwner=Class'\"/Script/RTD.TowerAttributeSet\"')") 1e+02) 0.1)) "CaseSensitive") "STUNDURATION" (Utilities|String|ToString(Float) (Math|Float|SnapToGrid(Float) (Class|GSCCoreComponent|GetCurrentAttributeValue _gsccore "(AttributeName=\"StunDuration\",Attribute=/Script/RTD.TowerAttributeSet:StunDuration,AttributeOwner=Class'\"/Script/RTD.TowerAttributeSet\"')") 0.01)) "CaseSensitive") "TARGETS" (Utilities|String|ToString(Integer) (Math|Float|Round (Class|GSCCoreComponent|GetCurrentAttributeValue _gsccore "(AttributeName=\"CurrentTargets\",Attribute=/Script/RTD.TowerAttributeSet:CurrentTargets,AttributeOwner=Class'\"/Script/RTD.TowerAttributeSet\"')"))) "CaseSensitive") "CRITCHANCE" (Utilities|String|ToString(Text) (Class|KismetTextLibrary|AsPercentFloat (Class|GSCCoreComponent|GetCurrentAttributeValue _gsccore_2 "(AttributeName=\"CritChance\",Attribute=/Script/RTD.TowerAttributeSet:CritChance,AttributeOwner=Class'\"/Script/RTD.TowerAttributeSet\"')") "HalfToEven")) "CaseSensitive") "CRITX" (Utilities|String|ToString(Float) (Math|Float|SnapToGrid(Float) (Class|GSCCoreComponent|GetCurrentAttributeValue _gsccore_2 "(AttributeName=\"CritX\",Attribute=/Script/RTD.TowerAttributeSet:CritX,AttributeOwner=Class'\"/Script/RTD.TowerAttributeSet\"')") 0.01)) "CaseSensitive"))) (Variables|Default|GetUpgradeCost) (Variables|Default|GetSellValue) (Variables|Default|GetItems) (Variables|Default|GetAvailableModes) (Variables|Default|GetTargetingMode) (Variables|Default|GetTargetingPriority)))