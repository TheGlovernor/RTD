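; Gatling tower building, a child of a shared tower parent, that fires BP_Bullet actors at the first entry in its target list.
; Attack is a self-calling delay loop that spawns bullets at a rate set by GSCCore attributes, with a random roll for multiplied damage, and polls when unable to fire.
; Rotating movement components spin the barrel and gears only while firing, and RotateGun pitches the body toward the target.
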(event Custom|toggleBarrel
  (params (on :type Boolean))
  (if on
    (Variables|/Script/Engine.RotatingMovementComponent|SetRotationRate (Variables|Default|GetBarrel_RotatingMovement) "0, 0,720.000000")
    (Variables|/Script/Engine.RotatingMovementComponent|SetRotationRate (Variables|Default|GetBodyGearRotatingMovement) "0.000000,0.000000,360.000000")
    (Variables|/Script/Engine.RotatingMovementComponent|SetRotationRate (Variables|Default|GetBottomGear_RotatingMovement) "0.000000,360.000000, 0")
    (else
      (Variables|/Script/Engine.RotatingMovementComponent|SetRotationRate (Variables|Default|GetBarrel_RotatingMovement) "0, 0, 0")
      (Variables|/Script/Engine.RotatingMovementComponent|SetRotationRate (Variables|Default|GetBodyGearRotatingMovement) "0, 0, 0")
      (Variables|/Script/Engine.RotatingMovementComponent|SetRotationRate (Variables|Default|GetBottomGear_RotatingMovement) "0, 0, 0"))))

(event Custom|RotateGun
  (bind _targetables (Variables|Default|GetTargetables))
  (bind _body (Variables|Default|GetBody))
  (if (Utilities|Array|IsNotEmpty _targetables)
    (Transformation|SetWorldRotation _body (Math|Rotator|MakeRotator 0.0 (.pitch (Math|Rotator|FindLookatRotation (Transformation|GetWorldLocation _body) (Transformation|GetActorLocation (Utilities|Array|Get(acopy) _targetables)))) 0.0) false false)))

(event EventBeginPlay
  (|CallParentFunction)
  (Components|Movement|SetUpdatedComponent (Variables|Default|GetBarrel_RotatingMovement) (Variables|Default|GetBarrel))
  (Components|Movement|SetUpdatedComponent (Variables|Default|GetBodyGearRotatingMovement) (Variables|Default|GetGear_Body))
  (Components|Movement|SetUpdatedComponent (Variables|Default|GetBottomGear_RotatingMovement) (Variables|Default|GetGear_Bottom))
  (Variables|Default|SetAmmo (Class|GSCCoreComponent|GetCurrentAttributeValue (Variables|Default|GetGSCCore) "(AttributeName=\"MagSize\",Attribute=/Script/RTD.TowerAttributeSet:MagSize,AttributeOwner=Class'\"/Script/RTD.TowerAttributeSet\"')")))

(event EventTick
  (params (DeltaSeconds :type Float%20%28single-precision%29))
  (|CallParentFunction DeltaSeconds))

(event EventAttack
  (bind _self self)
  (bind _gsccore (Variables|Default|GetGSCCore))
  (bind _barrel (Variables|Default|GetBarrel))
  (bind _returnvalue (Class|GSCCoreComponent|GetCurrentAttributeValue _gsccore "(AttributeName=\"AttackPower\",Attribute=/Script/RTD.TowerAttributeSet:AttackPower,AttributeOwner=Class'\"/Script/RTD.TowerAttributeSet\"')"))
  (bind _returnvalue_2 (CallFunction|CanAttack))
  (if _returnvalue_2
    (Utilities|IsValid (Utilities|Array|Get(acopy) (Variables|Default|GetTargetables))
      (:Is%20Valid
        (CallFunction|ToggleBarrel true)
        (Game|SpawnActorfromClass "/Game/Blueprints/Building/Tower/Projs_Beams/BP_Bullet.BP_Bullet_C" (Math|Transform|MakeTransform (Transformation|GetSocketLocation _barrel "RBarrel") (Math|Rotator|MakeRotationfromAxes (Math|Vector|GetForwardVector _barrel) (Math|Vector|GetRightVector _barrel) "0, 0,1.000000")) "AlwaysSpawn" _self (Math|Float|SelectFloat _returnvalue (* _returnvalue (Class|GSCCoreComponent|GetCurrentAttributeValue _gsccore "(AttributeName=\"CritX\",Attribute=/Script/RTD.TowerAttributeSet:CritX,AttributeOwner=Class'\"/Script/RTD.TowerAttributeSet\"')")) (> (Class|GSCCoreComponent|GetCurrentAttributeValue _gsccore "(AttributeName=\"CritChance\",Attribute=/Script/RTD.TowerAttributeSet:CritChance,AttributeOwner=Class'\"/Script/RTD.TowerAttributeSet\"')") (Math|Random|RandomFloat))) (Variables|Default|GetDamageTypeClass) _self (Math|Float|Round (Class|GSCCoreComponent|GetCurrentAttributeValue _gsccore "(AttributeName=\"CurrentTargets\",Attribute=/Script/RTD.TowerAttributeSet:CurrentTargets,AttributeOwner=Class'\"/Script/RTD.TowerAttributeSet\"')")) 0)
        (CallFunction|PlayShootingSound)
        (Utilities|FlowControl|Delay (/ 1.0 (Class|GSCCoreComponent|GetCurrentAttributeValue (Variables|Default|GetGSCCore) "(AttributeName=\"AttackSpeed\",Attribute=/Script/RTD.TowerAttributeSet:AttackSpeed,AttributeOwner=Class'\"/Script/RTD.TowerAttributeSet\"')")))
        (CallFunction|Attack))
      (:Is%20Not%20Valid
        (CallFunction|ToggleBarrel false :!label _label)
        (Utilities|FlowControl|Delay 0.1)
        (CallFunction|Attack)))
    (else
      (goto _label))))

(fn ConstructionScript
  (|CallParentFunction)
  (CallFunction|CalculateTowerStats)
  (CallFunction|ToggleSelect false))