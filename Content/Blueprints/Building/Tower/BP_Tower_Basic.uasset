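; Base tower-defense tower that attacks enemies inside its range sphere by Projectile, AOE, Beam or Trace.
; TowerData and an optional Item drive power, speed, range, target count and damage type.
; Targets are ordered by progress or health priority, attacks re-fire on a timer, and Beam towers match spawned beam actors to target count.
; A four-point spline with spline meshes draws the circular range indicator.
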(event OnComponentBeginOverlap(RangeSphere)
  (params (OverlappedComponent :type Primitive%20Component%20Object%20Reference) (OtherActor :type Actor%20Object%20Reference) (OtherComp :type Primitive%20Component%20Object%20Reference) (OtherBodyIndex :type Integer) (bFromSweep :type Boolean) (SweepResult :type Hit%20Result%20Structure%20%28by%20ref%29))
  (bind _asbp_enemy_base_01 (Utilities|Casting|CastToBP_Enemy_Base_01 OtherActor))
  (Variables|/Game/Blueprints/Mobs/BP_Enemy_Base_01.BP_Enemy_Base_01_C|SetMovementSpeed _asbp_enemy_base_01 (Variables|/Game/Blueprints/Mobs/BP_Enemy_Base_01.BP_Enemy_Base_01_C|GetTargetableSpeed _asbp_enemy_base_01)))

(event Custom|Attack
  (bind _didattack (CallFunction|AttemptAttack))
  (if _didattack
    (bind _returnvalue (Utilities|Time|SetTimerbyEvent (delegate Custom|Attack) (Variables|CalculatedStats|GetCalculatedAttackSpeed)))
    (Variables|Default|SetAttack%20Timer _returnvalue)))

(event EventBeginPlay)

(event EventTick
  (params (DeltaSeconds :type Float%20%28single-precision%29))
  (CallFunction|CheckBeamCount)
  (if (<= (Utilities|Time|GetTimerRemainingTimebyHandle (Variables|Default|GetAttack%20Timer)) 0.0)
    (CallFunction|Attack)))

(fn ConstructionScript
  (bind _staticmesh (Variables|Default|GetStaticMesh))
  (bind _towerdata (Variables|Default|GetTowerData))
  (bind _targetingmesh (Variables|Default|GetTargetingMesh))
  (Variables|Targeting|SetAttackType (.attacktype _towerdata))
  (Variables|Default|SetName (.name _towerdata))
  (Variables|Default|SetDamageTypeClass (.damagetypeclass _towerdata))
  (CallFunction|CalculateStats)
  (CallFunction|ToggleRangeIndicator false)
  (Components|StaticMesh|SetStaticMesh _staticmesh (.mesh1 _towerdata))
  (Transformation|SetRelativeTransform _staticmesh (.mesh1tfm _towerdata) false false)
  (Components|StaticMesh|SetStaticMesh _targetingmesh (.mesh2 _towerdata))
  (Transformation|SetRelativeTransform _targetingmesh (.mesh2tfm _towerdata) false false))

(fn CalculateStats
  (bind _towerdata (Variables|Default|GetTowerData))
  (bind _towerdata_2 (Variables|Default|GetTowerData))
  (bind _item (Variables|Default|GetItem)
    (:then
      (Utilities|FlowControl|Sequence
        (:then_0
          (Variables|CalculatedStats|SetCalculatedPower (* (.powermultiplier (Variables|/Game/Blueprints/Item/BP_TowerItem_DataObj.BP_TowerItem_DataObj_C|GetItemData _item)) (+ (.powerdelta (Variables|/Game/Blueprints/Item/BP_TowerItem_DataObj.BP_TowerItem_DataObj_C|GetItemData _item)) (.power _towerdata_2))))
          (if (Utilities|IsValidClass (.damagetypemodifier (Variables|/Game/Blueprints/Item/BP_TowerItem_DataObj.BP_TowerItem_DataObj_C|GetItemData _item)))
            (Variables|Default|SetDamageTypeClass (.damagetypemodifier (Variables|/Game/Blueprints/Item/BP_TowerItem_DataObj.BP_TowerItem_DataObj_C|GetItemData _item)))))
        (:then_1
          (Variables|CalculatedStats|SetCalculatedAttackSpeed (* (.attackspeedmultiplier (Variables|/Game/Blueprints/Item/BP_TowerItem_DataObj.BP_TowerItem_DataObj_C|GetItemData _item)) (+ (.attackspeeddelta (Variables|/Game/Blueprints/Item/BP_TowerItem_DataObj.BP_TowerItem_DataObj_C|GetItemData _item)) (.speed _towerdata_2)))))
        (:then_2
          (Variables|CalculatedStats|SetCalculatedRange (* (.rangemultiplier (Variables|/Game/Blueprints/Item/BP_TowerItem_DataObj.BP_TowerItem_DataObj_C|GetItemData _item)) (+ (.rangedelta (Variables|/Game/Blueprints/Item/BP_TowerItem_DataObj.BP_TowerItem_DataObj_C|GetItemData _item)) (.range _towerdata_2)))))
        (:then_3
          (Variables|CalculatedStats|SetCalculatedTargets (* (.targetmultiplier (Variables|/Game/Blueprints/Item/BP_TowerItem_DataObj.BP_TowerItem_DataObj_C|GetItemData _item)) (+ (.targetdelta (Variables|/Game/Blueprints/Item/BP_TowerItem_DataObj.BP_TowerItem_DataObj_C|GetItemData _item)) (.targets _towerdata_2))))
          (Variables|CalculatedStats|SetMaxTargets (.maxtargets _towerdata_2))
          (CallFunction|UpdateRange)
          (if (> (Variables|CalculatedStats|GetCalculatedTargets) (Variables|CalculatedStats|GetMaxTargets))
            (Variables|CalculatedStats|SetCalculatedTargets (Variables|CalculatedStats|GetMaxTargets))))
        (:then_4
          (Actor|Tick|SetActorTickInterval (Variables|CalculatedStats|GetCalculatedAttackSpeed) :!label _label)
          (CallFunction|SetTimer)
          (CallFunction|UpdateRange)
          (if (> (Variables|CalculatedStats|GetCalculatedTargets) (Variables|CalculatedStats|GetMaxTargets))
            (Variables|CalculatedStats|SetCalculatedTargets (Variables|CalculatedStats|GetMaxTargets))))))
    (:else
      (Utilities|FlowControl|Sequence
        (:then_0
          (Variables|CalculatedStats|SetCalculatedPower (.power _towerdata)))
        (:then_1
          (Variables|CalculatedStats|SetCalculatedAttackSpeed (.speed _towerdata)))
        (:then_2
          (Variables|CalculatedStats|SetCalculatedRange (.range _towerdata)))
        (:then_3
          (Variables|CalculatedStats|SetCalculatedTargets (.targets _towerdata)))
        (:then_4
          (Variables|CalculatedStats|SetMaxTargets (.maxtargets _towerdata)))
        (:then_5
          (Variables|Default|SetDamageTypeClass (.damagetypeclass _towerdata)))
        (:then_6
          (goto _label))))))

(fn UpdateRange
  (bind _rangesphere (Variables|Default|GetRangeSphere))
  (bind _splineheight (LocalVariables|GetSplineHeight))
  (bind _splineheight_2 (LocalVariables|GetSplineHeight))
  (bind _rangespline (Variables|Default|GetRangeSpline))
  (bind _calculatedrange (Variables|CalculatedStats|GetCalculatedRange))
  (bind _calculatedrange_2 (Variables|CalculatedStats|GetCalculatedRange))
  (bind _returnvalue (* _calculatedrange -1.0))
  (Components|Sphere|SetSphereRadius _rangesphere (Variables|CalculatedStats|GetCalculatedRange) true)
  (Transformation|SetRelativeLocation _rangesphere (Math|Vector|MakeVector 0.0 0.0 (LocalVariables|GetSplineHeight)) false false)
  (Utilities|FlowControl|Sequence
    (:then_0
      (Spline|SetLocationatSplinePoint _rangespline 0 (Math|Vector|MakeVector _calculatedrange_2 0.0 _splineheight_2) "Local" false)
      (Spline|SetTangentatSplinePoint _rangespline 0 (Math|Vector|MakeVector 0.0 (* (Variables|CalculatedStats|GetCalculatedRange) (Variables|Components|GetTangentConst)) 0.0) "Local" false))
    (:then_1
      (Spline|SetLocationatSplinePoint _rangespline 1 (Math|Vector|MakeVector 0.0 _calculatedrange_2 _splineheight_2) "Local" false)
      (Spline|SetTangentatSplinePoint _rangespline 1 (Math|Vector|MakeVector (* (Variables|CalculatedStats|GetCalculatedRange) (Variables|Components|GetTangentConst) -1.0) 0.0 0.0) "Local" false))
    (:then_2
      (Spline|SetLocationatSplinePoint _rangespline 2 (Math|Vector|MakeVector _returnvalue 0.0 _splineheight) "Local" false)
      (Spline|SetTangentatSplinePoint _rangespline 2 (Math|Vector|MakeVector 0.0 (* (Variables|CalculatedStats|GetCalculatedRange) (Variables|Components|GetTangentConst) -1.0) 0.0) "Local" false))
    (:then_3
      (Spline|SetLocationatSplinePoint _rangespline 3 (Math|Vector|MakeVector 0.0 _returnvalue _splineheight) "Local" false)
      (Spline|SetTangentatSplinePoint _rangespline 3 (Math|Vector|MakeVector (* (Variables|CalculatedStats|GetCalculatedRange) (Variables|Components|GetTangentConst)) 0.0 0.0) "Local" false))
    (:then_4
      (Spline|UpdateSpline (Variables|Default|GetRangeSpline))
      (CallFunction|UpdateRangeMesh)
      (for _array_element (Variables|Default|GetBeams)
        (Utilities|IsValid _array_element
          (:Is%20Valid
            (Variables|/Game/Blueprints/Building/Tower/Projs_Beams/BP_Beam_Basic.BP_Beam_Basic_C|Setrange _array_element (Variables|CalculatedStats|GetCalculatedRange))))))))

(fn UpdateRangeMesh
  (for (_array_element _array_index) (Variables|Components|GetRangeMeshes)
    (Utilities|IsValid _array_element
      (:Is%20Valid
        _)
      (:Is%20Not%20Valid
        (bind _returnvalue (AddComponent|AddSplineMeshComponent false))
        (Utilities|Array|SetArrayElem (Variables|Components|GetRangeMeshes) _array_index _returnvalue)))
    (|SetStart/End _array_element _array_index)))

(fn ToggleRangeIndicator
  (params (show :type Boolean))
  (bind _selectionwidget (Variables|Default|GetSelectionWidget))
  (for _array_element (Variables|Components|GetRangeMeshes)
    (Rendering|SetVisibility _array_element show true))
  (if show
    (Components|Activation|Activate _selectionwidget false)
    (Development|SetHiddeninGame _selectionwidget false false)
    (else
      (Components|Activation|Deactivate _selectionwidget)
      (Development|SetHiddeninGame _selectionwidget true false))))

(fn AttemptLevelUp
  (if true
    (Math|Integer|IncrementInt (Variables|CalculatedStats|GetLevel)
      (:%20%20
        (CallFunction|CalculateStats)))))

(fn AqcuireTargets
  (bind _rangesphere (Variables|Default|GetRangeSphere))
  (bind _overlappingactors (Collision|GetOverlappingActors _rangesphere "/Game/Blueprints/Mobs/BP_Enemy_Base_01.BP_Enemy_Base_01_C" :!class /Script/Engine.PrimitiveComponent))
  (if (Utilities|Array|IsNotEmpty _overlappingactors)
    (for _array_element _overlappingactors
      (bind _asbp_enemy_base_01 (Utilities|Casting|CastToBP_Enemy_Base_01 _array_element))
      (if (Utilities|Array|IsEmpty (LocalVariables|GetTargets))
        (Utilities|Array|AddUnique (LocalVariables|GetTargets) _asbp_enemy_base_01)
        (else
          (bind (_array_element_2 _array_index) (Utilities|Array|ForEachLoopwithBreak (LocalVariables|GetTargets) :!label _label)
            (:LoopBody
              (bind _usenew (CallFunction|Compare _asbp_enemy_base_01 _array_element_2))
              (if _usenew
                (Utilities|Array|Insert (LocalVariables|GetTargets) _asbp_enemy_base_01 _array_index)
                (LocalVariables|SetWasInserted true)
                (goto _label Break)))
            (:Completed
              (if (LocalVariables|GetWasInserted)
                (LocalVariables|SetWasInserted false)
                (else
                  (Utilities|Array|Add (LocalVariables|GetTargets) _asbp_enemy_base_01)))))))))
  (return (LocalVariables|GetTargets)))

(fn Compare
  (params (NewEnemy :type BP%20Enemy%20Base%2001%20Object%20Reference) (OldEnemy :type BP%20Enemy%20Base%2001%20Object%20Reference))
  (LocalVariables|SetEnemy1 NewEnemy)
  (LocalVariables|SetEnemy2 OldEnemy)
  (switch Utilities|FlowControl|Switch|SwitchonETargetPriority (Variables|Targeting|GetTargetingPriority)
    (:NewEnumerator0
      (switch Utilities|FlowControl|Switch|SwitchonETargetMode (Variables|Targeting|GetTargetingMode)
        (:NewEnumerator0
          (return (> (Variables|/Game/Blueprints/Mobs/BP_Enemy_Base_01.BP_Enemy_Base_01_C|GetDistanceToBase (LocalVariables|GetEnemy1)) (Variables|/Game/Blueprints/Mobs/BP_Enemy_Base_01.BP_Enemy_Base_01_C|GetDistanceToBase (LocalVariables|GetEnemy2)))))
        (:NewEnumerator1
          (return (< (Variables|/Game/Blueprints/Mobs/BP_Enemy_Base_01.BP_Enemy_Base_01_C|GetHealth (LocalVariables|GetEnemy1)) (Variables|/Game/Blueprints/Mobs/BP_Enemy_Base_01.BP_Enemy_Base_01_C|GetHealth (LocalVariables|GetEnemy2)))))))
    (:NewEnumerator1
      (switch Utilities|FlowControl|Switch|SwitchonETargetMode (Variables|Targeting|GetTargetingMode)
        (:NewEnumerator0
          (return (< (Variables|/Game/Blueprints/Mobs/BP_Enemy_Base_01.BP_Enemy_Base_01_C|GetDistanceToBase (LocalVariables|GetEnemy1)) (Variables|/Game/Blueprints/Mobs/BP_Enemy_Base_01.BP_Enemy_Base_01_C|GetDistanceToBase (LocalVariables|GetEnemy2)))))
        (:NewEnumerator1
          (return (> (Variables|/Game/Blueprints/Mobs/BP_Enemy_Base_01.BP_Enemy_Base_01_C|GetHealth (LocalVariables|GetEnemy1)) (Variables|/Game/Blueprints/Mobs/BP_Enemy_Base_01.BP_Enemy_Base_01_C|GetHealth (LocalVariables|GetEnemy2)))))))))

(fn AttemptAttack
  (bind _targetingmesh (Variables|Default|GetTargetingMesh))
  (bind _targetingmesh_2 (Variables|Default|GetTargetingMesh))
  (bind _returnvalue (Transformation|GetWorldLocation _targetingmesh))
  (bind _returnvalue_2 (- _returnvalue ""))
  (Utilities|FlowControl|Sequence
    (:then_0
      (switch Utilities|FlowControl|Switch|SwitchonETowerMode (Variables|Targeting|GetAttackType)
        (:NewEnumerator1
          (bind _targets1 (CallFunction|AqcuireTargets))
          (for _index (range 0 (- (Math|Integer|Min(Integer) (Utilities|Array|Length _targets1) (Variables|CalculatedStats|GetCalculatedTargets)) 1))
            (Utilities|IsValid (Utilities|Array|Get(acopy) _targets1 _index)
              (:Is%20Valid
                (Game|SpawnActorfromClass "/Game/Blueprints/Building/Tower/Projs_Beams/BP_Projectile_Basic.BP_Projectile_Basic_C" (Math|Transform|MakeTransform (Transformation|GetWorldLocation (Variables|Default|GetTargetingMesh))) "AlwaysSpawn" 0 (Utilities|Array|Get(acopy) _targets1 _index) (Transformation|GetWorldLocation (Variables|/Game/Blueprints/Mobs/BP_Enemy_Base_01.BP_Enemy_Base_01_C|GetTargetPoint (Utilities|Array|Get(acopy) _targets1 _index))) 0)
                (Utilities|IsValid (Utilities|Array|Get(acopy) _targets1 _index)
                  (:Is%20Valid
                    (Game|Damage|ApplyDamage (Utilities|Array|Get(acopy) _targets1 _index) (Variables|CalculatedStats|GetCalculatedPower) (Game|GetPlayerController 0) self (Variables|Default|GetDamageTypeClass))
                    (LocalVariables|SetAttacked true)))))))
        (:NewEnumerator0
          (for _array_element (Collision|GetOverlappingActors (Variables|Default|GetRangeSphere) "/Game/Blueprints/Mobs/BP_Enemy_Base_01.BP_Enemy_Base_01_C" :!class /Script/Engine.PrimitiveComponent)
            (Game|Damage|ApplyDamage _array_element (Variables|CalculatedStats|GetCalculatedPower) (Game|GetPlayerController 0) self (Variables|Default|GetDamageTypeClass))
            (LocalVariables|SetAttacked true)))
        (:NewEnumerator2
          (bind _targets1_2 (CallFunction|AqcuireTargets))
          (for _index_2 (range 0 (- (Math|Integer|Min(Integer) (Utilities|Array|Length _targets1_2) (Utilities|Array|Length (Variables|Default|GetBeams))) 1))
            (Variables|/Game/Blueprints/Building/Tower/Projs_Beams/BP_Beam_Basic.BP_Beam_Basic_C|SetTarget (Utilities|Array|Get(acopy) (Variables|Default|GetBeams) _index_2) (Utilities|Array|Get(acopy) _targets1_2 _index_2))
            (if (Utilities|Array|IsNotEmpty _targets1_2)
              (LocalVariables|SetAttacked (Utilities|Array|IsNotEmpty _targets1_2)))))
        (:NewEnumerator3
          (bind _targets1_3 (CallFunction|AqcuireTargets))
          (for _index_3 (range 0 (- (Math|Integer|Min(Integer) (Utilities|Array|Length _targets1_3) (Variables|CalculatedStats|GetCalculatedTargets)) 1))
            (bind _outhits (Collision|MultiLineTraceByChannel _returnvalue_2 (+ _returnvalue_2 (* (Math|Vector|GetUnitDirection(Vector) _returnvalue_2 (Transformation|GetWorldLocation (Variables|/Game/Blueprints/Mobs/BP_Enemy_Base_01.BP_Enemy_Base_01_C|GetDamageCapsule (Utilities|Array|Get(acopy) _targets1_3 _index_3)))) (Variables|CalculatedStats|GetCalculatedRange) (Variables|Default|GetTraceRangeXr))) "TraceTypeQuery6" false 0 "ForDuration" true "(R=1.000000,G=0.000000,B=0.000000,A=1.000000)" "(R=0.000000,G=1.000000,B=0.000000,A=1.000000)" 2.0))
            (Transformation|SetRelativeRotation _targetingmesh_2 (Math|Rotator|FindLookatRotation (Transformation|GetWorldLocation _targetingmesh_2) (Transformation|GetWorldLocation (Variables|/Game/Blueprints/Mobs/BP_Enemy_Base_01.BP_Enemy_Base_01_C|GetDamageCapsule (Utilities|Array|Get(acopy) _targets1_3 _index_3)))) false false)
            (for _array_element_2 _outhits
              (bind _asbp_enemy_base_01 (Utilities|Casting|CastToBP_Enemy_Base_01 (.HitActor (Collision|BreakHitResult _array_element_2))))
              (Game|Damage|ApplyDamage _asbp_enemy_base_01 (Variables|CalculatedStats|GetCalculatedPower) (Game|GetPlayerController 0) self (Variables|Default|GetDamageTypeClass))
              (LocalVariables|SetAttacked true))))))
    (:then_1
      (return (LocalVariables|GetAttacked)))))

(fn SetTimer
  (bind _returnvalue (Utilities|Time|SetTimerbyEvent (EventDispatchers|CreateEvent :!event Custom|Attack) 0.0))
  (Variables|Default|SetAttack%20Timer _returnvalue))

(fn CheckBeamCount
  (bind _calculatedtargets (Variables|CalculatedStats|GetCalculatedTargets))
  (bind _beams (Variables|Default|GetBeams))
  (bind _beams_2 (Variables|Default|GetBeams))
  (bind _returnvalue (Utilities|Array|Length _beams_2))
  (bind _returnvalue_2 (Utilities|Array|Length _beams))
  (bind _returnvalue_3 (< _returnvalue_2 _calculatedtargets))
  (bind _returnvalue_4 (- _returnvalue 1))
  (bind _output (Utilities|Array|Get(acopy) _beams_2 _returnvalue_4))
  (if (and (Utilities|Enum|Equal(Enum) (Variables|Targeting|GetAttackType) "NewEnumerator2") (!= (Utilities|Array|Length (Variables|Default|GetBeams)) (Variables|CalculatedStats|GetCalculatedTargets)))
    (if _returnvalue_3
      (while _returnvalue_3
        (bind _returnvalue_5 (Game|SpawnActorfromClass "/Game/Blueprints/Building/Tower/Projs_Beams/BP_Beam_Basic.BP_Beam_Basic_C" (Math|Transform|MakeTransform (Transformation|GetWorldLocation (Variables|Default|GetTargetingMesh))) "AlwaysSpawn" 0 0 (Variables|CalculatedStats|GetCalculatedPower) (Variables|CalculatedStats|GetCalculatedRange) (Variables|Default|GetDamageTypeClass) 0))
        (Utilities|Array|Add (Variables|Default|GetBeams) _returnvalue_5))
      (else
        (while (> (Utilities|Array|Length (Variables|Default|GetBeams)) (Variables|CalculatedStats|GetCalculatedTargets))
          (Actor|DestroyActor _output)
          (Utilities|Array|RemoveItem _beams_2 _output))))))