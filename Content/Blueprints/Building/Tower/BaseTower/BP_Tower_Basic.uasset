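; Basic tower-defense tower that tracks enemies inside a range sphere and picks a target; Tick is empty, so no attack happens here.
; Overlaps maintain the targetable list, set entering enemies' speed and choose targets by distance to base under Progress mode.
; Construction sizes the sphere from base-data range and level, shaping a hidden four-point spline-mesh ring as range indicator.
; AttemptLevelUp increments Level unconditionally, but range still reads the base-data level.
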(event OnComponentEndOverlap(RangeSphere)
  (params (OverlappedComponent :type Primitive%20Component%20Object%20Reference) (OtherActor :type Actor%20Object%20Reference) (OtherComp :type Primitive%20Component%20Object%20Reference) (OtherBodyIndex :type Integer))
  (bind _asbp_enemy_base_01 (Utilities|Casting|CastToBP_Enemy_Base_01 OtherActor))
  (Utilities|Array|RemoveItem (Variables|Targeting|GetTargetableEnemies) _asbp_enemy_base_01)
  (if (== _asbp_enemy_base_01 (Variables|Targeting|GetTarget))
    (Variables|Targeting|SetTarget 0)
    (bind _newtarget (CallFunction|GetNewTarget))
    (Variables|Targeting|SetTarget _newtarget)))

(event OnComponentBeginOverlap(RangeSphere)
  (params (OverlappedComponent :type Primitive%20Component%20Object%20Reference) (OtherActor :type Actor%20Object%20Reference) (OtherComp :type Primitive%20Component%20Object%20Reference) (OtherBodyIndex :type Integer) (bFromSweep :type Boolean) (SweepResult :type Hit%20Result%20Structure%20%28by%20ref%29))
  (bind _asbp_enemy_base_01 (Utilities|Casting|CastToBP_Enemy_Base_01 OtherActor))
  (Utilities|Array|Add (Variables|Targeting|GetTargetableEnemies) _asbp_enemy_base_01)
  (CallFunction|UpdateTarget _asbp_enemy_base_01)
  (Variables|/Game/Blueprints/Mobs/BP_Enemy_Base_01.BP_Enemy_Base_01_C|SetMovementSpeed _asbp_enemy_base_01 (Variables|/Game/Blueprints/Mobs/BP_Enemy_Base_01.BP_Enemy_Base_01_C|GetTargetableSpeed _asbp_enemy_base_01)))

(event EventBeginPlay
  (Actor|Tick|SetActorTickInterval (Variables|Stats|GetAttackRate)))

(event EventTick
  (params (DeltaSeconds :type Float%20%28single-precision%29)))

(fn ConstructionScript
  (Variables|Components|SetTangentConst (Variables|/Game/Blueprints/Building/Tower/BaseTower/BP_TowerData_Basic.BP_TowerData_Basic_C|GetTangentConst (Variables|Default|GetMyBaseData)))
  (CallFunction|SetLevel)
  (CallFunction|UpdateAllStats)
  (CallFunction|ToggleRangeIndicator false))

(fn UpdateAllStats
  (CallFunction|UpdateRange))

(fn UpdateRange
  (bind _mybasedata (Variables|Default|GetMyBaseData))
  (bind _rangesphere (Variables|Default|GetRangeSphere))
  (bind _splineheight (LocalVariables|GetSplineHeight))
  (bind _splineheight_2 (LocalVariables|GetSplineHeight))
  (bind _rangespline (Variables|Default|GetRangeSpline))
  (bind _output_get (Variables|Stats|SetRange (* (+ (* (Variables|/Game/Blueprints/Building/Tower/BaseTower/BP_TowerData_Basic.BP_TowerData_Basic_C|GetLevel _mybasedata) 0.1) 1) (Variables|/Game/Blueprints/Building/Tower/BaseTower/BP_TowerData_Basic.BP_TowerData_Basic_C|GetRange _mybasedata))))
  (Components|Sphere|SetSphereRadius _rangesphere _output_get true)
  (Transformation|SetRelativeLocation _rangesphere (Math|Vector|MakeVector 0.0 0.0 (LocalVariables|GetSplineHeight)) false false)
  (Utilities|FlowControl|Sequence
    (:then_0
      (Spline|SetLocationatSplinePoint _rangespline 0 (Math|Vector|MakeVector (Variables|Stats|GetRange) 0.0 _splineheight_2) "Local" false)
      (Spline|SetTangentatSplinePoint _rangespline 0 (Math|Vector|MakeVector 0.0 (* (Variables|Stats|GetRange) (Variables|Components|GetTangentConst)) 0.0) "Local" false))
    (:then_1
      (Spline|SetLocationatSplinePoint _rangespline 1 (Math|Vector|MakeVector 0.0 (Variables|Stats|GetRange) _splineheight_2) "Local" false)
      (Spline|SetTangentatSplinePoint _rangespline 1 (Math|Vector|MakeVector (* (Variables|Stats|GetRange) (Variables|Components|GetTangentConst) -1.0) 0.0 0.0) "Local" false))
    (:then_2
      (Spline|SetLocationatSplinePoint _rangespline 2 (Math|Vector|MakeVector (* (Variables|Stats|GetRange) -1.0) 0.0 _splineheight) "Local" false)
      (Spline|SetTangentatSplinePoint _rangespline 2 (Math|Vector|MakeVector 0.0 (* (Variables|Stats|GetRange) (Variables|Components|GetTangentConst) -1.0) 0.0) "Local" false))
    (:then_3
      (Spline|SetLocationatSplinePoint _rangespline 3 (Math|Vector|MakeVector 0.0 (* (Variables|Stats|GetRange) -1.0) _splineheight) "Local" false)
      (Spline|SetTangentatSplinePoint _rangespline 3 (Math|Vector|MakeVector (* (Variables|Stats|GetRange) (Variables|Components|GetTangentConst)) 0.0 0.0) "Local" false))
    (:then_4
      (Spline|UpdateSpline (Variables|Default|GetRangeSpline))
      (CallFunction|UpdateRangeMesh))))

(fn UpdateRangeMesh
  (for (_array_element _array_index) (Variables|Components|GetRangeMeshes)
    (Utilities|IsValid _array_element
      (:Is%20Valid
        _)
      (:Is%20Not%20Valid
        (bind _returnvalue (AddComponent|AddSplineMeshComponent false))
        (Utilities|Array|SetArrayElem (Variables|Components|GetRangeMeshes) _array_index _returnvalue)))
    (|SetStart/End _array_element _array_index)))

(fn GetNewTarget
  (switch Utilities|FlowControl|Switch|SwitchonETargetMode (Variables|Targeting|GetTargetingMode)
    (:NewEnumerator0
      (switch Utilities|FlowControl|Switch|SwitchonETargetPriority (Variables|Targeting|GetTargetingPriority)
        (:NewEnumerator0
          (for _array_element (Variables|Targeting|GetTargetableEnemies)
            (LocalVariables|GetTempTarget
              (:then
                (if (> (Variables|/Game/Blueprints/Mobs/BP_Enemy_Base_01.BP_Enemy_Base_01_C|GetDistanceToBase _array_element) (Variables|/Game/Blueprints/Mobs/BP_Enemy_Base_01.BP_Enemy_Base_01_C|GetDistanceToBase (stale _output_get)))
                  (LocalVariables|SetTempTarget _array_element)))
              (:else
                (bind _output_get (LocalVariables|SetTempTarget _array_element)))))
          (return (LocalVariables|GetTempTarget)))
        (:NewEnumerator1
          (for _array_element_2 (Variables|Targeting|GetTargetableEnemies)
            (LocalVariables|GetTempTarget
              (:then
                (if (< (Variables|/Game/Blueprints/Mobs/BP_Enemy_Base_01.BP_Enemy_Base_01_C|GetDistanceToBase _array_element_2) (Variables|/Game/Blueprints/Mobs/BP_Enemy_Base_01.BP_Enemy_Base_01_C|GetDistanceToBase (stale _output_get_2)))
                  (LocalVariables|SetTempTarget _array_element_2)))
              (:else
                (bind _output_get_2 (LocalVariables|SetTempTarget _array_element_2)))))
          (return (LocalVariables|GetTempTarget)))))))

(fn UpdateTarget
  (params (IncomingEnemy :type BP%20Enemy%20Base%2001%20Object%20Reference))
  (Variables|Targeting|GetTarget
    (:then
      (LocalVariables|SetNewEnemy IncomingEnemy)
      (switch Utilities|FlowControl|Switch|SwitchonETargetMode (Variables|Targeting|GetTargetingMode)
        (:NewEnumerator0
          (switch Utilities|FlowControl|Switch|SwitchonETargetPriority (Variables|Targeting|GetTargetingPriority)
            (:NewEnumerator0
              (if (> (Variables|/Game/Blueprints/Mobs/BP_Enemy_Base_01.BP_Enemy_Base_01_C|GetDistanceToBase (LocalVariables|GetNewEnemy)) (Variables|/Game/Blueprints/Mobs/BP_Enemy_Base_01.BP_Enemy_Base_01_C|GetDistanceToBase (Variables|Targeting|GetTarget)))
                (Variables|Targeting|SetTarget (LocalVariables|GetNewEnemy))))
            (:NewEnumerator1
              (if (< (Variables|/Game/Blueprints/Mobs/BP_Enemy_Base_01.BP_Enemy_Base_01_C|GetDistanceToBase (LocalVariables|GetNewEnemy)) (Variables|/Game/Blueprints/Mobs/BP_Enemy_Base_01.BP_Enemy_Base_01_C|GetDistanceToBase (Variables|Targeting|GetTarget)))
                (Variables|Targeting|SetTarget (LocalVariables|GetNewEnemy))))))))
    (:else
      (Variables|Targeting|SetTarget IncomingEnemy))))

(fn ToggleRangeIndicator
  (params (show :type Boolean))
  (for _array_element (Variables|Components|GetRangeMeshes)
    (Rendering|SetVisibility _array_element show true)))

(fn SetLevel
  (Variables|Stats|SetLevel (Variables|/Game/Blueprints/Building/Tower/BaseTower/BP_TowerData_Basic.BP_TowerData_Basic_C|GetLevel (Variables|Default|GetMyBaseData))))

(fn AttemptLevelUp
  (if true
    (Math|Integer|IncrementInt (Variables|Stats|GetLevel)
      (:%20%20
        (CallFunction|UpdateAllStats)))))