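; Gear-driven tower, apparently a base class, whose large gear turns to face its first target.
; Each tick the large gear yaws toward that target at a fixed rate, slowing when nearly aligned to limit overshoot.
; Six small gears roll at a multiple of the large gear's yaw to look meshed.
; Construction calculates stats and clears selection, ReportStats feeds the selection widget, and the venting events are empty stubs.
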(event Custom|StartVenting)

(event Custom|RotateGears
  (params (DeltaSeconds :type Float%20%28double-precision%29))
  (bind _largegear (Variables|Default|GetLargeGear))
  (bind _targetables (Variables|Default|GetTargetables))
  (bind _largegear_2 (Variables|Default|GetLargeGear))
  (bind _returnvalue (Transformation|GetWorldTransform _largegear))
  (bind _output (Utilities|Array|Get(acopy) _targetables))
  (bind _returnvalue_2 (Transformation|GetActorLocation _output))
  (bind _returnvalue_3 (Math|Rotator|FindRelativeLookatRotation _returnvalue _returnvalue_2))
  (bind _returnvalue_4 (Math|Float|Sign(Float) (.yaw _returnvalue_3)))
  (bind _returnvalue_5 (* DeltaSeconds 9e+01 _returnvalue_4))
  (if (Utilities|Array|IsNotEmpty _targetables)
    (Utilities|IsValid _output
      (:Is%20Valid
        (Transformation|AddRelativeRotation _largegear_2 (Math|Rotator|MakeRotator 0.0 0.0 (select (< (Math|Float|Absolute(Float) (.yaw _returnvalue_3)) 5.0) (/ _returnvalue_5 1e+01) _returnvalue_5)) false false)
        (for _array_element (Variables|Default|GetSmallGears)
          (Transformation|SetRelativeRotation _array_element (Math|Rotator|MakeRotator (* (.yaw (Variables|/Script/Engine.SceneComponent|GetRelativeRotation _largegear_2)) 4.0) 0.0 0.0) false false))))))

(event Custom|StopVenting)

(event EventBeginPlay
  (|CallParentFunction)
  (Variables|Default|SetSmallGears (Utilities|Array|MakeArray (Variables|Default|GetSmallGear1) (Variables|Default|GetSmallGear2) (Variables|Default|GetSmallGear3) (Variables|Default|GetSmallGear4) (Variables|Default|GetSmallGear5) (Variables|Default|GetSmallGear6))))

(event EventTick
  (params (DeltaSeconds :type Float%20%28single-precision%29))
  (|CallParentFunction DeltaSeconds)
  (CallFunction|RotateGears DeltaSeconds))

(fn ConstructionScript
  (|CallParentFunction)
  (CallFunction|CalculateTowerStats)
  (CallFunction|ToggleSelect false))

(fn ReportStats
  (Class|BPISelectionWidget|ReportStats(Message) (UserInterface|GetWidget (Variables|Default|GetSelectionWidget)) self (Components|GetOwner) (Variables|Default|GetTowerName) (Variables|Default|GetIcon) (Utilities|Array|MakeArray "") (Variables|Default|GetUpgradeCost) (Variables|Default|GetSellValue) (Variables|Default|GetItems) (Variables|Default|GetAvailableModes) (Variables|Default|GetTargetingMode) (Variables|Default|GetTargetingPriority)))