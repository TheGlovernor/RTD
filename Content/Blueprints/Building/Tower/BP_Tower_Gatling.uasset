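; Gatling tower for a tower defense game that aims at enemies in range and fires damaging multi-line traces on a looping timer.
; CalculateTowerStats builds level-scaled stats from base stats and item bonuses, then resizes the range sphere.
; AqcuireTargets orders overlapping enemies by progress or health priority, and Attack shoots toward the first.
; A four-point spline with tangent-shaped spline meshes draws the range ring, toggled with the selection widget.
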(event OnComponentBeginOverlap(RangeSphere)
  (params (OverlappedComponent :type Primitive%20Component%20Object%20Reference) (OtherActor :type Actor%20Object%20Reference) (OtherComp :type Primitive%20Component%20Object%20Reference) (OtherBodyIndex :type Integer) (bFromSweep :type Boolean) (SweepResult :type Hit%20Result%20Structure%20%28by%20ref%29))
  (bind _asbp_enemy_base_01 (Utilities|Casting|CastToBP_Enemy_Base_01 OtherActor))
  (Variables|/Game/Blueprints/Mobs/BP_Enemy_Base_01.BP_Enemy_Base_01_C|SetMovementSpeed _asbp_enemy_base_01 (Variables|/Game/Blueprints/Mobs/BP_Enemy_Base_01.BP_Enemy_Base_01_C|GetTargetableSpeed _asbp_enemy_base_01)))

(event Custom|AttemptAttack
  (if (<= (Utilities|Time|GetTimerRemainingTimebyHandle (Variables|Default|GetAttack%20Timer)) 0.0)
    (CallFunction|Attack)))

(event EventBeginPlay
  (CallFunction|CalculateTowerStats))

(event EventSelect
  (params (UI :type CUI%20Start%20Screen%20Object%20Reference))
  (CallFunction|ToggleSelect true)
  (Variables|/Game/UI/CUI_StartScreen.CUI_StartScreen_C|SetNoTowerSelected UI false)
  (Default|UpdateHoverView UI))

(event EventTick
  (params (DeltaSeconds :type Float%20%28single-precision%29))
  (CallFunction|AttemptAttack))

(event EventDeselect
  (params (UI :type CUI%20Start%20Screen%20Object%20Reference))
  (CallFunction|ToggleSelect false)
  (Variables|/Game/UI/CUI_StartScreen.CUI_StartScreen_C|SetNoTowerSelected UI true))

(event EventAttack
  (bind _targetingmesh (Variables|Default|GetTargetingMesh))
  (bind _returnvalue (Transformation|GetWorldLocation _targetingmesh))
  (bind _newparam (CallFunction|AqcuireTargets))
  (if (Utilities|Array|IsNotEmpty _newparam)
    (Transformation|SetRelativeRotation (Variables|Default|GetTargetingMesh) (Math|Rotator|FindLookatRotation (Transformation|GetWorldLocation (Variables|Default|GetTargetingMesh)) (Transformation|GetActorLocation (Utilities|Array|Get(acopy) _newparam))) false false)
    (bind _outhits (Collision|MultiLineTraceByChannel _returnvalue (+ _returnvalue (* (Math|Vector|GetUnitDirection(Vector) _returnvalue (Transformation|GetActorLocation (Utilities|Array|Get(acopy) _newparam))) (.Value (Utilities|Map|Find (Variables|CalculatedStats|GetCalculatedStats) "NewEnumerator4")) (Variables|Default|GetTraceRangeXr))) "TraceTypeQuery6" false 0 "ForDuration" true "(R=1.000000,G=0.000000,B=0.000000,A=1.000000)" "(R=0.000000,G=1.000000,B=0.000000,A=1.000000)" 2.0))
    (for _array_element _outhits
      (Game|Damage|ApplyDamage (.HitActor (Collision|BreakHitResult _array_element)) (.Value (Utilities|Map|Find (Variables|CalculatedStats|GetCalculatedStats) "NewEnumerator2")) (Game|GetPlayerController 0) self (Variables|Default|GetDamageTypeClass)))
    (bind _returnvalue_2 (Utilities|Time|SetTimerbyEvent (delegate EventAttack) (.Value (Utilities|Map|Find (Variables|CalculatedStats|GetCalculatedStats) "NewEnumerator3")) true))
    (Variables|Default|SetAttack%20Timer _returnvalue_2)))

(event EventCalculateTowerStats
  (bind _key (Utilities|ForEach (Variables|CalculatedStats|GetBaseStats))
    (:LoopBody
      (Variables|CalculatedStats|SetTemp+ 0.0)
      (Variables|CalculatedStats|SetTemp* 1.0)
      (Utilities|FlowControl|Sequence
        (:then_0
          (if (.ReturnValue (Utilities|Map|Find (Variables|CalculatedStats|GetBaseStatsAdd) _key))
            (Variables|CalculatedStats|SetTemp+ (.Value (Utilities|Map|Find (Variables|CalculatedStats|GetBaseStatsAdd) _key)))))
        (:then_1
          (for _array_element (Variables|Default|GetItems)
            (Utilities|FlowControl|Sequence
              (:then_0
                (if (.ReturnValue (Utilities|Map|Find (Variables|/Game/Blueprints/Item/BP_TowerItem_DataObj.BP_TowerItem_DataObj_C|GetAddStats _array_element) _key))
                  (Variables|CalculatedStats|SetTemp+ (+ (.Value (Utilities|Map|Find (Variables|/Game/Blueprints/Item/BP_TowerItem_DataObj.BP_TowerItem_DataObj_C|GetAddStats _array_element) _key)) (Variables|CalculatedStats|GetTemp+)))))
              (:then_1
                (if (.ReturnValue (Utilities|Map|Find (Variables|/Game/Blueprints/Item/BP_TowerItem_DataObj.BP_TowerItem_DataObj_C|GetAddStats _array_element) _key))
                  (Variables|CalculatedStats|SetTemp* (+ (.Value (Utilities|Map|Find (Variables|/Game/Blueprints/Item/BP_TowerItem_DataObj.BP_TowerItem_DataObj_C|GetAddStats _array_element) _key)) (Variables|CalculatedStats|GetTemp*)))))))
          (Utilities|Map|Add (Variables|CalculatedStats|GetStatsPerLevel) _key (* (Variables|CalculatedStats|GetTemp+) (Variables|CalculatedStats|GetTemp*)))
          (Utilities|Map|Add (Variables|CalculatedStats|GetCalculatedStats) _key (+ (.Value (Utilities|Map|Find (Variables|CalculatedStats|GetBaseStats) _key)) (* (* (Variables|CalculatedStats|GetTemp+) (Variables|CalculatedStats|GetTemp*)) (- (Variables|CalculatedStats|GetLevel) 1)))))))
    (:Completed
      (CallFunction|UpdateRange))))

(fn ConstructionScript
  (CallFunction|CalculateTowerStats)
  (CallFunction|ToggleSelect false))

(fn AqcuireTargets
  (for _array_element (Collision|GetOverlappingActors (Variables|Default|GetRangeSphere) "/Game/Blueprints/Mobs/BP_Enemy_Base_01.BP_Enemy_Base_01_C" :!class /Script/Engine.PrimitiveComponent)
    (LocalVariables|SetTarget _array_element)
    (if (Utilities|DoesObjectImplementInterface _array_element "/Game/Blueprints/Mobs/EnemyInterface.EnemyInterface_C")
      (if (Utilities|Array|IsEmpty (LocalVariables|GetTargets))
        (Utilities|Array|AddUnique (LocalVariables|GetTargets) (LocalVariables|GetTarget))
        (else
          (bind (_array_element_2 _array_index) (Utilities|Array|ForEachLoopwithBreak (LocalVariables|GetTargets) :!label _label)
            (:LoopBody
              (LocalVariables|Setindex _array_index)
              (Utilities|FlowControl|Sequence
                (:then_0
                  (bind (_distancetobase _health) (Class|EnemyInterface|ReportStats(Message) (LocalVariables|GetTarget))))
                (:then_1
                  (bind (_distancetobase_2 _health_2) (Class|EnemyInterface|ReportStats(Message) _array_element_2))
                  (switch Utilities|FlowControl|Switch|SwitchonETargetMode (Variables|Targeting|GetTargetingMode)
                    (:NewEnumerator0
                      (switch Utilities|FlowControl|Switch|SwitchonETargetPriority (Variables|Targeting|GetTargetingPriority)
                        (:NewEnumerator0
                          (if (> _distancetobase _distancetobase_2)
                            (Utilities|Array|Insert (LocalVariables|GetTargets) (LocalVariables|GetTarget) (LocalVariables|Getindex))
                            (LocalVariables|SetInserted true :!label _label_2)
                            (goto _label Break)))
                        (:NewEnumerator1
                          (if (< _distancetobase _distancetobase_2)
                            (Utilities|Array|Insert (LocalVariables|GetTargets) (LocalVariables|GetTarget) (LocalVariables|Getindex))
                            (goto _label_2)))))
                    (:NewEnumerator1
                      (switch Utilities|FlowControl|Switch|SwitchonETargetPriority (Variables|Targeting|GetTargetingPriority)
                        (:NewEnumerator0
                          (if (< _health _health_2)
                            (Utilities|Array|Insert (LocalVariables|GetTargets) (LocalVariables|GetTarget) (LocalVariables|Getindex))
                            (goto _label_2)))
                        (:NewEnumerator1
                          (if (> _health _health_2)
                            (Utilities|Array|Insert (LocalVariables|GetTargets) (LocalVariables|GetTarget) (LocalVariables|Getindex))
                            (goto _label_2)))))))))
            (:Completed
              (if (LocalVariables|GetInserted)
                (LocalVariables|SetInserted false)
                (else
                  (Utilities|Array|Add (LocalVariables|GetTargets) (LocalVariables|GetTarget))))))))))
  (return (LocalVariables|GetTargets)))

(fn ToggleSelect
  (params (show :type Boolean))
  (bind _selectionwidget (Variables|Default|GetSelectionWidget))
  (for _array_element (Variables|Components|GetRangeMeshes)
    (Rendering|SetVisibility _array_element show true))
  (if show
    (Development|SetHiddeninGame _selectionwidget false true)
    (else
      (Development|SetHiddeninGame _selectionwidget true true))))

(fn UpdateRange
  (bind _calculatedstats (Variables|CalculatedStats|GetCalculatedStats))
  (bind _rangesphere (Variables|Default|GetRangeSphere))
  (bind _splineheight (LocalVariables|GetSplineHeight))
  (bind _splineheight_2 (LocalVariables|GetSplineHeight))
  (bind _rangespline (Variables|Default|GetRangeSpline))
  (bind _value (Utilities|Map|Find _calculatedstats "NewEnumerator4"))
  (LocalVariables|SetRange _value)
  (Components|Sphere|SetSphereRadius _rangesphere _value true)
  (Transformation|SetRelativeLocation _rangesphere (Math|Vector|MakeVector 0.0 0.0 (LocalVariables|GetSplineHeight)) false false)
  (Utilities|FlowControl|Sequence
    (:then_0
      (Spline|SetLocationatSplinePoint _rangespline 0 (Math|Vector|MakeVector (LocalVariables|GetRange) 0.0 _splineheight_2) "Local" false)
      (Spline|SetTangentatSplinePoint _rangespline 0 (Math|Vector|MakeVector 0.0 (* (LocalVariables|GetRange) (Variables|Components|GetTangentConst)) 0.0) "Local" false))
    (:then_1
      (Spline|SetLocationatSplinePoint _rangespline 1 (Math|Vector|MakeVector 0.0 (LocalVariables|GetRange) _splineheight_2) "Local" false)
      (Spline|SetTangentatSplinePoint _rangespline 1 (Math|Vector|MakeVector (* (LocalVariables|GetRange) (Variables|Components|GetTangentConst) -1.0) 0.0 0.0) "Local" false))
    (:then_2
      (Spline|SetLocationatSplinePoint _rangespline 2 (Math|Vector|MakeVector (* (LocalVariables|GetRange) -1.0) 0.0 _splineheight) "Local" false)
      (Spline|SetTangentatSplinePoint _rangespline 2 (Math|Vector|MakeVector 0.0 (* (LocalVariables|GetRange) (Variables|Components|GetTangentConst) -1.0) 0.0) "Local" false))
    (:then_3
      (Spline|SetLocationatSplinePoint _rangespline 3 (Math|Vector|MakeVector 0.0 (* (LocalVariables|GetRange) -1.0) _splineheight) "Local" false)
      (Spline|SetTangentatSplinePoint _rangespline 3 (Math|Vector|MakeVector (* (LocalVariables|GetRange) (Variables|Components|GetTangentConst)) 0.0 0.0) "Local" false))
    (:then_4
      (Spline|UpdateSpline (Variables|Default|GetRangeSpline))
      (for (_array_element _array_index) (Variables|Components|GetRangeMeshes)
        (Utilities|IsValid _array_element
          (:Is%20Valid
            _)
          (:Is%20Not%20Valid
            (bind _returnvalue (AddComponent|AddSplineMeshComponent false))
            (Utilities|Array|SetArrayElem (Variables|Components|GetRangeMeshes) _array_index _returnvalue)))
        (|SetStart/End_2 _array_element _array_index)))))

(fn UpdateRangeMesh
  (for (_array_element _array_index) (Variables|Components|GetRangeMeshes)
    (Utilities|IsValid _array_element
      (:Is%20Valid
        _)
      (:Is%20Not%20Valid
        (bind _returnvalue (AddComponent|AddSplineMeshComponent false))
        (Utilities|Array|SetArrayElem (Variables|Components|GetRangeMeshes) _array_index _returnvalue)))
    (|SetStart/End _array_element _array_index)))

(fn GetReportedStats
  (return (Variables|CalculatedStats|GetCalculatedStats) (Variables|CalculatedStats|GetStatsPerLevel)))