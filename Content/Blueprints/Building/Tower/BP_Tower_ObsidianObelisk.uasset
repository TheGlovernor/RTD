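; Obsidian Obelisk tower Blueprint that fires damaging, crit-capable beams at multiple enemies through its beam component.
; ReportStats reads current GAS Companion attributes and fills a rich-text description template, sent to the selection widget with cost, sell value, items and targeting settings.
; The same call pushes beam count, damage, range, attack speed, crit stats and damage type into BPBeamComponent, so reporting stats also refreshes the beams.
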(fn ConstructionScript
  (|CallParentFunction))

(fn ReportStats
  (bind _gsccore (Variables|Default|GetGSCCore))
  (bind _gsccore_2 (Variables|Default|GetGSCCore))
  (bind _bp_beamcomponent (Variables|Default|GetBP_BeamComponent))
  (bind _gsccore_3 (Variables|Default|GetGSCCore))
  (bind _rowname (CallFunction|GetDisplayData (Variables|Default|GetDamageTypeClass)))
  (Class|BPISelectionWidget|ReportStats(Message) (UserInterface|GetWidget (Variables|Default|GetSelectionWidget)) self (Components|GetOwner) (Variables|Default|GetTowerName) (Variables|Default|GetIcon) (Utilities|Array|MakeArray (Utilities|Text|ToText(String) (Utilities|String|Replace (Utilities|String|Replace (Utilities|String|Replace (Utilities|String|Replace (Utilities|String|Replace (Utilities|String|Replace (Utilities|String|ToString(Text) (Utilities|Text|MakeLiteralText "Shoots beams at up to <RichText.Emphasis>TARGETS</> enemies, dealing <img id=\"ROW\"/><RichText.ROW> DMG</> damage to each every <RichText.Emphasis>TIME</> seconds.  This tower has a <RichText.Emphasis>CRITCHANCE</> chance to crit, dealing <RichText.Emphasis>CRITX</>x the damage.")) "TARGETS" (Utilities|String|ToString(Integer) (Math|Float|Round (Class|GSCCoreComponent|GetCurrentAttributeValue _gsccore_3 "(AttributeName=\"CurrentTargets\",Attribute=/Script/RTD.TowerAttributeSet:CurrentTargets,AttributeOwner=Class'\"/Script/RTD.TowerAttributeSet\"')"))) "CaseSensitive") "ROW" _rowname "CaseSensitive") "DMG" (Utilities|String|ToString(Float) (Math|Float|SnapToGrid(Float) (Class|GSCCoreComponent|GetCurrentAttributeValue _gsccore_3 "(AttributeName=\"AttackPower\",Attribute=/Script/RTD.TowerAttributeSet:AttackPower,AttributeOwner=Class'\"/Script/RTD.TowerAttributeSet\"')") 0.01)) "CaseSensitive") "TIME" (Utilities|String|ToString(Float) (Math|Float|SnapToGrid(Float) (/ 1.0 (Class|GSCCoreComponent|GetCurrentAttributeValue _gsccore_3 "(AttributeName=\"AttackSpeed\",Attribute=/Script/RTD.TowerAttributeSet:AttackSpeed,AttributeOwner=Class'\"/Script/RTD.TowerAttributeSet\"')")) 0.01)) "CaseSensitive") "CRITCHANCE" (Utilities|String|ToString(Text) (Class|KismetTextLibrary|AsPercentFloat (Class|GSCCoreComponent|GetCurrentAttributeValue _gsccore "(AttributeName=\"CritChance\",Attribute=/Script/RTD.TowerAttributeSet:CritChance,AttributeOwner=Class'\"/Script/RTD.TowerAttributeSet\"')") "HalfToEven")) "CaseSensitive") "CRITX" (Utilities|String|ToString(Float) (Math|Float|SnapToGrid(Float) (Class|GSCCoreComponent|GetCurrentAttributeValue _gsccore "(AttributeName=\"CritX\",Attribute=/Script/RTD.TowerAttributeSet:CritX,AttributeOwner=Class'\"/Script/RTD.TowerAttributeSet\"')") 0.01)) "CaseSensitive"))) (Variables|Default|GetUpgradeCost) (Variables|Default|GetSellValue) (Variables|Default|GetItems) (Variables|Default|GetAvailableModes) (Variables|Default|GetTargetingMode1) (Variables|Default|GetTargetingPriority1))
  (Variables|/Game/Blueprints/Building/Tower/BP_BeamComponent.BP_BeamComponent_C|SetBeamCount _bp_beamcomponent (Math|Float|Floor (Class|GSCCoreComponent|GetCurrentAttributeValue (Variables|Default|GetGSCCore) "(AttributeName=\"CurrentTargets\",Attribute=/Script/RTD.TowerAttributeSet:CurrentTargets,AttributeOwner=Class'\"/Script/RTD.TowerAttributeSet\"')")))
  (Default|CheckBeamCount _bp_beamcomponent)
  (Default|UpdateBeamStats (Variables|Default|GetBP_BeamComponent) (Class|GSCCoreComponent|GetCurrentAttributeValue _gsccore_2 "(AttributeName=\"AttackPower\",Attribute=/Script/RTD.TowerAttributeSet:AttackPower,AttributeOwner=Class'\"/Script/RTD.TowerAttributeSet\"')") (Class|GSCCoreComponent|GetCurrentAttributeValue _gsccore_2 "(AttributeName=\"Range\",Attribute=/Script/RTD.TowerAttributeSet:Range,AttributeOwner=Class'\"/Script/RTD.TowerAttributeSet\"')") (Class|GSCCoreComponent|GetCurrentAttributeValue _gsccore_2 "(AttributeName=\"AttackSpeed\",Attribute=/Script/RTD.TowerAttributeSet:AttackSpeed,AttributeOwner=Class'\"/Script/RTD.TowerAttributeSet\"')") (Class|GSCCoreComponent|GetCurrentAttributeValue _gsccore_2 "(AttributeName=\"CritChance\",Attribute=/Script/RTD.TowerAttributeSet:CritChance,AttributeOwner=Class'\"/Script/RTD.TowerAttributeSet\"')") (Class|GSCCoreComponent|GetCurrentAttributeValue _gsccore_2 "(AttributeName=\"CritX\",Attribute=/Script/RTD.TowerAttributeSet:CritX,AttributeOwner=Class'\"/Script/RTD.TowerAttributeSet\"')") (Variables|Default|GetDamageTypeClass)))