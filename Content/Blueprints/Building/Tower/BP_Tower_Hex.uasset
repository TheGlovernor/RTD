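; Hex tower Blueprint that fires slow projectiles which, per its tooltip, implode on the target, damaging enemies in range and slowing them by proximity to the edge.
; A self-repeating Attack loop spawns BP_Hex_Projectile from a mesh socket at the first targetable, waits by an attribute-driven rate, or polls briefly when none exist.
; GSCCore attributes supply projectile stats and fill placeholders in the rich-text description that ReportStats sends to the selection widget.
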(event EventAttack
  (bind _targetables (Variables|Default|GetTargetables))
  (bind _gsccore (Variables|Default|GetGSCCore))
  (if (Utilities|Array|IsNotEmpty _targetables)
    (Game|SpawnActorfromClass "/Game/Blueprints/Building/Tower/Projs_Beams/BP_Hex_Projectile.BP_Hex_Projectile_C" (Math|Transform|MakeTransform (Transformation|GetSocketLocation (Variables|Default|Getobs_Circle_011) "ProjSpawn")) "Undefined" 0 (Utilities|Array|Get(acopy) _targetables) (Variables|Default|GetDamageTypeClass) (Class|GSCCoreComponent|GetCurrentAttributeValue _gsccore "(AttributeName=\"ExplosionRadius\",Attribute=/Script/RTD.TowerAttributeSet:ExplosionRadius,AttributeOwner=Class'\"/Script/RTD.TowerAttributeSet\"')") (Class|GSCCoreComponent|GetCurrentAttributeValue _gsccore "(AttributeName=\"AttackPower\",Attribute=/Script/RTD.TowerAttributeSet:AttackPower,AttributeOwner=Class'\"/Script/RTD.TowerAttributeSet\"')") (Class|GSCCoreComponent|GetCurrentAttributeValue _gsccore "(AttributeName=\"CritChance\",Attribute=/Script/RTD.TowerAttributeSet:CritChance,AttributeOwner=Class'\"/Script/RTD.TowerAttributeSet\"')") (Class|GSCCoreComponent|GetCurrentAttributeValue _gsccore "(AttributeName=\"CritX\",Attribute=/Script/RTD.TowerAttributeSet:CritX,AttributeOwner=Class'\"/Script/RTD.TowerAttributeSet\"')") 0)
    (CallFunction|PlayShootingSound)
    (Utilities|FlowControl|Delay (/ 1.0 (Class|GSCCoreComponent|GetCurrentAttributeValue (Variables|Default|GetGSCCore) "(AttributeName=\"AttackSpeed\",Attribute=/Script/RTD.TowerAttributeSet:AttackSpeed,AttributeOwner=Class'\"/Script/RTD.TowerAttributeSet\"')")))
    (CallFunction|Attack)
    (else
      (Utilities|FlowControl|Delay 0.1)
      (CallFunction|Attack))))

(fn ConstructionScript
  (|CallParentFunction))

(fn ReportStats
  (bind _gsccore (Variables|Default|GetGSCCore))
  (bind _gsccore_2 (Variables|Default|GetGSCCore))
  (bind _rowname (CallFunction|GetDisplayData (Variables|Default|GetDamageTypeClass)))
  (Class|BPISelectionWidget|ReportStats(Message) (UserInterface|GetWidget (Variables|Default|GetSelectionWidget)) self (Components|GetOwner) (Variables|Default|GetTowerName) (Variables|Default|GetIcon) (Utilities|Array|MakeArray (Utilities|Text|ToText(String) (Utilities|String|Replace (Utilities|String|Replace (Utilities|String|Replace (Utilities|String|Replace (Utilities|String|Replace (Utilities|String|ToString(Text) (Utilities|Text|MakeLiteralText "Every <RichText.Emphasis>TIME</>s attacks with a slow moving projectile that implodes on it's target, causing <img id=\"ROW\"/><RichText.ROW>DAM</> damage in it's range and slows affected enemies by their proximity to it's edge.  This tower has a <RichText.Emphasis>CRITCHANCE</> chance to crit, dealing <RichText.Emphasis>CRITX</>x the damage.")) "DAM" (Utilities|String|ToString(Float) (Math|Float|SnapToGrid(Float) (Class|GSCCoreComponent|GetCurrentAttributeValue _gsccore_2 "(AttributeName=\"AttackPower\",Attribute=/Script/RTD.TowerAttributeSet:AttackPower,AttributeOwner=Class'\"/Script/RTD.TowerAttributeSet\"')") 0.1)) "CaseSensitive") "TIME" (Utilities|String|ToString(Float) (Math|Float|SnapToGrid(Float) (/ 1.0 (Class|GSCCoreComponent|GetCurrentAttributeValue _gsccore_2 "(AttributeName=\"AttackSpeed\",Attribute=/Script/RTD.TowerAttributeSet:AttackSpeed,AttributeOwner=Class'\"/Script/RTD.TowerAttributeSet\"')")) 0.1)) "CaseSensitive") "ROW" _rowname "CaseSensitive") "CRITCHANCE" (Utilities|String|ToString(Text) (Class|KismetTextLibrary|AsPercentFloat (Class|GSCCoreComponent|GetCurrentAttributeValue _gsccore "(AttributeName=\"CritChance\",Attribute=/Script/RTD.TowerAttributeSet:CritChance,AttributeOwner=Class'\"/Script/RTD.TowerAttributeSet\"')") "HalfToEven")) "CaseSensitive") "CRITX" (Utilities|String|ToString(Float) (Math|Float|SnapToGrid(Float) (Class|GSCCoreComponent|GetCurrentAttributeValue _gsccore "(AttributeName=\"CritX\",Attribute=/Script/RTD.TowerAttributeSet:CritX,AttributeOwner=Class'\"/Script/RTD.TowerAttributeSet\"')") 0.01)) "CaseSensitive"))) 0 0 (Variables|Default|GetItems) (Variables|Default|GetAvailableModes) (Variables|Default|GetTargetingMode) (Variables|Default|GetTargetingPriority)))