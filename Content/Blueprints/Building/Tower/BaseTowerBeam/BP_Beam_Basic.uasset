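; BP_Beam_Basic is a tower beam actor that deals damage to an assigned target while it is within range.
; Each tick, at an interval set by TickRate in the construction script, it checks that the target is valid and in range, hiding itself otherwise.
; When in range, it shows itself, stretches a spline mesh to the target's TargetPoint and applies damage with player controller 0 as instigator.
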(event EventBeginPlay)

(event Collision|EventActorBeginOverlap
  (params (OtherActor :type Actor%20Object%20Reference)))

(event EventTick
  (params (DeltaSeconds :type Float%20%28single-precision%29))
  (Utilities|IsValid (Variables|Default|GetTarget)
    (:Is%20Valid
      (if (> (Variables|Default|Getrange) (Math|Vector|Distance(Vector) (Transformation|GetActorLocation) (Transformation|GetActorLocation (Variables|Default|GetTarget))))
        (Rendering|SetActorHiddenInGame false)
        (CallFunction|UpdateDraw)
        (CallFunction|Damage)
        (else
          (Rendering|SetActorHiddenInGame true :!label _label))))
    (:Is%20Not%20Valid
      (goto _label))))

(fn ConstructionScript
  (Actor|Tick|SetActorTickInterval (Variables|Default|GetTickRate)))

(fn Damage
  (bind _target (Variables|Default|GetTarget))
  (Utilities|IsValid _target
    (:Is%20Valid
      (Game|Damage|ApplyDamage _target (Variables|Default|Getdmg) (Game|GetPlayerController 0) 0))))

(fn UpdateDraw
  (SplineMesh|SetStartandEnd (Variables|Default|GetSplineMesh) "0, 0, 0" "0, 0, 0" (- (Transformation|GetWorldLocation (Variables|/Game/Blueprints/Mobs/BP_Enemy_Base_01.BP_Enemy_Base_01_C|GetTargetPoint (Variables|Default|GetTarget))) (Transformation|GetActorLocation)) "0, 0, 0" true :!class /Script/Engine.SplineMeshComponent))