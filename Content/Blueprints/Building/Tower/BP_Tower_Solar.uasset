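; Solar tower that fires beams at multiple enemies through BPBeamComponent, with its stats held as GAS Companion attributes.
; Attribute changes are clamped, then refresh range or beam count where relevant, the beam's combat stats and the selection widget's description.
; Attack passes current targetables to the beam component and sets a looping timer to retarget.
; Level-ups apply a gameplay effect, and selling destroys the beam component.
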(event OnPostGameplayEffectExecute(GSCCore)
  (params (Attribute :type Gameplay%20Attribute%20Structure) (SourceActor :type Actor%20Object%20Reference) (TargetActor :type Actor%20Object%20Reference) (SourceTags :type Gameplay%20Tag%20Container%20Structure%20%28by%20ref%29) (Payload :type GSC%20Gameplay%20Effect%20Execute%20Data%20Structure))
  (bind _gsccore (Variables|Default|GetGSCCore))
  (bind _gsccore_2 (Variables|Default|GetGSCCore))
  (bind _bp_beamcomponent (Variables|Default|GetBP_BeamComponent))
  (|SwitchGameplayAttribute Attribute
    (:Level
      (Class|GSCCoreComponent|ClampAttributeValue (Variables|Default|GetGSCCore) "(AttributeName=\"Level\",Attribute=/Script/RTD.TowerAttributeSet:Level,AttributeOwner=Class'\"/Script/RTD.TowerAttributeSet\"')" 0.0 1e+08))
    (:AttackPower
      (Class|GSCCoreComponent|ClampAttributeValue (Variables|Default|GetGSCCore) "(AttributeName=\"AttackPower\",Attribute=/Script/RTD.TowerAttributeSet:AttackPower,AttributeOwner=Class'\"/Script/RTD.TowerAttributeSet\"')" 0.0 1e+08))
    (:AttackSpeed
      (Class|GSCCoreComponent|ClampAttributeValue (Variables|Default|GetGSCCore) "(AttributeName=\"AttackSpeed\",Attribute=/Script/RTD.TowerAttributeSet:AttackSpeed,AttributeOwner=Class'\"/Script/RTD.TowerAttributeSet\"')" 0.01 1e+08))
    (:Range
      (Class|GSCCoreComponent|ClampAttributeValue (Variables|Default|GetGSCCore) "(AttributeName=\"Range\",Attribute=/Script/RTD.TowerAttributeSet:Range,AttributeOwner=Class'\"/Script/RTD.TowerAttributeSet\"')" 0.0 1e+08)
      (CallFunction|UpdateRange))
    (:CurrentTargets
      (Class|GSCCoreComponent|ClampAttributeValue _gsccore_2 "(AttributeName=\"CurrentTargets\",Attribute=/Script/RTD.TowerAttributeSet:CurrentTargets,AttributeOwner=Class'\"/Script/RTD.TowerAttributeSet\"')" 1.0 (Class|GSCCoreComponent|GetCurrentAttributeValue _gsccore_2 "(AttributeName=\"MaxTargets\",Attribute=/Script/RTD.TowerAttributeSet:MaxTargets,AttributeOwner=Class'\"/Script/RTD.TowerAttributeSet\"')"))
      (Variables|/Game/Blueprints/Building/Tower/BP_BeamComponent.BP_BeamComponent_C|SetBeamCount _bp_beamcomponent (Math|Float|Floor (Class|GSCCoreComponent|GetCurrentAttributeValue _gsccore_2 "(AttributeName=\"CurrentTargets\",Attribute=/Script/RTD.TowerAttributeSet:CurrentTargets,AttributeOwner=Class'\"/Script/RTD.TowerAttributeSet\"')")))
      (Default|CheckBeamCount _bp_beamcomponent))
    (:MaxTargets
      (Class|GSCCoreComponent|ClampAttributeValue (Variables|Default|GetGSCCore) "(AttributeName=\"MaxTargets\",Attribute=/Script/RTD.TowerAttributeSet:MaxTargets,AttributeOwner=Class'\"/Script/RTD.TowerAttributeSet\"')" 0.0 1e+08))
    (:CritChance
      (Class|GSCCoreComponent|ClampAttributeValue (Variables|Default|GetGSCCore) "(AttributeName=\"CritChance\",Attribute=/Script/RTD.TowerAttributeSet:CritChance,AttributeOwner=Class'\"/Script/RTD.TowerAttributeSet\"')" 0.0 1e+08))
    (:CritX
      (Class|GSCCoreComponent|ClampAttributeValue (Variables|Default|GetGSCCore) "(AttributeName=\"CritChance\",Attribute=/Script/RTD.TowerAttributeSet:CritChance,AttributeOwner=Class'\"/Script/RTD.TowerAttributeSet\"')" 1.0 1e+08))
    (:MaxItems
      (Class|GSCCoreComponent|ClampAttributeValue (Variables|Default|GetGSCCore) "(AttributeName=\"MaxItems\",Attribute=/Script/RTD.TowerAttributeSet:MaxItems,AttributeOwner=Class'\"/Script/RTD.TowerAttributeSet\"')" 0.0 1e+08))
    (:BuyValue
      (Class|GSCCoreComponent|ClampAttributeValue (Variables|Default|GetGSCCore) "(AttributeName=\"BuyValue\",Attribute=/Script/RTD.TowerAttributeSet:BuyValue,AttributeOwner=Class'\"/Script/RTD.TowerAttributeSet\"')" 0.0 1e+08))
    (:UpgradeValue
      (Class|GSCCoreComponent|ClampAttributeValue (Variables|Default|GetGSCCore) "(AttributeName=\"UpgradeValue\",Attribute=/Script/RTD.TowerAttributeSet:UpgradeValue,AttributeOwner=Class'\"/Script/RTD.TowerAttributeSet\"')" 0.0 1e+08))
    (:SellValue
      (Class|GSCCoreComponent|ClampAttributeValue (Variables|Default|GetGSCCore) "(AttributeName=\"SellValue\",Attribute=/Script/RTD.TowerAttributeSet:SellValue,AttributeOwner=Class'\"/Script/RTD.TowerAttributeSet\"')" 0.0 1e+08)))
  (CallFunction|ReportStats)
  (Default|UpdateBeamStats (Variables|Default|GetBP_BeamComponent) (Class|GSCCoreComponent|GetCurrentAttributeValue _gsccore "(AttributeName=\"AttackPower\",Attribute=/Script/RTD.TowerAttributeSet:AttackPower,AttributeOwner=Class'\"/Script/RTD.TowerAttributeSet\"')") (Class|GSCCoreComponent|GetCurrentAttributeValue _gsccore "(AttributeName=\"Range\",Attribute=/Script/RTD.TowerAttributeSet:Range,AttributeOwner=Class'\"/Script/RTD.TowerAttributeSet\"')") (Class|GSCCoreComponent|GetCurrentAttributeValue _gsccore "(AttributeName=\"AttackSpeed\",Attribute=/Script/RTD.TowerAttributeSet:AttackSpeed,AttributeOwner=Class'\"/Script/RTD.TowerAttributeSet\"')") (Utilities|Array|MakeArray (Variables|Default|GetDamageTypeClass))))

(event OnInitAbilityActorInfo(GSCCore)
  (bind _bp_beamcomponent (Variables|Default|GetBP_BeamComponent))
  (Variables|/Game/Blueprints/Building/Tower/BP_BeamComponent.BP_BeamComponent_C|SetBeamCount _bp_beamcomponent (Math|Float|Floor (Class|GSCCoreComponent|GetCurrentAttributeValue (Variables|Default|GetGSCCore) "(AttributeName=\"CurrentTargets\",Attribute=/Script/RTD.TowerAttributeSet:CurrentTargets,AttributeOwner=Class'\"/Script/RTD.TowerAttributeSet\"')")))
  (Default|CheckBeamCount _bp_beamcomponent))

(event EventBeginPlay
  (bind _gsccore (Variables|Default|GetGSCCore))
  (bind _bp_beamcomponent (Variables|Default|GetBP_BeamComponent))
  (|CallParentFunction)
  (CallFunction|ToggleSelect false)
  (Variables|/Game/Blueprints/Building/Tower/BP_BeamComponent.BP_BeamComponent_C|SetBeamCount _bp_beamcomponent (Math|Float|Floor (Class|GSCCoreComponent|GetCurrentAttributeValue (Variables|Default|GetGSCCore) "(AttributeName=\"CurrentTargets\",Attribute=/Script/RTD.TowerAttributeSet:CurrentTargets,AttributeOwner=Class'\"/Script/RTD.TowerAttributeSet\"')")))
  (Default|CheckBeamCount _bp_beamcomponent)
  (CallFunction|ReportStats)
  (Default|UpdateBeamStats (Variables|Default|GetBP_BeamComponent) (Class|GSCCoreComponent|GetCurrentAttributeValue _gsccore "(AttributeName=\"AttackPower\",Attribute=/Script/RTD.TowerAttributeSet:AttackPower,AttributeOwner=Class'\"/Script/RTD.TowerAttributeSet\"')") (Class|GSCCoreComponent|GetCurrentAttributeValue _gsccore "(AttributeName=\"Range\",Attribute=/Script/RTD.TowerAttributeSet:Range,AttributeOwner=Class'\"/Script/RTD.TowerAttributeSet\"')") (Class|GSCCoreComponent|GetCurrentAttributeValue _gsccore "(AttributeName=\"AttackSpeed\",Attribute=/Script/RTD.TowerAttributeSet:AttackSpeed,AttributeOwner=Class'\"/Script/RTD.TowerAttributeSet\"')") (Utilities|Array|MakeArray (Variables|Default|GetDamageTypeClass))))

(event Collision|EventActorBeginOverlap
  (params (OtherActor :type Actor%20Object%20Reference))
  (|CallParentFunction OtherActor) ; This node is disabled and will not be called.\nDrag off pins to build functionality.
)

(event EventTick
  (params (DeltaSeconds :type Float%20%28single-precision%29))
  (|CallParentFunction DeltaSeconds) ; This node is disabled and will not be called.\nDrag off pins to build functionality.
)

(event EventAttack
  (Default|UpdateBeamTargets (Variables|Default|GetBP_BeamComponent) (Variables|Default|GetTargetables))
  (bind _returnvalue (Utilities|Time|SetTimerbyEvent (delegate EventAttack) 0.1 true))
  (Variables|Default|SetAttack%20Timer _returnvalue))

(event EventLevelUp
  (|CallParentFunction)
  (GameplayEffects|ApplyGameplayEffectToSelf :self (Variables|Default|GetGSCAbilitySystem) :GameplayEffectClass "/Game/Blueprints/Building/Tower/Stats/GE_Solar_LevelUp.GE_Solar_LevelUp_C" :Level 1.0))

(event EventSell
  (Components|DestroyComponent (Variables|Default|GetBP_BeamComponent))
  (|CallParentFunction))

(fn ConstructionScript
  (|CallParentFunction))

(fn ReportStats
  (bind _gsccore (Variables|Default|GetGSCCore))
  (bind _gsccore_2 (Variables|Default|GetGSCCore))
  (bind _rowname (CallFunction|GetDisplayData (Variables|Default|GetDamageTypeClass)))
  (Class|BPISelectionWidget|ReportStats(Message) (UserInterface|GetWidget (Variables|Default|GetSelectionWidget)) self (Components|GetOwner) (Variables|Default|GetTowerName) (Variables|Default|GetIcon) (Utilities|Array|MakeArray (Utilities|Text|ToText(String) (Utilities|String|Replace (Utilities|String|Replace (Utilities|String|Replace (Utilities|String|Replace (Utilities|String|ToString(Text) (Utilities|Text|MakeLiteralText "Shoots beams at up to <RichText.Emphasis>TARGETS</> enemies, dealing <img id=\"ROW\"/><RichText.ROW> DMG</> damage to each every <RichText.Emphasis>TIME</> seconds.")) "TARGETS" (Utilities|String|ToString(Integer) (Math|Float|Round (Class|GSCCoreComponent|GetCurrentAttributeValue _gsccore "(AttributeName=\"CurrentTargets\",Attribute=/Script/RTD.TowerAttributeSet:CurrentTargets,AttributeOwner=Class'\"/Script/RTD.TowerAttributeSet\"')"))) "CaseSensitive") "ROW" _rowname "CaseSensitive") "DMG" (Utilities|String|ToString(Float) (Class|GSCCoreComponent|GetCurrentAttributeValue _gsccore "(AttributeName=\"AttackPower\",Attribute=/Script/RTD.TowerAttributeSet:AttackPower,AttributeOwner=Class'\"/Script/RTD.TowerAttributeSet\"')")) "CaseSensitive") "TIME" (Utilities|String|ToString(Float) (Class|GSCCoreComponent|GetCurrentAttributeValue _gsccore "(AttributeName=\"AttackSpeed\",Attribute=/Script/RTD.TowerAttributeSet:AttackSpeed,AttributeOwner=Class'\"/Script/RTD.TowerAttributeSet\"')")) "CaseSensitive"))) (Math|Float|Truncate (Class|GSCCoreComponent|GetCurrentAttributeValue _gsccore_2 "(AttributeName=\"Level\",Attribute=/Script/RTD.TowerAttributeSet:Level,AttributeOwner=Class'\"/Script/RTD.TowerAttributeSet\"')")) (Class|GSCCoreComponent|GetCurrentAttributeValue _gsccore_2 "(AttributeName=\"AttackPower\",Attribute=/Script/RTD.TowerAttributeSet:AttackPower,AttributeOwner=Class'\"/Script/RTD.TowerAttributeSet\"')") (Class|GSCCoreComponent|GetCurrentAttributeValue _gsccore_2 "(AttributeName=\"AttackSpeed\",Attribute=/Script/RTD.TowerAttributeSet:AttackSpeed,AttributeOwner=Class'\"/Script/RTD.TowerAttributeSet\"')") (Class|GSCCoreComponent|GetCurrentAttributeValue _gsccore_2 "(AttributeName=\"Range\",Attribute=/Script/RTD.TowerAttributeSet:Range,AttributeOwner=Class'\"/Script/RTD.TowerAttributeSet\"')") (Class|GSCCoreComponent|GetCurrentAttributeValue _gsccore_2 "(AttributeName=\"CritChance\",Attribute=/Script/RTD.TowerAttributeSet:CritChance,AttributeOwner=Class'\"/Script/RTD.TowerAttributeSet\"')") (Math|Float|Floor (Class|GSCCoreComponent|GetCurrentAttributeValue _gsccore_2 "(AttributeName=\"CurrentTargets\",Attribute=/Script/RTD.TowerAttributeSet:CurrentTargets,AttributeOwner=Class'\"/Script/RTD.TowerAttributeSet\"')")) (Variables|Default|GetUpgradeCost) (Variables|Default|GetSellValue) (Variables|Default|GetItems) (Variables|Default|GetAvailableModes) (Variables|Default|GetTargetingMode) (Variables|Default|GetTargetingPriority)))