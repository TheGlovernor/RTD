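; Beam tower Blueprint, kept under DeprecatedTowers, that attacks by assigning targets to persistent beam actors.
; On BeginPlay it spawns one BP_Beam_Basic at its point light, passing calculated power, range and physical damage type, and stores it in a beam array.
; AttemptAttack pairs acquired targets with beams by index, up to the smaller count, leaving the rest of the attack to the beam actors.
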(event EventBeginPlay
  (|CallParentFunction)
  (bind _returnvalue (Game|SpawnActorfromClass "/Game/Blueprints/Building/Tower/Projs_Beams/BP_Beam_Basic.BP_Beam_Basic_C" (Math|Transform|MakeTransform (Transformation|GetWorldLocation (Variables|Default|GetPointLight))) "Undefined" self 0 (Variables|Default|GetCalculatedPower) (Variables|Default|GetCalculatedRange) "/Game/Blueprints/HealthDamage/DamageClasses/DamageType_Phys.DamageType_Phys_C" 0))
  (Utilities|Array|Add (Variables|Targeting|GetBeams_0) _returnvalue))

(event Collision|EventActorBeginOverlap
  (params (OtherActor :type Actor%20Object%20Reference))
  (|CallParentFunction OtherActor) ; This node is disabled and will not be called.\nDrag off pins to build functionality.
)

(event EventTick
  (params (DeltaSeconds :type Float%20%28single-precision%29))
  (|CallParentFunction DeltaSeconds))

(fn ConstructionScript
  (|CallParentFunction))

(fn AttemptAttack
  (bind _targets1 (CallFunction|AqcuireTargets))
  (for _index (range 0 (- (Math|Integer|Min(Integer) (Utilities|Array|Length _targets1) (Utilities|Array|Length (Variables|Targeting|GetBeams_0))) 1))
    (Variables|/Game/Blueprints/Building/Tower/Projs_Beams/BP_Beam_Basic.BP_Beam_Basic_C|SetTarget (Utilities|Array|Get(acopy) (Variables|Targeting|GetBeams_0) _index) (Utilities|Array|Get(acopy) _targets1 _index))))