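; Deprecated area-of-effect tower Blueprint, meant to damage enemies inside a circular or wedge-shaped zone around it.
; Tick applies CalculatedPower damage every frame, but its loop's array input shows no source.
; Disconnected logic would build a procedural fan mesh with convex collision from AOEAngle, Sections and CalculatedRange.
; Overlap events and CreateAOEMesh are empty, leaving enemy tracking and mesh generation inactive.
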(event OnComponentEndOverlap(AOEMesh)
  (params (OverlappedComponent :type Primitive%20Component%20Object%20Reference) (OtherActor :type Actor%20Object%20Reference) (OtherComp :type Primitive%20Component%20Object%20Reference) (OtherBodyIndex :type Integer)))

(event OnComponentBeginOverlap(AOEMesh)
  (params (OverlappedComponent :type Primitive%20Component%20Object%20Reference) (OtherActor :type Actor%20Object%20Reference) (OtherComp :type Primitive%20Component%20Object%20Reference) (OtherBodyIndex :type Integer) (bFromSweep :type Boolean) (SweepResult :type Hit%20Result%20Structure%20%28by%20ref%29)))

(event EventBeginPlay
  (|CallParentFunction))

(event Collision|EventActorBeginOverlap
  (params (OtherActor :type Actor%20Object%20Reference)))

(event EventTick
  (params (DeltaSeconds :type Float%20%28single-precision%29))
  (for _array_element 0
    (Game|Damage|ApplyDamage _array_element (Variables|Default|GetCalculatedPower) (Game|GetPlayerController 0) self)))

(fn ConstructionScript
  (|CallParentFunction))

(fn CreateAOEMesh)