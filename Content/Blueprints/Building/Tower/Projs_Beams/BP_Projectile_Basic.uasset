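; Basic tower projectile that homes in on an assigned enemy Target and deals Power damage of its DamageType on overlap, then destroys itself.
; The construction script sets the ProjectileMovement homing target to the enemy's DamageCapsule, destroying the projectile if Target is not a BP_Enemy_Base_01.
; A manual movement routine toward the target's last known location remains in the graph but is never run.
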(event Collision|EventActorBeginOverlap
  (params (OtherActor :type Actor%20Object%20Reference))
  (if (== OtherActor (Variables|Default|GetTarget))
    (Game|Damage|ApplyDamage OtherActor (Variables|Default|GetPower) 0 0 (Variables|Default|GetDamageType))
    (Actor|DestroyActor)))

(event EventDestroyed
  (Actor|Tick|SetActorTickEnabled false))

(fn ConstructionScript
  (bind _asbp_enemy_base_01 (Utilities|Casting|CastToBP_Enemy_Base_01 (Variables|Default|GetTarget))
    (:then
      (Variables|/Script/Engine.ProjectileMovementComponent|SetHomingTargetComponent (Variables|Default|GetProjectileMovement) (Variables|/Game/Blueprints/Mobs/EnemyBPs/BP_Enemy_Base_01.BP_Enemy_Base_01_C|GetDamageCapsule _asbp_enemy_base_01)))
    (:CastFailed
      (Actor|DestroyActor))))