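; BP_ArtilleryShell is an artillery shell projectile that explodes when it nears a surface below it.
; The construction script sets the projectile movement's initial speed from InitialVelocity.
; A timer opens a gate shortly after spawn, letting Tick run a short downward line trace as a proximity check.
; The first hit spawns BP_Explosion once, passing on owner, damage, radius, damage type and status-effect settings, then destroys the shell.
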(event Custom|OpenGate
  (bind _returnvalue (Transformation|GetActorLocation))
  (Utilities|FlowControl|Gate true) ; enters at Open
)

(event EventTick
  (params (DeltaSeconds :type Float%20%28single-precision%29))
  (bind _returnvalue (Transformation|GetActorLocation))
  (Utilities|FlowControl|Gate true
    (:Exit
      (bind _returnvalue_2 (Collision|LineTraceByChannel _returnvalue (- _returnvalue "0.000000,0.000000,50.000000") "TraceTypeQuery5" false 0 "None" true "(R=1.000000,G=0.000000,B=0.000000,A=1.000000)" "(R=0.000000,G=1.000000,B=0.000000,A=1.000000)" 1e+01))
      (if _returnvalue_2
        (Utilities|FlowControl|DoOnce false
          (:Completed
            (Game|SpawnActorfromClass "/Game/Blueprints/Building/Tower/Projs_Beams/BP_Explosion.BP_Explosion_C" (Math|Transform|MakeTransform (Transformation|GetActorLocation) "0, 0, 0" "1.000000,1.000000,1.000000") "AlwaysSpawn" "OverrideRootScale" (Components|GetOwner) (Variables|Default|GetDamage) (Variables|Default|GetRadius) (Variables|Default|GetDamageTypeClass) (Variables|Default|GetbForceFrost) (Variables|Default|GetbForceEntangle) (Variables|Default|GetbForceBleed) (Variables|Default|GetbForceEngulf) (Variables|Default|GetbForceStun) 0)
            (Actor|DestroyActor)))))))

(event EventBeginPlay
  (Utilities|Time|SetTimerbyEvent (delegate Custom|OpenGate) 0.5))

(fn ConstructionScript
  (Variables|/Script/Engine.ProjectileMovementComponent|SetInitialSpeed (Variables|Default|GetProjectileMovement) (Variables|Default|GetInitialVelocity)))