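; Chain beam projectile for towers that jumps from its initial target to nearby enemies, damaging each one.
; On BeginPlay it repeatedly sphere-traces around the last target to add a new ticking enemy, up to the jump limit.
; It creates a Niagara arc per target, has the owning tower apply status effects, and deals damage.
; A fast looping timer keeps arc endpoints on the targets until the actor self-destructs shortly afterward.
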(event Custom|updateArcs
  (bind _returnvalue (Transformation|GetActorLocation))
  (bind _targets (Variables|Default|GetTargets))
  (bind _output (Utilities|Array|Get(acopy) _targets))
  (for (_array_element _array_index) (Variables|Default|Getarcs)
    (if (== _array_index 0)
      (Effects|Components|ParticleSystem|SetVectorParameter _array_element "User.BeamStartPoint" _returnvalue)
      (Utilities|IsValid _output
        (:Is%20Valid
          (bind _location (Class|EnemyInterface|ReportTargetPoint(Message) _output))
          (Effects|Components|ParticleSystem|SetVectorParameter _array_element "User.BeamEndpoint" _location))
        (:Is%20Not%20Valid
          (Effects|Components|ParticleSystem|SetVectorParameter _array_element "User.BeamEndpoint" _returnvalue)))
      (else
        (Utilities|IsValid (Utilities|Array|Get(acopy) _targets (- _array_index 1))
          (:Is%20Valid
            (bind _location_2 (Class|EnemyInterface|ReportTargetPoint(Message) (Utilities|Array|Get(acopy) _targets (- _array_index 1))))
            (Utilities|IsValid (Utilities|Array|Get(acopy) _targets (+ _array_index 0))
              (:Is%20Valid
                (bind _location_3 (Class|EnemyInterface|ReportTargetPoint(Message) (Utilities|Array|Get(acopy) _targets (+ _array_index 0))))
                (Effects|Components|ParticleSystem|SetVectorParameter _array_element "User.BeamStartPoint" _location_2)
                (Effects|Components|ParticleSystem|SetVectorParameter _array_element "User.BeamEndpoint" _location_3))))))))
  (if (Variables|Default|GetFirst)
    (Variables|Default|SetFirst false)
    (for _array_element_2 (Variables|Default|Getarcs)
      (Components|Activation|Activate _array_element_2 false))))

(event EventBeginPlay
  (bind _targets (Variables|Default|GetTargets))
  (bind _targets_2 (Variables|Default|GetTargets))
  (Utilities|Array|Add _targets_2 (Variables|Default|GetTarget))
  (Utilities|FlowControl|Sequence
    (:then_0
      (bind _index (Utilities|FlowControl|ForLoopwithBreak 0 (- (Variables|Default|GetJumps) 2) :!label _label)
        (:LoopBody
          (Utilities|IsValid (Utilities|Array|Get(acopy) _targets_2 _index)
            (:Is%20Valid
              (bind (_outhits _returnvalue) (Collision|MultiSphereTraceByChannel (Transformation|GetActorLocation (Utilities|Array|Get(acopy) _targets_2 _index)) (Transformation|GetActorLocation (Utilities|Array|Get(acopy) _targets_2 _index)) 2e+02 "TraceTypeQuery1" false 0 "None"))
              (if _returnvalue
                (bind _array_element (Utilities|Array|ForEachLoopwithBreak _outhits :!label _label_2)
                  (:LoopBody
                    (bind _asbp_enemy_base_01 (Utilities|Casting|CastToBP_Enemy_Base_01 (.HitActor (Collision|BreakHitResult _array_element))))
                    (if (and (Class|Actor|IsActorTickEnabled _asbp_enemy_base_01) (not (Utilities|Array|ContainsItem (Variables|Default|GetTargets) (.HitActor (Collision|BreakHitResult _array_element)))))
                      (Utilities|Array|Add (Variables|Default|GetTargets) (.HitActor (Collision|BreakHitResult _array_element)))
                      (goto _label_2 Break))))
                (else
                  (goto _label Break))))))))
    (:then_1
      (for _index_2 (range 0 (- (Utilities|Array|Length (Variables|Default|GetTargets)) 1))
        (bind _returnvalue_2 (AddComponent|AddNiagaraComponent false))
        (Utilities|Array|Add (Variables|Default|Getarcs) _returnvalue_2))
      (CallFunction|UpdateArcs)
      (bind _asbp_tower_1parent (Utilities|Casting|CastToBP_Tower_1Parent (Components|GetOwner))
        (:then
          (Default|ApplyStatusEffectstoAll _asbp_tower_1parent _targets))
        (:CastFailed
          _))
      (for _array_element_2 _targets
        (Game|Damage|ApplyDamage _array_element_2 (Variables|Default|GetDamage) 0 0 (Variables|Default|GetDamage%20Type%20Class))))
    (:then_2
      (Utilities|Time|SetTimerbyEvent (delegate Custom|updateArcs) 0.01 true)
      (Utilities|FlowControl|Delay 0.2)
      (Actor|DestroyActor))))

(fn ConstructionScript)