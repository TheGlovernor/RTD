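; Tower-fired roots projectile that chases its target horizontally and applies the tower's status effect on overlap or arrival.
; Tick steers and moves the actor, snapping onto the target when in reach, while a downward trace keeps the Vines effect just below ground.
; Vines deactivate after a tower attribute-based delay or on target loss, and their finish event destroys the actor.
; Audio volume follows saved settings on a log scale.
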(event OnSystemFinished(Vines)
  (params (PSystem :type Niagara%20Component%20Object%20Reference))
  (Actor|DestroyActor))

(event EventBeginPlay
  (Utilities|FlowControl|Delay 0.1)
  (Components|Activation|Activate (Variables|Default|GetVines) false)
  (bind _returnvalue (SaveGame|LoadGamefromSlot "GameConfig"))
  (bind _assave_game_config (Utilities|Casting|CastToSave_GameConfig _returnvalue))
  (Audio|Components|Audio|SetVolumeMultiplier (Variables|Default|GetAudio) (Math|Float|Log (+ (* (Variables|/Game/Blueprints/Saves/Save_GameConfig.Save_GameConfig_C|GetSEVol _assave_game_config) (Variables|/Game/Blueprints/Saves/Save_GameConfig.Save_GameConfig_C|GetMainVol _assave_game_config)) 1.0) 1e+01) :!class /Script/Engine.AudioComponent))

(event EventUpdateSFXVol
  (bind _returnvalue (SaveGame|LoadGamefromSlot "GameConfig"))
  (bind _assave_game_config (Utilities|Casting|CastToSave_GameConfig _returnvalue))
  (Audio|Components|Audio|SetVolumeMultiplier (Variables|Default|GetAudio) (Math|Float|Log (+ (* (Variables|/Game/Blueprints/Saves/Save_GameConfig.Save_GameConfig_C|GetSEVol _assave_game_config) (Variables|/Game/Blueprints/Saves/Save_GameConfig.Save_GameConfig_C|GetMainVol _assave_game_config)) 1.0) 1e+01) :!class /Script/Engine.AudioComponent))

(event EventTick
  (params (DeltaSeconds :type Float%20%28single-precision%29))
  (bind _returnvalue (Transformation|GetActorLocation))
  (bind _returnvalue_2 (Transformation|GetActorLocation))
  (bind _target (Variables|Default|GetTarget))
  (bind _speed (Variables|Default|GetSpeed))
  (bind _target_2 (Variables|Default|GetTarget))
  (bind _returnvalue_3 (Transformation|GetActorLocation _target))
  (bind (_x _y) (Class|KismetMathLibrary|BreakVector3f _returnvalue))
  (bind _returnvalue_4 (Transformation|GetActorLocation _target_2))
  (bind _returnvalue_5 (Math|Vector|GetUnitDirection(Vector) (Math|Vector|MakeVector (.x _returnvalue_2) (.y _returnvalue_2) 0.0) (Math|Vector|MakeVector (.x _returnvalue_3) (.y _returnvalue_3) 0.0)))
  (bind (_x_2 _y_2) (Math|Vector|BreakVector _returnvalue_5))
  (Variables|Default|GetTarget
    (:then
      (Transformation|SetActorRotation (Math|Conversions|RotationFromXVector (Math|Vector|MakeVector _x_2 _y_2 0.0)))
      (if (> (* DeltaSeconds _speed) (Math|Vector|Distance(Vector) (Math|Vector|MakeVector (.x _returnvalue_2) (.y _returnvalue_2) 0.0) (Math|Vector|MakeVector (.x _returnvalue_3) (.y _returnvalue_3) 0.0)))
        (Transformation|SetActorLocation (Math|Vector|MakeVector (.x _returnvalue_4) (.y _returnvalue_4) (.z (Transformation|GetActorLocation))) false false)
        (Utilities|FlowControl|Sequence
          (:then_0
            (Utilities|FlowControl|DoOnce false
              (:Completed
                (Default|ApplyStatusEffect (Variables|Default|GetTower) (Variables|Default|GetTarget))
                (Utilities|FlowControl|Delay (Class|GSCCoreComponent|GetCurrentAttributeValue (Variables|/Game/Blueprints/Building/Tower/BP_Tower_1Parent.BP_Tower_1Parent_C|GetGSCCore (Variables|Default|GetTower)) "(AttributeName=\"EntangleDuration\",Attribute=/Script/RTD.TowerAttributeSet:EntangleDuration,AttributeOwner=Class'\"/Script/RTD.TowerAttributeSet\"')"))
                (Components|Activation|Deactivate (Variables|Default|GetVines)))))
          (:then_1
            (bind _outhit (Collision|LineTraceByChannel _returnvalue (Math|Vector|MakeVector _x _y -1e+03) "TraceTypeQuery5" false 0 "None" :!label _label))
            (Transformation|SetWorldLocation (Variables|Default|GetVines) (- (.Location (Collision|BreakHitResult _outhit)) "0,0,25.000000") false false)))
        (else
          (Transformation|AddActorWorldOffset (* DeltaSeconds _speed _returnvalue_5))
          (goto _label))))
    (:else
      (Components|Activation|Deactivate (Variables|Default|GetVines)))))

(event Collision|EventActorBeginOverlap
  (params (OtherActor :type Actor%20Object%20Reference))
  (bind _target (Variables|Default|GetTarget))
  (if (== OtherActor _target)
    (Default|ApplyStatusEffect (Variables|Default|GetTower) _target)))

(fn ConstructionScript)