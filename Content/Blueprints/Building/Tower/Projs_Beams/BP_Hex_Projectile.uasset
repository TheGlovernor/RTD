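; Homing tower projectile that implodes on reaching its target, applying Frost and area damage, with effects colored by damage type.
; Homing acceleration grows every tick toward the enemy's damage capsule.
; On first target overlap it stops, sphere-traces the radius and stacks Frost on each hit enemy, with more applications the farther it is from the center.
; Radial damage lands when the implosion effect finishes, and the actor is destroyed after its smoke trail ends.
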(event OnSystemFinished(Implosion)
  (params (PSystem :type Niagara%20Component%20Object%20Reference))
  (bind _damage (Variables|Default|GetDamage))
  (bind _radius (Variables|Default|GetRadius))
  (Class|GameplayStatics|ApplyRadialDamagewithFalloff _damage (/ _damage 5.0) (+ (Transformation|GetActorLocation) "0,0,10.000000") (* _radius 2.0) _radius 1.0 (Variables|Default|GetDamageType) 0 0 0 "ECC_GameTraceChannel2")
  (Components|Activation|Deactivate (Variables|Default|GetSmokeTrail)))

(event OnSystemFinished(SmokeTrail)
  (params (PSystem :type Niagara%20Component%20Object%20Reference))
  (Actor|DestroyActor))

(event EventTick
  (params (DeltaSeconds :type Float%20%28single-precision%29))
  (bind _projectilemovement (Variables|Default|GetProjectileMovement))
  (Variables|/Script/Engine.ProjectileMovementComponent|SetHomingAccelerationMagnitude _projectilemovement (+ (* DeltaSeconds 5e+03) (Variables|/Script/Engine.ProjectileMovementComponent|GetHomingAccelerationMagnitude _projectilemovement))))

(event EventBeginPlay
  (bind _implosion (Variables|Default|GetImplosion))
  (bind _smoketrail (Variables|Default|GetSmokeTrail))
  (bind _ac_effectcolor (Variables|Default|GetAC_EffectColor))
  (bind _damagetype (Variables|Default|GetDamageType))
  (bind _stencilvalue (Variables|/Game/Blueprints/Building/Tower/Projs_Beams/AC_EffectColor.AC_EffectColor_C|GetStencilValue _ac_effectcolor))
  (bind _primarycolor (Variables|/Game/Blueprints/Building/Tower/Projs_Beams/AC_EffectColor.AC_EffectColor_C|GetPrimaryColor _ac_effectcolor))
  (bind _value (Utilities|Map|Find _primarycolor _damagetype))
  (bind _value_2 (Utilities|Map|Find _stencilvalue _damagetype))
  (Effects|Components|ParticleSystem|SetColorParameter _implosion "User.Color" _value)
  (Rendering|SetCustomDepthStencilValue _implosion _value_2)
  (Effects|Components|ParticleSystem|SetColorParameter _smoketrail "User.Color" _value)
  (Effects|Components|ParticleSystem|SetColorParameter _smoketrail "User.SecondaryColor" (.Value (Utilities|Map|Find (Variables|/Game/Blueprints/Building/Tower/Projs_Beams/AC_EffectColor.AC_EffectColor_C|GetSecondaryColor _ac_effectcolor) _damagetype)))
  (Rendering|SetCustomDepthStencilValue _smoketrail _value_2))

(event Collision|EventActorBeginOverlap
  (params (OtherActor :type Actor%20Object%20Reference))
  (bind _returnvalue (Transformation|GetActorLocation))
  (if (== OtherActor (Variables|Default|GetTarget))
    (Utilities|FlowControl|DoOnce false
      (:Completed
        (Components|Activation|Activate (Variables|Default|GetImplosion) false)
        (Components|Activation|Deactivate (Variables|Default|GetProjectileMovement))
        (bind _outhits (Collision|MultiSphereTraceByChannel _returnvalue _returnvalue (Variables|Default|GetRadius) "TraceTypeQuery6" false 0 "ForDuration"))
        (for _array_element _outhits
          (Utilities|Array|AddUnique (Variables|Default|GetHitEnemies) (.HitActor (Collision|BreakHitResult _array_element))))
        (for _array_element_2 (Variables|Default|GetHitEnemies)
          (for _index (range 0 (Math|Float|Floor (Math|Float|Clamp(Float) (* (/ (Math|Vector|Distance(Vector) (Transformation|GetActorLocation _array_element_2) (Transformation|GetActorLocation)) (Variables|Default|GetRadius)) 1e+01) 0.0 9.0)))
            (Class|GASInterface|ApplyEffect(Message) _array_element_2 (Variables|Default|GetGSCAbilitySystem) "/Game/Blueprints/Effects/GE_Frost.GE_Frost_C" 0.0)))))))

(fn ConstructionScript
  (bind _asbp_enemy_base_01 (Utilities|Casting|CastToBP_Enemy_Base_01 (Variables|Default|GetTarget)))
  (Variables|/Script/Engine.ProjectileMovementComponent|SetHomingTargetComponent (Variables|Default|GetProjectileMovement) (Variables|/Game/Blueprints/Mobs/EnemyBPs/BP_Enemy_Base_01.BP_Enemy_Base_01_C|GetDamageCapsule _asbp_enemy_base_01))
  (Effects|Components|ParticleSystem|SetFloatParameter (Variables|Default|GetImplosion) "User.Radius" (Variables|Default|GetRadius)))