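; BP_Projectile_Instant is an instant tower projectile that stretches a spline mesh from its own origin to a target.
; The construction script pins the spline's first point locally and places the second at the target's reported point, or at LastKnownLocation if the target is invalid.
; A newly added spline mesh component then takes those points as its start and end positions.
; The event graph contains no active logic.
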(event EventBeginPlay
  (|CallParentFunction) ; This node is disabled and will not be called.\nDrag off pins to build functionality.
)

(event Collision|EventActorBeginOverlap
  (params (OtherActor :type Actor%20Object%20Reference))
  (|CallParentFunction OtherActor) ; This node is disabled and will not be called.\nDrag off pins to build functionality.
)

(fn ConstructionScript
  (bind _spline (Variables|Default|GetSpline))
  (bind _returnvalue (AddComponent|AddSplineMeshComponent false))
  (Spline|SetLocationatSplinePoint (Variables|Default|GetSpline) 0 (Math|Vector|MakeVector 0.0 0.0 0.0) "Local" true)
  (bind _target (Variables|Default|GetTarget)
    (:then
      (bind _target_2 (Class|EnemyInterface|ReportTargetPoint(Message) _target))
      (Spline|SetLocationatSplinePoint (Variables|Default|GetSpline) 1 (Transformation|GetWorldLocation _target_2) "World" true))
    (:else
      (Spline|SetLocationatSplinePoint (Variables|Default|GetSpline) 1 (Variables|Default|GetLastKnownLocation) "World" true)))
  (SplineMesh|SetStartandEnd _returnvalue (Spline|GetLocationatSplinePoint _spline 0 "Local") "0, 0, 0" (Spline|GetLocationatSplinePoint _spline 1 "Local") "0, 0, 0" true :!class /Script/Engine.SplineMeshComponent))