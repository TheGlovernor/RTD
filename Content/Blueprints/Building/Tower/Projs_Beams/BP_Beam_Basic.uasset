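; Basic tower beam actor that draws a Niagara beam to its Target and damages it.
; Tick shows the beam only within range, updating its endpoint from the target's reported point.
; A self-rescheduling timer applies every damage type at AttackSpeed, polling when targetless, without checking range.
; UpdateStats sets combat stats and colors the beam red for leading fire damage, otherwise blue.
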(event Custom|ApplyDamage
  (Variables|Default|GetTarget
    (:then
      (CallFunction|Damage)
      (bind _returnvalue (Utilities|Time|SetTimerbyEvent (delegate Custom|ApplyDamage) (/ 1.0 (Variables|Default|GetAttackSpeed)) true))
      (Variables|Default|SetDamageTimer _returnvalue))
    (:else
      (bind _returnvalue_2 (Utilities|Time|SetTimerbyEvent (delegate Custom|ApplyDamage) 0.1 true))
      (Variables|Default|SetDamageTimer _returnvalue_2))))

(event EventBeginPlay
  (bind _returnvalue (Utilities|Time|SetTimerbyEvent (delegate Custom|ApplyDamage) 0.1 true))
  (Variables|Default|SetDamageTimer _returnvalue))

(event EventTick
  (params (DeltaSeconds :type Float%20%28single-precision%29))
  (bind _returnvalue (Transformation|GetActorLocation))
  (bind _target (Variables|Default|GetTarget))
  (bind _beameffect (Variables|Default|GetBeamEffect))
  (bind _returnvalue_2 (Transformation|GetActorLocation _target))
  (Utilities|IsValid (Variables|Default|GetTarget)
    (:Is%20Valid
      (if (> (+ (Variables|Default|Getrange) 2e+01) (Math|Vector|Distance(Vector) (Math|Vector|MakeVector (.x _returnvalue) (.y _returnvalue) 0.0) (Math|Vector|MakeVector (.x _returnvalue_2) (.y _returnvalue_2) 0.0)))
        (Components|Activation|Activate _beameffect false)
        (CallFunction|UpdateDraw)
        (else
          (Components|Activation|Deactivate _beameffect :!label _label))))
    (:Is%20Not%20Valid
      (goto _label))))

(fn ConstructionScript
  (Class|ActorComponent|SetComponentTickInterval (Variables|Default|GetBeamEffect) (Variables|Default|GetAttackSpeed)))

(fn Damage
  (bind _target (Variables|Default|GetTarget))
  (for _array_element (Variables|Default|GetDamageTypes)
    (Utilities|IsValid _target
      (:Is%20Valid
        (Game|Damage|ApplyDamage _target (Variables|Default|Getdmg) (Game|GetPlayerController 0) self _array_element)))))

(fn UpdateDraw
  (bind _target (Variables|Default|GetTarget))
  (Utilities|IsValid _target
    (:Is%20Valid
      (bind _location (Class|EnemyInterface|ReportTargetPoint(Message) _target))
      (Effects|Components|ParticleSystem|SetVectorParameter (Variables|Default|GetBeamEffect) "User.BeamEndpoint" (- _location (Transformation|GetActorLocation))))))

(fn UpdateStats
  (params (Damage :type Float%20%28double-precision%29) (Range :type Float%20%28double-precision%29) (AttackSpeed :type Float%20%28double-precision%29) (DamageTypes :type Array%20of%20Damage%20Type%20Class%20References))
  (bind _beameffect (Variables|Default|GetBeamEffect))
  (Utilities|FlowControl|Sequence
    (:then_0
      (Variables|Default|Setdmg Damage))
    (:then_1
      (Variables|Default|Setrange Range))
    (:then_2
      (Variables|Default|SetAttackSpeed AttackSpeed))
    (:then_3
      (bind _output_get (Variables|Default|SetDamageTypes DamageTypes))
      (if (== (Utilities|Array|Get(acopy) _output_get) "/Game/Blueprints/HealthDamage/DamageClasses/BP_FireDamage.BP_FireDamage_C")
        (Effects|Components|ParticleSystem|SetColorParameter _beameffect "User.BeamColor" (Utilities|Struct|MakeLinearColor 1.0 0.0 0.0 1.0))
        (else
          (Effects|Components|ParticleSystem|SetColorParameter _beameffect "User.BeamColor" (Utilities|Struct|MakeLinearColor 0.0 0.0 1.0 1.0)))))))