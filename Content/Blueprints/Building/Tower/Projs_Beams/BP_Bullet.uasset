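; BP_Bullet is a tower projectile that damages enemies it overlaps and can hit several before it is spent.
; Its construction script feeds Speed into the projectile movement's initial speed.
; While active, each overlap applies damage with the Tower as causer, then notifies the still-valid enemy and has the Tower apply status effects.
; Each such hit decrements Targets; below one, the bullet goes inactive and deactivates NSBullet a tick later.
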(event EventBeginPlay)

(event Collision|EventActorBeginOverlap
  (params (OtherActor :type Actor%20Object%20Reference))
  (bind _asbp_enemy_base_01 (Utilities|Casting|CastToBP_Enemy_Base_01 OtherActor))
  (if (Variables|Default|GetActive)
    (Game|Damage|ApplyDamage _asbp_enemy_base_01 (Variables|Default|GetDamage) (Game|GetPlayerController 0) (Variables|Default|GetTower) (Variables|Default|GetDamageClass))
    (Utilities|IsValid _asbp_enemy_base_01
      (:Is%20Valid
        (Class|EnemyInterface|BulletHit(Message) _asbp_enemy_base_01)
        (Default|ApplyStatusEffects (Variables|Default|GetTower) _asbp_enemy_base_01)
        (Variables|Default|SetTargets (- (Variables|Default|GetTargets) 1))
        (if (< (Variables|Default|GetTargets) 1)
          (Variables|Default|SetActive false)
          (Utilities|FlowControl|DelayUntilNextTick)
          (Components|Activation|Deactivate (Variables|Default|GetNS_Bullet)))))))

(fn ConstructionScript
  (Variables|/Script/Engine.ProjectileMovementComponent|SetInitialSpeed (Variables|Default|GetProjectileMovement) (Variables|Default|GetSpeed)))