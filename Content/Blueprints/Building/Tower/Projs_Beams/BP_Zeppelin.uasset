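; Zeppelin unit, apparently tower-spawned, that rises to a cruising altitude, then follows its target while bombing from above.
; Tick handles the ascent, then hands movement to the FloatingAIMovement component, which ChangeTarget retargets.
; From BeginPlay, Attack re-arms its own timer and drops a BP_ZeppelinBomb using damage stats set through UpdateStats.
; Bombs drop regardless of target or altitude, as a ground sphere-trace check is left disconnected.
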(event Custom|Attack
  (Utilities|Time|SetTimerbyEvent (delegate Custom|Attack) (Variables|Default|GetAttackSpeed))
  (Game|SpawnActorfromClass "/Game/Blueprints/Building/Tower/Projs_Beams/BP_ZeppelinBomb.BP_ZeppelinBomb_C" (Math|Transform|MakeTransform (+ (Transformation|GetActorLocation) "0,0.000000,-50.000000")) "AlwaysSpawn" 0 (Variables|Default|GetDamageType) (Variables|Default|GetDamage) (Variables|Default|GetRadius) 0))

(event Custom|ChangeTarget
  (params (NewTarget :type Actor%20Object%20Reference))
  (bind _output_get (Variables|Default|SetTarget NewTarget))
  (Default|ChangeTarget (Variables|Default|GetFloating_AI_Movement) _output_get 0 true))

(event Custom|Ascend
  (params (DeltaSeconds :type Float%20%28double-precision%29))
  (Transformation|SetActorLocation (+ (* DeltaSeconds "0,0,500.000000") (Transformation|GetActorLocation)) false false))

(event EventBeginPlay
  (Default|EasySetup (Variables|Default|GetFloating_AI_Movement))
  (Default|ChangeTarget (Variables|Default|GetFloating_AI_Movement) (Variables|Default|GetTarget) 0 true)
  (CallFunction|Attack))

(event EventTick
  (params (DeltaSeconds :type Float%20%28single-precision%29))
  (if (>= (.z (Transformation|GetActorLocation)) 1.99e+03)
    (Variables|Default|GetTarget
      (:then
        (Default|Move (Variables|Default|GetFloating_AI_Movement)))
      (:else))
    (else
      (CallFunction|Ascend DeltaSeconds))))

(fn ConstructionScript)

(fn UpdateStats
  (params (DamageType :type Damage%20Type%20Class%20Reference) (Damage :type Float%20%28double-precision%29) (AttackSpeed :type Float%20%28double-precision%29) (ExplosionRadius :type Float%20%28double-precision%29))
  (Variables|Default|SetDamageType DamageType)
  (Variables|Default|SetDamage Damage)
  (Variables|Default|SetAttackSpeed AttackSpeed)
  (Variables|Default|SetRadius ExplosionRadius))