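; BP_Explosion is a one-shot explosion actor in the tower projectiles and beams set that deals area damage when it spawns.
; On BeginPlay it applies radial damage with linear falloff from full to half damage between Radius and twice Radius, slightly above its location.
; The damage is credited to the actor's owner and can be blocked on a custom trace channel.
; The actor destroys itself when its Niagara effect finishes.
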(event OnSystemFinished(Niagara)
  (params (PSystem :type Niagara%20Component%20Object%20Reference))
  (Actor|DestroyActor))

(event EventBeginPlay
  (bind _damage (Variables|Default|GetDamage))
  (bind _radius (Variables|Default|GetRadius))
  (Class|GameplayStatics|ApplyRadialDamagewithFalloff _damage (/ _damage 2.0) (+ (Transformation|GetActorLocation) "0,0,10.000000") _radius (* _radius 2.0) 1.0 (Variables|Default|GetDamage%20Type%20Class) 0 (Components|GetOwner) 0 "ECC_GameTraceChannel2"))

(fn ConstructionScript)