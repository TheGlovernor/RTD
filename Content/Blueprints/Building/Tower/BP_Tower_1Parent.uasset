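; Parent tower actor for tower defense that attacks enemies in range and handles selection, selling and item slots.
; A looping-by-re-arm timer gathers overlapping enemies ordered by progress or health priority.
; Tick fires when the cooldown timer expires, aiming at the first target and damaging every multi-line-trace hit.
; GAS attributes via GSCCore drive stats, refreshing the selection widget and resizing the range sphere and four-point spline-mesh ring.
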(event OnPostGameplayEffectExecute(GSCCore)
  (params (Attribute :type Gameplay%20Attribute%20Structure) (SourceActor :type Actor%20Object%20Reference) (TargetActor :type Actor%20Object%20Reference) (SourceTags :type Gameplay%20Tag%20Container%20Structure%20%28by%20ref%29) (Payload :type GSC%20Gameplay%20Effect%20Execute%20Data%20Structure))
  (|SwitchGameplayAttribute Attribute
    (:Level
      (Class|GSCCoreComponent|ClampAttributeValue (Variables|Default|GetGSCCore) "(AttributeName=\"Level\",Attribute=/Script/RTD.TowerAttributeSet:Level,AttributeOwner=Class'\"/Script/RTD.TowerAttributeSet\"')" 0.0 1e+08))
    (:AttackPower
      (Class|GSCCoreComponent|ClampAttributeValue (Variables|Default|GetGSCCore) "(AttributeName=\"AttackPower\",Attribute=/Script/RTD.TowerAttributeSet:AttackPower,AttributeOwner=Class'\"/Script/RTD.TowerAttributeSet\"')" 0.0 1e+08))
    (:AttackSpeed
      (Class|GSCCoreComponent|ClampAttributeValue (Variables|Default|GetGSCCore) "(AttributeName=\"AttackSpeed\",Attribute=/Script/RTD.TowerAttributeSet:AttackSpeed,AttributeOwner=Class'\"/Script/RTD.TowerAttributeSet\"')" 0.0 1e+08))
    (:Range
      (Class|GSCCoreComponent|ClampAttributeValue (Variables|Default|GetGSCCore) "(AttributeName=\"Range\",Attribute=/Script/RTD.TowerAttributeSet:Range,AttributeOwner=Class'\"/Script/RTD.TowerAttributeSet\"')" 0.0 1e+08)
      (CallFunction|UpdateRange))
    (:CurrentTargets
      (Class|GSCCoreComponent|ClampAttributeValue (Variables|Default|GetGSCCore) "(AttributeName=\"CurrentTargets\",Attribute=/Script/RTD.TowerAttributeSet:CurrentTargets,AttributeOwner=Class'\"/Script/RTD.TowerAttributeSet\"')" 0.0 1e+08))
    (:MaxTargets
      (Class|GSCCoreComponent|ClampAttributeValue (Variables|Default|GetGSCCore) "(AttributeName=\"MaxTargets\",Attribute=/Script/RTD.TowerAttributeSet:MaxTargets,AttributeOwner=Class'\"/Script/RTD.TowerAttributeSet\"')" 0.0 1e+08))
    (:CritChance
      (Class|GSCCoreComponent|ClampAttributeValue (Variables|Default|GetGSCCore) "(AttributeName=\"CritChance\",Attribute=/Script/RTD.TowerAttributeSet:CritChance,AttributeOwner=Class'\"/Script/RTD.TowerAttributeSet\"')" 0.0 1e+08))
    (:MaxItems
      (Class|GSCCoreComponent|ClampAttributeValue (Variables|Default|GetGSCCore) "(AttributeName=\"MaxItems\",Attribute=/Script/RTD.TowerAttributeSet:MaxItems,AttributeOwner=Class'\"/Script/RTD.TowerAttributeSet\"')" 0.0 1e+08))
    (:BuyValue
      (Class|GSCCoreComponent|ClampAttributeValue (Variables|Default|GetGSCCore) "(AttributeName=\"BuyValue\",Attribute=/Script/RTD.TowerAttributeSet:BuyValue,AttributeOwner=Class'\"/Script/RTD.TowerAttributeSet\"')" 0.0 1e+08))
    (:UpgradeValue
      (Class|GSCCoreComponent|ClampAttributeValue (Variables|Default|GetGSCCore) "(AttributeName=\"UpgradeValue\",Attribute=/Script/RTD.TowerAttributeSet:UpgradeValue,AttributeOwner=Class'\"/Script/RTD.TowerAttributeSet\"')" 0.0 1e+08))
    (:SellValue
      (Class|GSCCoreComponent|ClampAttributeValue (Variables|Default|GetGSCCore) "(AttributeName=\"SellValue\",Attribute=/Script/RTD.TowerAttributeSet:SellValue,AttributeOwner=Class'\"/Script/RTD.TowerAttributeSet\"')" 0.0 1e+08)))
  (CallFunction|ReportStats))

(event OnComponentBeginOverlap(RangeSphere)
  (params (OverlappedComponent :type Primitive%20Component%20Object%20Reference) (OtherActor :type Actor%20Object%20Reference) (OtherComp :type Primitive%20Component%20Object%20Reference) (OtherBodyIndex :type Integer) (bFromSweep :type Boolean) (SweepResult :type Hit%20Result%20Structure%20%28by%20ref%29))
  (bind _asbp_enemy_base_01 (Utilities|Casting|CastToBP_Enemy_Base_01 OtherActor))
  (Variables|/Game/Blueprints/Mobs/BP_Enemy_Base_01.BP_Enemy_Base_01_C|SetMovementSpeed _asbp_enemy_base_01 (Variables|/Game/Blueprints/Mobs/BP_Enemy_Base_01.BP_Enemy_Base_01_C|GetTargetableSpeed _asbp_enemy_base_01)))

(event OnInitAbilityActorInfo(GSCCore)
  (CallFunction|ReportStats))

(event Custom|AttemptAttack
  (if (<= (Utilities|Time|GetTimerRemainingTimebyHandle (Variables|info|GetAttack%20Timer)) 0.0)
    (CallFunction|Attack)))

(event Custom|GetTargets
  (bind _targetableenemies (CallFunction|AcquireTargets))
  (Variables|Targeting|SetTargetables _targetableenemies)
  (if (Utilities|Array|IsNotEmpty _targetableenemies)
    (Utilities|Time|SetTimerbyEvent (delegate Custom|GetTargets) 0.5)
    (else
      (Utilities|Time|SetTimerbyEvent (delegate Custom|GetTargets) 0.1))))

(event EventBeginPlay
  (Utilities|Time|SetTimerbyEvent (delegate Custom|GetTargets) 0.5))

(event EventSelect
  (params (UI :type CUI%20Start%20Screen%20Object%20Reference))
  (CallFunction|ToggleSelect true)
  (Variables|/Game/UI/CUI_StartScreen.CUI_StartScreen_C|SetNoTowerSelected UI false)
  (Variables|/Game/UI/CUI_StartScreen.CUI_StartScreen_C|SetSelectedTower UI self))

(event EventRemoveItem
  (params (ToRemove :type BP%20Tower%20Item%20Data%20Obj%20Object%20Reference))
  (bind _foundwidgets (Class|WidgetBlueprintLibrary|GetAllWidgetswithInterface "/Game/UI/BPI_MainUI.BPI_MainUI_C" false))
  (Class|BPIMainUI|AddItem(Message) (Utilities|Array|Get(acopy) _foundwidgets) ToRemove)
  (Utilities|Array|RemoveItem (Variables|stats|GetItems) ToRemove))

(event EventTick
  (params (DeltaSeconds :type Float%20%28single-precision%29))
  (CallFunction|AttemptAttack))

(event EventDeselect
  (params (UI :type CUI%20Start%20Screen%20Object%20Reference))
  (CallFunction|ToggleSelect false)
  (Variables|/Game/UI/CUI_StartScreen.CUI_StartScreen_C|SetNoTowerSelected UI true))

(event EventAttack
  (bind _targetables (Variables|Targeting|GetTargetables))
  (bind _targetingmesh (Variables|Default|GetTargetingMesh))
  (bind _returnvalue (Transformation|GetWorldLocation _targetingmesh))
  (bind _output (Utilities|Array|Get(acopy) _targetables))
  (if (Utilities|Array|IsNotEmpty _targetables)
    (Utilities|IsValid _output
      (:Is%20Valid
        (bind _target (Class|EnemyInterface|ReportTargetPoint(Message) _output))
        (Transformation|SetRelativeRotation (Variables|Default|GetTargetingMesh) (Math|Rotator|FindLookatRotation (Transformation|GetWorldLocation (Variables|Default|GetTargetingMesh)) (Transformation|GetWorldLocation _target)) false false)
        (bind _outhits (Collision|MultiLineTraceByChannel _returnvalue (+ _returnvalue (* (Math|Vector|GetUnitDirection(Vector) _returnvalue (Transformation|GetWorldLocation _target)) (Class|GSCCoreComponent|GetCurrentAttributeValue (Variables|Default|GetGSCCore) "(AttributeName=\"Range\",Attribute=/Script/RTD.TowerAttributeSet:Range,AttributeOwner=Class'\"/Script/RTD.TowerAttributeSet\"')") (Variables|stats|GetTraceRangeXr))) "TraceTypeQuery6" false 0 "ForDuration" true "(R=1.000000,G=0.000000,B=0.000000,A=1.000000)" "(R=0.000000,G=1.000000,B=0.000000,A=1.000000)" 2.0))
        (for _array_element _outhits
          (Utilities|IsValid (.HitActor (Collision|BreakHitResult _array_element))
            (:Is%20Valid
              (Game|Damage|ApplyDamage (.HitActor (Collision|BreakHitResult _array_element)) (Class|GSCCoreComponent|GetCurrentAttributeValue (Variables|Default|GetGSCCore) "(AttributeName=\"AttackPower\",Attribute=/Script/RTD.TowerAttributeSet:AttackPower,AttributeOwner=Class'\"/Script/RTD.TowerAttributeSet\"')") (Game|GetPlayerController 0) self (Variables|info|GetDamageTypeClass)))))
        (bind _returnvalue_2 (Utilities|Time|SetTimerbyEvent (delegate EventAttack) (Class|GSCCoreComponent|GetCurrentAttributeValue (Variables|Default|GetGSCCore) "(AttributeName=\"AttackSpeed\",Attribute=/Script/RTD.TowerAttributeSet:AttackSpeed,AttributeOwner=Class'\"/Script/RTD.TowerAttributeSet\"')")))
        (Variables|info|SetAttack%20Timer _returnvalue_2)))))

(event EventSell
  (Class|BPIPlayer|ChangeMoney(Message) (Components|GetOwner) (Variables|Stats|GetSellValue))
  (Class|BPIPlayer|RemoveTower(Message) (Components|GetOwner) (Variables|Default|GetMyInstanceID))
  (Actor|DestroyActor))

(event EventLevelUp
  (Class|BPIPlayer|ChangeMoney(Message) (Components|GetOwner) (* (Variables|Stats|GetUpgradeCost) -1)))

(event EventSetTargetMode
  (params (Mode :type ETargetMode%20Enum :default "NewEnumerator0"))
  (Variables|Targeting|SetTargetingMode Mode))

(event EventSetTargetPriority
  (params (Priority :type ETargetPriority%20Enum :default "NewEnumerator0"))
  (Variables|Targeting|SetTargetingPriority Priority))

(fn ConstructionScript
  (bind _mydata (Variables|Info|GetMyData))
  (bind (_towername _icon _tower _basestats _addstats) (Utilities|Struct|BreakS_TowerDataStruct _mydata))
  (CallFunction|ReportStats)
  (CallFunction|UpdateRangeMesh)
  (Variables|Info|SetTowerName _towername)
  (Variables|info|SetIcon _icon)
  (Variables|Stats|SetBaseStats _basestats)
  (Variables|Stats|SetBaseStatsAdd _addstats))

(fn AcquireTargets
  (for _array_element (Collision|GetOverlappingActors (Variables|Default|GetRangeSphere) "/Game/Blueprints/Mobs/BP_Enemy_Base_01.BP_Enemy_Base_01_C" :!class /Script/Engine.PrimitiveComponent)
    (LocalVariables|SetTarget _array_element)
    (if (Utilities|DoesObjectImplementInterface _array_element "/Game/Blueprints/Mobs/EnemyInterface.EnemyInterface_C")
      (if (Utilities|Array|IsEmpty (LocalVariables|GetTargets))
        (Utilities|Array|AddUnique (LocalVariables|GetTargets) (LocalVariables|GetTarget))
        (else
          (bind (_array_element_2 _array_index) (Utilities|Array|ForEachLoopwithBreak (LocalVariables|GetTargets) :!label _label)
            (:LoopBody
              (LocalVariables|Setindex _array_index)
              (Utilities|FlowControl|Sequence
                (:then_0
                  (bind (_distancetobase _health) (Class|EnemyInterface|ReportStats(Message) (LocalVariables|GetTarget))))
                (:then_1
                  (bind (_distancetobase_2 _health_2) (Class|EnemyInterface|ReportStats(Message) _array_element_2))
                  (switch Utilities|FlowControl|Switch|SwitchonETargetMode (Variables|Targeting|GetTargetingMode)
                    (:NewEnumerator0
                      (switch Utilities|FlowControl|Switch|SwitchonETargetPriority (Variables|Targeting|GetTargetingPriority)
                        (:NewEnumerator0
                          (if (> _distancetobase _distancetobase_2)
                            (Utilities|Array|Insert (LocalVariables|GetTargets) (LocalVariables|GetTarget) (LocalVariables|Getindex))
                            (LocalVariables|SetInserted true :!label _label_2)
                            (goto _label Break)))
                        (:NewEnumerator1
                          (if (< _distancetobase _distancetobase_2)
                            (Utilities|Array|Insert (LocalVariables|GetTargets) (LocalVariables|GetTarget) (LocalVariables|Getindex))
                            (goto _label_2)))))
                    (:NewEnumerator1
                      (switch Utilities|FlowControl|Switch|SwitchonETargetPriority (Variables|Targeting|GetTargetingPriority)
                        (:NewEnumerator0
                          (if (< _health _health_2)
                            (Utilities|Array|Insert (LocalVariables|GetTargets) (LocalVariables|GetTarget) (LocalVariables|Getindex))
                            (goto _label_2)))
                        (:NewEnumerator1
                          (if (> _health _health_2)
                            (Utilities|Array|Insert (LocalVariables|GetTargets) (LocalVariables|GetTarget) (LocalVariables|Getindex))
                            (goto _label_2)))))))))
            (:Completed
              (if (LocalVariables|GetInserted)
                (LocalVariables|SetInserted false)
                (else
                  (Utilities|Array|Add (LocalVariables|GetTargets) (LocalVariables|GetTarget))))))))))
  (return (LocalVariables|GetTargets)))

(fn ToggleSelect
  (params (show :type Boolean))
  (bind _selectionwidget (Variables|Default|GetSelectionWidget))
  (for _array_element (Variables|Components|GetRangeMeshes)
    (Rendering|SetVisibility _array_element show true))
  (if show
    (Development|SetHiddeninGame _selectionwidget false true)
    (else
      (Development|SetHiddeninGame _selectionwidget true true))))

(fn UpdateRange
  (bind _rangesphere (Variables|Default|GetRangeSphere))
  (bind _splineheight (LocalVariables|GetSplineHeight))
  (bind _splineheight_2 (LocalVariables|GetSplineHeight))
  (bind _rangespline (Variables|Default|GetRangeSpline))
  (bind _output_get (LocalVariables|SetRange (Class|GSCCoreComponent|GetCurrentAttributeValue (Variables|Default|GetGSCCore) "(AttributeName=\"Range\",Attribute=/Script/RTD.TowerAttributeSet:Range,AttributeOwner=Class'\"/Script/RTD.TowerAttributeSet\"')")))
  (Components|Sphere|SetSphereRadius _rangesphere _output_get true)
  (Transformation|SetRelativeLocation _rangesphere (Math|Vector|MakeVector 0.0 0.0 (LocalVariables|GetSplineHeight)) false false)
  (Utilities|FlowControl|Sequence
    (:then_0
      (Spline|SetLocationatSplinePoint _rangespline 0 (Math|Vector|MakeVector (LocalVariables|GetRange) 0.0 _splineheight_2) "Local" false)
      (Spline|SetTangentatSplinePoint _rangespline 0 (Math|Vector|MakeVector 0.0 (* (LocalVariables|GetRange) (Variables|Components|GetTangentConst)) 0.0) "Local" false))
    (:then_1
      (Spline|SetLocationatSplinePoint _rangespline 1 (Math|Vector|MakeVector 0.0 (LocalVariables|GetRange) _splineheight_2) "Local" false)
      (Spline|SetTangentatSplinePoint _rangespline 1 (Math|Vector|MakeVector (* (LocalVariables|GetRange) (Variables|Components|GetTangentConst) -1.0) 0.0 0.0) "Local" false))
    (:then_2
      (Spline|SetLocationatSplinePoint _rangespline 2 (Math|Vector|MakeVector (* (LocalVariables|GetRange) -1.0) 0.0 _splineheight) "Local" false)
      (Spline|SetTangentatSplinePoint _rangespline 2 (Math|Vector|MakeVector 0.0 (* (LocalVariables|GetRange) (Variables|Components|GetTangentConst) -1.0) 0.0) "Local" false))
    (:then_3
      (Spline|SetLocationatSplinePoint _rangespline 3 (Math|Vector|MakeVector 0.0 (* (LocalVariables|GetRange) -1.0) _splineheight) "Local" false)
      (Spline|SetTangentatSplinePoint _rangespline 3 (Math|Vector|MakeVector (* (LocalVariables|GetRange) (Variables|Components|GetTangentConst)) 0.0 0.0) "Local" false))
    (:then_4
      (Spline|UpdateSpline (Variables|Default|GetRangeSpline))
      (for (_array_element _array_index) (Variables|Components|GetRangeMeshes)
        (Utilities|IsValid _array_element
          (:Is%20Valid
            _)
          (:Is%20Not%20Valid
            (bind _returnvalue (AddComponent|AddSplineMeshComponent false))
            (Utilities|Array|SetArrayElem (Variables|Components|GetRangeMeshes) _array_index _returnvalue)))
        (|SetStart/End_2 _array_element _array_index)))))

(fn UpdateRangeMesh
  (for (_array_element _array_index) (Variables|Components|GetRangeMeshes)
    (Utilities|IsValid _array_element
      (:Is%20Valid
        _)
      (:Is%20Not%20Valid
        (bind _returnvalue (AddComponent|AddSplineMeshComponent false))
        (Utilities|Array|SetArrayElem (Variables|Components|GetRangeMeshes) _array_index _returnvalue)))
    (|SetStart/End _array_element _array_index)))

(fn ReportStats
  (bind _gsccore (Variables|Default|GetGSCCore))
  (Class|BPISelectionWidget|ReportStats(Message) (UserInterface|GetWidget (Variables|Default|GetSelectionWidget)) self (Components|GetOwner) (Variables|Info|GetTowerName) (Variables|info|GetIcon) (Math|Float|Truncate (Class|GSCCoreComponent|GetCurrentAttributeValue _gsccore "(AttributeName=\"Level\",Attribute=/Script/RTD.TowerAttributeSet:Level,AttributeOwner=Class'\"/Script/RTD.TowerAttributeSet\"')")) (Class|GSCCoreComponent|GetCurrentAttributeValue _gsccore "(AttributeName=\"AttackPower\",Attribute=/Script/RTD.TowerAttributeSet:AttackPower,AttributeOwner=Class'\"/Script/RTD.TowerAttributeSet\"')") (Class|GSCCoreComponent|GetCurrentAttributeValue _gsccore "(AttributeName=\"AttackSpeed\",Attribute=/Script/RTD.TowerAttributeSet:AttackSpeed,AttributeOwner=Class'\"/Script/RTD.TowerAttributeSet\"')") (Class|GSCCoreComponent|GetCurrentAttributeValue _gsccore "(AttributeName=\"Range\",Attribute=/Script/RTD.TowerAttributeSet:Range,AttributeOwner=Class'\"/Script/RTD.TowerAttributeSet\"')") (Class|GSCCoreComponent|GetCurrentAttributeValue _gsccore "(AttributeName=\"CritChance\",Attribute=/Script/RTD.TowerAttributeSet:CritChance,AttributeOwner=Class'\"/Script/RTD.TowerAttributeSet\"')") (Math|Float|Truncate (Class|GSCCoreComponent|GetCurrentAttributeValue _gsccore "(AttributeName=\"CurrentTargets\",Attribute=/Script/RTD.TowerAttributeSet:CurrentTargets,AttributeOwner=Class'\"/Script/RTD.TowerAttributeSet\"')")) (Variables|Stats|GetUpgradeCost) (Variables|Stats|GetSellValue) (Variables|stats|GetItems) (Variables|Targeting|GetAvailableModes) (Variables|Targeting|GetTargetingMode) (Variables|Targeting|GetTargetingPriority)))

(fn InsertItem
  (params (Item :type Object%20Object%20Reference))
  (bind _asbp_tower_item_data_obj (Utilities|Casting|CastToBP_TowerItem_DataObj Item)
    (:then
      (if (< (Utilities|Array|Length (Variables|stats|GetItems)) (Class|GSCCoreComponent|GetCurrentAttributeValue (Variables|Default|GetGSCCore) "(AttributeName=\"MaxItems\",Attribute=/Script/RTD.TowerAttributeSet:MaxItems,AttributeOwner=Class'\"/Script/RTD.TowerAttributeSet\"')"))
        (Utilities|Array|Add (Variables|stats|GetItems) _asbp_tower_item_data_obj)
        (return true)
        (else
          _)))
    (:CastFailed
      _))
  (return false))