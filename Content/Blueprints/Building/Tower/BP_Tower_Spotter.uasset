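; Spotter tower that reveals hidden enemies and marks targets to take increased damage.
; Range sphere overlaps apply GE_Reveal on entry and remove it on exit.
; AttemptAttack is empty; Attack instead reapplies GE_Spot to every valid Targetable on a short self-repeating delay, passing an attribute-driven magnitude via SetByCaller.
; ReportStats fills the selection widget with attribute-based description text, costs, items and targeting settings.
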(event OnComponentBeginOverlap(RangeSphere)
  (params (OverlappedComponent :type Primitive%20Component%20Object%20Reference) (OtherActor :type Actor%20Object%20Reference) (OtherComp :type Primitive%20Component%20Object%20Reference) (OtherBodyIndex :type Integer) (bFromSweep :type Boolean) (SweepResult :type Hit%20Result%20Structure%20%28by%20ref%29))
  (bind _gscabilitysystem (Variables|Default|GetGSCAbilitySystem))
  (Class|GASInterface|ApplySpec(Message) OtherActor _gscabilitysystem (GameplayEffects|MakeOutgoingSpec :self _gscabilitysystem :GameplayEffectClass "/Game/Blueprints/Effects/GE_Reveal.GE_Reveal_C")))

(event OnComponentEndOverlap(RangeSphere)
  (params (OverlappedComponent :type Primitive%20Component%20Object%20Reference) (OtherActor :type Actor%20Object%20Reference) (OtherComp :type Primitive%20Component%20Object%20Reference) (OtherBodyIndex :type Integer))
  (Class|GASInterface|RemoveEffect(Message) OtherActor (Variables|Default|GetGSCAbilitySystem) "/Game/Blueprints/Effects/GE_Reveal.GE_Reveal_C"))

(event EventAttack
  (for _array_element (Variables|Default|GetTargetables)
    (bind _returnvalue (Ability|GameplayEffect|AssignTagSetbyCallerMagnitude (GameplayEffects|MakeOutgoingSpec :self (Variables|Default|GetGSCAbilitySystem) :GameplayEffectClass "/Game/Blueprints/Effects/GE_Spot.GE_Spot_C") "(TagName=\"EffectMagnitude\")" (Class|GSCCoreComponent|GetCurrentAttributeValue (Variables|Default|GetGSCCore) "(AttributeName=\"EffectPower\",Attribute=/Script/RTD.TowerAttributeSet:EffectPower,AttributeOwner=Class'\"/Script/RTD.TowerAttributeSet\"')")))
    (Utilities|IsValid _array_element
      (:Is%20Valid
        (Class|GASInterface|ApplySpec(Message) _array_element (Variables|Default|GetGSCAbilitySystem) _returnvalue))))
  (Utilities|FlowControl|Delay 0.1)
  (CallFunction|Attack))

(event EventAttemptAttack)

(fn ConstructionScript
  (|CallParentFunction))

(fn ReportStats
  (bind _gsccore (Variables|Default|GetGSCCore))
  (Class|BPISelectionWidget|ReportStats(Message) (UserInterface|GetWidget (Variables|Default|GetSelectionWidget)) self (Components|GetOwner) (Variables|Default|GetTowerName) (Variables|Default|GetIcon) (Utilities|Array|MakeArray (Utilities|Text|ToText(String) (Utilities|String|Replace (Utilities|String|Replace (Utilities|String|ToString(Text) (Utilities|Text|MakeLiteralText "Reveals hidden enemies. <img id=\"Spotted\"/>Spots up to <RichText.Emphasis>TARGETS</> enemie(s), increasing their damage taken by <RichText.Emphasis>AMOUNT</>%.")) "TARGETS" (Utilities|String|ToString(Integer) (Math|Float|Round (Class|GSCCoreComponent|GetCurrentAttributeValue _gsccore "(AttributeName=\"CurrentTargets\",Attribute=/Script/RTD.TowerAttributeSet:CurrentTargets,AttributeOwner=Class'\"/Script/RTD.TowerAttributeSet\"')"))) "CaseSensitive") "AMOUNT" (Utilities|String|ToString(Float) (Math|Float|SnapToGrid(Float) (* (Class|GSCCoreComponent|GetCurrentAttributeValue _gsccore "(AttributeName=\"SpotPower\",Attribute=/Script/RTD.TowerAttributeSet:SpotPower,AttributeOwner=Class'\"/Script/RTD.TowerAttributeSet\"')") 1e+02) 0.1)) "CaseSensitive"))) (Variables|Default|GetUpgradeCost) (Variables|Default|GetSellValue) (Variables|Default|GetItems) (Variables|Default|GetAvailableModes) (Variables|Default|GetTargetingMode) (Variables|Default|GetTargetingPriority)))