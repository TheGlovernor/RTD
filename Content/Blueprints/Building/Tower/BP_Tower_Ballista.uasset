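; Ballista tower Blueprint that repeatedly fires basic projectiles at the first entry in its target list.
; Attack plays the firing animation and sound, spawns the projectile with attribute-driven power and a random bonus roll, then re-calls itself after an attribute-based delay, polling briefly when unable to fire.
; LevelUp extends the parent with a ballista-specific Gameplay Effect.
; An ammo and venting timer chain is left disconnected and never runs.
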(event EventAttack
  (bind _targetables (Variables|Default|GetTargetables))
  (bind _gsccore (Variables|Default|GetGSCCore))
  (bind _returnvalue (Class|GSCCoreComponent|GetCurrentAttributeValue _gsccore "(AttributeName=\"AttackPower\",Attribute=/Script/RTD.TowerAttributeSet:AttackPower,AttributeOwner=\"/Script/CoreUObject.Class'/Script/RTD.TowerAttributeSet'\")"))
  (bind _output (Utilities|Array|Get(acopy) _targetables))
  (bind _returnvalue_2 (CallFunction|CanAttack))
  (if _returnvalue_2
    (Utilities|IsValid _output
      (:Is%20Valid
        (bind _location (Class|EnemyInterface|ReportTargetPoint(Message) _output))
        (Components|Animation|PlayAnimation (Variables|Default|GetBallista) "/Game/Assets/Buildings/Towers/TowerModels/Ballista/Ballista_Anim.Ballista_Anim" false)
        (Game|SpawnActorfromClass "/Game/Blueprints/Building/Tower/Projs_Beams/BP_Projectile_Basic.BP_Projectile_Basic_C" (Math|Transform|MakeTransform (Transformation|GetWorldLocation (Variables|Default|GetBallista))) "AlwaysSpawn" "OverrideRootScale" self _output _location (Variables|Default|GetDamageTypeClass) (select (> (Class|GSCCoreComponent|GetCurrentAttributeValue _gsccore "(AttributeName=\"CritChance\",Attribute=/Script/RTD.TowerAttributeSet:CritChance,AttributeOwner=\"/Script/CoreUObject.Class'/Script/RTD.TowerAttributeSet'\")") (Math|Random|RandomFloat)) (* _returnvalue (Class|GSCCoreComponent|GetCurrentAttributeValue _gsccore "(AttributeName=\"CritX\",Attribute=/Script/RTD.TowerAttributeSet:CritX,AttributeOwner=\"/Script/CoreUObject.Class'/Script/RTD.TowerAttributeSet'\")")) _returnvalue) 0)
        (CallFunction|PlayShootingSound)
        (Utilities|FlowControl|Delay (/ 1.0 (Class|GSCCoreComponent|GetCurrentAttributeValue (Variables|Default|GetGSCCore) "(AttributeName=\"AttackSpeed\",Attribute=/Script/RTD.TowerAttributeSet:AttackSpeed,AttributeOwner=\"/Script/CoreUObject.Class'/Script/RTD.TowerAttributeSet'\")")))
        (CallFunction|Attack))
      (:Is%20Not%20Valid
        (Utilities|FlowControl|Delay 0.1 :!label _label)
        (CallFunction|Attack)))
    (else
      (goto _label))))

(event EventLevelUp
  (|CallParentFunction)
  (GameplayEffects|ApplyGameplayEffectToSelf :self (Variables|Default|GetGSCAbilitySystem) :GameplayEffectClass "/Game/Blueprints/Building/Tower/Stats/GE_Ballista_LevelUp.GE_Ballista_LevelUp_C" :Level 1.0))

(fn ConstructionScript
  (|CallParentFunction))