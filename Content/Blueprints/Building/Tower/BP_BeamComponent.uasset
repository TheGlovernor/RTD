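; Tower component that maintains a pool of beam actors and drives their targets and stats.
; CheckBeamCount spawns BP_Beam_Basic actors at the owning BP_Tower_1Parent's targeting mesh, or destroys surplus ones, until the pool matches BeamCount.
; UpdateBeamTargets pairs targets with beams by index, leaving extra beams unchanged.
; UpdateBeamStats pushes damage, range, damage type and a clamped tick rate to every beam.
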(event Custom|CheckBeamCount
  (bind _beamcount (Variables|Default|GetBeamCount))
  (bind _beams (Variables|Default|GetBeams))
  (bind _beams_2 (Variables|Default|GetBeams))
  (bind _returnvalue (Utilities|Array|Length _beams))
  (bind _returnvalue_2 (Utilities|Array|Length _beams_2))
  (bind _returnvalue_3 (< _returnvalue_2 _beamcount))
  (bind _returnvalue_4 (- _returnvalue 1))
  (bind _output (Utilities|Array|Get(acopy) _beams _returnvalue_4))
  (if (!= (Variables|Default|GetBeamCount) (Utilities|Array|Length (Variables|Default|GetBeams)))
    (if _returnvalue_3
      (while _returnvalue_3
        (bind _asbp_tower_1parent (Utilities|Casting|CastToBP_Tower_1Parent (Components|GetOwner)))
        (bind _returnvalue_5 (Game|SpawnActorfromClass "/Game/Blueprints/Building/Tower/Projs_Beams/BP_Beam_Basic.BP_Beam_Basic_C" (Math|Transform|MakeTransform (Transformation|GetWorldLocation (Variables|/Game/Blueprints/Building/Tower/BP_Tower_1Parent.BP_Tower_1Parent_C|GetTargetingMesh _asbp_tower_1parent))) "AlwaysSpawn" 0 0 0.0 0.0 0 0))
        (Utilities|Array|Add (Variables|Default|GetBeams) _returnvalue_5))
      (else
        (while (> (Utilities|Array|Length (Variables|Default|GetBeams)) (Variables|Default|GetBeamCount))
          (Actor|DestroyActor _output)
          (Utilities|Array|RemoveItem _beams _output))))))

(event Custom|UpdateBeamTargets
  (params (Targets :type Array%20of%20Actor%20Object%20References))
  (if (Utilities|Array|IsNotEmpty Targets)
    (for _index (range 0 (- (Math|Integer|Min(Integer) (Utilities|Array|Length Targets) (Utilities|Array|Length (Variables|Default|GetBeams))) 1))
      (Variables|/Game/Blueprints/Building/Tower/Projs_Beams/BP_Beam_Basic.BP_Beam_Basic_C|SetTarget (Utilities|Array|Get(acopy) (Variables|Default|GetBeams) _index) (Utilities|Array|Get(acopy) Targets _index)))))

(event Custom|UpdateBeamStats
  (params (Damage :type Float%20%28double-precision%29) (Range :type Float%20%28double-precision%29) (DamageTickRate :type Float%20%28double-precision%29) (DamageType :type Array%20of%20Damage%20Type%20Class%20References))
  (for _array_element (Variables|Default|GetBeams)
    (Default|UpdateStats _array_element Damage Range (Math|Float|Clamp(Float) DamageTickRate 0.01) DamageType)))