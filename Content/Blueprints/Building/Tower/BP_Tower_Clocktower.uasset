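; Clocktower tower that alters the passage of time for enemies and friendly towers within its bounds, without targeting.
; Overlapping actors receive GE_Time scaled by a GSC attribute, with basic buildings also needing their location within range.
; The effect is removed when overlap ends or the tower ends play.
; Level-ups apply GE_ClockTower_LU to itself, and ReportStats sends its current values to the selection widget.
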(event Collision|EventActorBeginOverlap
  (params (OtherActor :type Actor%20Object%20Reference))
  (bind _returnvalue (Transformation|GetActorLocation OtherActor))
  (bind _returnvalue_2 (Transformation|GetActorLocation))
  (if (not (Utilities|ClassIsChildOf (Utilities|GetClass OtherActor) "/Game/Blueprints/Building/BP_Building_Basic.BP_Building_Basic_C"))
    (Class|GASInterface|ApplyEffect(Message) OtherActor (Variables|Default|GetGSCAbilitySystem) "/Game/Blueprints/Effects/GE_Time.GE_Time_C" (Class|GSCCoreComponent|GetCurrentAttributeValue (Variables|Default|GetGSCCore) "(AttributeName=\"EffectPower\",Attribute=/Script/RTD.TowerAttributeSet:EffectPower,AttributeOwner=Class'\"/Script/RTD.TowerAttributeSet\"')") :!label _label)
    (elif (<= (Math|Vector|Distance(Vector) (Math|Vector|MakeVector (.x _returnvalue) (.y _returnvalue) 0.0) (Math|Vector|MakeVector (.x _returnvalue_2) (.y _returnvalue_2) 0.0)) (Class|GSCCoreComponent|GetCurrentAttributeValue (Variables|Default|GetGSCCore) "(AttributeName=\"Range\",Attribute=/Script/RTD.TowerAttributeSet:Range,AttributeOwner=Class'\"/Script/RTD.TowerAttributeSet\"')"))
      (goto _label))))

(event Collision|EventActorEndOverlap
  (params (OtherActor :type Actor%20Object%20Reference))
  (Class|GASInterface|RemoveEffect(Message) OtherActor (Variables|Default|GetGSCAbilitySystem) "/Game/Blueprints/Effects/GE_Time.GE_Time_C"))

(event EventLevelUp
  (|CallParentFunction)
  (GameplayEffects|ApplyGameplayEffectToSelf :self (Variables|Default|GetGSCAbilitySystem) :GameplayEffectClass "/Game/Blueprints/Building/Tower/Stats/GE_ClockTower_LU.GE_ClockTower_LU_C"))

(event EventEndPlay
  (params (EndPlayReason :type EEndPlayReason%20Enum :default "Destroyed"))
  (for _array_element (Collision|GetOverlappingActors 0 :!class /Script/Engine.Actor)
    (Class|GASInterface|RemoveEffect(Message) _array_element (Variables|Default|GetGSCAbilitySystem) "/Game/Blueprints/Effects/GE_Time.GE_Time_C")))

(fn ConstructionScript
  (|CallParentFunction))

(fn AcquireTargets
  (return 0))

(fn ReportStats
  (bind _gsccore (Variables|Default|GetGSCCore))
  (Class|BPISelectionWidget|ReportStats(Message) (UserInterface|GetWidget (Variables|Default|GetSelectionWidget)) self (Components|GetOwner) (Variables|Default|GetTowerName) (Variables|Default|GetIcon) (Utilities|Array|MakeArray (Utilities|Text|ToText(String) (Utilities|String|Replace (Utilities|String|ToString(Text) (Utilities|Text|MakeLiteralText "Changes the passage of time in it's bounds by <RichText.Emphasis>PWR%</>. Affects both enemies and friendly towers. This effect does not stack.")) "PWR" (Utilities|String|ToString(Integer) (Math|Float|Round (* (Class|GSCCoreComponent|GetCurrentAttributeValue _gsccore "(AttributeName=\"EffectPower\",Attribute=/Script/RTD.TowerAttributeSet:EffectPower,AttributeOwner=Class'\"/Script/RTD.TowerAttributeSet\"')") 1e+02))) "CaseSensitive"))) (Math|Float|Round (Class|GSCCoreComponent|GetCurrentAttributeValue _gsccore "(AttributeName=\"Level\",Attribute=/Script/RTD.TowerAttributeSet:Level,AttributeOwner=Class'\"/Script/RTD.TowerAttributeSet\"')")) -1.0 -1.0 (Class|GSCCoreComponent|GetCurrentAttributeValue _gsccore "(AttributeName=\"Range\",Attribute=/Script/RTD.TowerAttributeSet:Range,AttributeOwner=Class'\"/Script/RTD.TowerAttributeSet\"')") -1.0 0 (Variables|Default|GetUpgradeCost) (Variables|Default|GetSellValue) (Variables|Default|GetItems) (Variables|Default|GetAvailableModes) (Variables|Default|GetTargetingMode) (Variables|Default|GetTargetingPriority)))