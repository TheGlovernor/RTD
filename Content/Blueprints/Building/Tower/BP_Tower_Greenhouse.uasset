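; Greenhouse tower that attacks by spawning BP_Roots actors aimed at its first targetable.
; Attack is a self-calling loop: when CanAttack passes, it spawns the roots high above the tower with the tower and target passed in.
; It then waits for the inverse of a GSCCore attribute value before repeating, or rechecks after a short delay when it cannot attack.
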(event EventAttack
  (bind _self self)
  (bind _returnvalue (CallFunction|CanAttack))
  (if _returnvalue
    (Game|SpawnActorfromClass "/Game/Blueprints/Building/Tower/Projs_Beams/BP_Roots.BP_Roots_C" (Math|Transform|MakeTransform (+ (Transformation|GetActorLocation) "0,0,500.000000")) "Undefined" "OverrideRootScale" _self _self (Utilities|Array|Get(acopy) (Variables|Default|GetTargetables)) 0)
    (Utilities|FlowControl|Delay (/ 1.0 (Class|GSCCoreComponent|GetCurrentAttributeValue (Variables|Default|GetGSCCore) "(AttributeName=\"AttackSpeed\",Attribute=/Script/RTD.TowerAttributeSet:AttackSpeed,AttributeOwner=\"/Script/CoreUObject.Class'/Script/RTD.TowerAttributeSet'\")")))
    (CallFunction|Attack)
    (else
      (Utilities|FlowControl|Delay 0.1)
      (CallFunction|Attack))))

(fn ConstructionScript
  (|CallParentFunction))