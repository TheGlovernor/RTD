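; Artillery tower, a child tower that lobs BP_ArtilleryShell projectiles in ballistic arcs at its first target.
; Each tick pitches the barrel toward a launch angle computed from 2D distance, gravity and velocity; attacks wait until it is aimed.
; Range updates raise launch velocity as needed for a 45-degree shot to reach.
; A self-rescheduling attack timer spawns shells with randomly reduced velocity, attribute-driven damage, crits and radius, plus forced status effects.
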(event Custom|AimBarrel
  (params (DeltaSeconds :type Float%20%28double-precision%29))
  (if (Utilities|Array|IsNotEmpty (Variables|Default|GetTargetables))
    (if (> (Math|Float|Absolute(Float) (- (.pitch (Variables|/Script/Engine.SceneComponent|GetRelativeRotation (Variables|Default|GetArt_Cylinder_032))) (CallFunction|GetLaunchAngle))) 0.5)
      (Transformation|AddRelativeRotation (Variables|Default|GetArt_Cylinder_032) (Math|Rotator|MakeRotator 0.0 (Math|Float|SelectFloat (* DeltaSeconds 3e+01) (* DeltaSeconds 3e+01 -1.0) (< (.pitch (Variables|/Script/Engine.SceneComponent|GetRelativeRotation (Variables|Default|GetArt_Cylinder_032))) (CallFunction|GetLaunchAngle))) 0.0) false false)
      (Variables|Default|SetbLaunchAngleAimed false)
      (else
        (Transformation|SetRelativeRotation (Variables|Default|GetArt_Cylinder_032) (Math|Rotator|MakeRotator 0.0 (CallFunction|GetLaunchAngle) 0.0) false false)
        (Variables|Default|SetbLaunchAngleAimed true)))))

(event EventAttack
  (bind _gsccore (Variables|Default|GetGSCCore))
  (bind _art_cylinder_031 (Variables|Default|GetArt_Cylinder_031))
  (bind _returnvalue (Class|GSCCoreComponent|GetCurrentAttributeValue _gsccore "(AttributeName=\"AttackPower\",Attribute=/Script/RTD.TowerAttributeSet:AttackPower,AttributeOwner=\"/Script/CoreUObject.Class'/Script/RTD.TowerAttributeSet'\")"))
  (bind _returnvalue_2 (Transformation|GetSocketTransform _art_cylinder_031 "Barrel" "RTS_World"))
  (bind _returnvalue_3 (CallFunction|CanAttack))
  (if _returnvalue_3
    (if (Utilities|Array|IsNotEmpty (Variables|Default|GetTargetables))
      (bind (_bforcefrost _bforceentangle _bforcebleed _bforceengulf _bforcestun) (CallFunction|GetForceStatusEffects))
      (Game|SpawnActorfromClass "/Game/Blueprints/Building/Tower/Projs_Beams/BP_ArtilleryShell.BP_ArtilleryShell_C" (Math|Transform|MakeTransform (.location _returnvalue_2) (.rotation _returnvalue_2) "1.000000,1.000000,1.000000") "AlwaysSpawn" "MultiplyWithRoot" self (- (Variables|Default|GetInitialVelocity) (Math|Random|RandomFloatinRange 0.0 2.5e+02)) (select (> (Class|GSCCoreComponent|GetCurrentAttributeValue _gsccore "(AttributeName=\"CritChance\",Attribute=/Script/RTD.TowerAttributeSet:CritChance,AttributeOwner=\"/Script/CoreUObject.Class'/Script/RTD.TowerAttributeSet'\")") (Math|Random|RandomFloat)) (* _returnvalue (Class|GSCCoreComponent|GetCurrentAttributeValue _gsccore "(AttributeName=\"CritX\",Attribute=/Script/RTD.TowerAttributeSet:CritX,AttributeOwner=\"/Script/CoreUObject.Class'/Script/RTD.TowerAttributeSet'\")")) _returnvalue) (Class|GSCCoreComponent|GetCurrentAttributeValue _gsccore "(AttributeName=\"ExplosionRadius\",Attribute=/Script/RTD.TowerAttributeSet:ExplosionRadius,AttributeOwner=\"/Script/CoreUObject.Class'/Script/RTD.TowerAttributeSet'\")") (Variables|Default|GetDamageTypeClass) _bforcefrost _bforceentangle _bforcebleed _bforceengulf _bforcestun 0)
      (CallFunction|PlayShootingSound)
      (Utilities|Time|SetTimerbyEvent (delegate EventAttack) (/ 1.0 (Class|GSCCoreComponent|GetCurrentAttributeValue (Variables|Default|GetGSCCore) "(AttributeName=\"AttackSpeed\",Attribute=/Script/RTD.TowerAttributeSet:AttackSpeed,AttributeOwner=\"/Script/CoreUObject.Class'/Script/RTD.TowerAttributeSet'\")")))
      (else
        (Utilities|Time|SetTimerbyEvent (delegate EventAttack) 0.1 :!label _label)))
    (else
      (goto _label))))

(event EventTick
  (params (DeltaSeconds :type Float%20%28single-precision%29))
  (|CallParentFunction DeltaSeconds)
  (CallFunction|AimBarrel DeltaSeconds))

(fn ConstructionScript
  (|CallParentFunction)
  (CallFunction|CalculateTowerStats)
  (CallFunction|ToggleSelect false))

(fn UpdateRange
  (|CallParentFunction)
  (Variables|Default|SetInitialVelocity (Math|Float|Max(Float) (Variables|Default|GetInitialVelocity) (.Velocity (Utilities|GetInitialVelocitySimple :EndLocation (Math|Vector|MakeVector (Class|GSCCoreComponent|GetCurrentAttributeValue (Variables|Default|GetGSCCore) "(AttributeName=\"Range\",Attribute=/Script/RTD.TowerAttributeSet:Range,AttributeOwner=\"/Script/CoreUObject.Class'/Script/RTD.TowerAttributeSet'\")") 0.0 0.0) :Angle%28Degrees%29 45.0 :ProjectileGravity (Variables|Default|GetProjectileGravity))))))

(fn GetLaunchAngle
  (bind _returnvalue (Transformation|GetActorLocation))
  (bind _targetables (Variables|Default|GetTargetables))
  (bind _output (Utilities|Array|Get(acopy) _targetables))
  (bind _returnvalue_2 (Transformation|GetActorLocation _output))
  (return (- 9e+01 (Utilities|GetLaunchAngle (Variables|Default|GetProjectileGravity) (Math|Vector|Distance2D(Vector) (Math|Vector2D|MakeVector2D (.x _returnvalue_2) (.y _returnvalue_2)) (Math|Vector2D|MakeVector2D (.x _returnvalue) (.y _returnvalue))) (Variables|Default|GetInitialVelocity)))))

(fn CanAttack
  (bind _returnvalue (|CallParentFunction))
  (return (and _returnvalue (Variables|Default|GetbLaunchAngleAimed))))