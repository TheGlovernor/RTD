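; Basic homing projectile fired by a tower, damaging only its assigned target on overlap and then destroying itself.
; Each tick it offsets toward the target by a fixed step, without sweep or delta-time scaling, and rotates to face it.
; If the target becomes invalid, it adopts the current target of its owning BP_Tower_Basic, or destroys itself when that tower has none.
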(event EventBeginPlay
  (Actor|Tick|SetActorTickEnabled true))

(event Collision|EventActorBeginOverlap
  (params (OtherActor :type Actor%20Object%20Reference))
  (if (== OtherActor (Variables|Default|GetTarget))
    (Game|Damage|ApplyDamage OtherActor (Variables|Default|GetDamage) 0 self)
    (Actor|Tick|SetActorTickEnabled false)
    (Actor|DestroyActor)))

(event EventTick
  (params (DeltaSeconds :type Float%20%28single-precision%29))
  (Utilities|IsValid (Variables|Default|GetTarget)
    (:Is%20Valid
      (Transformation|AddActorWorldOffset (* (Variables|Default|GetMovementSpeed) (Math|Vector|GetUnitDirection(Vector) (Transformation|GetWorldLocation (Variables|Default|GetDefaultSceneRoot)) (Transformation|GetWorldLocation (Variables|/Game/Blueprints/Mobs/BP_Enemy_Base_01.BP_Enemy_Base_01_C|GetDefaultSceneRoot (Variables|Default|GetTarget))))) :!label _label)
      (if (Class|Actor|IsActorTickEnabled)
        (Transformation|SetActorRotation (Math|Conversions|RotationFromXVector (Math|Vector|GetUnitDirection(Vector) (Transformation|GetWorldLocation (Variables|Default|GetDefaultSceneRoot)) (Transformation|GetWorldLocation (Variables|/Game/Blueprints/Mobs/BP_Enemy_Base_01.BP_Enemy_Base_01_C|GetDefaultSceneRoot (Variables|Default|GetTarget))))))))
    (:Is%20Not%20Valid
      (bind _asbase_tower (Utilities|Casting|CastToBP_Tower_Basic (Components|GetOwner)))
      (Utilities|IsValid (Variables|/Game/Blueprints/Building/Tower/BaseTower/BP_Tower_Basic.BP_Tower_Basic_C|GetTarget _asbase_tower)
        (:Is%20Valid
          (Variables|Default|SetTarget (Variables|/Game/Blueprints/Building/Tower/BaseTower/BP_Tower_Basic.BP_Tower_Basic_C|GetTarget _asbase_tower))
          (goto _label))
        (:Is%20Not%20Valid
          (Actor|Tick|SetActorTickEnabled false)
          (Actor|DestroyActor))))))

(fn ConstructionScript)