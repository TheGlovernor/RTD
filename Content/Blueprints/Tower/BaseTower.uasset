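; Tower defense base tower that fires Projectile_Base at one enemy within range, using its tick interval as the attack rate.
; A sphere overlap maintains the candidate list, and targets are picked by DistanceToBase under the Progress targeting mode.
; Range scales with MyBaseData.Level, sizing the sphere and a four-point spline circle drawn with spline meshes, hidden on construction.
; AttemptLevelUp increments a separate Level variable, which the range formula does not read.
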(event OnComponentEndOverlap(Sphere)
  (params (OverlappedComponent :type Primitive%20Component%20Object%20Reference) (OtherActor :type Actor%20Object%20Reference) (OtherComp :type Primitive%20Component%20Object%20Reference) (OtherBodyIndex :type Integer))
  (if (== (Utilities|GetClass OtherActor) "/Game/Blueprints/Mobs/TD_enemy_base.TD_enemy_base_C")
    (bind _astd_enemy_base (Utilities|Casting|CastToTD_enemy_base OtherActor))
    (Utilities|Array|RemoveItem (Variables|Targeting|GetTargetableEnemies) _astd_enemy_base)
    (if (== _astd_enemy_base (Variables|Targeting|GetTarget))
      (Variables|Targeting|SetTarget 0)
      (CallFunction|GetNewTarget))))

(event OnComponentBeginOverlap(Sphere)
  (params (OverlappedComponent :type Primitive%20Component%20Object%20Reference) (OtherActor :type Actor%20Object%20Reference) (OtherComp :type Primitive%20Component%20Object%20Reference) (OtherBodyIndex :type Integer) (bFromSweep :type Boolean) (SweepResult :type Hit%20Result%20Structure%20%28by%20ref%29))
  (if (== (Utilities|GetClass OtherActor) "/Game/Blueprints/Mobs/TD_enemy_base.TD_enemy_base_C")
    (bind _astd_enemy_base (Utilities|Casting|CastToTD_enemy_base OtherActor))
    (Utilities|Array|Add (Variables|Targeting|GetTargetableEnemies) _astd_enemy_base)
    (CallFunction|UpdateTarget _astd_enemy_base)))

(event EventBeginPlay
  (Actor|Tick|SetActorTickInterval (Variables|Stats|GetAttackRate)))

(event EventTick
  (params (DeltaSeconds :type Float%20%28single-precision%29))
  (bind _target (Variables|Targeting|GetTarget)
    (:then
      (Game|SpawnActorfromClass "/Game/Blueprints/Tower/Projectiles/Projectile_Base.Projectile_Base_C" (Math|Transform|MakeTransform (Transformation|GetWorldLocation (Variables|Default|GetCannon)) "0, 0, 0" "5.000000,5.000000,5.000000") "Undefined" 0 _target (Variables|Stats|GetAttackPower) 0))
    (:else
      (CallFunction|GetNewTarget))))

(fn ConstructionScript
  (Variables|Components|SetTangentConst (Variables|/Game/Blueprints/Tower/BaseTowerData.BaseTowerData_C|GetTangentConst (Variables|Default|GetMyBaseData)))
  (CallFunction|SetLevel)
  (CallFunction|UpdateAllStats)
  (CallFunction|ToggleRangeIndicator false))

(fn UpdateAllStats
  (CallFunction|UpdateRange))

(fn UpdateRange
  (bind _mybasedata (Variables|Default|GetMyBaseData))
  (bind _sphere (Variables|Default|GetSphere))
  (bind _splineheight (LocalVariables|GetSplineHeight))
  (bind _splineheight_2 (LocalVariables|GetSplineHeight))
  (bind _rangespline (Variables|Default|GetRangeSpline))
  (bind _output_get (Variables|Stats|SetRange (* (+ (* (Variables|/Game/Blueprints/Tower/BaseTowerData.BaseTowerData_C|GetLevel _mybasedata) 0.1) 1) (Variables|/Game/Blueprints/Tower/BaseTowerData.BaseTowerData_C|GetRange _mybasedata))))
  (Components|Sphere|SetSphereRadius _sphere _output_get true)
  (Transformation|SetRelativeLocation _sphere (Math|Vector|MakeVector 0.0 0.0 (LocalVariables|GetSplineHeight)) false false)
  (Utilities|FlowControl|Sequence
    (:then_0
      (Spline|SetLocationatSplinePoint _rangespline 0 (Math|Vector|MakeVector (Variables|Stats|GetRange) 0.0 _splineheight_2) "Local" false)
      (Spline|SetTangentatSplinePoint _rangespline 0 (Math|Vector|MakeVector 0.0 (* (Variables|Stats|GetRange) (Variables|Components|GetTangentConst)) 0.0) "Local" false))
    (:then_1
      (Spline|SetLocationatSplinePoint _rangespline 1 (Math|Vector|MakeVector 0.0 (Variables|Stats|GetRange) _splineheight_2) "Local" false)
      (Spline|SetTangentatSplinePoint _rangespline 1 (Math|Vector|MakeVector (* (Variables|Stats|GetRange) (Variables|Components|GetTangentConst) -1.0) 0.0 0.0) "Local" false))
    (:then_2
      (Spline|SetLocationatSplinePoint _rangespline 2 (Math|Vector|MakeVector (* (Variables|Stats|GetRange) -1.0) 0.0 _splineheight) "Local" false)
      (Spline|SetTangentatSplinePoint _rangespline 2 (Math|Vector|MakeVector 0.0 (* (Variables|Stats|GetRange) (Variables|Components|GetTangentConst) -1.0) 0.0) "Local" false))
    (:then_3
      (Spline|SetLocationatSplinePoint _rangespline 3 (Math|Vector|MakeVector 0.0 (* (Variables|Stats|GetRange) -1.0) _splineheight) "Local" false)
      (Spline|SetTangentatSplinePoint _rangespline 3 (Math|Vector|MakeVector (* (Variables|Stats|GetRange) (Variables|Components|GetTangentConst)) 0.0 0.0) "Local" false))
    (:then_4
      (Spline|UpdateSpline (Variables|Default|GetRangeSpline))
      (CallFunction|UpdateSplineMesh))))

(fn UpdateSplineMesh
  (for (_array_element _array_index) (Variables|Components|GetRangeMeshes)
    (Utilities|IsValid _array_element
      (:Is%20Valid
        _)
      (:Is%20Not%20Valid
        (bind _returnvalue (AddComponent|AddSplineMeshComponent false))
        (Utilities|Array|SetArrayElem (Variables|Components|GetRangeMeshes) _array_index _returnvalue)))
    (|SetStart/End _array_element _array_index)))

(fn GetNewTarget
  (switch Utilities|FlowControl|Switch|SwitchonETargetMode (Variables|Targeting|GetTargetingMode)
    (:NewEnumerator0
      (switch Utilities|FlowControl|Switch|SwitchonETargetPriority (Variables|Targeting|GetTargetingPriority)
        (:NewEnumerator0
          (for _array_element (Variables|Targeting|GetTargetableEnemies)
            (LocalVariables|GetTempTarget
              (:then
                (if (> (Variables|/Game/Blueprints/Mobs/TD_enemy_base.TD_enemy_base_C|GetDistanceToBase _array_element) (Variables|/Game/Blueprints/Mobs/TD_enemy_base.TD_enemy_base_C|GetDistanceToBase (stale _output_get)))
                  (LocalVariables|SetTempTarget _array_element)))
              (:else
                (bind _output_get (LocalVariables|SetTempTarget _array_element)))))
          (Variables|Targeting|SetTarget (LocalVariables|GetTempTarget)))
        (:NewEnumerator1
          (for _array_element_2 (Variables|Targeting|GetTargetableEnemies)
            (LocalVariables|GetTempTarget
              (:then
                (if (< (Variables|/Game/Blueprints/Mobs/TD_enemy_base.TD_enemy_base_C|GetDistanceToBase _array_element_2) (Variables|/Game/Blueprints/Mobs/TD_enemy_base.TD_enemy_base_C|GetDistanceToBase (stale _output_get_2)))
                  (LocalVariables|SetTempTarget _array_element_2)))
              (:else
                (bind _output_get_2 (LocalVariables|SetTempTarget _array_element_2)))))
          (Variables|Targeting|SetTarget (LocalVariables|GetTempTarget)))))))

(fn UpdateTarget
  (params (IncomingEnemy :type TD%20Enemy%20Base%20Object%20Reference))
  (Variables|Targeting|GetTarget
    (:then
      (LocalVariables|SetNewEnemy IncomingEnemy)
      (switch Utilities|FlowControl|Switch|SwitchonETargetMode (Variables|Targeting|GetTargetingMode)
        (:NewEnumerator0
          (switch Utilities|FlowControl|Switch|SwitchonETargetPriority (Variables|Targeting|GetTargetingPriority)
            (:NewEnumerator0
              (if (> (Variables|/Game/Blueprints/Mobs/TD_enemy_base.TD_enemy_base_C|GetDistanceToBase (LocalVariables|GetNewEnemy)) (Variables|/Game/Blueprints/Mobs/TD_enemy_base.TD_enemy_base_C|GetDistanceToBase (Variables|Targeting|GetTarget)))
                (Variables|Targeting|SetTarget (LocalVariables|GetNewEnemy))))))))
    (:else
      (Variables|Targeting|SetTarget IncomingEnemy))))

(fn ToggleRangeIndicator
  (params (show :type Boolean))
  (for _array_element (Variables|Components|GetRangeMeshes)
    (Rendering|SetVisibility _array_element show true)))

(fn SetLevel
  (Variables|Stats|SetLevel (Variables|/Game/Blueprints/Tower/BaseTowerData.BaseTowerData_C|GetLevel (Variables|Default|GetMyBaseData))))

(fn AttemptLevelUp
  (if true
    (Math|Integer|IncrementInt (Variables|Stats|GetLevel)
      (:%20%20
        (CallFunction|UpdateAllStats)))))