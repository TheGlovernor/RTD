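; TowerTypeData is a lookup that supplies a data object for each tower type.
; InitData loops over every ETowerType, constructs an object from each class found in RefMap and stores it in DataMap under that type.
; Types without a RefMap entry are skipped.
; GetTowerDataFromEnum returns the DataMap value for a given type, without checking whether the entry was found.
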(fn GetTowerDatafromEnum
  (params (TowerType :type ETowerType%20Enum :default "NewEnumerator0"))
  (return (.Value (Utilities|Map|Find (Variables|Default|GetDataMap) TowerType))))

(fn InitData
  (bind _enumvalue (|ForEachETowerType)
    (:LoopBody
      (if (.ReturnValue (Utilities|Map|Find (Variables|Default|GetRefMap) _enumvalue))
        (bind _returnvalue (Game|ConstructObjectfromClass (.Value (Utilities|Map|Find (Variables|Default|GetRefMap) _enumvalue))))
        (Utilities|Map|Add (Variables|Default|GetDataMap) _enumvalue _returnvalue)))))