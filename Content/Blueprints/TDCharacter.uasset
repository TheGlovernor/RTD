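; TDCharacter is a player-controlled flying Character that provides a movable, rotatable, zoomable camera with a visible cursor and Game-and-UI input.
; WASD and Q/E set movement and yaw values, which Tick applies along the capsule's axes and to controller yaw.
; Tick also sets the spring arm rotation from control rotation, offset by a CameraAngle pitch.
; The mouse wheel zooms by adjusting arm length within min and max limits.
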(event Custom|Rotate
  (Pawn|Input|AddControllerYawInput (Variables|Default|GetRotationSpeed))
  (Transformation|SetRelativeRotation (Variables|Camera|GetSpringArm) (Math|Rotator|Delta(Rotator) (Pawn|GetControlRotation :!class /Script/Engine.Pawn) (Math|Rotator|MakeRotator 0.0 (Variables|Default|GetCameraAngle) 0.0)) false false))

(event Custom|MoveForwards
  (Pawn|Input|AddMovementInput (Math|Vector|GetForwardVector (Variables|Collision|GetCapsuleComponent)) (Variables|Default|GetForwards) false))

(event Custom|MoveSideways
  (Pawn|Input|AddMovementInput (Math|Vector|GetRightVector (Variables|Collision|GetCapsuleComponent)) (Variables|Default|GetSideways) false))

(event EventBeginPlay
  (bind _returnvalue (Game|GetPlayerController 0))
  (Pawn|Components|CharacterMovement|SetMovementMode (Variables|Character|GetCharacterMovement) "MOVE_Flying" 0)
  (Variables|/Script/Engine.PlayerController|SetbShowMouseCursor _returnvalue true)
  (Input|SetInputModeGameandUI _returnvalue 0 "DoNotLock" true)
  (Variables|/Script/Engine.SpringArmComponent|SetTargetArmLength (Variables|Camera|GetSpringArm) (Variables|Default|GetMinArmLength)))

(event EventTick
  (params (DeltaSeconds :type Float%20%28single-precision%29))
  (CallFunction|MoveForwards)
  (CallFunction|MoveSideways)
  (CallFunction|Rotate))

(event Input|MouseEvents|MouseWheelAxis
  (params (AxisValue :type Float%20%28single-precision%29))
  (bind _springarm (Variables|Camera|GetSpringArm))
  (Variables|/Script/Engine.SpringArmComponent|SetTargetArmLength _springarm (Math|Float|Clamp(Float) (+ (* AxisValue -1.0 (Variables|Default|GetZoomScalar)) (Variables|/Script/Engine.SpringArmComponent|GetTargetArmLength _springarm)) (Variables|Default|GetMinArmLength) (Variables|Default|GetMaxArmLength))))

(event Input|KeyboardEvents|W
  (params (Key :type Key%20Structure :default "None"))
  (:Pressed
    (Variables|Default|SetForwards 1.0))
  (:Released
    (Variables|Default|SetForwards 0.0)))

(event Input|KeyboardEvents|A
  (params (Key :type Key%20Structure :default "None"))
  (:Pressed
    (Variables|Default|SetSideways -1.0))
  (:Released
    (Variables|Default|SetSideways 0.0)))

(event Input|KeyboardEvents|S
  (params (Key :type Key%20Structure :default "None"))
  (:Pressed
    (Variables|Default|SetForwards -1.0))
  (:Released
    (Variables|Default|SetForwards 0.0)))

(event Input|KeyboardEvents|D
  (params (Key :type Key%20Structure :default "None"))
  (:Pressed
    (Variables|Default|SetSideways 1.0))
  (:Released
    (Variables|Default|SetSideways 0.0)))

(event Input|KeyboardEvents|Q
  (params (Key :type Key%20Structure :default "None"))
  (:Pressed
    (Variables|Default|SetRotationSpeed 0.2))
  (:Released
    (Variables|Default|SetRotationSpeed 0.0)))

(event Input|KeyboardEvents|E
  (params (Key :type Key%20Structure :default "None"))
  (:Pressed
    (Variables|Default|SetRotationSpeed -0.2))
  (:Released
    (Variables|Default|SetRotationSpeed 0.0)))

(fn ConstructionScript)